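; BP_QuietDirectionalLight is the directional light actor of the Quiet runtime editor, with a thumbnail and arrow as editor visuals.
; A looping timer started on BeginPlay retries until it finds the outliner component, then clears itself and binds to that component's selection changes.
; Selection state, including any already active at binding, is forwarded to the thumbnail.
; EnableDebugMode toggles the visibility of the arrow and thumbnail.
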(event `self.ReceiveBeginPlay`
  (bind _returnvalue (`KismetSystemLibrary.K2_SetTimerDelegate` (delegate `TryToBindToSelect`) 1.0 true)))

(event `TryToBindToSelect`
  (bind _pinned (`/Game/QuietRuntimeEditor/Common/Blueprints/BP_QuietJsonMacroLibrary.Pin` (`self.GetComponentByClass` "/Game/QuietRuntimeEditor/Outliner/Blueprints/BP_QuietOutlinerComponent.BP_QuietOutlinerComponent_C")))
  (`/Engine/EditorBlueprintResources/StandardMacros.IsValid` _pinned
    (:`Is Valid`
      (`KismetSystemLibrary.K2_ClearAndInvalidateTimerHandle` (stale `self.ReceiveBeginPlay` _returnvalue))
      (add `/Game/QuietRuntimeEditor/Outliner/Blueprints/BP_QuietOutlinerComponent.NotifyOnSelectionStateChanged` _pinned (delegate `HandleOnSelectionStateChange`))
      (if (`/Game/QuietRuntimeEditor/Outliner/Blueprints/BP_QuietOutlinerComponent.GetSelectionState` _pinned)
        (`/Game/QuietRuntimeEditor/Common/QuietActors/Blueprints/BP_ThumbnailComponent.ChangeSelectionState` (`self.Thumbnail`) true)))))

(event `HandleOnSelectionStateChange`
  (params (NewState :type Boolean))
  (`/Game/QuietRuntimeEditor/Common/QuietActors/Blueprints/BP_ThumbnailComponent.ChangeSelectionState` (`self.Thumbnail`) NewState))

(event `/Game/QuietRuntimeEditor/Common/QuietActors/Blueprints/BI_QuietActorsInterface.EnableDebugMode`
  (params (Enable :type Boolean))
  (`SceneComponent.SetVisibility` (`self.Arrow`) Enable false)
  (`/Game/QuietRuntimeEditor/Common/QuietActors/Blueprints/BP_ThumbnailComponent.SetThumbnailVisibility` (`self.Thumbnail`) Enable))

(fn `UserConstructionScript`)