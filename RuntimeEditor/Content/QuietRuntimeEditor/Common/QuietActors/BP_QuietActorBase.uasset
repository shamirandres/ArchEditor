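; Base actor for the Quiet Runtime Editor that shows a thumbnail reflecting the actor's selection state.
; On BeginPlay it adds a thumbnail component, then polls on a looping timer for a BP_QuietOutlinerComponent until found or the retry limit runs out.
; Once bound, it forwards the current selection and later changes to the thumbnail.
; EnableDebugMode toggles the thumbnail's visibility.
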(event `self.ReceiveBeginPlay`
  (bind _returnvalue (`AddComponent|NODE_AddBP_ThumbnailComponent-0`))
  (set `self.ThumbnailComponent` _returnvalue)
  (bind _returnvalue_2 (`KismetSystemLibrary.K2_SetTimerDelegate` (delegate `TryToBindToSelect`) 0.5 true))
  (`self.TryToBindToSelect`)
  (`/Game/QuietRuntimeEditor/Common/QuietActors/Blueprints/BP_ThumbnailComponent.SetThumbnail` (`self.ThumbnailComponent`) (`self.Thumbnail`)))

(event `TryToBindToSelect`
  (bind _pinned (`/Game/QuietRuntimeEditor/Common/Blueprints/BP_QuietJsonMacroLibrary.Pin` (`self.GetComponentByClass` "/Game/QuietRuntimeEditor/Outliner/Blueprints/BP_QuietOutlinerComponent.BP_QuietOutlinerComponent_C")))
  (`/Engine/EditorBlueprintResources/StandardMacros.IsValid` _pinned
    (:`Is Valid`
      (`KismetSystemLibrary.K2_ClearAndInvalidateTimerHandle` (stale `self.ReceiveBeginPlay` _returnvalue_2))
      (add `/Game/QuietRuntimeEditor/Outliner/Blueprints/BP_QuietOutlinerComponent.NotifyOnSelectionStateChanged` _pinned (delegate `HandleOnSelectionStateChanged`))
      (if (`/Game/QuietRuntimeEditor/Outliner/Blueprints/BP_QuietOutlinerComponent.GetSelectionState` _pinned)
        (`/Game/QuietRuntimeEditor/Common/QuietActors/Blueprints/BP_ThumbnailComponent.ChangeSelectionState` (`self.ThumbnailComponent`) true)))
    (:`Is Not Valid`
      (bind _result (`/Engine/EditorBlueprintResources/StandardMacros.IncrementInt` (`self.BindingAttempts`))
        (:`  `
          (if (> _result 20)
            (`KismetSystemLibrary.K2_ClearAndInvalidateTimerHandle` (stale `self.ReceiveBeginPlay` _returnvalue_2))))))))

(event `HandleOnSelectionStateChanged`
  (params (NewState :type Boolean))
  (`/Game/QuietRuntimeEditor/Common/QuietActors/Blueprints/BP_ThumbnailComponent.ChangeSelectionState` (`self.ThumbnailComponent`) NewState))

(event `/Game/QuietRuntimeEditor/Common/QuietActors/Blueprints/BI_QuietActorsInterface.EnableDebugMode`
  (params (Enable :type Boolean))
  (`/Game/QuietRuntimeEditor/Common/QuietActors/Blueprints/BP_ThumbnailComponent.SetThumbnailVisibility` (`self.ThumbnailComponent`) Enable))

(fn `UserConstructionScript`)