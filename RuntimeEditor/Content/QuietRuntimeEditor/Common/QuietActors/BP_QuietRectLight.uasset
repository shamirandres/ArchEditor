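; Rect light actor for the Quiet runtime editor that visualizes its source rectangle and barn doors with a debug mesh.
; A procedural mesh is built at BeginPlay from width, height, barn door angle and length.
; Tick rewrites its vertices when those light parameters change.
; A looping timer waits for the outliner component, then binds selection changes to drive the thumbnail and, in debug mode, mesh visibility.
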(event `self.ReceiveBeginPlay`
  (`self.CreatePlane`)
  (`self.WriteParams`)
  (bind _returnvalue (`KismetSystemLibrary.K2_SetTimerDelegate` (delegate `TryToBindToSelect`) 1.0 true)))

(event `TryToBindToSelect`
  (bind _pinned (`/Game/QuietRuntimeEditor/Common/Blueprints/BP_QuietJsonMacroLibrary.Pin` (`self.GetComponentByClass` "/Game/QuietRuntimeEditor/Outliner/Blueprints/BP_QuietOutlinerComponent.BP_QuietOutlinerComponent_C")))
  (`/Engine/EditorBlueprintResources/StandardMacros.IsValid` _pinned
    (:`Is Valid`
      (`KismetSystemLibrary.K2_ClearAndInvalidateTimerHandle` (stale `self.ReceiveBeginPlay` _returnvalue))
      (add `/Game/QuietRuntimeEditor/Outliner/Blueprints/BP_QuietOutlinerComponent.NotifyOnSelectionStateChanged` _pinned (delegate `HandleOnSelectionStateChanged`))
      (`KismetSystemLibrary.DelayUntilNextTick`)
      (if (`/Game/QuietRuntimeEditor/Outliner/Blueprints/BP_QuietOutlinerComponent.GetSelectionState` _pinned)
        (`/Game/QuietRuntimeEditor/Common/QuietActors/Blueprints/BP_ThumbnailComponent.ChangeSelectionState` (`self.Thumbnail`) true)
        (if (`self.DebugVisibility`)
          (`self.Set Debug Mesh Visibility` true)
          (`self.UpdatePlanes`))))))

(event `HandleOnSelectionStateChanged`
  (params (NewState :type Boolean))
  (`/Game/QuietRuntimeEditor/Common/QuietActors/Blueprints/BP_ThumbnailComponent.ChangeSelectionState` (`self.Thumbnail`) NewState)
  (if (`self.DebugVisibility`)
    (`self.Set Debug Mesh Visibility` NewState)
    (`self.UpdatePlanes`)))

(event `/Game/QuietRuntimeEditor/Common/QuietActors/Blueprints/BI_QuietActorsInterface.EnableDebugMode`
  (params (Enable :type Boolean))
  (bind _output_get (set `self.DebugVisibility` Enable))
  (`SceneComponent.SetVisibility` (`self.Arrow`) _output_get false)
  (`/Game/QuietRuntimeEditor/Common/QuietActors/Blueprints/BP_ThumbnailComponent.SetThumbnailVisibility` (`self.Thumbnail`) (`self.DebugVisibility`))
  (if (`self.DebugVisibility`)
    (if (`self.IsSelected`)
      (`self.Set Debug Mesh Visibility` true))
    (elif (`self.IsSelected`)
      (`self.Set Debug Mesh Visibility` false))))

(event `self.ReceiveTick`
  (params (DeltaSeconds :type "Float (single-precision)"))
  (bind _rectlightcomponent (`self.RectLightComponent`))
  (if (or (not (`KismetMathLibrary.NearlyEqual_FloatFloat` (`self.Width`) (`RectLightComponent.SourceWidth` _rectlightcomponent) 0.001)) (not (`KismetMathLibrary.NearlyEqual_FloatFloat` (`RectLightComponent.BarnDoorAngle` _rectlightcomponent) (`self.Angle`) 0.001)) (not (`KismetMathLibrary.NearlyEqual_FloatFloat` (`RectLightComponent.BarnDoorLength` _rectlightcomponent) (`self.Length`) 0.001)) (not (`KismetMathLibrary.NearlyEqual_FloatFloat` (`RectLightComponent.SourceHeight` _rectlightcomponent) (`self.Height`) 0.001)))
    (`self.WriteParams`)
    (`self.UpdatePlanes`)))

(fn `CreatePlane`
  (bind _returnvalue (`AddComponent|NODE_AddProceduralMeshComponent-2`))
  (set `self.DebugMesh` _returnvalue)
  (bind _vertices (`self.UpdateDebugVertices`))
  (`ProceduralMeshComponent.CreateMeshSection_LinearColor` :`self` (`self.DebugMesh`) :`Vertices` _vertices :`Triangles` (`|MakeArray` 1 2 0 0 2 3 5 1 4 4 1 0 2 6 3 3 6 7 3 9 0 0 9 8 1 10 2 2 10 11) :`UV0` (`|MakeArray` (0.0 1.0) (1.0 1.0) (1.0 0.0) (0.0 0.0) (0.0 0.0) (1.0 0.0) (1.0 1.0) (0.0 1.0) (0.0 0.0) (1.0 0.0) (0.0 1.0) (0.0 0.0) :!type "Vector2D Structure"))
  (`PrimitiveComponent.SetMaterial` (`self.DebugMesh`) 0 "/Game/QuietRuntimeEditor/Common/QuietActors/Materials/M_DebugLighting.M_DebugLighting")
  (`self.UpdatePlanes`))

(fn `IsSelected`
  (returns (State :type Boolean))
  (bind _pinned (`/Game/QuietRuntimeEditor/Common/Blueprints/BP_QuietJsonMacroLibrary.Pin` (`self.GetComponentByClass` "/Game/QuietRuntimeEditor/Outliner/Blueprints/BP_QuietOutlinerComponent.BP_QuietOutlinerComponent_C")))
  (`/Engine/EditorBlueprintResources/StandardMacros.IsValid` _pinned
    (:`Is Valid`
      (return (`/Game/QuietRuntimeEditor/Outliner/Blueprints/BP_QuietOutlinerComponent.GetSelectionState` _pinned)))))

(fn `Set Debug Mesh Visibility`
  (params (NewState :type Boolean))
  (`SceneComponent.SetVisibility` (`self.DebugMesh`) NewState true))

(fn `UpdateDebugVertices`
  (returns (Vertices :type "Array of Vector Structure"))
  (bind _length (`self.Length`))
  (bind _length_2 (`self.Length`))
  (bind _returnvalue (`KismetMathLibrary.RotateAngleAxis` (1.0 0.0 0.0) (`self.Angle`) (0.0 1.0 0.0)))
  (bind _returnvalue_2 (/ (`self.Height`) 2.0))
  (bind _returnvalue_3 (/ (`self.Width`) 2.0))
  (bind _returnvalue_4 (`KismetMathLibrary.MakeVector` 0.0 _returnvalue_3 _returnvalue_2))
  (bind _returnvalue_5 (`KismetMathLibrary.RotateAngleAxis` (1.0 0.0 0.0) (* (`self.Angle`) -1.0) (0.0 1.0 0.0)))
  (bind _returnvalue_6 (* _returnvalue_2 -1.0))
  (bind _returnvalue_7 (* _returnvalue_3 -1.0))
  (bind _returnvalue_8 (`KismetMathLibrary.MakeVector` 0.0 _returnvalue_3 _returnvalue_6))
  (bind _returnvalue_9 (`KismetMathLibrary.MakeVector` 0.0 _returnvalue_7 _returnvalue_6))
  (bind _returnvalue_10 (`KismetMathLibrary.MakeVector` 0.0 _returnvalue_7 _returnvalue_2))
  (bind _returnvalue_11 (+ _returnvalue_9 (* (`KismetMathLibrary.RotateAngleAxis` _returnvalue -45.0 (1.0 0.0 0.0)) _length_2)))
  (bind _returnvalue_12 (+ _returnvalue_8 (* (`KismetMathLibrary.RotateAngleAxis` _returnvalue 45.0 (1.0 0.0 0.0)) _length_2)))
  (bind _returnvalue_13 (+ _returnvalue_10 (* (`KismetMathLibrary.RotateAngleAxis` _returnvalue_5 45.0 (1.0 0.0 0.0)) _length)))
  (bind _returnvalue_14 (+ _returnvalue_4 (* (`KismetMathLibrary.RotateAngleAxis` _returnvalue_5 -45.0 (1.0 0.0 0.0)) _length)))
  (return (`|MakeArray` _returnvalue_8 _returnvalue_9 _returnvalue_10 _returnvalue_4 _returnvalue_12 _returnvalue_11 _returnvalue_13 _returnvalue_14 _returnvalue_12 _returnvalue_14 _returnvalue_11 _returnvalue_13)))

(fn `UpdatePlanes`
  (bind _vertices (`self.UpdateDebugVertices`))
  (`ProceduralMeshComponent.UpdateMeshSection_LinearColor` :`self` (`self.DebugMesh`) :`Vertices` _vertices))

(fn `UserConstructionScript`)

(fn `WriteParams`
  (bind _rectlightcomponent (`self.RectLightComponent`))
  (set `self.Width` (`RectLightComponent.SourceWidth` _rectlightcomponent))
  (set `self.Height` (`RectLightComponent.SourceHeight` _rectlightcomponent))
  (set `self.Length` (`RectLightComponent.BarnDoorLength` _rectlightcomponent))
  (set `self.Angle` (`RectLightComponent.BarnDoorAngle` _rectlightcomponent)))