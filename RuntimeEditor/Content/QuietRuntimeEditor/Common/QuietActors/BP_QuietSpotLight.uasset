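; Spot light actor for the Quiet runtime editor that draws debug cone and sphere meshes showing the light's shape.
; Meshes are scaled from inner/outer cone angles and attenuation radius, refreshed on Tick when these change, with a dynamic material mask on the sphere.
; A looping timer retries binding to the outliner component's selection event, which updates the thumbnail.
; In debug mode, the arrow and thumbnail show, and the meshes appear only while selected.
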(event `self.ReceiveBeginPlay`
  (`self.SetupDebugMeshes`)
  (`self.UpdateDebugMesh`)
  (bind _returnvalue (`KismetSystemLibrary.K2_SetTimerDelegate` (delegate `TryToBindToSelect`) 1.0 true)))

(event `TryToBindToSelect`
  (bind _pinned (`/Game/QuietRuntimeEditor/Common/Blueprints/BP_QuietJsonMacroLibrary.Pin` (`self.GetComponentByClass` "/Game/QuietRuntimeEditor/Outliner/Blueprints/BP_QuietOutlinerComponent.BP_QuietOutlinerComponent_C")))
  (`/Engine/EditorBlueprintResources/StandardMacros.IsValid` _pinned
    (:`Is Valid`
      (`KismetSystemLibrary.K2_ClearAndInvalidateTimerHandle` (stale `self.ReceiveBeginPlay` _returnvalue))
      (add `/Game/QuietRuntimeEditor/Outliner/Blueprints/BP_QuietOutlinerComponent.NotifyOnSelectionStateChanged` _pinned (delegate `HandleOnSelectionStateChanged`))
      (if (`/Game/QuietRuntimeEditor/Outliner/Blueprints/BP_QuietOutlinerComponent.GetSelectionState` _pinned)
        (`/Game/QuietRuntimeEditor/Common/QuietActors/Blueprints/BP_ThumbnailComponent.ChangeSelectionState` (`self.Thumbnail`) true)))))

(event `HandleOnSelectionStateChanged`
  (params (NewState :type Boolean))
  (`/Game/QuietRuntimeEditor/Common/QuietActors/Blueprints/BP_ThumbnailComponent.ChangeSelectionState` (`self.Thumbnail`) NewState)
  (if (`self.DebugVisibility`)
    (`self.Set Debug Mesh Visibility` NewState)))

(event `/Game/QuietRuntimeEditor/Common/QuietActors/Blueprints/BI_QuietActorsInterface.EnableDebugMode`
  (params (Enable :type Boolean))
  (bind _output_get (set `self.DebugVisibility` Enable))
  (`SceneComponent.SetVisibility` (`self.Arrow`) _output_get false)
  (`/Game/QuietRuntimeEditor/Common/QuietActors/Blueprints/BP_ThumbnailComponent.SetThumbnailVisibility` (`self.Thumbnail`) (`self.DebugVisibility`))
  (if (`self.DebugVisibility`)
    (if (`self.IsSelected`)
      (`self.Set Debug Mesh Visibility` true))
    (elif (`self.IsSelected`)
      (`self.Set Debug Mesh Visibility` false))))

(event `self.ReceiveTick`
  (params (DeltaSeconds :type "Float (single-precision)"))
  (bind _spotlightcomponent (`self.SpotLightComponent`))
  (if (or (not (`KismetMathLibrary.NearlyEqual_FloatFloat` (`SpotLightComponent.OuterConeAngle` _spotlightcomponent) (`self.Angle`) 0.001)) (not (`KismetMathLibrary.NearlyEqual_FloatFloat` (`LocalLightComponent.AttenuationRadius` _spotlightcomponent) (`self.Radius`) 0.001)) (not (`KismetMathLibrary.NearlyEqual_FloatFloat` (`SpotLightComponent.InnerConeAngle` _spotlightcomponent) (`self.InnerAngle`) 0.001)))
    (`self.UpdateDebugMesh`)))

(fn `IsSelected`
  (returns (State :type Boolean))
  (bind _pinned (`/Game/QuietRuntimeEditor/Common/Blueprints/BP_QuietJsonMacroLibrary.Pin` (`self.GetComponentByClass` "/Game/QuietRuntimeEditor/Outliner/Blueprints/BP_QuietOutlinerComponent.BP_QuietOutlinerComponent_C")))
  (`/Engine/EditorBlueprintResources/StandardMacros.IsValid` _pinned
    (:`Is Valid`
      (return (`/Game/QuietRuntimeEditor/Outliner/Blueprints/BP_QuietOutlinerComponent.GetSelectionState` _pinned)))))

(fn `Set Debug Mesh Visibility`
  (params (NewState :type Boolean))
  (`SceneComponent.SetVisibility` (`self.SM_SpotOuter`) NewState true)
  (`SceneComponent.SetVisibility` (`self.SM_SpotInner`) NewState true)
  (`SceneComponent.SetVisibility` (`self.SM_SpotConeSphere`) NewState true))

(fn `SetupDebugMeshes`
  (bind _returnvalue (`PrimitiveComponent.CreateDynamicMaterialInstance` (`self.SM_SpotConeSphere`) 0 "/Game/QuietRuntimeEditor/Common/QuietActors/Materials/MI_SpotOuterSphere.MI_SpotOuterSphere" "None"))
  (set `self.OuterSphereMat` _returnvalue)
  (`self.UpdateDebugMesh`))

(fn `UpdateDebugMesh`
  (bind _spotlightcomponent (`self.SpotLightComponent`))
  (bind _spotlightcomponent_2 (`self.SpotLightComponent`))
  (bind _relativescale3d_x (`KismetMathLibrary.BreakVector` (`SceneComponent.RelativeScale3D` (`self.SM_SpotConeSphere`))))
  (bind _relativescale3d_x_2 (`KismetMathLibrary.BreakVector` (`SceneComponent.RelativeScale3D` (`self.SM_SpotOuter`))))
  (bind _outerconeangle (`SpotLightComponent.OuterConeAngle` _spotlightcomponent_2))
  (bind _attenuationradius (`LocalLightComponent.AttenuationRadius` _spotlightcomponent_2))
  (bind _innerconeangle (`SpotLightComponent.InnerConeAngle` _spotlightcomponent_2))
  (bind _returnvalue (`KismetMathLibrary.FClamp` (/ (* (`KismetMathLibrary.DegSin` _innerconeangle) _attenuationradius) 50.0) 0.01 100000.0))
  (bind _returnvalue_2 (`KismetMathLibrary.FClamp` (/ (* (`KismetMathLibrary.DegSin` _outerconeangle) _attenuationradius) 50.0) 0.01 100000.0))
  (set `self.Radius` (`LocalLightComponent.AttenuationRadius` _spotlightcomponent))
  (set `self.Angle` (`SpotLightComponent.OuterConeAngle` _spotlightcomponent))
  (set `self.InnerAngle` (`SpotLightComponent.InnerConeAngle` _spotlightcomponent))
  (`SceneComponent.SetRelativeScale3D` (`self.SM_SpotOuter`) (`KismetMathLibrary.MakeVector` (* (`KismetMathLibrary.DegCos` _outerconeangle) (/ _attenuationradius 100.0)) _returnvalue_2 _returnvalue_2))
  (`SceneComponent.SetRelativeScale3D` (`self.SM_SpotInner`) (`KismetMathLibrary.MakeVector` (* (`KismetMathLibrary.DegCos` _innerconeangle) (/ _attenuationradius 100.0)) _returnvalue _returnvalue))
  (`SceneComponent.SetRelativeScale3D` (`self.SM_SpotConeSphere`) (`KismetMathLibrary.Conv_DoubleToVector` (/ (`LocalLightComponent.AttenuationRadius` (`self.SpotLightComponent`)) 50.0)))
  (`MaterialInstanceDynamic.SetScalarParameterValue` (`self.OuterSphereMat`) "VerticalMask" (/ _relativescale3d_x_2 (/ _relativescale3d_x 2.0))))

(fn `UserConstructionScript`)