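; BP_DatasmithImporter is a Quiet runtime editor actor that imports Datasmith files from a path or file browser.
; Import clears attached actors and polls progress on Tick through gates, with a delayed missing-file warning.
; On completion it applies any requested JSON restore recursively, matching actors by tags, then takes a unique name and registers with the Outliner.
; Its thumbnail mirrors Outliner selection, bound through a retrying timer.
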(event `Import`
  (bind _returnvalue (`BlueprintFileUtilsBPLibrary.FileExists` (`self.File`)))
  (if _returnvalue
    (bind _returnvalue_2 (`self.LoadFile` (`self.File`)))
    (if _returnvalue_2
      (`self.Clear` :!label _label)
      (bind _progressbar (`/Game/QuietRuntimeEditor/Common/Blueprints/BP_QuietDialogLibrary.CallProgressbar` (`GameplayStatics.GetPlayerController` 0)))
      (`/Game/QuietRuntimeEditor/Common/Widgets/WBP_Progressbar.Subscribe` _progressbar self)
      (`|ExecutionSequence`
        (:`then_0`
          (`KismetSystemLibrary.Delay` 10.0)
          (`/Engine/EditorBlueprintResources/StandardMacros.Gate` true :!label _label_2
            (:`Exit`
              (bind _returnvalue_3 (`BlueprintFileUtilsBPLibrary.FileExists` (`self.ExternalFile`)))
              (if (not _returnvalue_3)
                (`/Engine/EditorBlueprintResources/StandardMacros.IsValid` _progressbar
                  (:`Is Valid`
                    (`/Game/QuietRuntimeEditor/Common/Widgets/WBP_Progressbar.End` _progressbar))
                  (:`Is Not Valid`
                    _))
                (`/Game/QuietRuntimeEditor/Common/Blueprints/BP_QuietDialogLibrary.CallWarningDialogSimple` (`GameplayStatics.GetPlayerController` 0) "Datasmith.LoadingFailed")))))
        (:`then_1`
          (goto _label_2 :!via `Open`))
        (:`then_2`
          (goto _label_3 :!via `Open`))))))

(event `BrowseFile`
  (bind _returnvalue (`DatasmithRuntimeLibrary.LoadFileFromExplorer` self))
  (if _returnvalue
    (goto _label)))

(event `self.ReceiveTick`
  (params (DeltaSeconds :type "Float (single-precision)"))
  (`/Engine/EditorBlueprintResources/StandardMacros.Gate` true :!label _label_3
    (:`Exit`
      (`/Engine/EditorBlueprintResources/StandardMacros.IsValid` (stale `Import` _progressbar)
        (:`Is Valid`
          (`/Game/QuietRuntimeEditor/Common/Widgets/WBP_Progressbar.Progress` (stale `Import` _progressbar) self (`KismetMathLibrary.FClamp` (`self.Progress`))))
        (:`Is Not Valid`
          _))
      (if (and (>= (`self.Progress`) 0.5) (not (`self.bBuilding`)))
        (`|ExecutionSequence`
          (:`then_0`
            (`/Game/QuietRuntimeEditor/Common/Widgets/WBP_Progressbar.Progress` (stale `Import` _progressbar) self 1.0)
            (`KismetSystemLibrary.DelayUntilNextTick`)
            (`self.RestoreContentMacro` (stale `RestoreContent` ContentJson) :!label _label_4)
            (set `self.File` (`self.ExternalFile`))
            (`self.RenameImporter`)
            (`/Game/QuietRuntimeEditor/Common/Blueprints/BP_Router.ThrowActor` (`/Game/QuietRuntimeEditor/Common/Blueprints/BP_QuietEditorUtilities.GetRouter`) (struct :`TagName` "Manager") (struct :`TagName` "Outliner.RegisterAttachment") self)
            (`/Engine/EditorBlueprintResources/StandardMacros.IsValid` (stale `Import` _progressbar)
              (:`Is Valid`
                (`/Game/QuietRuntimeEditor/Common/Widgets/WBP_Progressbar.RemoveSubscriber` (stale `Import` _progressbar) self))))
          (:`then_1`
            (goto _label_2 :!via `Close`))
          (:`then_2`
            (goto _label_3 :!via `Close`)))))))

(event `RestoreContent`
  (params (ContentJson :type "JsonObjectWrapper Structure"))
  (goto _label_4 :!via `Request`))

(event `self.ReceiveBeginPlay`
  (bind _returnvalue (`KismetSystemLibrary.K2_SetTimerDelegate` (delegate `TryToBindToSelect`) 1.0 true)))

(event `TryToBindToSelect`
  (bind _pinned (`/Game/QuietRuntimeEditor/Common/Blueprints/BP_QuietJsonMacroLibrary.Pin` (`self.GetComponentByClass` "/Game/QuietRuntimeEditor/Outliner/Blueprints/BP_QuietOutlinerComponent.BP_QuietOutlinerComponent_C")))
  (`/Engine/EditorBlueprintResources/StandardMacros.IsValid` _pinned
    (:`Is Valid`
      (`KismetSystemLibrary.K2_ClearAndInvalidateTimerHandle` (stale `self.ReceiveBeginPlay` _returnvalue))
      (add `/Game/QuietRuntimeEditor/Outliner/Blueprints/BP_QuietOutlinerComponent.NotifyOnSelectionStateChanged` _pinned (delegate `HandleOnSelectionStateChanged`))
      (if (`/Game/QuietRuntimeEditor/Outliner/Blueprints/BP_QuietOutlinerComponent.GetSelectionState` _pinned)
        (`/Game/QuietRuntimeEditor/Common/QuietActors/Blueprints/BP_ThumbnailComponent.ChangeSelectionState` (`self.Thumbnail`) true)))))

(event `HandleOnSelectionStateChanged`
  (params (NewState :type Boolean))
  (`/Game/QuietRuntimeEditor/Common/QuietActors/Blueprints/BP_ThumbnailComponent.ChangeSelectionState` (`self.Thumbnail`) NewState))

(event `/Game/QuietRuntimeEditor/Common/QuietActors/Blueprints/BI_QuietActorsInterface.EnableDebugMode`
  (params (Enable :type Boolean))
  (`/Game/QuietRuntimeEditor/Common/QuietActors/Blueprints/BP_ThumbnailComponent.SetThumbnailVisibility` (`self.Thumbnail`) Enable))

(fn `Clear`
  (bind (_arrayindex _arrayelement) (`/Engine/EditorBlueprintResources/StandardMacros.ReverseForEachLoop` (`self.GetAttachedActors` true true))
    (:`LoopBody`
      (`self.K2_DestroyActor` _arrayelement))))

(fn `FindActorByTags`
  (params (Parent :type "Actor Object Reference") (JsonObject :type "JsonObjectWrapper Structure (by ref)"))
  (returns (`Array Element` :type "Actor Object Reference"))
  (bind _outvalue (`|GetJsonField` JsonObject "Tags"))
  (for _array_element (`self.GetAttachedActors` Parent true true)
    (if (`KismetArrayLibrary.Array_Identical` (`Actor.Tags` _array_element) _outvalue)
      (return _array_element))))

(fn `RenameImporter`
  (locals (RawName :type String))
  (set `local.RawName` (`self.LoadedScene`))
  (bind _actors (`/Game/QuietRuntimeEditor/Common/Blueprints/BP_Router.GetActorsWithTag` (`/Game/QuietRuntimeEditor/Common/Blueprints/BP_QuietEditorUtilities.GetRouter`) (struct :`TagName` "Manager") (struct :`TagName` "Outliner.GetAllActors")))
  (bind _names (`/Game/QuietRuntimeEditor/Outliner/Blueprints/BP_QuietOutlinerLibrary.CollectActorNames` _actors))
  (`/Game/QuietRuntimeEditor/Common/Blueprints/BP_QuietEditorUtilities.UnifyName` (`local.RawName`) _names)
  (bind _treecomponent (`/Game/QuietRuntimeEditor/Outliner/Blueprints/BP_QuietOutlinerLibrary.AcquireOutlinerComponent` self))
  (`/Game/QuietRuntimeEditor/Outliner/Blueprints/BP_QuietOutlinerComponent.Rename` _treecomponent (`local.RawName`) false))

(fn `RestoreContentImpl`
  (params (Actor :type "Actor Object Reference") (Json :type "JsonObjectWrapper Structure"))
  (bind _outvalue (`|GetJsonField` Json "Attachment"))
  (for _array_element _outvalue
    (bind _array_element_2 (`self.FindActorByTags` Actor _array_element))
    (`/Game/QuietRuntimeEditor/Common/Blueprints/BP_QuietEditorUtilities.DeserializeObject` _array_element_2 _array_element)
    (bind _outvalue_2 (`|GetJsonField` _array_element "Transform"))
    (`self.K2_SetActorTransform` _array_element_2 _outvalue_2 false true)
    (`self.RestoreContentImpl` _array_element_2 _array_element)))

(fn `UserConstructionScript`)