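; Sun and sky actor that orients the sun and drives a sky sphere material, with selectable thumbnails for the Quiet runtime editor.
; Construction rotates Orbit from SunAngle and Azimuth, then pushes parameters to a lazily created dynamic material.
; Sun pitch drives color curves, horizon falloff and stars; UpdateSunDirection reapplies curve colors even when RefreshMaterial uses manual ones.
; At play, it polls for an outliner component to mirror selection onto thumbnails.
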(event `self.ReceiveBeginPlay`
  (bind _returnvalue (`KismetSystemLibrary.K2_SetTimerDelegate` (delegate `TryToBindToSelect`) 1.0 true)))

(event `TryToBindToSelect`
  (bind _returnvalue (`self.GetComponentByClass` "/Game/QuietRuntimeEditor/Outliner/Blueprints/BP_QuietOutlinerComponent.BP_QuietOutlinerComponent_C"))
  (`/Game/QuietRuntimeEditor/Common/Blueprints/BP_QuietJsonMacroLibrary.Pin` _returnvalue)
  (`/Engine/EditorBlueprintResources/StandardMacros.IsValid` _returnvalue
    (:`Is Valid`
      (`KismetSystemLibrary.K2_ClearAndInvalidateTimerHandle` (stale `self.ReceiveBeginPlay` _returnvalue))
      (add `/Game/QuietRuntimeEditor/Outliner/Blueprints/BP_QuietOutlinerComponent.NotifyOnSelectionStateChanged` _returnvalue (delegate `HandleOnSelectionStateChange`))
      (if (`/Game/QuietRuntimeEditor/Outliner/Blueprints/BP_QuietOutlinerComponent.GetSelectionState` _returnvalue)
        (`/Game/QuietRuntimeEditor/Common/QuietActors/Blueprints/BP_ThumbnailComponent.ChangeSelectionState` (`self.SunThumbnail`) true)
        (`/Game/QuietRuntimeEditor/Common/QuietActors/Blueprints/BP_ThumbnailComponent.ChangeSelectionState` (`self.SkyThumbnail`) true)))))

(event `HandleOnSelectionStateChange`
  (params (NewState :type Boolean))
  (`/Game/QuietRuntimeEditor/Common/QuietActors/Blueprints/BP_ThumbnailComponent.ChangeSelectionState` (`self.SunThumbnail`) NewState)
  (`/Game/QuietRuntimeEditor/Common/QuietActors/Blueprints/BP_ThumbnailComponent.ChangeSelectionState` (`self.SkyThumbnail`) NewState))

(event `/Game/QuietRuntimeEditor/Common/QuietActors/Blueprints/BI_QuietActorsInterface.EnableDebugMode`
  (params (Enable :type Boolean))
  (`/Game/QuietRuntimeEditor/Common/QuietActors/Blueprints/BP_ThumbnailComponent.SetThumbnailVisibility` (`self.SunThumbnail`) Enable)
  (`/Game/QuietRuntimeEditor/Common/QuietActors/Blueprints/BP_ThumbnailComponent.SetThumbnailVisibility` (`self.SkyThumbnail`) Enable))

(fn `AcquireSkyMaterial`
  (returns (`Sky material` :type "MaterialInstanceDynamic Object Reference"))
  (bind _skymaterial (`self.SkyMaterial`)
    (:`then`
      (return _skymaterial))
    (:`else`
      (bind _returnvalue (`PrimitiveComponent.CreateDynamicMaterialInstance` (`self.SkySphereMesh`) 0 "/Engine/EngineSky/M_Sky_Panning_Clouds2.M_Sky_Panning_Clouds2" "None"))
      (bind _output_get (set `self.SkyMaterial` _returnvalue))
      (return _output_get))))

(fn `RefreshMaterial`
  (bind _sky_material (`self.AcquireSkyMaterial`))
  (bind _sunheight (`self.SunHeight`))
  (bind _sunheight_2 (`self.SunHeight`))
  (bind _returnvalue (`SceneComponent.K2_GetComponentRotation` (`self.SUN`)))
  (`MaterialInstanceDynamic.SetVectorParameterValue` _sky_material "Light direction" (`KismetMathLibrary.Conv_VectorToLinearColor` (`KismetMathLibrary.Conv_RotatorToVector` _returnvalue)))
  (`MaterialInstanceDynamic.SetVectorParameterValue` _sky_material "Sun color" (`KismetMathLibrary.Conv_ColorToLinearColor` (`LightComponentBase.LightColor` (`self.SUN`))))
  (set `self.SunHeight` (`KismetMathLibrary.MapRangeUnclamped` (.pitch _returnvalue) 0.0 -90.0 0.0 1.0))
  (if (`self.Colors determined by sun position`)
    (`MaterialInstanceDynamic.SetVectorParameterValue` _sky_material "Horizon color" (`CurveLinearColor.GetClampedLinearColorValue` (`self.HorizonColorCurve`) (`self.SunHeight`)))
    (`MaterialInstanceDynamic.SetVectorParameterValue` _sky_material "Zenith color" (`CurveLinearColor.GetClampedLinearColorValue` (`self.ZenithColorCurve`) (`self.SunHeight`)))
    (`MaterialInstanceDynamic.SetVectorParameterValue` _sky_material "Cloud color" (`CurveLinearColor.GetClampedLinearColorValue` (`self.CloudColorCurve`) _sunheight_2))
    (`MaterialInstanceDynamic.SetScalarParameterValue` _sky_material "Horizon falloff" (`KismetMathLibrary.Lerp` 3.0 7.0 (`KismetMathLibrary.Abs` _sunheight_2)))
    (else
      (`MaterialInstanceDynamic.SetVectorParameterValue` _sky_material "Horizon color" (`self.HorizonColor`))
      (`MaterialInstanceDynamic.SetVectorParameterValue` _sky_material "Zenith color" (`self.ZenithColor`))
      (`MaterialInstanceDynamic.SetVectorParameterValue` _sky_material "Overall color" (`self.OverallColor`))
      (`MaterialInstanceDynamic.SetVectorParameterValue` _sky_material "Cloud color" (`self.CloudColor`))
      (`MaterialInstanceDynamic.SetScalarParameterValue` _sky_material "Horizon falloff" (`self.HorizonFalloff`))))
  (`MaterialInstanceDynamic.SetScalarParameterValue` _sky_material "Cloud speed" (`self.CloudSpeed`))
  (`MaterialInstanceDynamic.SetScalarParameterValue` _sky_material "Sun brightness" (`self.SunBrightness`))
  (`MaterialInstanceDynamic.SetScalarParameterValue` _sky_material "Sun height" (`KismetMathLibrary.SelectFloat` (`KismetMathLibrary.Abs` _sunheight) 0.0 (< _sunheight 0.0)))
  (`MaterialInstanceDynamic.SetScalarParameterValue` _sky_material "Cloud opacity" (`self.CloudOpacity`))
  (`MaterialInstanceDynamic.SetScalarParameterValue` _sky_material "Stars brightness" (`self.StarsBrightness`)))

(fn `UpdateOrientation`
  (`SceneComponent.K2_SetRelativeRotation` (`self.Orbit`) (`KismetMathLibrary.MakeRotator` 0.0 (`self.SunAngle`) (`self.Azimuth`)) false false))

(fn `UpdateSunDirection`
  (bind _sky_material (`self.AcquireSkyMaterial`))
  (bind _sunheight (`self.SunHeight`))
  (bind _sunheight_2 (`self.SunHeight`))
  (bind _returnvalue (`SceneComponent.K2_GetComponentRotation` (`self.SUN`)))
  (`MaterialInstanceDynamic.SetVectorParameterValue` _sky_material "Light direction" (`KismetMathLibrary.Conv_VectorToLinearColor` (`KismetMathLibrary.Conv_RotatorToVector` _returnvalue)))
  (`MaterialInstanceDynamic.SetVectorParameterValue` _sky_material "Sun color" (`KismetMathLibrary.Conv_ColorToLinearColor` (`LightComponentBase.LightColor` (`self.SUN`))))
  (set `self.SunHeight` (`KismetMathLibrary.MapRangeUnclamped` (.pitch _returnvalue) 0.0 -90.0 0.0 1.0))
  (`MaterialInstanceDynamic.SetVectorParameterValue` _sky_material "Horizon color" (`CurveLinearColor.GetClampedLinearColorValue` (`self.HorizonColorCurve`) (`self.SunHeight`)))
  (`MaterialInstanceDynamic.SetVectorParameterValue` _sky_material "Zenith color" (`CurveLinearColor.GetClampedLinearColorValue` (`self.ZenithColorCurve`) (`self.SunHeight`)))
  (`MaterialInstanceDynamic.SetVectorParameterValue` _sky_material "Cloud color" (`CurveLinearColor.GetClampedLinearColorValue` (`self.CloudColorCurve`) _sunheight_2))
  (`MaterialInstanceDynamic.SetScalarParameterValue` _sky_material "Horizon falloff" (`KismetMathLibrary.Lerp` 3.0 8.0 (`KismetMathLibrary.Abs` _sunheight_2)))
  (`MaterialInstanceDynamic.SetScalarParameterValue` _sky_material "Sun height" (`KismetMathLibrary.SelectFloat` (`KismetMathLibrary.Abs` _sunheight) 0.0 (< _sunheight 0.0))))

(fn `UserConstructionScript`
  (`self.UpdateOrientation`)
  (`self.RefreshMaterial`)
  (`self.UpdateSunDirection`))