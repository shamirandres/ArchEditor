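; BP_QuietPointLight is a point light actor for the Quiet runtime editor, with a thumbnail and debug meshes showing attenuation and source radius.
; A looping timer retries until it finds the actor's outliner component, then binds to its selection changes to update the thumbnail.
; In debug mode the thumbnail is visible and the meshes appear while selected.
; Tick rescales the meshes when either radius changes.
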(event `self.ReceiveBeginPlay`
  (`self.UpdateDebugMesh`)
  (set `self.Radius` (`LocalLightComponent.AttenuationRadius` (`self.PointLightComponent`)))
  (set `self.Source Radius` (`PointLightComponent.SourceRadius` (`self.PointLightComponent`)))
  (bind _returnvalue (`KismetSystemLibrary.K2_SetTimerDelegate` (delegate `TryToBindToSelect`) 0.5 true)))

(event `TryToBindToSelect`
  (bind _pinned (`/Game/QuietRuntimeEditor/Common/Blueprints/BP_QuietJsonMacroLibrary.Pin` (`self.GetComponentByClass` "/Game/QuietRuntimeEditor/Outliner/Blueprints/BP_QuietOutlinerComponent.BP_QuietOutlinerComponent_C")))
  (`/Engine/EditorBlueprintResources/StandardMacros.IsValid` _pinned
    (:`Is Valid`
      (`KismetSystemLibrary.K2_ClearAndInvalidateTimerHandle` (stale `self.ReceiveBeginPlay` _returnvalue))
      (add `/Game/QuietRuntimeEditor/Outliner/Blueprints/BP_QuietOutlinerComponent.NotifyOnSelectionStateChanged` _pinned (delegate `HandleOnSelectionStateChanged`))
      (if (`/Game/QuietRuntimeEditor/Outliner/Blueprints/BP_QuietOutlinerComponent.GetSelectionState` _pinned)
        (`/Game/QuietRuntimeEditor/Common/QuietActors/Blueprints/BP_ThumbnailComponent.ChangeSelectionState` (`self.Thumbnail`) true)))))

(event `HandleOnSelectionStateChanged`
  (params (NewState :type Boolean))
  (`/Game/QuietRuntimeEditor/Common/QuietActors/Blueprints/BP_ThumbnailComponent.ChangeSelectionState` (`self.Thumbnail`) NewState)
  (if (`self.DebugVisibility`)
    (`self.Set Debug Mesh Visibility` NewState)))

(event `/Game/QuietRuntimeEditor/Common/QuietActors/Blueprints/BI_QuietActorsInterface.EnableDebugMode`
  (params (Enable :type Boolean))
  (bind _output_get (set `self.DebugVisibility` Enable))
  (`/Game/QuietRuntimeEditor/Common/QuietActors/Blueprints/BP_ThumbnailComponent.SetThumbnailVisibility` (`self.Thumbnail`) _output_get)
  (if (`self.DebugVisibility`)
    (if (`self.IsSelected`)
      (`self.Set Debug Mesh Visibility` true))
    (elif (`self.IsSelected`)
      (`self.Set Debug Mesh Visibility` false))))

(event `self.ReceiveTick`
  (params (DeltaSeconds :type "Float (single-precision)"))
  (if (`self.DebugVisibility`)
    (if (or (not (`KismetMathLibrary.NearlyEqual_FloatFloat` (`self.Radius`) (`LocalLightComponent.AttenuationRadius` (`self.PointLightComponent`)) 0.001)) (not (`KismetMathLibrary.NearlyEqual_FloatFloat` (`self.Source Radius`) (`PointLightComponent.SourceRadius` (`self.PointLightComponent`)) 0.001)))
      (set `self.Radius` (`LocalLightComponent.AttenuationRadius` (`self.PointLightComponent`)))
      (set `self.Source Radius` (`PointLightComponent.SourceRadius` (`self.PointLightComponent`)))
      (`self.UpdateDebugMesh`))))

(fn `IsSelected`
  (returns (State :type Boolean))
  (bind _pinned (`/Game/QuietRuntimeEditor/Common/Blueprints/BP_QuietJsonMacroLibrary.Pin` (`self.GetComponentByClass` "/Game/QuietRuntimeEditor/Outliner/Blueprints/BP_QuietOutlinerComponent.BP_QuietOutlinerComponent_C")))
  (`/Engine/EditorBlueprintResources/StandardMacros.IsValid` _pinned
    (:`Is Valid`
      (return (`/Game/QuietRuntimeEditor/Outliner/Blueprints/BP_QuietOutlinerComponent.GetSelectionState` _pinned)))))

(fn `Set Debug Mesh Visibility`
  (params (NewState :type Boolean))
  (`SceneComponent.SetVisibility` (`self.PointLightSphere`) NewState true)
  (`SceneComponent.SetVisibility` (`self.SourceRadiusMesh`) NewState true))

(fn `UpdateDebugMesh`
  (`SceneComponent.SetRelativeScale3D` (`self.PointLightSphere`) (`KismetMathLibrary.Conv_DoubleToVector` (/ (`LocalLightComponent.AttenuationRadius` (`self.PointLightComponent`)) 50.0)))
  (`SceneComponent.SetRelativeScale3D` (`self.SourceRadiusMesh`) (`KismetMathLibrary.Conv_DoubleToVector` (/ (`PointLightComponent.SourceRadius` (`self.PointLightComponent`)) 50.0))))

(fn `UserConstructionScript`
  (`self.UpdateDebugMesh`))