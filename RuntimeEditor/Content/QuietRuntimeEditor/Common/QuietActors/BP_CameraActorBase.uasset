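; Base camera actor for the runtime editor that can take over the player's view and travel along a spline.
; Activate and Deactivate blend the view target between this camera and the player pawn, tracking an active flag.
; MoveAlongSpline drives location and rotation along the attach parent's root spline, using a timeline scaled by spline Duration, and warns when none is valid.
; A debug mode toggles the camera mesh's visibility.
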(event `/Game/QuietRuntimeEditor/Common/QuietActors/Blueprints/BI_QuietActorsInterface.EnableDebugMode`
  (params (Enable :type Boolean))
  (`SceneComponent.SetVisibility` (`self.Mesh`) Enable false))

(event `MoveAlongSpline`
  (bind _spline (`self.GetSpline`))
  (`/Engine/EditorBlueprintResources/StandardMacros.IsValid` _spline
    (:`Is Valid`
      (`TimelineComponent.SetPlayRate` (`self.Move`) (/ 1.0 (`SplineComponent.Duration` _spline)))
      (bind (_direction _driver) (`Timeline|Move` :!label _label)
        (:`Update`
          (bind _returnvalue (* _driver (`SplineComponent.GetSplineLength` _spline)))
          (`self.K2_SetActorLocationAndRotation` (`SplineComponent.GetLocationAtDistanceAlongSpline` _spline _returnvalue "World") (`SplineComponent.GetRotationAtDistanceAlongSpline` _spline _returnvalue "World")))
        (:`Finished`
          (`TimelineComponent.SetPlaybackPosition` (`self.Move`) 0.0 false true))))
    (:`Is Not Valid`
      (`/Game/QuietRuntimeEditor/Common/Blueprints/BP_QuietDialogLibrary.CallWarningDialogSimple` (`GameplayStatics.GetPlayerController` 0) "Camera.InvalidSpline"))))

(event `Stop`
  (goto _label :!via `Stop`))

(fn `Activate`
  (if (not (`self.IsActive`))
    (set `self.IsActive` true)
    (`PlayerController.SetViewTargetWithBlend` (`GameplayStatics.GetPlayerController` 0) self 1.0 "VTBlend_Linear" 0.0 false)))

(fn `Deactivate`
  (if (`self.IsActive`)
    (set `self.IsActive` false)
    (`PlayerController.SetViewTargetWithBlend` (`GameplayStatics.GetPlayerController` 0) (`GameplayStatics.GetPlayerPawn` 0) 1.0 "VTBlend_Linear" 0.0 false)))

(fn `GetCamera`
  (returns (ReturnValue :type "CameraComponent Object Reference"))
  (return (`self.GetComponentByClass` "/Script/Engine.CameraComponent")))

(fn `GetIsActive`
  (returns (IsActive :type Boolean))
  (return (`self.IsActive`)))

(fn `GetSpline`
  (returns (Spline :type "SplineComponent Object Reference"))
  (bind _returnvalue (`self.GetAttachParentActor`))
  (`/Engine/EditorBlueprintResources/StandardMacros.IsValid` _returnvalue
    (:`Is Valid`
      (bind _asspline_component (cast `SplineComponent` (`Actor.RootComponent` _returnvalue)))
      (return _asspline_component))))

(fn `UserConstructionScript`)