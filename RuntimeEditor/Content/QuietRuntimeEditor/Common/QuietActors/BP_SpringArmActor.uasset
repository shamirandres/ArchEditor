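; BP_SpringArmActor is a runtime-editor actor with a Thumbnail component that reflects its selection state in the outliner.
; On BeginPlay, a looping timer retries through a MultiGate until it finds a BP_QuietOutlinerComponent, then binds to its selection changes, or gives up after a fixed number of tries.
; Selection changes drive the thumbnail's state, debug mode toggles its visibility, and Tick keeps it at the actor's location.
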(event `self.ReceiveBeginPlay`
  (bind _returnvalue (`KismetSystemLibrary.K2_SetTimerDelegate` (delegate `TryToBindToSelect`) 0.5 true)))

(event `TryToBindToSelect`
  (`|MultiGate` false
    (:`Out 0`
      (bind _pinned (`/Game/QuietRuntimeEditor/Common/Blueprints/BP_QuietJsonMacroLibrary.Pin` (`self.GetComponentByClass` "/Game/QuietRuntimeEditor/Outliner/Blueprints/BP_QuietOutlinerComponent.BP_QuietOutlinerComponent_C") :!label _label))
      (`/Engine/EditorBlueprintResources/StandardMacros.IsValid` _pinned
        (:`Is Valid`
          (`KismetSystemLibrary.K2_ClearAndInvalidateTimerHandle` (stale `self.ReceiveBeginPlay` _returnvalue))
          (add `/Game/QuietRuntimeEditor/Outliner/Blueprints/BP_QuietOutlinerComponent.NotifyOnSelectionStateChanged` _pinned (delegate `HandleOnSelectionStateChanged`))
          (if (`/Game/QuietRuntimeEditor/Outliner/Blueprints/BP_QuietOutlinerComponent.GetSelectionState` _pinned)
            (`self.HandleOnSelectionStateChanged` true)))))
    (:`Out 1`
      (goto _label))
    (:`Out 2`
      (goto _label))
    (:`Out 3`
      (goto _label))
    (:`Out 4`
      (goto _label))
    (:`Out 5`
      (goto _label))
    (:`Out 6`
      (goto _label))
    (:`Out 7`
      (goto _label))
    (:`Out 8`
      (goto _label))
    (:`Out 9`
      (goto _label))
    (:`Out 10`
      (goto _label))
    (:`Out 11`
      (`KismetSystemLibrary.K2_ClearAndInvalidateTimerHandle` (stale `self.ReceiveBeginPlay` _returnvalue)))))

(event `HandleOnSelectionStateChanged`
  (params (NewState :type Boolean))
  (`/Game/QuietRuntimeEditor/Common/QuietActors/Blueprints/BP_ThumbnailComponent.ChangeSelectionState` (`self.Thumbnail`) NewState))

(event `/Game/QuietRuntimeEditor/Common/QuietActors/Blueprints/BI_QuietActorsInterface.EnableDebugMode`
  (params (Enable :type Boolean))
  (`/Game/QuietRuntimeEditor/Common/QuietActors/Blueprints/BP_ThumbnailComponent.SetThumbnailVisibility` (`self.Thumbnail`) Enable))

(event `self.ReceiveTick`
  (params (DeltaSeconds :type "Float (single-precision)"))
  (`SceneComponent.K2_SetWorldLocation` (`self.Thumbnail`) (`self.K2_GetActorLocation`) false false))

(fn `UserConstructionScript`)