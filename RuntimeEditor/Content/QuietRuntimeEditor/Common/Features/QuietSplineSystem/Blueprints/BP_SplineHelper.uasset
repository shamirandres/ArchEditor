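; BP_SplineHelper is a spline utility that creates and updates parallel, sideways-shifted copies of a spline and can cache or restore spline points.
; MakeShiftedSpline adds a SplineComponent to the outer component's owning actor, then UpdateShiftedSpline rebuilds its points.
; Offset positions use miter-style joins of neighboring segments' right vectors, handling open and closed ends.
; Tangents are scaled by offset-to-source distance ratios sampled a quarter key away.
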(event `CustomEvent_0`
  (bind _asactor (cast `Actor` (`KismetSystemLibrary.GetOuterObject` self)))
  (`|AddComponentByClass` :`self` _asactor :`Class` "/Script/Engine.SplineComponent"))

(fn `CachePoint`
  (params (Spline :type "SplineComponent Object Reference") (Index :type Integer))
  (returns (SplinePoint :type "SplinePoint Structure"))
  (return (make `SplinePoint` (`KismetMathLibrary.Conv_IntToDouble` Index) (`SplineComponent.GetLocationAtSplinePoint` Spline Index "Local") (`SplineComponent.GetArriveTangentAtSplinePoint` Spline Index "Local") (`SplineComponent.GetLeaveTangentAtSplinePoint` Spline Index "Local") (`SplineComponent.GetRotationAtSplinePoint` Spline Index "Local") (`SplineComponent.GetScaleAtSplinePoint` Spline Index) (`SplineComponent.GetSplinePointType` Spline Index))))

(fn `CacheSpline`
  (params (Spline :type "SplineComponent Object Reference"))
  (returns (Cache :type "Array of SplinePoint Structure"))
  (locals (Points :type "Array of SplinePoint Structure"))
  (for _index (range (`SplineComponent.GetNumberOfSplinePoints` Spline))
    (bind _splinepoint (`self.CachePoint` Spline _index))
    (`KismetArrayLibrary.Array_Add` (`local.Points`) _splinepoint))
  (return (`local.Points`)))

(fn `CalcArriveTangentOffset`
  (params (Index :type Integer) (Shift :type "Float (double-precision)"))
  (returns (ArriveTangent :type "Vector Structure"))
  (bind _spline (`self.Spline`))
  (bind _returnvalue (`SplineComponent.GetArriveTangentAtSplinePoint` (`self.Spline`) Index "Local"))
  (bind _returnvalue_2 (- (`KismetMathLibrary.Conv_IntToDouble` (`KismetMathLibrary.SelectInt` (`SplineComponent.GetNumberOfSplinePoints` (`self.Spline`)) Index (== Index 0))) 0.25))
  (if (`KismetMathLibrary.Vector_IsNormal` _returnvalue)
    (return _returnvalue)
    (else
      (return (* (`self.SafeDivideVector` (- (`self.GetOffsetPointAtInputKey` (`KismetMathLibrary.Conv_IntToDouble` Index) Shift) (`self.GetOffsetPointAtInputKey` _returnvalue_2 Shift)) (- (`SplineComponent.GetLocationAtSplinePoint` _spline Index "Local") (`SplineComponent.GetLocationAtSplineInputKey` _spline _returnvalue_2 "Local"))) _returnvalue)))))

(fn `CalcLeaveTangentOffset`
  (params (Index :type Integer) (Shift :type "Float (double-precision)"))
  (returns (LeaveTangent :type "Vector Structure"))
  (bind _returnvalue (`KismetMathLibrary.Conv_IntToDouble` Index))
  (bind _spline (`self.Spline`))
  (bind _returnvalue_2 (`SplineComponent.GetLeaveTangentAtSplinePoint` (`self.Spline`) Index "Local"))
  (bind _returnvalue_3 (+ _returnvalue 0.25))
  (if (`KismetMathLibrary.Vector_IsNormal` _returnvalue_2)
    (return _returnvalue_2)
    (else
      (return (* (`KismetMathLibrary.Vector_GetAbs` (`self.SafeDivideVector` (- (`self.GetOffsetPointAtInputKey` _returnvalue Shift) (`self.GetOffsetPointAtInputKey` _returnvalue_3 Shift)) (- (`SplineComponent.GetLocationAtSplineInputKey` _spline _returnvalue_3 "Local") (`SplineComponent.GetLocationAtSplinePoint` _spline Index "Local")))) _returnvalue_2)))))

(fn `CalcPointOffset`
  (params (VectorA :type "Vector Structure") (VectorB :type "Vector Structure") (LineOffset :type "Float (double-precision)"))
  (returns (ReturnValue :type "Vector Structure"))
  (bind _lineoffset (`local.LineOffset`))
  (bind _returnvalue (`KismetMathLibrary.Normal` (/ (+ VectorA VectorB) 2.0)))
  (bind _returnvalue_2 (`KismetMathLibrary.DegAcos` (`KismetMathLibrary.Abs` (`KismetMathLibrary.Dot_VectorVector` (`local.VectorA`) _returnvalue))))
  (return (* _returnvalue (`KismetMathLibrary.SelectFloat` (/ _lineoffset (`KismetMathLibrary.DegCos` (- 90.0 _returnvalue_2))) (/ _lineoffset (`KismetMathLibrary.DegCos` _returnvalue_2)) (> (`KismetMathLibrary.DegAcos` (`KismetMathLibrary.Abs` (`KismetMathLibrary.Dot_VectorVector` _returnvalue (`local.VectorA`)))) 90.0)))))

(fn `FindCurrentRightVector`
  (params (Start :type Integer) (End :type Integer))
  (returns (Source :type "Vector Structure") (Direction :type "Vector Structure"))
  (bind _spline (`self.Spline`))
  (bind _returnvalue (`SplineComponent.GetLocationAtSplinePoint` _spline Start "Local"))
  (return _returnvalue (`KismetMathLibrary.Cross_VectorVector` (`KismetMathLibrary.GetDirectionUnitVector` _returnvalue (`SplineComponent.GetLocationAtSplinePoint` _spline End "Local")) (`SplineComponent.GetUpVectorAtSplinePoint` _spline Start "Local"))))

(fn `FindCurrentRightVector_0`
  (params (Start :type Integer) (End :type Integer))
  (returns (Source :type "Vector Structure") (Direction :type "Vector Structure"))
  (bind _spline (`self.Spline`))
  (bind _returnvalue (`SplineComponent.GetLocationAtSplinePoint` _spline (`local.End`) "Local"))
  (bind _returnvalue_2 (`SplineComponent.GetLocationAtSplinePoint` _spline (`local.Start`) "Local"))
  (bind _returnvalue_3 (`SplineComponent.GetLeaveTangentAtSplinePoint` _spline (`local.Start`) "Local"))
  (bind _returnvalue_4 (`KismetMathLibrary.SelectVector` (`SplineComponent.GetLeaveTangentAtSplinePoint` _spline (`local.End`) "Local") _returnvalue_3 (> (`local.Start`) (`local.End`))))
  (return _returnvalue_2 (`KismetMathLibrary.Cross_VectorVector` (`KismetMathLibrary.VLerp` (`KismetMathLibrary.GetDirectionUnitVector` _returnvalue_2 _returnvalue) (`KismetMathLibrary.Normal` (`KismetMathLibrary.SelectVector` _returnvalue_3 _returnvalue_4 (and (== (`local.Start`) (- (`SplineComponent.GetNumberOfSplinePoints` (`self.Spline`)) 1)) (== (`local.End`) 0)))) (`KismetMathLibrary.FClamp` (/ (`KismetMathLibrary.VSize` _returnvalue_4) (`KismetMathLibrary.Vector_Distance` _returnvalue_2 _returnvalue)))) (`SplineComponent.GetUpVectorAtSplinePoint` _spline (`local.Start`) "Local"))))

(fn `GetLocationAtSplinePointWithOffset`
  (params (Index :type Integer) (Shift :type "Float (double-precision)"))
  (returns (ReturnValue :type "Vector Structure"))
  (bind _spline (`self.Spline`))
  (bind _returnvalue (`KismetMathLibrary.Normal` (`SplineComponent.GetArriveTangentAtSplinePoint` _spline Index "Local")))
  (return (+ (`SplineComponent.GetLocationAtSplinePoint` _spline Index "Local") (* (`KismetMathLibrary.RotateAngleAxis` _returnvalue (/ (`KismetMathLibrary.DegAcos` (`KismetMathLibrary.Dot_VectorVector` _returnvalue (`KismetMathLibrary.Normal` (`KismetMathLibrary.NegateVector` (`SplineComponent.GetLeaveTangentAtSplinePoint` _spline Index "Local"))))) 2.0) (`SplineComponent.GetUpVectorAtSplinePoint` _spline Index "Local")) Shift -1.0))))

(fn `GetOffsetLocationAtSplinePoint`
  (params (Index :type Integer) (Shift :type "Float (double-precision)") (Outline :type Boolean))
  (returns (ReturnValue :type "Vector Structure"))
  (locals (LastPoint :type Integer :default 0))
  (bind (_source _direction) (`self.FindCurrentRightVector` 0 1))
  (bind (_source_2 _direction_2) (`self.FindCurrentRightVector` 0 1))
  (bind _lastpoint (`local.LastPoint`))
  (bind _index (`local.Index`))
  (bind (_source_3 _direction_3) (`self.FindCurrentRightVector` _lastpoint))
  (bind (_source_4 _direction_4) (`self.FindCurrentRightVector` _index (+ _index 1)))
  (bind _output_get (set `local.LastPoint` (- (`SplineComponent.GetNumberOfSplinePoints` (`self.Spline`)) 1)))
  (if (== _output_get (`local.Index`))
    (if (`local.Outline`)
      _
      (elif (not (`SplineComponent.IsClosedLoop` (`self.Spline`)))
        _
        (else
          (return (+ _source_3 (`self.CalcPointOffset` (`.Direction` (`self.FindCurrentRightVector` (- _lastpoint 1) _lastpoint)) _direction_3 (`local.Shift`)))))))
    (return (+ (`SplineComponent.GetLocationAtSplinePoint` (`self.Spline`) (`local.LastPoint`) "Local") (* (`.Direction` (`self.FindCurrentRightVector` (- (`local.LastPoint`) 1) (`local.LastPoint`))) (`local.Shift`))))
    (elif (== 0 (`local.Index`))
      (if (`local.Outline`)
        _
        (elif (not (`SplineComponent.IsClosedLoop` (`self.Spline`)))
          _
          (else
            (return (+ _source_2 (`self.CalcPointOffset` (`.Direction` (`self.FindCurrentRightVector` (`local.LastPoint`))) _direction_2 (`local.Shift`)))))))
      (return (+ _source (* _direction (`local.Shift`))))
      (else
        ;[0 0 0] Middle Points
        (return (+ _source_4 (`self.CalcPointOffset` _direction_4 (`.Direction` (`self.FindCurrentRightVector` (- _index 1) _index)) (`local.Shift`))))))))

(fn `GetOffsetPointAtInputKey`
  (params (InKey :type "Float (single-precision)") (Shift :type "Float (double-precision)"))
  (returns (ReturnValue :type "Vector Structure"))
  (bind _spline (`self.Spline`))
  (return (+ (`SplineComponent.GetLocationAtSplineInputKey` _spline InKey "Local") (* (`SplineComponent.GetRightVectorAtSplineInputKey` _spline InKey "Local") Shift -1.0))))

(fn `MakeShiftedSpline`
  (params (Shift :type "Float (double-precision)"))
  (returns (NewSpline :type "SplineComponent Object Reference"))
  (bind _asactor_component (cast `ActorComponent` (`KismetSystemLibrary.GetOuterObject` self)))
  (bind _returnvalue (`|AddComponentByClass` :`self` (`ActorComponent.GetOwner` _asactor_component) :`Class` "/Script/Engine.SplineComponent"))
  (`self.UpdateShiftedSpline` _returnvalue Shift)
  (return _returnvalue))

(fn `RestorePoint`
  (params (Spline :type "SplineComponent Object Reference") (Point :type "SplinePoint Structure"))
  (bind (_inputkey _position _arrivetangent _leavetangent _rotation _scale _type) (break `SplinePoint` Point))
  (bind _pinned (`/Game/QuietRuntimeEditor/Common/Blueprints/BP_QuietJsonMacroLibrary.Pin` (`KismetMathLibrary.FTrunc` _inputkey)))
  (`SplineComponent.SetLocationAtSplinePoint` Spline _pinned _position "Local" true)
  (`SplineComponent.SetRotationAtSplinePoint` Spline _pinned _rotation "Local" true)
  (`SplineComponent.SetScaleAtSplinePoint` Spline _pinned _scale true)
  (`SplineComponent.SetSplinePointType` Spline _pinned _type true)
  (switch `ESplinePointType` _type
    (:`Linear`
      _)
    (:`Constant`
      _)
    (:`CurveClamped`
      _)
    (:`CurveCustomTangent`
      _))
  (`SplineComponent.SetTangentsAtSplinePoint` Spline _pinned _arrivetangent _leavetangent "Local" true)
  (return))

(fn `SafeDivideVector`
  (params (A :type "Vector Structure") (B :type "Vector Structure"))
  (returns (ReturnValue :type "Vector Structure"))
  (return (`KismetMathLibrary.MakeVector` (`KismetMathLibrary.SafeDivide` (.x A) (.x B)) (`KismetMathLibrary.SafeDivide` (.y A) (.y B)) (`KismetMathLibrary.SafeDivide` (.z A) (.z B)))))

(fn `UpdateShiftedSpline`
  (params (Spline :type "SplineComponent Object Reference") (Shift :type "Float (double-precision)"))
  (bind _spline (`self.Spline`))
  (`SplineComponent.ClearSplinePoints` Spline true)
  (`SplineComponent.SetClosedLoop` Spline (`SplineComponent.IsClosedLoop` (`self.Spline`)) false)
  (for _index (range (`SplineComponent.GetNumberOfSplinePoints` (`self.Spline`)))
    (bind _pinned (`/Game/QuietRuntimeEditor/Common/Blueprints/BP_QuietJsonMacroLibrary.Pin` (`self.GetOffsetLocationAtSplinePoint` _index Shift)))
    (`SplineComponent.AddPoint` Spline (make `SplinePoint` (`KismetMathLibrary.Conv_IntToDouble` _index) _pinned (`self.CalcArriveTangentOffset` _index Shift) (`self.CalcLeaveTangentOffset` _index Shift) (`SplineComponent.GetRotationAtSplinePoint` _spline _index "Local") (`SplineComponent.GetScaleAtSplinePoint` _spline _index) (`SplineComponent.GetSplinePointType` _spline _index)) false))
  (`SplineComponent.UpdateSpline` Spline)
  (return))