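; BP_Circle is a spline shape Blueprint in the QuietSplineSystem that procedurally builds a circle from a radius and point count.
; MakeCircle clears the spline and rotates evenly spaced points around Z, with custom tangents scaled by CalcTangentMult to approximate the arc.
; Construction, restore and update rebuild the circle before calling parent logic, though update does nothing when CustomSpline is set.
; DrawShape takes the radius from the dragged rectangle's vector length.
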(fn `DrawShape`
  (params (DraggedRectangle :type "Vector Structure"))
  (set `self.Radius` (`KismetMathLibrary.VSize` DraggedRectangle))
  (`self.MakeCircle`))

(fn `MakeCircle`
  (`SplineComponent.ClearSplinePoints` (`self.Spline`) true)
  (bind _pinned (`/Game/QuietRuntimeEditor/Common/Blueprints/BP_QuietJsonMacroLibrary.Pin` (/ 360.0 (`KismetMathLibrary.Conv_IntToDouble` (`self.PointsCount`))))) ; Angle
  (bind _returnvalue (`self.CalcTangentMult` (`self.Radius`) _pinned))
  (for _index (range (`self.PointsCount`))
    (bind _returnvalue_2 (* _index _pinned))
    (bind _returnvalue_3 (* (`KismetMathLibrary.RotateAngleAxis` (0.0 1.0 0.0) _returnvalue_2 (0.0 0.0 1.0)) _returnvalue -1.0))
    (`SplineComponent.AddPoint` (`self.Spline`) (make `SplinePoint` (`KismetMathLibrary.Conv_IntToDouble` _index) (`KismetMathLibrary.RotateAngleAxis` (`KismetMathLibrary.MakeVector` (`self.Radius`)) _returnvalue_2 (0.0 0.0 1.0)) _returnvalue_3 _returnvalue_3 (`KismetMathLibrary.MakeRotator` 0.0 0.0 _returnvalue_2) (1.0 1.0 1.0) "CurveCustomTangent") false))
  (`SplineComponent.UpdateSpline` (`self.Spline`)))

(fn `RestoreShape`
  (`self.MakeCircle`)
  (`parent.RestoreShape`))

(fn `UpdateShape`
  (if (not (`self.CustomSpline`))
    (`self.MakeCircle`)
    (`parent.UpdateShape`)))

(fn `UserConstructionScript`
  (`self.MakeCircle`)
  (`parent.UserConstructionScript`))