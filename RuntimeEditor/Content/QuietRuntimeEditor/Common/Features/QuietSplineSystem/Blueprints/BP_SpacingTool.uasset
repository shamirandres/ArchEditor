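; Spline spacing tool that scatters a set count of instances along a spline.
; PopulateEvent debounces rebuilds with a retriggerable delay, then Populate clears and re-adds instances using spline transforms, start-to-end offset blends and random jitter.
; A power-curve bias skews spacing toward either end, and a random chance leaves holes.
; A nonzero Shift uses a temporary shifted spline from BP_SplineHelper, destroyed after populating.
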(event `self.ReceiveEndPlay`
  (params (EndPlayReason :type "EEndPlayReason Enum" :default "Destroyed"))
  (switch `EEndPlayReason` EndPlayReason
    (:`Destroyed`
      (bind _shiftedspline (`self.ShiftedSpline`)
        (:`then`
          (`self.RequestToDestroyComponent` _shiftedspline))
        (:`else`)))))

(event `PopulateEvent`
  (`KismetSystemLibrary.RetriggerableDelay` 0.001)
  (`self.Populate`))

(fn `AcquireHelper`
  (returns (Helper :type "/Game/QuietRuntimeEditor/Common/Features/QuietSplineSystem/Blueprints/BP_SplineHelper Object Reference"))
  (`self.Helper`
    (:`then`
      _)
    (:`else`
      (bind _returnvalue (`|GenericCreateObject` "/Game/QuietRuntimeEditor/Common/Features/QuietSplineSystem/Blueprints/BP_SplineHelper.BP_SplineHelper_C" (`self.Spline`)))
      (set `self.Helper` _returnvalue)))
  (return (`self.Helper`)))

(fn `AcquireShiftedSpline`
  (returns (ShiftedSpline :type "SplineComponent Object Reference"))
  (`self.ShiftedSpline`
    (:`then`
      _)
    (:`else`
      (bind _newspline (`/Game/QuietRuntimeEditor/Common/Features/QuietSplineSystem/Blueprints/BP_SplineHelper.MakeShiftedSpline` (`self.AcquireHelper`) (`self.Shift`)))
      (set `self.ShiftedSpline` _newspline)))
  (return (`self.ShiftedSpline`)))

(fn `Populate`
  (bind (_randomrotation_roll _randomrotation_pitch _randomrotation_yaw) (`KismetMathLibrary.BreakRotator` (`self.RandomRotation`)))
  (bind _returnvalue (`KismetMathLibrary.MapRangeClamped` (`KismetMathLibrary.Abs` (`self.Bias`)) 0.0 1.0 1.0 5.0))
  (`self.ClearInstances`)
  (bind _spline (`self.SelectSpline`))
  (for _index (range (`self.Count`))
    (if (> (`self.RandomHoleChance`) 0)
      (if (> (`KismetMathLibrary.RandomIntegerInRange` 1 100) (`self.RandomHoleChance`))
        (bind _returnvalue_2 (`KismetMathLibrary.SelectFloat` (- 1.0 (`KismetMathLibrary.MultiplyMultiply_FloatFloat` (/ (`KismetMathLibrary.Conv_IntToDouble` (- (`self.Count`) _index)) (`KismetMathLibrary.Conv_IntToDouble` (`self.Count`))) _returnvalue)) (`KismetMathLibrary.MultiplyMultiply_FloatFloat` (/ (`KismetMathLibrary.Conv_IntToDouble` _index) (`KismetMathLibrary.Conv_IntToDouble` (`self.Count`))) _returnvalue) (< (`KismetMathLibrary.SignOfFloat` (`self.Bias`)) 0.0)))
        (bind _pinned (`/Game/QuietRuntimeEditor/Common/Blueprints/BP_QuietJsonMacroLibrary.Pin` (* _returnvalue_2 (`SplineComponent.GetSplineLength` _spline)) :!label _label)) ; Step Distance
        (bind (_returnvalue_x _returnvalue_y _returnvalue_z) (`KismetMathLibrary.BreakVector` (+ (`KismetMathLibrary.MakeVector` (+ (.roll (`SplineComponent.GetRotationAtDistanceAlongSpline` _spline _pinned "Local")) (.roll (`KismetMathLibrary.RLerp` (`self.StartRotationOffset`) (`self.EndRotationOffset`) _returnvalue_2))) (+ (.pitch (`SplineComponent.GetRotationAtDistanceAlongSpline` _spline _pinned "Local")) (.pitch (`KismetMathLibrary.RLerp` (`self.StartRotationOffset`) (`self.EndRotationOffset`) _returnvalue_2))) (+ (.yaw (`SplineComponent.GetRotationAtDistanceAlongSpline` _spline _pinned "Local")) (.yaw (`KismetMathLibrary.RLerp` (`self.StartRotationOffset`) (`self.EndRotationOffset`) _returnvalue_2)))) (`KismetMathLibrary.MakeVector` (`KismetMathLibrary.RandomFloatInRange` (* _randomrotation_roll -1.0) _randomrotation_roll) (`KismetMathLibrary.RandomFloatInRange` (* _randomrotation_pitch -1.0) _randomrotation_pitch) (`KismetMathLibrary.RandomFloatInRange` (* _randomrotation_yaw -1.0) _randomrotation_yaw)))))
        (bind _returnvalue_3 (+ (`KismetMathLibrary.VLerp` (`self.StartScaleOffset`) (`self.EndScaleOffset`) _returnvalue_2) (`KismetMathLibrary.RandomPointInBoundingBox` (0.0 0.0 0.0) (`self.RandomScaleOffset`))))
        (`self.AddInstance` (`KismetMathLibrary.MakeTransform` (+ (+ (`KismetMathLibrary.VLerp` (`self.StartOffset`) (`self.EndOffset`) _returnvalue_2) (`KismetMathLibrary.RandomPointInBoundingBox` (0.0 0.0 0.0) (`self.RandomOffset`))) (`SplineComponent.GetLocationAtDistanceAlongSpline` _spline _pinned "Local")) (`KismetMathLibrary.MakeRotator` _returnvalue_x _returnvalue_y _returnvalue_z) (+ (`SplineComponent.GetScaleAtDistanceAlongSpline` _spline _pinned) (`KismetMathLibrary.SelectVector` (`KismetMathLibrary.Conv_DoubleToVector` (.x _returnvalue_3)) _returnvalue_3 (`self.UniformScale`))))))
      (else
        (goto _label))))
  (bind _shiftedspline (`self.ShiftedSpline`)
    (:`then`
      (`self.RequestToDestroyComponent` _shiftedspline))
    (:`else`)))

(fn `SelectSpline`
  (returns (Spline :type "SplineComponent Object Reference"))
  (if (`KismetMathLibrary.NearlyEqual_FloatFloat` (`self.Shift`) 0.0 0.001)
    (return (`self.Spline`))
    (else
      (return (`self.AcquireShiftedSpline`)))))