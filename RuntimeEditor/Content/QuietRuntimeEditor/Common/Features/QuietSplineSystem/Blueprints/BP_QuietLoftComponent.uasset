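; Quiet spline system loft component that lays a static mesh along a source spline as one spline mesh component per segment.
; A helper builds a laterally shifted spline for offset lofts, while point scale and distance-interpolated twist shape each segment.
; Point edits accumulate with their neighbors and update next tick, falling back to a full rebuild.
; New segments copy properties from a "Donor"-tagged mesh component through serialization.
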(event `UpdatePointEvent`
  (params (Index :type Integer))
  (`self.UpdateShiftedSpline`)
  (`|ExecutionSequence`
    (:`then_0`
      (bind _indices (`self.IndexAccumulator` Index :!label _label))
      (for _array_element _indices
        (`self.UpdatePoint` _array_element)))
    (:`then_1`
      (`KismetSystemLibrary.DelayUntilNextTick`)
      (goto _label :!via `Exec`))))

(event `self.ReceiveEndPlay`
  (params (EndPlayReason :type "EEndPlayReason Enum" :default "Destroyed"))
  (bind (_arrayindex _arrayelement) (`/Engine/EditorBlueprintResources/StandardMacros.ReverseForEachLoop` (`self.Meshes`))
    (:`LoopBody`
      (`self.RequestToDestroyComponent` _arrayelement))
    (:`Completed`
      (`self.RemoveShiftedSpline`))))

(fn `AcquireHelper`
  (returns (Helper :type "/Game/QuietRuntimeEditor/Common/Features/QuietSplineSystem/Blueprints/BP_SplineHelper Object Reference"))
  (`self.Helper`
    (:`then`
      _)
    (:`else`
      (bind _returnvalue (`|GenericCreateObject` "/Game/QuietRuntimeEditor/Common/Features/QuietSplineSystem/Blueprints/BP_SplineHelper.BP_SplineHelper_C" (`self.SourceSpline`)))
      (set `self.Helper` _returnvalue)))
  (return (`self.Helper`)))

(fn `AcquireShiftedSpline`
  (returns (ShiftedSpline :type "SplineComponent Object Reference"))
  (`self.ShiftedSpline`
    (:`then`
      _)
    (:`else`
      (bind _newspline (`/Game/QuietRuntimeEditor/Common/Features/QuietSplineSystem/Blueprints/BP_SplineHelper.MakeShiftedSpline` (`self.AcquireHelper`) (`self.Shift`)))
      (set `self.ShiftedSpline` _newspline)))
  (return (`self.ShiftedSpline`)))

(fn `AcquireSplineMesh`
  (params (Index :type Integer))
  (returns (SplineMesh :type "SplineMeshComponent Object Reference"))
  (if (`KismetArrayLibrary.Array_IsValidIndex` (`self.Meshes`) Index)
    (bind _pinned (`/Game/QuietRuntimeEditor/Common/Blueprints/BP_QuietJsonMacroLibrary.Pin` (`|GetArrayItem` (`self.Meshes`) Index)))
    (`/Engine/EditorBlueprintResources/StandardMacros.IsValid` _pinned
      (:`Is Valid`
        (return _pinned))
      (:`Is Not Valid`
        _)))
  (bind _returnvalue (`|AddComponentByClass` (`self.GetOwner`) "/Game/QuietRuntimeEditor/Common/Features/QuietSplineSystem/Blueprints/BP_CustomSplineMeshComponent.BP_CustomSplineMeshComponent_C" false (`KismetMathLibrary.MakeTransform` (`self.Offset`))))
  (`KismetArrayLibrary.Array_Set` (`self.Meshes`) Index _returnvalue true)
  (if (`self.OverrideMaterial`)
    (`PrimitiveComponent.SetMaterial` _returnvalue 0 (`self.Material`)))
  (bind (_success _json) (`/Game/QuietRuntimeEditor/Common/Blueprints/BP_QuietEditorUtilities.SerializeObject` (`|GetArrayItem` (`Actor.GetComponentsByTag` (`self.GetOwner`) "/Script/Engine.StaticMeshComponent" "Donor"))))
  (`/Game/QuietRuntimeEditor/Common/Blueprints/BP_QuietEditorUtilities.DeserializeObject` _returnvalue _json)
  (`SceneComponent.SetMobility` _returnvalue "Movable")
  (`StaticMeshComponent.SetStaticMesh` _returnvalue (`self.StaticMesh`))
  (if (`/Game/QuietRuntimeEditor/Common/Blueprints/BP_QuietEditorUtilities.IsActorSelected` (`self.GetOwner`))
    (`PrimitiveComponent.SetRenderCustomDepth` _returnvalue true))
  (return _returnvalue))

(fn `Clear`
  (bind (_arrayindex _arrayelement) (`/Engine/EditorBlueprintResources/StandardMacros.ReverseForEachLoop` (`self.Meshes`))
    (:`LoopBody`
      (`self.RequestToDestroyComponent` _arrayelement))
    (:`Completed`
      (`KismetArrayLibrary.Array_Clear` (`self.Meshes`)))))

(fn `GetOverrideMaterial`
  (returns (OverrideMaterial :type Boolean))
  (return (`self.OverrideMaterial`)))

(fn `GetStaticMesh`
  (returns (StaticMesh :type "StaticMesh Object Reference"))
  (return (`self.StaticMesh`)))

(fn `GetTwistAtSplinePoint`
  (params (PointIndex :type Integer))
  (returns (ReturnValue :type "Float (double-precision)"))
  (bind _shiftedspline (`self.AcquireShiftedSpline`))
  (return (+ (`KismetMathLibrary.Lerp` 0.0 (`self.Twist`) (/ (`SplineComponent.GetDistanceAlongSplineAtSplinePoint` _shiftedspline PointIndex) (`SplineComponent.GetSplineLength` _shiftedspline))) (`SplineComponent.GetRollAtSplinePoint` _shiftedspline 0 "Local"))))

(fn `RebuildSpline`
  (bind _shiftedspline (`self.AcquireShiftedSpline`))
  (bind _shiftedspline_2 (`self.AcquireShiftedSpline`))
  (bind _sourcespline (`self.SourceSpline`))
  (for _index (range (+ (- (`SplineComponent.GetNumberOfSplinePoints` _sourcespline) (`KismetMathLibrary.SelectInt` 1 2 (`SplineComponent.IsClosedLoop` _sourcespline))) 1))
    (bind _splinemesh (`self.AcquireSplineMesh` _index))
    (bind _returnvalue (+ _index 1))
    (`SplineMeshComponent.SetStartAndEnd` _splinemesh (`SplineComponent.GetLocationAtSplinePoint` _shiftedspline_2 _index "Local") (`SplineComponent.GetLeaveTangentAtSplinePoint` _shiftedspline_2 _index "Local") (`SplineComponent.GetLocationAtSplinePoint` _shiftedspline _returnvalue "Local") (`SplineComponent.GetArriveTangentAtSplinePoint` _shiftedspline _returnvalue "Local") true)
    (`SplineMeshComponent.SetStartRoll` _splinemesh (`self.GetTwistAtSplinePoint` _index) true)
    (bind (_returnvalue_x _returnvalue_y _returnvalue_z) (`KismetMathLibrary.BreakVector` (`SplineComponent.GetScaleAtSplinePoint` (`self.SourceSpline`) _index)))
    (`SplineMeshComponent.SetStartScale` _splinemesh (`KismetMathLibrary.MakeVector2D` _returnvalue_y _returnvalue_z) true)
    (bind _returnvalue_2 (+ _index 1))
    (`SplineMeshComponent.SetEndRoll` _splinemesh (`self.GetTwistAtSplinePoint` _returnvalue_2) true)
    (bind (_returnvalue_x_2 _returnvalue_y_2 _returnvalue_z_2) (`KismetMathLibrary.BreakVector` (`SplineComponent.GetScaleAtSplinePoint` (`self.SourceSpline`) _returnvalue_2)))
    (`SplineMeshComponent.SetEndScale` _splinemesh (`KismetMathLibrary.MakeVector2D` _returnvalue_y_2 _returnvalue_z_2) true))
  (bind (_arrayindex _arrayelement) (`/Engine/EditorBlueprintResources/StandardMacros.ReverseForEachLoop` (`self.Meshes`))
    (:`LoopBody`
      (if (>= _arrayindex _index)
        (`self.RequestToDestroyComponent` _arrayelement)
        (`KismetArrayLibrary.Array_Remove` (`self.Meshes`) _arrayindex)
        (else
          (`|ExecutionSequence` :!label _label
            (:`then_0`
              (bind _shiftedspline_3 (`self.ShiftedSpline`)
                (:`then`
                  (`self.RequestToDestroyComponent` _shiftedspline_3))
                (:`else`)))
            (:`then_1`
              (return))))))
    (:`Completed`
      (goto _label))))

(fn `RemovePoint`
  (params (Index :type Integer))
  (`self.RequestToDestroyComponent` (`|GetArrayItem` (`self.Meshes`) Index))
  (`KismetArrayLibrary.Array_Remove` (`self.Meshes`) Index)
  (`self.UpdateShiftedSpline`)
  (`self.UpdatePoint` (`KismetMathLibrary.SelectInt` Index (- Index 1) (< Index (`SplineComponent.GetNumberOfSplinePoints` (`self.SourceSpline`))))))

(fn `RemoveShiftedSpline`
  (bind _shiftedspline (`self.ShiftedSpline`)
    (:`then`
      (`self.RequestToDestroyComponent` _shiftedspline))
    (:`else`)))

(fn `SelectSpline`
  (returns (Spline :type "SplineComponent Object Reference"))
  (if (`KismetMathLibrary.NearlyEqual_FloatFloat` (`self.Shift`) 0.0 0.001)
    (return (`self.SourceSpline`))
    (else
      (return (`self.AcquireShiftedSpline`)))))

(fn `SetCommonProperty`
  (params (Property :type String) (Value :type "JsonObjectWrapper Structure"))
  (for _array_element (`self.Meshes`)
    (`/Game/QuietRuntimeEditor/Common/Blueprints/BP_QuietEditorUtilities.SetPropertyByName` _array_element Property Value)))

(fn `SetLoftOffset`
  (params (NewOffset :type "Vector Structure"))
  (set `self.Offset` NewOffset)
  (for _array_element (`self.Meshes`)
    (`SceneComponent.K2_SetRelativeLocation` _array_element (`self.Offset`) false false)))

(fn `SetMaterial`
  (params (NewMaterial :type "MaterialInterface Object Reference"))
  (set `self.Material` NewMaterial)
  (`self.StaticMesh`
    (:`then`
      (if (`self.OverrideMaterial`)
        (for _array_element (`self.Meshes`)
          (`PrimitiveComponent.SetMaterial` _array_element 0 (`self.Material`)))))
    (:`else`)))

(fn `SetOverrideMaterial`
  (params (NewState :type Boolean))
  (set `self.OverrideMaterial` NewState)
  (bind _staticmesh (`self.StaticMesh`)
    (:`then`
      (for _array_element (`self.Meshes`)
        (`PrimitiveComponent.SetMaterial` _array_element 0 (select `bool` (`self.OverrideMaterial`) :`false` (`StaticMesh.GetMaterial` _staticmesh 0) :`true` (`self.Material`)))))
    (:`else`)))

(fn `SetShift`
  (params (NewShift :type "Float (double-precision)"))
  (set `self.Shift` NewShift)
  (`self.UpdateShiftedSpline`)
  (`self.RebuildSpline`))

(fn `SetStaticMesh`
  (params (StaticMesh :type "StaticMesh Object Reference"))
  (set `self.StaticMesh` StaticMesh)
  (for _array_element (`self.Meshes`)
    (`StaticMeshComponent.SetStaticMesh` _array_element (`self.StaticMesh`))
    (if (`self.OverrideMaterial`)
      (`PrimitiveComponent.SetMaterial` _array_element 0 (`self.Material`))))
  (`self.RebuildSpline`))

(fn `UpdatePoint`
  (params (Index :type Integer))
  (bind _spline (`self.SelectSpline`))
  (bind _returnvalue (`self.GetTwistAtSplinePoint` Index))
  (bind (_returnvalue_x _returnvalue_y _returnvalue_z) (`KismetMathLibrary.BreakVector` (`SplineComponent.GetScaleAtSplinePoint` (`self.SourceSpline`) Index)))
  (bind (_returnvalue_x_2 _returnvalue_y_2 _returnvalue_z_2) (`KismetMathLibrary.BreakVector` (`SplineComponent.GetScaleAtSplinePoint` (`self.SourceSpline`) Index)))
  (bind _pinned (`/Game/QuietRuntimeEditor/Common/Blueprints/BP_QuietJsonMacroLibrary.Pin` (`SplineComponent.GetLocationAtSplinePoint` (`self.SelectSpline`) Index "Local")))
  (`|ExecutionSequence`
    (:`then_0`
      (if (`KismetArrayLibrary.Array_IsValidIndex` (`self.Meshes`) Index)
        (bind _pinned_2 (`/Game/QuietRuntimeEditor/Common/Blueprints/BP_QuietJsonMacroLibrary.Pin` (`|GetArrayItem` (`self.Meshes`) Index)))
        (`SplineMeshComponent.SetStartPosition` _pinned_2 _pinned true)
        (`SplineMeshComponent.SetStartTangent` _pinned_2 (`SplineComponent.GetLeaveTangentAtSplinePoint` _spline Index "Local") true)
        (`SplineMeshComponent.SetStartRoll` _pinned_2 _returnvalue true)
        (`SplineMeshComponent.SetStartScale` _pinned_2 (`KismetMathLibrary.MakeVector2D` _returnvalue_y_2 _returnvalue_z_2) true)
        (else
          (`self.RebuildSpline`)
          (return))))
    (:`then_1`
      (bind _pinned_3 (`/Game/QuietRuntimeEditor/Common/Blueprints/BP_QuietJsonMacroLibrary.Pin` (- Index 1)))
      (bind _returnvalue_2 (>= _pinned_3 0))
      (if _returnvalue_2
        (bind _output (`|GetArrayItem` (`self.Meshes`) (`KismetMathLibrary.SelectInt` _pinned_3 (`KismetArrayLibrary.Array_LastIndex` (`self.Meshes`)) _returnvalue_2)))
        (`SplineMeshComponent.SetEndPosition` _output _pinned true :!label _label)
        (`SplineMeshComponent.SetEndTangent` _output (`SplineComponent.GetArriveTangentAtSplinePoint` _spline Index "Local") true)
        (`SplineMeshComponent.SetEndRoll` _output _returnvalue true)
        (`SplineMeshComponent.SetEndScale` _output (`KismetMathLibrary.MakeVector2D` _returnvalue_y _returnvalue_z) true)
        (elif (`SplineComponent.IsClosedLoop` (`self.SourceSpline`))
          (goto _label))))))

(fn `UpdateShiftedSpline`
  (bind _helper (`self.AcquireHelper`))
  (bind _shift (`self.Shift`))
  (bind _shiftedspline (`self.ShiftedSpline`)
    (:`then`
      (`/Game/QuietRuntimeEditor/Common/Features/QuietSplineSystem/Blueprints/BP_SplineHelper.UpdateShiftedSpline` _helper _shiftedspline _shift))
    (:`else`
      (bind _newspline (`/Game/QuietRuntimeEditor/Common/Features/QuietSplineSystem/Blueprints/BP_SplineHelper.MakeShiftedSpline` _helper _shift))
      (set `self.ShiftedSpline` _newspline))))