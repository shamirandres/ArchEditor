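; Helix shape for the runtime editor's spline system that procedurally builds a spiral spline from turns, height and start/end radii.
; MakeHelix places custom-tangent points, interpolating radius and skewing vertical spacing with a signed Bias power curve.
; DrawShape sizes it in three mouse steps: base radius, height and end radius, using cursor-ray plane intersections for the latter two.
; Construction and restore rebuild the helix, as does UpdateShape unless CustomSpline is set.
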(fn `CalcDrawingHeight`
  (returns (Intersection :type "Vector Structure"))
  (bind _returnvalue (`WidgetLayoutLibrary.GetMousePositionOnViewport`))
  (bind (_worldposition _worlddirection) (`GameplayStatics.DeprojectScreenToWorld` (`GameplayStatics.GetPlayerController` 0) (* _returnvalue (`WidgetLayoutLibrary.GetViewportScale`))))
  (return (`.Intersection` (`KismetMathLibrary.LinePlaneIntersection_OriginNormal` _worldposition (+ _worldposition (* _worlddirection 10000.0)) (`self.K2_GetActorLocation`) (`KismetMathLibrary.NegateVector` (`SceneComponent.GetForwardVector` (`PlayerCameraManager.TransformComponent` (`GameplayStatics.GetPlayerCameraManager` 0))))))))

(fn `CalcDrawingRadius`
  (returns (Intersection :type "Vector Structure"))
  (bind (_returnvalue_x _returnvalue_y) (`KismetMathLibrary.BreakVector` (`self.K2_GetActorLocation`)))
  (bind (_returnvalue_x_2 _returnvalue_y_2 _returnvalue_z) (`KismetMathLibrary.BreakVector` (`SplineComponent.GetLocationAtSplinePoint` (`self.Spline`) (- (`SplineComponent.GetNumberOfSplinePoints` (`self.Spline`)) 1) "Local")))
  (bind _returnvalue (`WidgetLayoutLibrary.GetMousePositionOnViewport`))
  (bind (_worldposition _worlddirection) (`GameplayStatics.DeprojectScreenToWorld` (`GameplayStatics.GetPlayerController` 0) (* _returnvalue (`WidgetLayoutLibrary.GetViewportScale`))))
  (return (`.Intersection` (`KismetMathLibrary.LinePlaneIntersection_OriginNormal` _worldposition (+ _worldposition (* _worlddirection 10000.0)) (`KismetMathLibrary.MakeVector` _returnvalue_x _returnvalue_y _returnvalue_z) (0.0 0.0 1.0)))))

(fn `DrawShape`
  (params (DraggedRectangle :type "Vector Structure"))
  (switch `int` (`self.DrawingStep`)
    (:`0`
      (set `self.Height` 0.1)
      (bind _output_get (set `self.StartRadius` (`KismetMathLibrary.VSize` DraggedRectangle)))
      (set `self.EndRadius` _output_get)
      (`self.MakeHelix`))
    (:`1`
      (bind _intersection (`self.CalcDrawingHeight`))
      (if (not (`KismetMathLibrary.Vector_IsZero` (`self.DrawingHeightPoint`)))
        (bind (_returnvalue_x _returnvalue_y _returnvalue_z) (`KismetMathLibrary.BreakVector` (- _intersection (`self.DrawingHeightPoint`))))
        (set `self.Height` (+ _returnvalue_z (`self.Height`)))
        (`self.MakeHelix`))
      (set `self.DrawingHeightPoint` _intersection))
    (:`2`
      (bind _intersection_2 (`self.CalcDrawingRadius`))
      (if (`KismetMathLibrary.Vector_IsZero` (`self.DrawingRadiusPoint`))
        (set `self.DrawingRadiusPoint` _intersection_2)
        (else
          (set `self.EndRadius` (`KismetMathLibrary.Vector_Distance` _intersection_2 (`self.DrawingRadiusPoint`)))
          (`self.MakeHelix`))))))

(fn `MakeHelix`
  (locals (Step :type Integer) (HeightStep :type "Float (double-precision)") (Angle :type "Float (double-precision)") (CurrentHeight :type "Float (double-precision)") (LastHeight :type "Float (double-precision)"))
  (bind _returnvalue (* (`self.Turns`) (`self.PointsCount`)))
  (`SplineComponent.ClearSplinePoints` (`self.Spline`) true)
  (set `local.HeightStep` (/ (`self.Height`) (`self.Turns`) (`self.PointsCount`)))
  (set `local.Angle` (/ 360.0 (`KismetMathLibrary.Conv_IntToDouble` (`self.PointsCount`))))
  (for _ (range (`self.Turns`))
    (for _index (range (`self.PointsCount`))
      (bind _pinned (`/Game/QuietRuntimeEditor/Common/Blueprints/BP_QuietJsonMacroLibrary.Pin` (* (`local.HeightStep`) (`local.Step`)) :!label _label)) ; CurrentHeight
      (bind _pinned_2 (`/Game/QuietRuntimeEditor/Common/Blueprints/BP_QuietJsonMacroLibrary.Pin` (`KismetMathLibrary.Lerp` (`self.StartRadius`) (`self.EndRadius`) (/ _pinned (`self.Height`))))) ; CurrentRadius
      (bind _returnvalue_2 (`self.CalcTangentMult` _pinned_2 (`local.Angle`)))
      (bind _pinned_3 (`/Game/QuietRuntimeEditor/Common/Blueprints/BP_QuietJsonMacroLibrary.Pin` (`KismetMathLibrary.SelectFloat` (- (`self.Height`) (* (`KismetMathLibrary.MultiplyMultiply_FloatFloat` (/ (`KismetMathLibrary.Conv_IntToDouble` (- _returnvalue (`local.Step`))) (`KismetMathLibrary.Conv_IntToDouble` _returnvalue)) (`KismetMathLibrary.MapRangeClamped` (`KismetMathLibrary.Abs` (`self.Bias`)) 0.0 1.0 1.0 10.0)) (`self.Height`))) (* (`KismetMathLibrary.MultiplyMultiply_FloatFloat` (/ (`KismetMathLibrary.Conv_IntToDouble` (`local.Step`)) (`KismetMathLibrary.Conv_IntToDouble` (* (`self.Turns`) (`self.PointsCount`)))) (`KismetMathLibrary.MapRangeClamped` (`self.Bias`) 0.0 1.0 1.0 10.0)) (`self.Height`)) (< (`KismetMathLibrary.SignOfFloat` (`self.Bias`)) 0.0))))
      (bind _returnvalue_3 (* _index (`local.Angle`)))
      (bind _returnvalue_4 (+ (* (`KismetMathLibrary.RotateAngleAxis` (0.0 1.0 0.0) _returnvalue_3 (0.0 0.0 1.0)) _returnvalue_2 -1.0) (`KismetMathLibrary.MakeVector` 0.0 0.0 (- _pinned_3 (`local.LastHeight`)))))
      (`SplineComponent.AddPoint` (`self.Spline`) (make `SplinePoint` (`KismetMathLibrary.Conv_IntToDouble` (`local.Step`)) (`KismetMathLibrary.RotateAngleAxis` (`KismetMathLibrary.MakeVector` _pinned_2 0.0 _pinned_3) _returnvalue_3 (0.0 0.0 1.0)) _returnvalue_4 _returnvalue_4 (`KismetMathLibrary.MakeRotator` 0.0 0.0 _returnvalue_3) (1.0 1.0 1.0) "CurveCustomTangent") true)
      (`/Engine/EditorBlueprintResources/StandardMacros.IncrementInt` (`local.Step`)
        (:`  `
          (set `local.LastHeight` _pinned_3)))))
  (goto _label))

(fn `RestoreShape`
  (`self.MakeHelix`)
  (`parent.RestoreShape`))

(fn `UpdateShape`
  (if (not (`self.CustomSpline`))
    (`self.MakeHelix`)
    (`parent.UpdateShape`)))

(fn `UserConstructionScript`
  (`self.MakeHelix`)
  (`parent.UserConstructionScript`))