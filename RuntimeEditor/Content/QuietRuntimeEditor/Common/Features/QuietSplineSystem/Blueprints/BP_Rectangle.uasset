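; Rectangle shape for the Quiet spline system that generates its outline on a Spline component from Length, Width and Fillet.
; MakeRectangle rotates corners in 90-degree steps, placing two custom-tangent points per rounded corner, or one when Fillet is negligible.
; The construction script and shape overrides rebuild through it: DrawShape sizes from a drag vector, RestoreShape regenerates, and UpdateShape skips custom splines.
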(fn `DrawShape`
  (params (DraggedRectangle :type "Vector Structure"))
  (set `self.Length` (.x (* (`KismetMathLibrary.Vector_GetAbs` DraggedRectangle) 2.0)))
  (set `self.Width` (.y (* (`KismetMathLibrary.Vector_GetAbs` DraggedRectangle) 2.0)))
  (`self.MakeRectangle`))

(fn `MakeRectangle`
  (bind _returnvalue (/ (`self.Width`) 2.0))
  (bind _returnvalue_2 (/ (`self.Length`) 2.0))
  (bind _returnvalue_3 (/ (`self.Length`) 2.0))
  (bind _returnvalue_4 (/ (`self.Width`) 2.0))
  (`SplineComponent.ClearSplinePoints` (`self.Spline`) true)
  (if (> (`self.Fillet`) 0.00099)
    (for _index (range 4)
      (bind _pinned (`/Game/QuietRuntimeEditor/Common/Blueprints/BP_QuietJsonMacroLibrary.Pin` (* (`KismetMathLibrary.Conv_IntToDouble` _index) 90.0)))
      (for (_array_element _array_index) (`|MakeArray` (`KismetMathLibrary.RotateAngleAxis` (0.0 -1.0 0.0) _pinned (0.0 0.0 1.0)) (`KismetMathLibrary.RotateAngleAxis` (-1.0 0.0 0.0) _pinned (0.0 0.0 1.0)))
        (bind _pinned_2 (`/Game/QuietRuntimeEditor/Common/Blueprints/BP_QuietJsonMacroLibrary.Pin` (* _array_element (`self.Fillet`))))
        (bind _returnvalue_5 (* (`KismetMathLibrary.SelectVector` _pinned_2 (`KismetMathLibrary.NegateVector` _pinned_2) (`KismetMathLibrary.Conv_IntToBool` _array_index)) 2.0))
        (`SplineComponent.AddPoint` (`self.Spline`) (make `SplinePoint` (`KismetMathLibrary.Conv_IntToDouble` (`SplineComponent.GetNumberOfSplinePoints` (`self.Spline`))) (+ _pinned_2 (`KismetMathLibrary.RotateAngleAxis` (`KismetMathLibrary.SelectVector` (`KismetMathLibrary.MakeVector` _returnvalue_2 _returnvalue) (`KismetMathLibrary.MakeVector` _returnvalue _returnvalue_2) (`self.IsOdd` _index)) _pinned (0.0 0.0 1.0))) _returnvalue_5 _returnvalue_5 (`KismetMathLibrary.MakeRotator` 0.0 0.0 _pinned) (1.0 1.0 1.0) "CurveCustomTangent") false)))
    (`SplineComponent.UpdateSpline` (`self.Spline`))
    (else
      (for _index_2 (range 4)
        (bind _pinned_3 (`/Game/QuietRuntimeEditor/Common/Blueprints/BP_QuietJsonMacroLibrary.Pin` (* 90.0 (`KismetMathLibrary.Conv_IntToDouble` _index_2))))
        (`SplineComponent.AddPoint` (`self.Spline`) (make `SplinePoint` (`KismetMathLibrary.Conv_IntToDouble` _index_2) (`KismetMathLibrary.RotateAngleAxis` (`KismetMathLibrary.SelectVector` (`KismetMathLibrary.MakeVector` _returnvalue_3 _returnvalue_4) (`KismetMathLibrary.MakeVector` _returnvalue_4 _returnvalue_3) (== (mod _index_2 2) 0)) _pinned_3 (0.0 0.0 1.0)) (`KismetMathLibrary.RotateAngleAxis` (1.0 0.0 0.0) _pinned_3 (0.0 0.0 1.0)) (`KismetMathLibrary.RotateAngleAxis` (0.0 1.0 0.0) _pinned_3 (0.0 0.0 1.0)) (`KismetMathLibrary.MakeRotator` 0.0 0.0 _pinned_3) (1.0 1.0 1.0) "CurveCustomTangent") false))
      (`/Game/QuietRuntimeEditor/Common/Features/QuietSplineSystem/Blueprints/BP_QuietSplineEditorComponent.ValidateSplinePointTypes` (`self.SplineEditor`))
      (`SplineComponent.UpdateSpline` (`self.Spline`)))))

(fn `RestoreShape`
  (`self.MakeRectangle`)
  (`parent.RestoreShape`))

(fn `UpdateShape`
  (if (not (`self.CustomSpline`))
    (`self.MakeRectangle`)
    (`parent.UpdateShape`)))

(fn `UserConstructionScript`
  (`self.MakeRectangle`)
  (`parent.UserConstructionScript`))