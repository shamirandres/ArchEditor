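; Base spline actor for the Quiet runtime editor, drawn with the mouse and decorated with loft meshes and spacing-tool instances.
; Spawning suspends pawn input and drives an empty DrawShape hook from a cursor-to-plane hit, presumably for child shapes.
; SplineEditor edits rebuild lofts and repopulate instances, and manual point changes flag the shape as custom.
; Shape, loft and spacing-tool operations register JSON history for undo/redo, restoring removed components from serialized data.
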(event `/Game/QuietRuntimeEditor/QuietGizmo/Blueprints/BI_GizmoBlueprintInterface.NotifyOnTransformed`
  (params (Component :type "SceneComponent Object Reference") (Mode :type "/Game/QuietRuntimeEditor/Common/Blueprints/Enums/E_TransformMode Enum" :default "NewEnumerator0") (Delta :type "Transform Structure"))
  (if (!= Component (`self.Spline`))
    (`self.CheckShape`)
    (bind _index (`/Game/QuietRuntimeEditor/Common/Features/QuietSplineSystem/Blueprints/BP_QuietSplineEditorComponent.HandleOnPointTransformed` (`self.SplineEditor`) Component Mode))
    (`self.UpdateLoftPoint` _index)
    (`self.PopulateInstances`)))

(event `self.SplineEditor.OnPointChanged`
  (params (Index :type Integer))
  (`self.CheckShape`)
  (`self.UpdateLoftPoint` Index)
  (`self.PopulateInstances`))

(event `/Game/QuietRuntimeEditor/QuietGizmo/Blueprints/BI_GizmoBlueprintInterface.NotifyStart`
  (`/Engine/EditorBlueprintResources/StandardMacros.DoOnce` false :!label _label
    (:`Completed`
      (`/Game/QuietRuntimeEditor/Common/Features/QuietSplineSystem/Blueprints/BP_QuietSplineEditorComponent.HandleOnStartTransform` (`self.SplineEditor`))
      (goto _label_2 :!via `Reset`))))

(event `/Game/QuietRuntimeEditor/QuietGizmo/Blueprints/BI_GizmoBlueprintInterface.NotifyEnd`
  (`/Engine/EditorBlueprintResources/StandardMacros.DoOnce` true :!label _label_2
    (:`Completed`
      (`/Game/QuietRuntimeEditor/Common/Features/QuietSplineSystem/Blueprints/BP_QuietSplineEditorComponent.HandleEndOfTransform` (`self.SplineEditor`))
      (goto _label :!via `Reset`))))

(event `self.SplineEditor.RequestToDestroyComponent`
  (params (Component :type "ActorComponent Object Reference"))
  (`ActorComponent.K2_DestroyComponent` Component))

(event `self.SplineEditor.OnPointRemoved`
  (params (Index :type Integer))
  (`self.UpdateLoft` :!label _label_3)
  (`self.PopulateInstances`))

(event `self.SplineEditor.OnSplineUpdated`
  (goto _label_3))

(event `UpdateMeshes`
  (goto _label_3))

(event `Refresh`
  (`KismetSystemLibrary.RetriggerableDelay` 0.01)
  (`self.UpdateShape`))

(event `/Game/QuietRuntimeEditor/Common/QuietActors/Blueprints/BI_QuietActorsInterface.EnableDebugMode`
  (params (Enable :type Boolean))
  (`/Game/QuietRuntimeEditor/Common/Features/QuietSplineSystem/Blueprints/BP_QuietSplineEditorComponent.SetSplineVisibility` (`self.SplineEditor`) Enable))

(event `self.ReceiveTick`
  (params (DeltaSeconds :type "Float (single-precision)"))
  (`/Engine/EditorBlueprintResources/StandardMacros.Gate` true :!label _label
    (:`Exit`
      (bind _returnvalue (`self.GetDraggedRectangle`))
      (`self.DrawShape` _returnvalue)
      (`/Game/QuietRuntimeEditor/Common/Features/QuietSplineSystem/Blueprints/BP_QuietSplineEditorComponent.UpdateSpline` (`self.SplineEditor`) false))))

(event `/Game/QuietRuntimeEditor/Common/QuietActors/Blueprints/BI_QuietActorsInterface.OnSpawned`
  (`self.DisablePawnInput`)
  (goto _label :!via `Open`))

(event `Key|LeftMouseButton` :consume false
  (params (Key :type "Key Structure"))
  (:`Pressed`
    (`self.DrawNewPoint`)
    (`self.IsNotCustom`)
    (`/Engine/EditorBlueprintResources/StandardMacros.IncrementInt` (`self.DrawingStep`) :!label _label_2
      (:`  `
        (if (not (< (`self.DrawingStep`) (`self.DrawingStepsCount`)))
          (bind _jsonobject (`/Game/QuietRuntimeEditor/Common/Blueprints/BP_QuietJsonFunctionLibrary.NewJson`))
          (bind _jsonobject_2 (`/Game/QuietRuntimeEditor/Common/Blueprints/BP_QuietJsonFunctionLibrary.NewJson`))
          (`/Game/QuietRuntimeEditor/Common/Blueprints/BP_QuietEditorUtilities.SerializeRegisteredActor` self _jsonobject_2)
          (`|SetJsonField` _jsonobject "Cache" _jsonobject_2)
          (`/Game/QuietRuntimeEditor/Common/Blueprints/BP_QuietEditorUtilities.RegisterHistoryAction` _jsonobject)
          (`self.EnablePawnInput` :!label _label_3)
          (`|ExecutionSequence`
            (:`then_0`
              (goto _label :!via `Close`))
            (:`then_1`
              (`KismetSystemLibrary.DelayUntilNextTick`)
              (`/Game/QuietRuntimeEditor/Common/Blueprints/BP_QuietEditorUtilities.RefreshActorDetails` self)))))))
  (:`Released`
    (if (> (`self.DrawingStep`) 0)
      (`self.IsNotCustom`)
      (goto _label_2))))

(event `Key|RightMouseButton` :overrideparent false
  (params (Key :type "Key Structure"))
  (:`Pressed`
    (`self.IsNotCustom`)
    (goto _label_3))
  (:`Released`
    (`self.StopLine`)))

(event `DrawNewPoint`
  (`/Engine/EditorBlueprintResources/StandardMacros.Gate` true :!label _label_4
    (:`Exit`
      (`/Game/QuietRuntimeEditor/Common/Features/QuietSplineSystem/Blueprints/BP_QuietSplineEditorComponent.DrawLine` (`self.SplineEditor`)))))

(event `StartDrawing`
  (`self.DisablePawnInput`)
  (goto _label_4 :!via `Open`))

(event `self.SplineEditor.NotifyOnLineFinished`
  (`|ExecutionSequence`
    (:`then_0`
      (goto _label_4 :!via `Close`))
    (:`then_1`
      (`KismetSystemLibrary.DelayUntilNextTick`)
      (`self.EnablePawnInput`))))

(event `StopLine`
  (`/Game/QuietRuntimeEditor/Common/Features/QuietSplineSystem/Blueprints/BP_QuietSplineEditorComponent.StopDrawing` (`self.SplineEditor`)))

(event `DrawNewSpline`
  (`/Game/QuietRuntimeEditor/Common/Features/QuietSplineSystem/Blueprints/BP_QuietSplineEditorComponent.StartRegisterDrawing` (`self.SplineEditor`))
  (`/Game/QuietRuntimeEditor/Common/Features/QuietSplineSystem/Blueprints/BP_QuietSplineEditorComponent.ClearSpline` (`self.SplineEditor`) false)
  (`self.StartDrawing`))

(event `DrawLine`
  (`/Game/QuietRuntimeEditor/Common/Features/QuietSplineSystem/Blueprints/BP_QuietSplineEditorComponent.StartRegisterDrawing` (`self.SplineEditor`))
  (`self.StartDrawing`))

(event `/Game/QuietRuntimeEditor/Common/QuietActors/Blueprints/BI_QuietActorsInterface.SendCommandWithData`
  (params (Command :type String) (Json :type "JsonObjectWrapper Structure"))
  (bind _splineeditor (`self.SplineEditor`))
  (bind _outvalue (`|GetJsonField` Json "Operation"))
  (switch `string` _outvalue
    (:`Default`
      (switch `string` Command
        (:`Undo`
          (`/Game/QuietRuntimeEditor/Common/Features/QuietSplineSystem/Blueprints/BP_QuietSplineEditorComponent.UndoSpline` _splineeditor Json))
        (:`Redo`
          (`/Game/QuietRuntimeEditor/Common/Features/QuietSplineSystem/Blueprints/BP_QuietSplineEditorComponent.RedoSpline` _splineeditor Json))))
    (:`RestoreShape`
      (switch `string` Command
        (:`Undo`
          (set `self.CustomSpline` true :!label _label)
          (`/Game/QuietRuntimeEditor/Common/Blueprints/BP_QuietEditorUtilities.RefreshActorDetails` self))
        (:`Redo`
          (set `self.CustomSpline` false :!label _label_2)
          (`/Game/QuietRuntimeEditor/Common/Blueprints/BP_QuietEditorUtilities.RefreshActorDetails` self)
          (`/Game/QuietRuntimeEditor/Common/Features/QuietSplineSystem/Blueprints/BP_QuietSplineEditorComponent.UpdateSpline` (`self.SplineEditor`) true)
          (`self.UpdateMeshes`))))
    (:`EditSpline`
      (switch `string` Command
        (:`Undo`
          (goto _label_2))
        (:`Redo`
          (goto _label))))
    (:`RemoveLoft`
      (switch `string` Command
        (:`Undo`
          (bind _outvalue_2 (`|GetJsonField` Json "Loft"))
          (bind _outvalue_3 (`|GetJsonField` Json "Index"))
          (bind _returnvalue (`|AddComponentByClass` "/Game/QuietRuntimeEditor/Common/Features/QuietSplineSystem/Blueprints/BP_QuietLoftComponent.BP_QuietLoftComponent_C" (`self.Spline`) null))
          (`KismetArrayLibrary.Array_Set` (`self.Lofts`) _outvalue_3 _returnvalue true)
          (add `/Game/QuietRuntimeEditor/Common/Features/QuietSplineSystem/Blueprints/BP_QuietLoftComponent.RequestToDestroyComponent` _returnvalue (`|CreateDelegate` :!event `DestroyComponent`))
          (`/Game/QuietRuntimeEditor/Common/Blueprints/BP_QuietEditorUtilities.DeserializeObject` _returnvalue _outvalue_2)
          (`/Game/QuietRuntimeEditor/Common/Blueprints/BP_QuietEditorUtilities.RefreshActorDetails` self))
        (:`Redo`
          (bind _outvalue_4 (`|GetJsonField` Json "Index"))
          (`self.RemoveLoft` _outvalue_4))))
    (:`AddNewLoft`
      (switch `string` Command
        (:`Undo`
          (`self.RemoveLoft` (`KismetArrayLibrary.Array_LastIndex` (`self.Lofts`))))
        (:`Redo`
          (`self.AddNewLoft` false))))
    (:`AddNewSpacingTool`
      (switch `string` Command
        (:`Undo`
          (`self.RemoveSpacingTool` (`KismetArrayLibrary.Array_LastIndex` (`self.Instances`))))
        (:`Redo`
          (`self.AddNewSpacingTool` false))))
    (:`RemoveSpacingTool`
      (switch `string` Command
        (:`Undo`
          (bind _outvalue_5 (`|GetJsonField` Json "SpacingTool"))
          (bind _outvalue_6 (`|GetJsonField` Json "Index"))
          (bind _returnvalue_2 (`AddComponent|NODE_AddBP_SpacingTool-3` :`Spline` (`self.Spline`) :`Mesh` null))
          (`KismetArrayLibrary.Array_Set` (`self.Instances`) _outvalue_6 _returnvalue_2 true)
          (add `/Game/QuietRuntimeEditor/Common/Features/QuietSplineSystem/Blueprints/BP_SpacingTool.RequestToDestroyComponent` _returnvalue_2 (`|CreateDelegate` :!event `DestroyComponent`))
          (`/Game/QuietRuntimeEditor/Common/Blueprints/BP_QuietEditorUtilities.DeserializeObject` _returnvalue_2 _outvalue_5)
          (`/Game/QuietRuntimeEditor/Common/Blueprints/BP_QuietEditorUtilities.RefreshActorDetails` self))
        (:`Redo`
          (bind _outvalue_7 (`|GetJsonField` Json "Index"))
          (`self.RemoveSpacingTool` _outvalue_7))))))

(fn `AcquireSplinePoint`
  (params (Index :type Integer) (Point :type "SplinePoint Structure") (bUpdateSpline :type Boolean))
  (bind (_inputkey _position _arrivetangent _leavetangent _rotation _scale _type) (break `SplinePoint` Point))
  (if (> (- (`SplineComponent.GetNumberOfSplinePoints` (`self.Spline`)) 1) Index)
    (`SplineComponent.SetSplinePointType` (`self.Spline`) Index _type false)
    (`SplineComponent.SetLocationAtSplinePoint` (`self.Spline`) Index _position "Local" false)
    (`SplineComponent.SetRotationAtSplinePoint` (`self.Spline`) Index _rotation "Local" false)
    (`SplineComponent.SetScaleAtSplinePoint` (`self.Spline`) Index _scale false)
    (`SplineComponent.SetTangentsAtSplinePoint` (`self.Spline`) Index _arrivetangent _leavetangent "Local" bUpdateSpline)
    (else
      (`SplineComponent.AddPoint` (`self.Spline`) Point bUpdateSpline))))

(fn `AddNewLoft`
  (params (Register :type Boolean))
  (bind _loft (`self.CreateLoftComponent`))
  (`/Engine/EditorBlueprintResources/StandardMacros.IsValid` (`/Game/QuietRuntimeEditor/Common/Features/QuietSplineSystem/Blueprints/BP_QuietLoftComponent.GetStaticMesh` _loft)
    (:`Is Valid`
      (`/Game/QuietRuntimeEditor/Common/Features/QuietSplineSystem/Blueprints/BP_QuietLoftComponent.RebuildSpline` _loft))
    (:`Is Not Valid`
      _))
  (`/Game/QuietRuntimeEditor/Common/Blueprints/BP_QuietEditorUtilities.RefreshActorDetails` self)
  (bind (_success _json) (`/Game/QuietRuntimeEditor/Common/Blueprints/BP_QuietEditorUtilities.SerializeObject` (`self.MeshSettingsDonor`)))
  (`/Game/QuietRuntimeEditor/Common/Blueprints/BP_QuietEditorUtilities.DeserializeObject` _loft _json)
  (if Register
    (`/Game/QuietRuntimeEditor/Common/Features/QuietSplineSystem/Blueprints/BP_QuietSplineEditorComponent.RegisterHistoryAction` (`self.SplineEditor`) (make `JsonObjectWrapper`) "AddNewLoft")))

(fn `AddNewSpacingTool`
  (params (Register :type Boolean))
  (returns (SpacingTool :type "/Game/QuietRuntimeEditor/Common/Features/QuietSplineSystem/Blueprints/BP_SpacingTool Object Reference"))
  (bind _returnvalue (`AddComponent|NODE_AddBP_SpacingTool-1` :`Spline` (`self.Spline`) :`Mesh` null))
  (`KismetArrayLibrary.Array_Add` (`self.Instances`) _returnvalue)
  (add `/Game/QuietRuntimeEditor/Common/Features/QuietSplineSystem/Blueprints/BP_SpacingTool.RequestToDestroyComponent` _returnvalue (`|CreateDelegate` :!event `DestroyComponent`))
  (`/Game/QuietRuntimeEditor/Common/Features/QuietSplineSystem/Blueprints/BP_SpacingTool.PopulateEvent` _returnvalue)
  (bind (_success _json) (`/Game/QuietRuntimeEditor/Common/Blueprints/BP_QuietEditorUtilities.SerializeObject` (`self.MeshSettingsDonor`)))
  (`/Game/QuietRuntimeEditor/Common/Blueprints/BP_QuietEditorUtilities.DeserializeObject` _returnvalue _json)
  (if Register
    (`/Game/QuietRuntimeEditor/Common/Features/QuietSplineSystem/Blueprints/BP_QuietSplineEditorComponent.RegisterHistoryAction` (`self.SplineEditor`) (make `JsonObjectWrapper`) "AddNewSpacingTool"))
  (return _returnvalue))

(fn `CalcTangentMult`
  (params (InRadius :type "Float (double-precision)") (InAngle :type "Float (double-precision)"))
  (returns (ReturnValue :type "Float (double-precision)"))
  (locals (A :type "Float (double-precision)" :default 0.5) (AA :type "Float (double-precision)" :default 0.5) (AAA :type "Float (double-precision)") (T0 :type "Vector Structure" :default (1.0 0.0 0.0)) (T1 :type "Vector Structure") (P0 :type "Vector Structure") (P1 :type "Vector Structure" :default (0.0 0.0 0.0)))
  (bind _t0_x (`KismetMathLibrary.BreakVector` (`local.T0`)))
  (bind _t1_x (`KismetMathLibrary.BreakVector` (`local.T1`)))
  (bind _a (`local.A`))
  (set `local.AA` (* _a _a))
  (set `local.AAA` (* (`local.AA`) (`local.A`)))
  (set `local.T1` (`KismetMathLibrary.RotateAngleAxis` (`local.T0`) (`local.InAngle`) (0.0 0.0 1.0)))
  (set `local.P0` (* (0.0 1.0 0.0) (`local.InRadius`)))
  (set `local.P1` (`KismetMathLibrary.RotateAngleAxis` (`local.P0`) (`local.InAngle`) (0.0 0.0 1.0)))
  (bind _returnvalue (`self.CubicInterp` (`local.P0`) (`local.T0`) (`local.P1`) (`local.T1`) (`local.A`))) ; ActualVal
  (bind _pinned (`/Game/QuietRuntimeEditor/Common/Blueprints/BP_QuietJsonMacroLibrary.Pin` (* (+ (* (+ (- (`local.AAA`) (* (`local.AA`) 2.0)) (`local.A`)) _t0_x) (* (- (`local.AAA`) (`local.AA`)) _t1_x)) -1.0))) ; PartialInterp
  (if (`KismetMathLibrary.NearlyEqual_FloatFloat` _pinned 0.0 0.001)
    (return _pinned)
    (else
      (bind _returnvalue_x (`KismetMathLibrary.BreakVector` (- _returnvalue (`KismetMathLibrary.RotateAngleAxis` (`local.P0`) (* (`local.InAngle`) (`local.A`)) (0.0 0.0 1.0)))))
      (return (/ _returnvalue_x _pinned)))))

(fn `CheckShape`
  (if (not (`self.CustomSpline`))
    (set `self.CustomSpline` true)
    (`/Game/QuietRuntimeEditor/Common/Blueprints/BP_QuietEditorUtilities.RefreshActorDetails` self)))

(fn `CreateLoftComponent`
  (returns (Loft :type "/Game/QuietRuntimeEditor/Common/Features/QuietSplineSystem/Blueprints/BP_QuietLoftComponent Object Reference"))
  (bind _returnvalue (`|AddComponentByClass` "/Game/QuietRuntimeEditor/Common/Features/QuietSplineSystem/Blueprints/BP_QuietLoftComponent.BP_QuietLoftComponent_C" (`self.Spline`) null))
  (`KismetArrayLibrary.Array_Add` (`self.Lofts`) _returnvalue)
  (add `/Game/QuietRuntimeEditor/Common/Features/QuietSplineSystem/Blueprints/BP_QuietLoftComponent.RequestToDestroyComponent` _returnvalue (`|CreateDelegate` :!event `DestroyComponent`))
  (return _returnvalue))

(fn `CubicInterp`
  (params (P0 :type "Vector Structure") (T0 :type "Vector Structure") (P1 :type "Vector Structure") (T1 :type "Vector Structure") (A :type "Float (double-precision)"))
  (returns (ReturnValue :type "Vector Structure"))
  (locals (A2 :type "Float (double-precision)") (A3 :type "Float (double-precision)"))
  (bind _output_get (set `local.A2` (* A A)))
  (set `local.A3` (* _output_get A))
  (return (+ (* (+ (- (* (`local.A3`) 2.0) (* (`local.A2`) 3.0)) 1.0) (`local.P0`)) (* (+ (- (`local.A3`) (* (`local.A2`) 2.0)) (`local.A`)) (`local.T0`)) (* (- (`local.A3`) (`local.A2`)) (`local.T1`)) (* (+ (* (`local.A3`) -2.0) (* (`local.A2`) 3.0)) (`local.P1`)))))

(fn `CutSpline`
  (params (LastPoint :type Integer))
  (bind _returnvalue (- (`SplineComponent.GetNumberOfSplinePoints` (`self.Spline`)) 1))
  (while (< LastPoint _returnvalue)
    (`SplineComponent.RemoveSplinePoint` (`self.Spline`) _returnvalue false)))

(fn `DestroyComponent`
  (params (ActorComponent :type "ActorComponent Object Reference"))
  (`ActorComponent.K2_DestroyComponent` ActorComponent))

(fn `DisablePawnInput`
  (`self.EnableInput` (`GameplayStatics.GetPlayerController` 0))
  (message `/Game/QuietRuntimeEditor/Common/Blueprints/BI_QuietRoutingInterface.ForwardCommand` (`GameplayStatics.GetPlayerPawn` 0) (struct :`TagName` "EditorPawn.SuspendInput"))
  (set `PlayerController.bEnableClickEvents` false (`GameplayStatics.GetPlayerController` 0)))

(fn `DrawShape`
  (params (DraggedRectangle :type "Vector Structure")))

(fn `EditSpline`
  (set `self.CustomSpline` true)
  (`/Game/QuietRuntimeEditor/Common/Blueprints/BP_QuietEditorUtilities.RefreshActorDetails` self)
  (`/Game/QuietRuntimeEditor/Common/Features/QuietSplineSystem/Blueprints/BP_QuietSplineEditorComponent.RegisterHistoryAction` (`self.SplineEditor`) (make `JsonObjectWrapper`) "EditSpline"))

(fn `EnablePawnInput`
  (message `/Game/QuietRuntimeEditor/Common/Blueprints/BI_QuietRoutingInterface.ForwardCommand` (`GameplayStatics.GetPlayerPawn` 0) (struct :`TagName` "EditorPawn.ResumeInput"))
  (set `PlayerController.bEnableClickEvents` true (`GameplayStatics.GetPlayerController` 0))
  (`self.DisableInput` (`GameplayStatics.GetPlayerController` 0)))

(fn `GetAlignState`
  (returns (State :type Boolean))
  (return false))

(fn `GetDeltaStateByType`
  (returns (State :type Boolean))
  (return false))

(fn `GetDeltaValueByType`
  (returns (Value :type "Float (double-precision)"))
  (return 0.0))

(fn `GetDraggedRectangle`
  (returns (ReturnValue :type "Vector Structure"))
  (bind _returnvalue (`WidgetLayoutLibrary.GetMousePositionOnViewport`))
  (bind (_worldposition _worlddirection) (`GameplayStatics.DeprojectScreenToWorld` (`GameplayStatics.GetPlayerController` 0) (* _returnvalue (`WidgetLayoutLibrary.GetViewportScale`))))
  (return (- (`.Intersection` (`KismetMathLibrary.LinePlaneIntersection_OriginNormal` _worldposition (+ _worldposition (* _worlddirection 10000.0)) (`self.K2_GetActorLocation`) (`self.GetActorUpVector`))) (`self.K2_GetActorLocation`))))

(fn `GetInitialSize`
  (returns (ReturnValue :type "Float (double-precision)"))
  (locals (DesiredSize :type "Float (double-precision)" :default 100.0))
  (bind _returnvalue (`GameplayStatics.GetPlayerCameraManager` 0))
  (bind _returnvalue_2 (`self.K2_GetActorLocation` self))
  (bind _returnvalue_3 (- (`SceneComponent.K2_GetComponentLocation` (`PlayerCameraManager.TransformComponent` _returnvalue)) _returnvalue_2))
  (bind (_returnvalue_x _returnvalue_y _returnvalue_z) (`KismetMathLibrary.BreakVector` (* _returnvalue_3 _returnvalue_3)))
  (return (`KismetMathLibrary.FClamp` (* (* (`PlayerCameraManager.GetFOVAngle` _returnvalue) (`KismetMathLibrary.Sqrt` (+ _returnvalue_x _returnvalue_y _returnvalue_z)) (`KismetMathLibrary.Dot_VectorVector` (`self.GetActorForwardVector` _returnvalue) (`KismetMathLibrary.Conv_RotatorToVector` (`KismetMathLibrary.FindLookAtRotation` (`PlayerCameraManager.GetCameraLocation` _returnvalue) _returnvalue_2)))) 1e-05 (`local.DesiredSize`)) 0.1 10000.0)))

(fn `GetMainSelectedActor`
  (returns (MainActor :type "Actor Object Reference"))
  (return null))

(fn `GetPivotLocation`
  (returns (UseSelectionCenter :type Boolean))
  (return false))

(fn `GetRelativeByType`
  (returns (State :type Boolean))
  (return false))

(fn `GetScaleUniformState`
  (returns (State :type Boolean))
  (return false))

(fn `GetSelectedActors`
  (returns (Actors :type "Array of Actor Object Reference"))
  (return))

(fn `GetTransformMode`
  (returns (Mode :type "/Game/QuietRuntimeEditor/Common/Blueprints/Enums/E_TransformMode Enum"))
  (return "NewEnumerator0"))

(fn `GizmoOverState`
  (returns (State :type Boolean))
  (return false))

(fn `IsOdd`
  (params (Index :type Integer))
  (returns (ReturnValue :type Boolean))
  (return (== (mod Index 2) 0)))

(fn `PopulateInstances`
  (for _array_element (`self.Instances`)
    (`/Game/QuietRuntimeEditor/Common/Features/QuietSplineSystem/Blueprints/BP_SpacingTool.PopulateEvent` _array_element)))

(fn `RemoveLoft`
  (params (Index :type Integer) (Register :type Boolean))
  (if (`KismetArrayLibrary.Array_IsValidIndex` (`self.Lofts`) Index)
    (bind _pinned (`/Game/QuietRuntimeEditor/Common/Blueprints/BP_QuietJsonMacroLibrary.Pin` (`|GetArrayItem` (`self.Lofts`) Index)))
    (if Register
      (bind (_success _json) (`/Game/QuietRuntimeEditor/Common/Blueprints/BP_QuietEditorUtilities.SerializeObject` _pinned))
      (bind _jsonobject (`/Game/QuietRuntimeEditor/Common/Blueprints/BP_QuietJsonFunctionLibrary.NewJson`))
      (`|SetJsonField` _jsonobject "Loft" _json)
      (`|SetJsonField` _jsonobject "Index" Index)
      (`/Game/QuietRuntimeEditor/Common/Features/QuietSplineSystem/Blueprints/BP_QuietSplineEditorComponent.RegisterHistoryAction` (`self.SplineEditor`) _jsonobject "RemoveLoft"))
    (`KismetArrayLibrary.Array_Remove` (`self.Lofts`) Index)
    (`/Engine/EditorBlueprintResources/StandardMacros.IsValid` _pinned
      (:`Is Valid`
        (`ActorComponent.K2_DestroyComponent` _pinned)
        (`/Game/QuietRuntimeEditor/Common/Blueprints/BP_QuietEditorUtilities.RefreshActorDetails` self)))))

(fn `RemoveSpacingTool`
  (params (Index :type Integer) (Register :type Boolean))
  (if (`KismetArrayLibrary.Array_IsValidIndex` (`self.Instances`) Index)
    (bind _pinned (`/Game/QuietRuntimeEditor/Common/Blueprints/BP_QuietJsonMacroLibrary.Pin` (`|GetArrayItem` (`self.Instances`) Index)))
    (if Register
      (bind (_success _json) (`/Game/QuietRuntimeEditor/Common/Blueprints/BP_QuietEditorUtilities.SerializeObject` _pinned))
      (bind _jsonobject (`/Game/QuietRuntimeEditor/Common/Blueprints/BP_QuietJsonFunctionLibrary.NewJson`))
      (`|SetJsonField` _jsonobject "SpacingTool" _json)
      (`|SetJsonField` _jsonobject "Index" Index)
      (`/Game/QuietRuntimeEditor/Common/Features/QuietSplineSystem/Blueprints/BP_QuietSplineEditorComponent.RegisterHistoryAction` (`self.SplineEditor`) _jsonobject "RemoveSpacingTool"))
    (`KismetArrayLibrary.Array_Remove` (`self.Instances`) Index)
    (`/Engine/EditorBlueprintResources/StandardMacros.IsValid` _pinned
      (:`Is Valid`
        (`ActorComponent.K2_DestroyComponent` _pinned)
        (`/Game/QuietRuntimeEditor/Common/Blueprints/BP_QuietEditorUtilities.RefreshActorDetails` self)))))

(fn `RestoreShape`
  (set `self.CustomSpline` false)
  (`/Game/QuietRuntimeEditor/Common/Blueprints/BP_QuietEditorUtilities.RefreshActorDetails` self)
  (`/Game/QuietRuntimeEditor/Common/Features/QuietSplineSystem/Blueprints/BP_QuietSplineEditorComponent.UpdateSpline` (`self.SplineEditor`) true)
  (`self.UpdateMeshes`)
  (`/Game/QuietRuntimeEditor/Common/Features/QuietSplineSystem/Blueprints/BP_QuietSplineEditorComponent.RegisterHistoryAction` (`self.SplineEditor`) (make `JsonObjectWrapper`) "RestoreShape")
  (`/Game/QuietRuntimeEditor/Common/Blueprints/BP_QuietEditorUtilities.RefreshSelectedComponent`)
  (`/Game/QuietRuntimeEditor/Common/Features/QuietSplineSystem/Blueprints/BP_QuietSplineEditorComponent.UpdateTangents` (`self.SplineEditor`)))

(fn `UpdateLoft`
  (for _array_element (`self.Lofts`)
    (`/Game/QuietRuntimeEditor/Common/Features/QuietSplineSystem/Blueprints/BP_QuietLoftComponent.RebuildSpline` _array_element)))

(fn `UpdateLoftPoint`
  (params (Index :type Integer))
  (for _array_element (`self.Lofts`)
    (`/Game/QuietRuntimeEditor/Common/Features/QuietSplineSystem/Blueprints/BP_QuietLoftComponent.UpdatePointEvent` _array_element Index)))

(fn `UpdateShape`
  (`/Game/QuietRuntimeEditor/Common/Features/QuietSplineSystem/Blueprints/BP_QuietSplineEditorComponent.UpdateSpline` (`self.SplineEditor`) true)
  (`/Game/QuietRuntimeEditor/Common/Features/QuietSplineSystem/Blueprints/BP_QuietSplineEditorComponent.UpdateTangents` (`self.SplineEditor`))
  (`self.UpdateMeshes`))

(fn `UserConstructionScript`)