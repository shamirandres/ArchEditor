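; BP_NGon is a parametric spline shape that builds a regular polygon from side count, radius and corner fillet.
; MakeNGon rebuilds the spline by rotating points around Z, using two custom-tangent points per corner when filleted, otherwise one point followed by SplineEditor point-type validation.
; It runs on construction, restore and update, skipping updates for custom splines; DrawShape sets the radius from the dragged rectangle's vector length.
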(fn `DrawShape`
  (params (DraggedRectangle :type "Vector Structure"))
  (set `self.Radius` (`KismetMathLibrary.VSize` DraggedRectangle))
  (`self.MakeNGon`))

(fn `MakeNGon`
  (`SplineComponent.ClearSplinePoints` (`self.Spline`) true)
  (bind _pinned (`/Game/QuietRuntimeEditor/Common/Blueprints/BP_QuietJsonMacroLibrary.Pin` (/ 360.0 (`KismetMathLibrary.Conv_IntToDouble` (`self.Sides`))))) ; Angle
  (if (> (`self.Fillet`) 0.00099)
    (bind _pinned_2 (`/Game/QuietRuntimeEditor/Common/Blueprints/BP_QuietJsonMacroLibrary.Pin` (- 90.0 (/ 360.0 (* (`self.Sides`) 2.0)))))
    (for _index (range (`self.Sides`))
      (bind _pinned_3 (`/Game/QuietRuntimeEditor/Common/Blueprints/BP_QuietJsonMacroLibrary.Pin` (* _index _pinned)))
      (bind _returnvalue (* _pinned _index))
      (bind _returnvalue_2 (`KismetMathLibrary.RotateAngleAxis` (-1.0 0.0 0.0) (+ _returnvalue _pinned_2) (0.0 0.0 1.0)))
      (bind _returnvalue_3 (`KismetMathLibrary.RotateAngleAxis` (-1.0 0.0 0.0) (- _returnvalue _pinned_2) (0.0 0.0 1.0)))
      (for (_array_element _array_index) (`|MakeArray` _returnvalue_2 _returnvalue_3)
        (bind _pinned_4 (`/Game/QuietRuntimeEditor/Common/Blueprints/BP_QuietJsonMacroLibrary.Pin` (* _array_element (`self.Fillet`))))
        (bind _returnvalue_4 (* (`KismetMathLibrary.SelectVector` _pinned_4 (`KismetMathLibrary.NegateVector` _pinned_4) (`KismetMathLibrary.Conv_IntToBool` _array_index)) 2.0))
        (`SplineComponent.AddPoint` (`self.Spline`) (make `SplinePoint` (`KismetMathLibrary.Conv_IntToDouble` (`SplineComponent.GetNumberOfSplinePoints` (`self.Spline`))) (+ _pinned_4 (`KismetMathLibrary.RotateAngleAxis` (`KismetMathLibrary.MakeVector` (`self.Radius`)) (* _index _pinned) (0.0 0.0 1.0))) _returnvalue_4 _returnvalue_4 (`KismetMathLibrary.MakeRotator` 0.0 0.0 _pinned_3) (1.0 1.0 1.0) "CurveCustomTangent") false)))
    (`SplineComponent.UpdateSpline` (`self.Spline`))
    (else
      (for _index_2 (range (`self.Sides`))
        (bind _returnvalue_5 (* _index_2 _pinned))
        (`SplineComponent.AddPoint` (`self.Spline`) (make `SplinePoint` (`KismetMathLibrary.Conv_IntToDouble` _index_2) (`KismetMathLibrary.RotateAngleAxis` (`KismetMathLibrary.MakeVector` (`self.Radius`)) _returnvalue_5 (0.0 0.0 1.0)) _returnvalue_2 _returnvalue_3 (`KismetMathLibrary.MakeRotator` 0.0 0.0 _returnvalue_5) (1.0 1.0 1.0) "CurveCustomTangent") false))
      (`/Game/QuietRuntimeEditor/Common/Features/QuietSplineSystem/Blueprints/BP_QuietSplineEditorComponent.ValidateSplinePointTypes` (`self.SplineEditor`))
      (`SplineComponent.UpdateSpline` (`self.Spline`)))))

(fn `RestoreShape`
  (`self.MakeNGon`)
  (`parent.RestoreShape`))

(fn `UpdateShape`
  (if (not (`self.CustomSpline`))
    (`self.MakeNGon`)
    (`parent.UpdateShape`)))

(fn `UserConstructionScript`
  (`self.MakeNGon`)
  (`parent.UserConstructionScript`))