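; Procedural star shape for the Quiet runtime spline system, rebuilding its spline from a side count, two alternating radii and per-radius fillets.
; MakeStar rotates alternating radius points around Z, then writes them as custom-tangent spline points, splitting filleted corners into two points with tangents scaled by the radius ratio.
; Construction, restore and update rebuild the star, though update skips custom splines.
; DrawShape derives the radii from the dragged rectangle per drawing step.
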(fn `DrawShape`
  (params (DraggedRectangle :type "Vector Structure"))
  (bind _returnvalue (`KismetMathLibrary.VSize` DraggedRectangle))
  (switch `int` (`self.DrawingStep`)
    (:`0`
      (bind _output_get (set `self.Radius1` _returnvalue))
      (set `self.Radius2` (/ _output_get 2.0)))
    (:`1`
      (set `self.Radius2` (/ _returnvalue 2.0))))
  (`self.MakeStar`))

(fn `MakeStar`
  (locals (Points :type "Array of Vector Structure"))
  (`SplineComponent.ClearSplinePoints` (`self.Spline`) true)
  (bind _pinned (`/Game/QuietRuntimeEditor/Common/Blueprints/BP_QuietJsonMacroLibrary.Pin` (/ 360.0 (* (`self.Sides`) 2)))) ; Angle
  (for _index (range (* (`self.Sides`) 2))
    (`KismetArrayLibrary.Array_Add` (`local.Points`) (`KismetMathLibrary.RotateAngleAxis` (`KismetMathLibrary.MakeVector` (`KismetMathLibrary.SelectFloat` (`self.Radius1`) (`self.Radius2`) (`self.IsOdd` _index))) (* _index _pinned) (0.0 0.0 1.0))))
  (for (_array_element _array_index) (`local.Points`)
    (bind _pinned_2 (`/Game/QuietRuntimeEditor/Common/Blueprints/BP_QuietJsonMacroLibrary.Pin` (`KismetMathLibrary.SelectFloat` (`self.Fillet1`) (`self.Fillet2`) (`self.IsOdd` _array_index)))) ; Fillet
    (if (> _pinned_2 0.00099)
      (bind _returnvalue (- _array_index 1))
      (bind _returnvalue_2 (+ _array_index 1))
      (for (_array_element_2 _array_index_2) (`|MakeArray` (`KismetMathLibrary.Conv_RotatorToVector` (`KismetMathLibrary.FindLookAtRotation` (`|GetArrayItem` (`local.Points`) _array_index) (`|GetArrayItem` (`local.Points`) (`KismetMathLibrary.SelectInt` _returnvalue (`KismetArrayLibrary.Array_LastIndex` (`local.Points`)) (`KismetArrayLibrary.Array_IsValidIndex` (`local.Points`) _returnvalue))))) (`KismetMathLibrary.Conv_RotatorToVector` (`KismetMathLibrary.FindLookAtRotation` (`|GetArrayItem` (`local.Points`) _array_index) (`|GetArrayItem` (`local.Points`) (`KismetMathLibrary.SelectInt` _returnvalue_2 0 (`KismetArrayLibrary.Array_IsValidIndex` (`local.Points`) _returnvalue_2))))))
        (bind _returnvalue_3 (* _array_element_2 _pinned_2))
        (bind _returnvalue_4 (`KismetMathLibrary.SelectVector` (`KismetMathLibrary.NegateVector` _returnvalue_3) _returnvalue_3 (`self.IsOdd` _array_index_2)))
        (bind _returnvalue_5 (`KismetMathLibrary.SelectVector` (* _returnvalue_4 (/ (`self.Radius2`) (`self.Radius1`))) (* _returnvalue_4 (/ (`self.Radius1`) (`self.Radius2`))) (> (`self.Radius2`) (`self.Radius1`))))
        (`SplineComponent.AddPoint` (`self.Spline`) (make `SplinePoint` (`KismetMathLibrary.Conv_IntToDouble` (`SplineComponent.GetNumberOfSplinePoints` (`self.Spline`))) (+ _returnvalue_3 _array_element) _returnvalue_5 _returnvalue_5 (struct) (1.0 1.0 1.0) "CurveCustomTangent") false))
      (else
        (`SplineComponent.AddPoint` (`self.Spline`) (make `SplinePoint` (`KismetMathLibrary.Conv_IntToDouble` (`SplineComponent.GetNumberOfSplinePoints` (`self.Spline`))) _array_element (1.0 0.0 0.0) (1.0 0.0 0.0) (struct) (1.0 1.0 1.0) "CurveCustomTangent") false))))
  (`/Game/QuietRuntimeEditor/Common/Features/QuietSplineSystem/Blueprints/BP_QuietSplineEditorComponent.ValidateSplinePointTypes` (`self.SplineEditor`))
  (`SplineComponent.UpdateSpline` (`self.Spline`)))

(fn `RestoreShape`
  (`self.MakeStar`)
  (`parent.RestoreShape`))

(fn `UpdateShape`
  (if (not (`self.CustomSpline`))
    (`self.MakeStar`)
    (`parent.UpdateShape`)))

(fn `UserConstructionScript`
  (`self.MakeStar`)
  (`parent.UserConstructionScript`))