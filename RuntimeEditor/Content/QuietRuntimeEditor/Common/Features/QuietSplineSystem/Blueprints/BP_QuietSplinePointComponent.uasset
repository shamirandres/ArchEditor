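; Spline point component in the Quiet runtime editor's spline system that swaps its material to show whether the point is occluded.
; SetOcclusionState switches material slot 0 between the regular material and an occluded one.
; The occluded dynamic material instance is created lazily and cached, with its parent chosen by component tags so arrive and leave tangent handles differ from regular points.
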(fn `AcquireOccludedMat`
  (returns (Material :type "MaterialInstanceDynamic Object Reference"))
  (bind _occludedmaterial (`self.OccludedMaterial`)
    (:`then`
      (return _occludedmaterial))
    (:`else`
      (bind _returnvalue (`KismetMaterialLibrary.CreateDynamicMaterialInstance` (select `bool` (or (`self.ComponentHasTag` "ArriveTangent") (`self.ComponentHasTag` "LeaveTangent")) :`false` "/Game/QuietRuntimeEditor/Common/Features/QuietSplineSystem/Materials/M_SplinePointOccluded.M_SplinePointOccluded" :`true` "/Game/QuietRuntimeEditor/Common/Features/QuietSplineSystem/Materials/MI_TangentPoint.MI_TangentPoint" :!type "MaterialInterface Object Reference")))
      (bind _output_get (set `self.OccludedMaterial` _returnvalue))
      (return _output_get))))

(fn `SetOcclusionState`
  (params (NewState :type Boolean))
  (`self.SetMaterial` 0 (select `bool` NewState :`false` (`self.RegularMaterial`) :`true` (`self.AcquireOccludedMat`) :!type "MaterialInterface Object Reference"))
  (if NewState
    (set `self.Material` (`self.AcquireOccludedMat`))))