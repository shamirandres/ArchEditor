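; BP_QuietSplineMeshComponent is a spline mesh component for the Quiet Spline System that switches between regular and occluded looks.
; SetOcclusionState swaps the first material slot between RegularMaterial and a cached occluded dynamic instance.
; AcquireOccludedMat creates that instance on demand, parented to MI_SplineHandler for components tagged as arrive or leave tangents, otherwise to M_SplineMasterOccluded.
; InitMaterial creates it directly from M_SplineMasterOccluded, regardless of tags.
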(fn `AcquireOccludedMat`
  (returns (Material :type "MaterialInstanceDynamic Object Reference"))
  (bind _occludedmaterial (`self.OccludedMaterial`)
    (:`then`
      (return _occludedmaterial))
    (:`else`
      (bind _returnvalue (`KismetMaterialLibrary.CreateDynamicMaterialInstance` (select `bool` (or (`self.ComponentHasTag` "ArriveTangent") (`self.ComponentHasTag` "LeaveTangent")) :`false` "/Game/QuietRuntimeEditor/Common/Features/QuietSplineSystem/Materials/M_SplineMasterOccluded.M_SplineMasterOccluded" :`true` "/Game/QuietRuntimeEditor/Common/Features/QuietSplineSystem/Materials/MI_SplineHandler.MI_SplineHandler" :!type "MaterialInterface Object Reference")))
      (bind _output_get (set `self.OccludedMaterial` _returnvalue))
      (return _output_get))))

(fn `InitMaterial`
  (bind _returnvalue (`KismetMaterialLibrary.CreateDynamicMaterialInstance` "/Game/QuietRuntimeEditor/Common/Features/QuietSplineSystem/Materials/M_SplineMasterOccluded.M_SplineMasterOccluded"))
  (set `self.OccludedMaterial` _returnvalue))

(fn `SetOcclusionState`
  (params (NewState :type Boolean))
  (`self.SetMaterial` 0 (select `bool` NewState :`false` (`self.RegularMaterial`) :`true` (`self.AcquireOccludedMat`) :!type "MaterialInterface Object Reference")))