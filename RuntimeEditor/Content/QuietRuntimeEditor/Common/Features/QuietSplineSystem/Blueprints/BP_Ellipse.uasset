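; BP_Ellipse is a spline shape Blueprint in the Quiet runtime editor's spline system that generates an ellipse from Width, Length and PointsCount.
; MakeEllipse rebuilds the spline with evenly spaced angular steps, setting custom tangents from the sine/cosine derivative.
; Construction, drag-drawing and restore all call MakeEllipse, with DrawShape sizing the ellipse from twice the absolute drag vector.
; UpdateShape regenerates it only when CustomSpline is false, leaving custom splines untouched.
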(fn `DrawShape`
  (params (DraggedRectangle :type "Vector Structure"))
  (set `self.Width` (.x (* (`KismetMathLibrary.Vector_GetAbs` DraggedRectangle) 2.0)))
  (set `self.Length` (.y (* (`KismetMathLibrary.Vector_GetAbs` DraggedRectangle) 2.0)))
  (`self.MakeEllipse`))

(fn `MakeEllipse`
  (locals (CycleInc :type "Float (double-precision)") (CycleItr :type "Float (double-precision)"))
  (bind _returnvalue (`KismetMathLibrary.MakeVector` (* (`self.Width`) 0.5 -1.0 (`KismetMathLibrary.Sin` (`local.CycleItr`))) (* (`self.Length`) 0.5 (`KismetMathLibrary.Cos` (`local.CycleItr`)))))
  (`SplineComponent.ClearSplinePoints` (`self.Spline`) true)
  (bind _output_get (set `local.CycleInc` (/ (* (`KismetMathLibrary.GetPI`) 2.0) (`self.PointsCount`))))
  (set `local.CycleItr` (+ _output_get (* (`KismetMathLibrary.GetPI`) -1.0)))
  (for _index (range (`self.PointsCount`))
    (`SplineComponent.AddPoint` (`self.Spline`) (make `SplinePoint` (`KismetMathLibrary.Conv_IntToDouble` _index) (`KismetMathLibrary.MakeVector` (* (`self.Width`) 0.5 (`KismetMathLibrary.Cos` (`local.CycleItr`))) (* (`self.Length`) 0.5 (`KismetMathLibrary.Sin` (`local.CycleItr`)))) _returnvalue _returnvalue (`KismetMathLibrary.MakeRotator` 0.0) (1.0 1.0 1.0) "CurveCustomTangent") true)
    (set `local.CycleItr` (+ (`local.CycleItr`) (`local.CycleInc`)))))

(fn `RestoreShape`
  (`self.MakeEllipse`)
  (`parent.RestoreShape`))

(fn `UpdateShape`
  (if (not (`self.CustomSpline`))
    (`self.MakeEllipse`)
    (`parent.UpdateShape`)))

(fn `UserConstructionScript`
  (`self.MakeEllipse`)
  (`parent.UserConstructionScript`))