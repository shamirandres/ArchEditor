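; Instanced static mesh component for the QuietScatter feature that adds randomized mesh instances from a supplied location and surface normal.
; AddNewInstance rejects points outside optional height and slope limits, thinning those near the lower height limit with a steep probabilistic falloff.
; Accepted instances get random uniform scale, tilt and yaw, with Gravity blending their up axis from world up toward the normal.
; Helpers expose the mesh and return all instance transforms in local space.
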(fn `AddNewInstance`
  (params (Location :type "Vector Structure") (Normal :type "Vector Structure (by ref)"))
  (returns (Success :type Boolean))
  (bind (_scale_range_x _scale_range_y) (`KismetMathLibrary.BreakVector2D` (`self.Scale Range`)))
  (bind (_heightlimits_x _heightlimits_y) (`KismetMathLibrary.BreakVector2D` (`self.HeightLimits`)))
  (bind (_orientationlimit_x _orientationlimit_y) (`KismetMathLibrary.BreakVector2D` (`self.OrientationLimit`)))
  (bind (_heightlimits_x_2 _heightlimits_y_2) (`KismetMathLibrary.BreakVector2D` (`self.HeightLimits`)))
  (bind (_orientationlimit_x_2 _orientationlimit_y_2) (`KismetMathLibrary.BreakVector2D` (`self.OrientationLimit`)))
  (`|ExecutionSequence`
    (:`then_0`
      ;[0 0 0] Check Location
      (if (`KismetMathLibrary.NearlyEqual_FloatFloat` _heightlimits_x _heightlimits_y 0.0001)
        _
        (elif (`KismetMathLibrary.InRange_FloatFloat` (.z (`local.Location`)) _heightlimits_x_2 _heightlimits_y_2 false false)
          (if (not (`self.ApplyHeightFalloff` (`local.Location`)))
            (return false))
          (else
            (return false)))))
    (:`then_1`
      ;[0 0 0] Check Normal
      (if (`KismetMathLibrary.NearlyEqual_FloatFloat` _orientationlimit_x _orientationlimit_y 0.0001)
        _
        (elif (not (`KismetMathLibrary.InRange_FloatFloat` (`KismetMathLibrary.Dot_VectorVector` (`local.Normal`) (0.0 0.0 1.0)) _orientationlimit_x_2 _orientationlimit_y_2))
          (return false))))
    (:`then_2`
      ;[0 0 0] Add Instance
      (`self.AddInstance` (`KismetMathLibrary.MakeTransform` (`local.Location`) (`self.GetNewInstanceRotation` (`local.Normal`)) (`KismetMathLibrary.Conv_DoubleToVector` (`KismetMathLibrary.RandomFloatInRange` _scale_range_x _scale_range_y))) true)
      (return true))))

(fn `ApplyHeightFalloff`
  (params (targetLocation :type "Vector Structure"))
  (returns (ReturnValue :type Boolean))
  (bind _heightfallof (`self.HeightFallof`))
  (bind (_heightlimits_x _heightlimits_y) (`KismetMathLibrary.BreakVector2D` (`self.HeightLimits`)))
  (bind _returnvalue (`KismetMathLibrary.Abs` (- (/ (- _heightlimits_y targetLocation_Z) (- _heightlimits_y _heightlimits_x)) 1.0)))
  (if (< _returnvalue _heightfallof)
    (return (== (`KismetMathLibrary.RandomIntegerInRange` 0 (`KismetMathLibrary.FTrunc` (* (`KismetMathLibrary.MultiplyMultiply_FloatFloat` (- 1.0 (/ _returnvalue _heightfallof)) 10.0) 100.0))) 0))
    (else
      (return true))))

(fn `GetInstanceRandomScale`
  (returns (ReturnValue :type "Float (double-precision)"))
  (bind (_scale_range_x _scale_range_y) (`KismetMathLibrary.BreakVector2D` (`self.Scale Range`)))
  (return (`KismetMathLibrary.RandomFloatInRange` _scale_range_x _scale_range_y)))

(fn `GetInstances`
  (returns (Instances :type "Array of Transform Structure"))
  (locals (Transforms :type "Array of Transform Structure"))
  (for _index (range (`self.GetInstanceCount`))
    (`KismetArrayLibrary.Array_Add` (`local.Transforms`) (`self.GetInstanceTransform` _index)))
  (return (`local.Transforms`)))

(fn `GetMesh`
  (returns (`Static Mesh` :type "StaticMesh Object Reference"))
  (return (`self.StaticMesh`)))

(fn `GetNewInstanceRotation`
  (params (Normal :type "Vector Structure (by ref)"))
  (returns (ReturnValue :type "Rotator Structure"))
  (bind _maxrandomtilt (`self.MaxRandomTilt`))
  (bind _maxrotationangle (`self.MaxRotationAngle`))
  (return (`KismetMathLibrary.TransformRotation` (`KismetMathLibrary.MakeTransform` (0.0 0.0 0.0) (`KismetMathLibrary.MakeRotFromZ` (`KismetMathLibrary.RotateAngleAxis` (`KismetMathLibrary.VLerp` (0.0 0.0 1.0) Normal (`self.Gravity`)) (`KismetMathLibrary.RandomFloatInRange` (* _maxrandomtilt -1.0) _maxrandomtilt) (`KismetMathLibrary.SelectVector` (1.0 0.0 0.0) (0.0 1.0 0.0) (`KismetMathLibrary.RandomBool`))))) (`KismetMathLibrary.MakeRotator` 0.0 0.0 (`KismetMathLibrary.RandomFloatInRange` (* _maxrotationangle -1.0) _maxrotationangle)))))

(fn `SetMesh`
  (params (NewMesh :type "StaticMesh Object Reference"))
  (`self.SetStaticMesh` NewMesh))