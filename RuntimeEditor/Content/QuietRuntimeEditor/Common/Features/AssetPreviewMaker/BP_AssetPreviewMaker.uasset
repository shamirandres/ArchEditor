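; Preview actor that renders a mesh and/or material into a render target, keeping only one instance alive by destroying others on BeginPlay.
; Setup applies the mesh and an optional slot-0 material override, limits the scene capture to this actor, centers the mesh and sets camera distance from its bounds.
; Rotation functions orbit the capture with limited pitch.
; Capture runs on demand, optionally destroying the actor afterward, or every frame.
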(event `self.ReceiveBeginPlay`
  (`SceneComponent.K2_SetRelativeRotation` (`self.TargetCapture`) (`self.StartRotation`) false false)
  (`self.DestoryOtherCaptures`)
  (`self.Setup`))

(event `Rotate`
  (params (Axis :type "Vector2D Structure"))
  (bind _returnvalue (`self.ClampOrbit` Axis_Y))
  (`SceneComponent.K2_AddRelativeRotation` (`self.TargetCapture`) (`KismetMathLibrary.MakeRotator` 0.0 _returnvalue Axis_X) false false))

(fn `DestoryOtherCaptures`
  (bind _outactors (`GameplayStatics.GetAllActorsOfClass` "BP_AssetPreviewMaker_C"))
  (for _array_element _outactors
    (if (!= _array_element self)
      (`self.K2_DestroyActor` _array_element))))

(fn `MakePreview`
  (params (Destroy :type Boolean))
  (`SceneCaptureComponent2D.CaptureScene` (`self.SceneCaptureComponent2D`))
  (if Destroy
    (`self.K2_DestroyActor`)))

(fn `PlaceMeshToCenter`
  (bind (_min _max) (`StaticMeshComponent.GetLocalBounds` (`self.PreviewMesh`)))
  (`SceneComponent.K2_SetRelativeLocation` (`self.PreviewMesh`) (/ (+ _min _max) -2.0) false true))

(fn `Reinit`
  (params (Material :type "MaterialInterface Object Reference") (Mesh :type "StaticMesh Object Reference") (RenderTarget :type "TextureRenderTarget2D Object Reference"))
  (set `self.Material` Material)
  (set `self.Mesh` Mesh)
  (`/Engine/EditorBlueprintResources/StandardMacros.IsValid` RenderTarget
    (:`Is Valid`
      (set `self.RenderTarget` RenderTarget))
    (:`Is Not Valid`
      _))
  (`self.Setup`))

(fn `RelocateCameraByMeshSize`
  (bind (_origin _boxextent _sphereradius) (`KismetSystemLibrary.GetComponentBounds` (`self.PreviewMesh`)))
  (`SceneComponent.K2_SetRelativeLocation` (`self.SceneCaptureComponent2D`) (`KismetMathLibrary.MakeVector` (- (* _sphereradius (`KismetMathLibrary.DegTan` (- 90.0 20.0)) -1.0) (/ _sphereradius 2.0))) false true))

(fn `RotateNew`
  (params (Axis :type "Vector2D Structure"))
  (returns (TargetRotation :type "Rotator Structure"))
  (bind _returnvalue (`self.ClampOrbit` Axis_Y))
  (`SceneComponent.K2_AddRelativeRotation` (`self.TargetCapture`) (`KismetMathLibrary.MakeRotator` 0.0 _returnvalue Axis_X) false false)
  (return (`SceneComponent.RelativeRotation` (`self.TargetCapture`))))

(fn `SetCaptureEveryFrame`
  (params (NewState :type Boolean))
  (set `SceneCaptureComponent.bCaptureEveryFrame` NewState (`self.SceneCaptureComponent2D`)))

(fn `Setup`
  (`|ExecutionSequence`
    (:`then_0`
      (`/Engine/EditorBlueprintResources/StandardMacros.IsValid` (`self.Mesh`)
        (:`Is Valid`
          (`StaticMeshComponent.SetStaticMesh` (`self.PreviewMesh`) (`self.Mesh`))
          (for (_ _array_index) (`MeshComponent.GetMaterials` (`self.PreviewMesh`))
            (`PrimitiveComponent.SetMaterial` (`self.PreviewMesh`) _array_index (`StaticMesh.GetMaterial` (`self.Mesh`) _array_index))))))
    (:`then_1`
      (`/Engine/EditorBlueprintResources/StandardMacros.IsValid` (`self.Material`)
        (:`Is Valid`
          (`PrimitiveComponent.SetMaterial` (`self.PreviewMesh`) 0 (`self.Material`))))))
  (set `SceneCaptureComponent2D.TextureTarget` (`self.RenderTarget`) (`self.SceneCaptureComponent2D`))
  (set `SceneCaptureComponent.ShowOnlyActors` (`|MakeArray` self :!type "Actor Object Reference") (`self.SceneCaptureComponent2D`))
  (`self.RelocateCameraByMeshSize`)
  (`self.PlaceMeshToCenter`))

(fn `UserConstructionScript`)