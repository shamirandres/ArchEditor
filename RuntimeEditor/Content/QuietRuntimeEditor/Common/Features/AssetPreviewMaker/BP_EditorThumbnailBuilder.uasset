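; Editor tool that generates thumbnail textures for material instances, meshes and Blueprints, from one object or a package path scan.
; Each asset is temporarily spawned as an actor, with material instances shown on a sphere, then centered by its bounds.
; SceneCapture2D backs off by actor size and captures through a render target.
; The saved static texture replaces any existing one under QuietRuntimeEditor/Thumbnails, mirroring the asset's UserContent path.
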(event `MakeSeparateThumbnail`
  (`self.Make Simple Thumbnail`))

(event `MakePackageThumbnails`
  (bind _outassetdata (`AssetRegistry.GetAssetsByPath` (`AssetRegistryHelpers.GetAssetRegistry`) (`self.Package Path`) (`self.Recursive`) false))
  (for _array_element _outassetdata
    (if (`KismetArrayLibrary.Array_Contains` (`|MakeArray` "MaterialInstanceConstant" "StaticMesh" "SkeletalMesh" "Blueprint" "BlueprintGeneratedClass" :!type "Name") (`KismetStringLibrary.Conv_StringToName` (`KismetSystemLibrary.GetClassDisplayName` (`AssetRegistryHelpers.GetClass` _array_element))))
      (`self.Capture` (`AssetRegistryHelpers.GetAsset` _array_element)))))

(event `Capture`
  (params (Object :type "Object Object Reference"))
  (bind _asmaterial_instance_constant (cast `MaterialInstanceConstant` Object)
    (:`then`
      (bind _returnvalue (`EditorLevelLibrary.SpawnActorFromClass` "/Script/Engine.StaticMeshActor"))
      (bind _staticmeshcomponent (`StaticMeshActor.StaticMeshComponent` _returnvalue))
      (`StaticMeshComponent.SetStaticMesh` _staticmeshcomponent "/Engine/BasicShapes/Sphere.Sphere")
      (`PrimitiveComponent.SetMaterial` _staticmeshcomponent 0 _asmaterial_instance_constant)
      (`self.MakeThumbnail` _returnvalue _asmaterial_instance_constant))
    (:`CastFailed`
      (bind _returnvalue_2 (`EditorLevelLibrary.SpawnActorFromObject` Object))
      (`self.MakeThumbnail` _returnvalue_2 Object))))

(event `MakeThumbnail`
  (params (Actor :type "Actor Object Reference") (Object :type "Object Object Reference"))
  (bind (_pathpart _filenamepart) (`BlueprintPathsLibrary.Split` (`KismetSystemLibrary.GetPathName` Object)))
  (`self.PlaceActorToCenter` Actor)
  (`self.RelocateCameraByActorSize` Actor)
  (bind _pinned (`/Game/QuietRuntimeEditor/Common/Blueprints/BP_QuietJsonMacroLibrary.Pin` (`KismetStringLibrary.Concat_StrStr` "/Game/QuietRuntimeEditor/Thumbnails/" (`.RightS` (`KismetStringLibrary.Split` _pathpart "UserContent/")) "/" _filenamepart)))
  (`EditorAssetLibrary.DeleteAsset` (`KismetStringLibrary.Concat_StrStr` _pinned "." (`.FilenamePart` (`BlueprintPathsLibrary.Split` _pinned))))
  (`self.CaptureThumbnail` _pinned)
  (`self.K2_DestroyActor` Actor))

(fn `CaptureThumbnail`
  (params (Asset :type String))
  (`SceneCaptureComponent2D.CaptureScene` (`self.SceneCapture2D`))
  (bind _returnvalue (`KismetRenderingLibrary.RenderTargetCreateStaticTexture2DEditorOnly` "/Game/QuietRuntimeEditor/Common/Features/AssetPreviewMaker/RT_Thumbnail.RT_Thumbnail" Asset "TC_Default" "TMGS_NoMipmaps"))
  (`EditorAssetLibrary.SaveLoadedAsset` _returnvalue false))

(fn `Make Simple Thumbnail`
  (`/Engine/EditorBlueprintResources/StandardMacros.IsValid` (`self.SimpleObject`)
    (:`Is Valid`
      (if (`KismetArrayLibrary.Array_Contains` (`|MakeArray` "/Script/Engine.MaterialInstanceConstant" "/Script/Engine.StaticMesh" "/Script/Engine.SkeletalMesh" "/Script/Engine.Blueprint" :!type "Object Class Reference") (`GameplayStatics.GetObjectClass` (`self.SimpleObject`)))
        (`self.Capture` (`self.SimpleObject`))))))

(fn `PlaceActorToCenter`
  (params (Actor :type "Actor Object Reference"))
  (`self.K2_SetActorLocation` Actor (`KismetMathLibrary.NegateVector` (`self.GetActorBounds` Actor true false)) false false))

(fn `RelocateCameraByActorSize`
  (params (Actor :type "Actor Object Reference"))
  (bind _returnvalue (`KismetMathLibrary.GetMaxElement` (`.BoxExtent` (`self.GetActorBounds` Actor true false))))
  (`SceneComponent.K2_SetRelativeLocation` (`self.SceneCapture2D`) (`KismetMathLibrary.MakeVector` (- (* _returnvalue (`KismetMathLibrary.DegTan` (- 90.0 5.0)) -1.3) (/ _returnvalue 2.0))) false true))

(fn `UserConstructionScript`)