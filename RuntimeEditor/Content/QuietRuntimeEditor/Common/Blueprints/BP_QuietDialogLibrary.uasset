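; Blueprint function library that opens shared dialog and progress bar widgets for the Quiet Runtime Editor.
; The warning dialog functions create a WBP_QuietWarningDialog on the viewport, either with message type, default value and a completion callback, or with just a message.
; CallProgressbar reuses an existing top-level WBP_Progressbar or creates one at a high Z-order, returning it to the caller.
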(fn `CallProgressbar`
  (params (OwningPlayer :type "PlayerController Object Reference"))
  (returns (Progressbar :type "/Game/QuietRuntimeEditor/Common/Widgets/WBP_Progressbar Object Reference"))
  (bind _foundwidgets (`WidgetBlueprintLibrary.GetAllWidgetsOfClass` OwningPlayer "/Game/QuietRuntimeEditor/Common/Widgets/WBP_Progressbar.WBP_Progressbar_C"))
  (if (`KismetArrayLibrary.Array_IsValidIndex` _foundwidgets)
    (return (`|GetArrayItem` _foundwidgets))
    (else
      (bind _returnvalue (`|CreateWidget` "/Game/QuietRuntimeEditor/Common/Widgets/WBP_Progressbar.WBP_Progressbar_C" OwningPlayer))
      (`UserWidget.AddToViewport` _returnvalue 100)
      (return _returnvalue))))

(fn `CallWarningDialog`
  (params (OwningPlayer :type "PlayerController Object Reference") (MessageType :type "/Game/QuietRuntimeEditor/Common/Blueprints/Enums/E_QuietMsgType Enum" :default "NewEnumerator0") (DefaultValue :type "/Game/QuietRuntimeEditor/Common/Blueprints/Enums/E_QuietMsgReturnValue Enum" :default "NewEnumerator0") (Message :type Text) (Callback :type "Delegate (by ref)"))
  (bind _returnvalue (`|CreateWidget` "/Game/QuietRuntimeEditor/Common/Widgets/WBP_QuietWarningDialog.WBP_QuietWarningDialog_C" OwningPlayer MessageType DefaultValue Message))
  (`UserWidget.AddToViewport` _returnvalue 0)
  (add `/Game/QuietRuntimeEditor/Common/Widgets/WBP_QuietWarningDialog.NotifyOnMessageProcessed` _returnvalue Callback))

(fn `CallWarningDialogSimple`
  (params (OwningPlayer :type "PlayerController Object Reference") (Message :type Text))
  (bind _returnvalue (`|CreateWidget` "/Game/QuietRuntimeEditor/Common/Widgets/WBP_QuietWarningDialog.WBP_QuietWarningDialog_C" OwningPlayer "NewEnumerator0" "NewEnumerator0" Message))
  (`UserWidget.AddToViewport` _returnvalue 0))