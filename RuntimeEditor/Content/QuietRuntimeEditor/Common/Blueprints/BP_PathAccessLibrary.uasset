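; Blueprint function library that supplies the Quiet runtime editor's paths for user content, saved scenes and thumbnails.
; The content folder comes from a text literal, and both directory getters switch on a "SaveDirectory" text literal converted to a string.
; "User Directory" resolves under the user's game-named folder and "Project Saved Dir" under the project's Saved folder, creating missing directories.
; Any other value is returned unchanged as the path.
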(fn `GetContentFolder`
  (returns (ReturnValue :type String))
  (return (`KismetTextLibrary.Conv_TextToString` "UserContent")))

(fn `GetSaveDirectory`
  (returns (ReturnValue :type String))
  (bind _returnvalue (`KismetTextLibrary.Conv_TextToString` "SaveDirectory"))
  (bind _returnvalue_2 (`KismetStringLibrary.Concat_StrStr` (`BlueprintFileUtilsBPLibrary.GetUserDirectory`) "/" (`KismetSystemLibrary.GetGameName`) "/SaveScenes"))
  (bind _returnvalue_3 (`KismetStringLibrary.Concat_StrStr` (`BlueprintPathsLibrary.ProjectSavedDir`) "/SaveScenes"))
  (switch `string` _returnvalue
    (:`Default`
      (return _returnvalue))
    (:`UserDirectory`
      (bind _returnvalue_4 (`BlueprintFileUtilsBPLibrary.DirectoryExists` _returnvalue_2))
      (if (not _returnvalue_4)
        (`BlueprintFileUtilsBPLibrary.MakeDirectory` _returnvalue_2 true))
      (return _returnvalue_2))
    (:`ProjectSavedDir`
      (bind _returnvalue_5 (`BlueprintFileUtilsBPLibrary.DirectoryExists` _returnvalue_3))
      (if (not _returnvalue_5)
        (`BlueprintFileUtilsBPLibrary.MakeDirectory` _returnvalue_3))
      (return _returnvalue_3))))

(fn `GetThumbnailsDirectory`
  (returns (ReturnValue :type String))
  (bind _returnvalue (`KismetTextLibrary.Conv_TextToString` "SaveDirectory"))
  (bind _returnvalue_2 (`KismetStringLibrary.Concat_StrStr` (`BlueprintFileUtilsBPLibrary.GetUserDirectory`) "/" (`KismetSystemLibrary.GetGameName`) "/Thumbnails"))
  (bind _returnvalue_3 (`KismetStringLibrary.Concat_StrStr` (`BlueprintPathsLibrary.ProjectSavedDir`) "/Thumbnails"))
  (switch `string` _returnvalue
    (:`Default`
      (return _returnvalue))
    (:`UserDirectory`
      (bind _returnvalue_4 (`BlueprintFileUtilsBPLibrary.DirectoryExists` _returnvalue_2))
      (if (not _returnvalue_4)
        (`BlueprintFileUtilsBPLibrary.MakeDirectory` _returnvalue_2 true))
      (return _returnvalue_2))
    (:`ProjectSavedDir`
      (bind _returnvalue_5 (`BlueprintFileUtilsBPLibrary.DirectoryExists` _returnvalue_3))
      (if (not _returnvalue_5)
        (`BlueprintFileUtilsBPLibrary.MakeDirectory` _returnvalue_3))
      (return _returnvalue_3))))