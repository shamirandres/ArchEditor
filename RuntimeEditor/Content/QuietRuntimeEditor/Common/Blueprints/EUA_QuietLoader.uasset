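; Scene loader actor for the Quiet Runtime Editor that restores a saved scene from a file through a Serializer.
; LoadScene passes File to RestoreSceneMessage.
; ReturnDataByRequestWithTag spawns an actor from the JSON "Class" field, also reading its location from that field, and writes it back as "Actor".
; GetDataWithTag always reports failure and TakeActorsWithTag is empty, so only the restore direction is implemented.
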(event `Load Scene`
  (message `/Game/QuietRuntimeEditor/Serialization/BI_SerializerInterface.RestoreScene` (`self.Serializer`) (`self.File`)))

(fn `GetDataWithTag`
  (params (Request :type "GameplayTag Structure"))
  (returns (Success :type Boolean) (Data :type "JsonObjectWrapper Structure"))
  (return false))

(fn `ReturnDataByRequestWithTag`
  (params (Request :type "GameplayTag Structure") (InputData :type "JsonObjectWrapper Structure"))
  (returns (Success :type Boolean) (Data :type "JsonObjectWrapper Structure"))
  (bind _outvalue (`|GetJsonField` InputData "Class"))
  (bind _outvalue_2 (`|GetJsonField` InputData "Class"))
  (bind _returnvalue (`EditorLevelLibrary.SpawnActorFromClass` _outvalue_2 (.location _outvalue)))
  (bind _returnvalue_2 (`|SetJsonField` InputData "Actor" _returnvalue))
  (return _returnvalue_2 InputData))

(fn `TakeActorsWithTag`
  (params (Request :type "GameplayTag Structure"))
  (returns (Actors :type "Array of Actor Object Reference"))
  (return))

(fn `UserConstructionScript`)