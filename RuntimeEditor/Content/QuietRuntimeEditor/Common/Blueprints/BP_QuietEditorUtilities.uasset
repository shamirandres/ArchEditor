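; Utility function library for the Quiet Runtime Editor, giving shared access to editor services and common helpers.
; String helpers strip asset prefixes and suffixes, make names unique with numeric suffixes, and quicksort with index-aware comparison; others compute actor bounds and find components by name.
; Editor calls go through a BP_Router fetched from the GameState, sending tagged messages to Manager, Details and UI, or using the registered Serializer for scene save/load, duplication and by-name property access.
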(fn `CallFunction`
  (params (Object :type "Object Object Reference (by ref)") (Action :type "JsonObjectWrapper Structure (by ref)"))
  (returns (Success :type Boolean))
  (bind (_success _value) (`/Game/QuietRuntimeEditor/Common/Blueprints/BP_Router.GetRegisterdObject` (`self.GetRouter` null) (struct :`TagName` "Serializer")))
  (if _success
    (bind _success_2 (message `/Game/QuietRuntimeEditor/Serialization/BI_SerializerInterface.CallFunctionByName` _value Object Action))
    (return _success_2)
    (else
      (return false))))

(fn `ClearSelectedComponents`
  (`/Game/QuietRuntimeEditor/Common/Blueprints/BP_Router.ThrowCommand` (`self.GetRouter` null) (struct :`TagName` "Manager") (struct :`TagName` "Gizmo.ClearSelectedComponents")))

(fn `CollectObjectDetails`
  (params (Object :type "Object Object Reference"))
  (returns (Success :type Boolean) (ReturnValue :type "JsonObjectWrapper Structure"))
  (bind _outjsonobject (`JsonBlueprintFunctionLibrary.FromString` "{ }"))
  (bind (_success _value) (`/Game/QuietRuntimeEditor/Common/Blueprints/BP_Router.GetRegisterdObject` (`self.GetRouter` null) (struct :`TagName` "Serializer")))
  (if _success
    (message `/Game/QuietRuntimeEditor/Serialization/BI_SerializerInterface.GrabDetails` _value Object _outjsonobject)
    (return true _outjsonobject)
    (else
      (return false (make `JsonObjectWrapper`)))))

(fn `DeserializeActor`
  (params (Cache :type "JsonObjectWrapper Structure (by ref)") (IncludeAttachment :type Boolean))
  (returns (Actor :type "Actor Object Reference"))
  (bind (_success _value) (`/Game/QuietRuntimeEditor/Common/Blueprints/BP_Router.GetRegisterdObject` (`self.GetRouter` null) (struct :`TagName` "Serializer")))
  (if _success
    (bind _actor (message `/Game/QuietRuntimeEditor/Serialization/BI_SerializerInterface.RestoreCachedActor` _value Cache IncludeAttachment))
    (return _actor)))

(fn `DeserializeObject`
  (params (Object :type "Object Object Reference") (Json :type "JsonObjectWrapper Structure"))
  (returns (Success :type Boolean))
  (bind (_success _value) (`/Game/QuietRuntimeEditor/Common/Blueprints/BP_Router.GetRegisterdObject` (`self.GetRouter` null) (struct :`TagName` "Serializer")))
  (if _success
    (message `/Game/QuietRuntimeEditor/Serialization/BI_SerializerInterface.RestoreObject` _value Object Json)
    (return true)
    (else
      (return false))))

(fn `DuplicateActor`
  (params (Actor :type "Actor Object Reference") (IncludeAttachment :type Boolean))
  (returns (Copy :type "Actor Object Reference"))
  (bind (_success _value) (`/Game/QuietRuntimeEditor/Common/Blueprints/BP_Router.GetRegisterdObject` (`self.GetRouter` null) (struct :`TagName` "Serializer")))
  (if _success
    (bind _copy (message `/Game/QuietRuntimeEditor/Serialization/BI_SerializerInterface.DuplicateRegisteredActor` _value Actor IncludeAttachment))
    (return _copy)))

(fn `EndsWithNumber`
  (params (String :type String))
  (returns (ReturnValue :type Boolean))
  (return (`KismetStringLibrary.IsNumeric` (`KismetStringLibrary.Right` String 1))))

(fn `ExtractIndex`
  (params (String :type String))
  (returns (Index :type Integer))
  (bind _returnvalue (`KismetStringLibrary.Len` String))
  (for _index (range 1 (+ _returnvalue 1))
    (bind _returnvalue_2 (- _returnvalue _index))
    (if (not (`KismetMathLibrary.InRange_IntInt` (`KismetStringLibrary.GetCharacterAsNumber` String _returnvalue_2) 48 57))
      (return (`KismetStringLibrary.Conv_StringToInt` (`KismetStringLibrary.GetSubstring` String _returnvalue_2 _index)))))
  (return (`KismetStringLibrary.Conv_StringToInt` String)))

(fn `GetActorsBounds`
  (params (Actors :type "Array of Actor Object Reference (by ref)"))
  (returns (Center :type "Vector Structure") (Radius :type "Float (double-precision)"))
  (bind (_center _boxextent) (`GameplayStatics.GetActorArrayBounds` Actors))
  (bind _returnvalue (`KismetMathLibrary.GetMaxElement` _boxextent))
  (return _center (`KismetMathLibrary.VSize` (`KismetMathLibrary.MakeVector` _returnvalue _returnvalue _returnvalue))))

(fn `GetCenterOfActors`
  (params (Actors :type "Array of Actor Object Reference"))
  (returns (Center :type "Vector Structure"))
  (locals (LocalAverages :type "Array of Vector Structure"))
  (for _array_element Actors
    (`KismetArrayLibrary.Array_Add` (`local.LocalAverages`) (`Actor.GetActorBounds` _array_element false false)))
  (return (`KismetMathLibrary.GetVectorArrayAverage` (`local.LocalAverages`))))

(fn `GetComponentByName`
  (params (Actor :type "Actor Object Reference") (Name :type String))
  (returns (Component :type "ActorComponent Object Reference"))
  (if (`KismetStringLibrary.EqualEqual_StrStr` Name "Root")
    (return (`Actor.RootComponent` Actor))
    (else
      (for _array_element (`Actor.K2_GetComponentsByClass` Actor "/Script/Engine.ActorComponent")
        (if (`KismetStringLibrary.EqualEqual_StrStr` Name (`KismetSystemLibrary.GetDisplayName` _array_element))
          (return _array_element))))))

(fn `GetComponentName`
  (params (Component :type "ActorComponent Object Reference"))
  (returns (Name :type String))
  (return (`KismetMathLibrary.SelectString` "Root" (`KismetSystemLibrary.GetDisplayName` Component) (== Component (`Actor.RootComponent` (`ActorComponent.GetOwner` Component))))))

(fn `GetPropertyByName`
  (params (Object :type "Object Object Reference") (Name :type String))
  (returns (Success :type Boolean) (Property :type "JsonObjectWrapper Structure"))
  (bind (_success _value) (`/Game/QuietRuntimeEditor/Common/Blueprints/BP_Router.GetRegisterdObject` (`self.GetRouter` null) (struct :`TagName` "Serializer")))
  (if _success
    (bind (_success_2 _boxedvalue) (message `/Game/QuietRuntimeEditor/Serialization/BI_SerializerInterface.GetValueByName` _value Object Name))
    (return _success_2 _boxedvalue)
    (else
      (return false (make `JsonObjectWrapper`)))))

(fn `GetRouter`
  (returns (Router :type "/Game/QuietRuntimeEditor/Common/Blueprints/BP_Router Object Reference"))
  (bind _object (message `/Game/QuietRuntimeEditor/Common/Blueprints/BI_QuietRoutingInterface.TakeObjectWithTag` (`GameplayStatics.GetGameState` null) (struct)))
  (bind _asbp_router (cast `/Game/QuietRuntimeEditor/Common/Blueprints/BP_Router` _object))
  (return _asbp_router))

(fn `GetSelectedActors`
  (returns (Actors :type "Array of Actor Object Reference"))
  (bind _actors (`/Game/QuietRuntimeEditor/Common/Blueprints/BP_Router.GetActorsWithTag` (`self.GetRouter` null) (struct :`TagName` "Manager") (struct :`TagName` "Outliner.GetSelection")))
  (return _actors))

(fn `Greater`
  (params (lhs :type String) (rhs :type String))
  (returns (ReturnValue :type Boolean))
  (locals (LhsLen :type Integer) (RhsLen :type Integer) (LhsChar :type Integer) (RhsChar :type Integer))
  (set `local.LhsLen` (`KismetStringLibrary.Len` lhs))
  (set `local.RhsLen` (`KismetStringLibrary.Len` rhs))
  (for _index (range (`KismetMathLibrary.Min` (`local.LhsLen`) (`local.RhsLen`)))
    (set `local.LhsChar` (`KismetStringLibrary.GetCharacterAsNumber` (`local.lhs`) _index))
    (set `local.RhsChar` (`KismetStringLibrary.GetCharacterAsNumber` (`local.rhs`) _index))
    (if (not (== (`local.LhsChar`) (`local.RhsChar`)))
      (return (> (`local.LhsChar`) (`local.RhsChar`)))))
  (return (> (`local.LhsLen`) (`local.RhsLen`))))

(fn `GreaterWithIndices`
  (params (A :type String) (B :type String))
  (returns (ReturnValue :type Boolean))
  (if (and (`self.EndsWithNumber` A) (`self.EndsWithNumber` B))
    (bind (_string _index) (`self.SplitStringByIndex` A))
    (bind (_string_2 _index_2) (`self.SplitStringByIndex` B))
    (if (== _string _string_2)
      (return (> _index _index_2))
      (else
        (bind _returnvalue (`self.Greater` _string _string_2))
        (return _returnvalue)))
    (else
      (bind _returnvalue_2 (`self.Greater` (`local.A`) (`local.B`)))
      (return _returnvalue_2))))

(fn `IsActorSelected`
  (params (Actor :type "Actor Object Reference (by ref)"))
  (returns (ReturnValue :type Boolean))
  (bind _actors (`/Game/QuietRuntimeEditor/Common/Blueprints/BP_Router.GetActorsWithTag` (`self.GetRouter` null) (struct :`TagName` "Manager") (struct :`TagName` "Outliner.GetSelection")))
  (return (`KismetArrayLibrary.Array_Contains` _actors Actor)))

(fn `LoadScene`
  (params (File :type "FilePath Structure"))
  (returns (RootActors :type "Array of Actor Object Reference") (SceneJson :type "JsonObjectWrapper Structure") (DynamicMaterials :type "Map of MaterialInterface Object Reference to JsonObjectWrapper Structure"))
  (bind (_success _value) (`/Game/QuietRuntimeEditor/Common/Blueprints/BP_Router.GetRegisterdObject` (`self.GetRouter` null) (struct :`TagName` "Serializer")))
  (if _success
    (bind (_actors _cache _materials) (message `/Game/QuietRuntimeEditor/Serialization/BI_SerializerInterface.RestoreScene` _value File))
    (return _actors _cache _materials)))

(fn `Partition`
  (params (In :type "Array of String") (lo :type Integer) (hi :type Integer))
  (returns (`Pivot Index` :type Integer))
  (locals (Pivot :type String) (i :type Integer))
  (set `local.Pivot` (`|GetArrayItem` In hi))
  (set `local.i` (- lo 1))
  (for _index (range lo hi)
    (bind _returnvalue (`self.GreaterWithIndices` (`|GetArrayItem` In _index) (`local.Pivot`)))
    (if (not _returnvalue)
      (bind _result (`/Engine/EditorBlueprintResources/StandardMacros.IncrementInt` (`local.i`))
        (:`  `
          (`KismetArrayLibrary.Array_Swap` In _result _index)))))
  (bind _result_2 (`/Engine/EditorBlueprintResources/StandardMacros.IncrementInt` (`local.i`))
    (:`  `
      (`KismetArrayLibrary.Array_Swap` In _result_2 hi)
      (return (`local.i`)))))

(fn `QuickSort`
  (params (In :type "Array of String"))
  (`self.QuickSortImpl` In 0 (`KismetArrayLibrary.Array_LastIndex` In)))

(fn `QuickSortImpl`
  (params (In :type "Array of String") (lo :type Integer) (hi :type Integer))
  (if (not (or (>= lo hi) (< lo 0)))
    (bind _pivot_index (`self.Partition` In lo hi))
    (`self.QuickSortImpl` In lo (- _pivot_index 1))
    (`self.QuickSortImpl` In (+ _pivot_index 1) hi)))

(fn `RefreshActorDetails`
  (params (Actor :type "Actor Object Reference"))
  (if (`self.IsActorSelected` Actor)
    (bind (_success _returnvalue) (`self.CollectObjectDetails` Actor))
    (bind _outjsonobject (`JsonBlueprintFunctionLibrary.FromString` "{ }"))
    (`|SetJsonField` _outjsonobject "Message" _returnvalue)
    (`|SetJsonField` _outjsonobject "Actor" Actor)
    (`/Game/QuietRuntimeEditor/Common/Blueprints/BP_Router.ThrowJson` (`self.GetRouter` null) (struct :`TagName` "Details") (struct :`TagName` "Details.Setup") _outjsonobject)
    (return)))

(fn `RefreshSelectedComponent`
  (`/Game/QuietRuntimeEditor/Common/Blueprints/BP_Router.ThrowCommand` (`self.GetRouter` null) (struct :`TagName` "Manager") (struct :`TagName` "Gizmo.RefreshComponent")))

(fn `RegisterActor`
  (params (Actor :type "Actor Object Reference"))
  (`/Game/QuietRuntimeEditor/Common/Blueprints/BP_Router.ThrowActor` (`self.GetRouter` null) (struct :`TagName` "Manager") (struct :`TagName` "ContentBrowser.RegisterActor") Actor)
  (`/Game/QuietRuntimeEditor/Common/Blueprints/BP_Router.ThrowActor` (`self.GetRouter` null) (struct :`TagName` "Manager") (struct :`TagName` "ContentBrowser.FinishSpawning") Actor))

(fn `RegisterHistoryAction`
  (params (Action :type "JsonObjectWrapper Structure"))
  (returns (Success :type Boolean))
  (bind _returnvalue (`/Game/QuietRuntimeEditor/Common/Blueprints/BP_Router.ThrowJson` (`self.GetRouter` null) (struct :`TagName` "Manager") (struct :`TagName` "History.Register") Action))
  (return _returnvalue))

(fn `RemoveAssetPrefix`
  (params (Name :type String))
  (returns (ReturnValue :type String))
  (locals (Prefixes :type "Array of String"))
  (for _array_element (`local.Prefixes`)
    (if (`KismetStringLibrary.StartsWith` Name _array_element)
      (return (`self.RemoveAssetSuffix` (`KismetStringLibrary.Replace` Name _array_element)))))
  (return (`self.RemoveAssetSuffix` Name)))

(fn `RemoveAssetPrefixPure`
  (params (Name :type String))
  (returns (ReturnValue :type String))
  (locals (Prefixes :type "Array of String"))
  (for _array_element (`local.Prefixes`)
    (if (`KismetStringLibrary.StartsWith` Name _array_element)
      (return (`self.RemoveAssetSuffix` (`KismetStringLibrary.Replace` Name _array_element)))))
  (return (`self.RemoveAssetSuffix` Name)))

(fn `RemoveAssetSuffix`
  (params (SourceString :type String))
  (returns (ReturnValue :type String))
  (if (`KismetStringLibrary.EndsWith` SourceString "_C")
    (return (`KismetStringLibrary.LeftChop` SourceString 2))
    (elif (`KismetStringLibrary.Contains` SourceString "_C_")
      (return (`KismetStringLibrary.Replace` SourceString "_C_" "_" "CaseSensitive"))
      (else
        (return SourceString)))))

(fn `SaveScene`
  (params (File :type "FilePath Structure") (TargetJson :type "JsonObjectWrapper Structure (by ref)") (Actors :type "Array of Actor Object Reference (by ref)") (DynamicMaterials :type "Map of MaterialInstanceDynamic Object Reference to JsonObjectWrapper Structure"))
  (returns (Success :type Boolean))
  (bind (_success _value) (`/Game/QuietRuntimeEditor/Common/Blueprints/BP_Router.GetRegisterdObject` (`self.GetRouter` null) (struct :`TagName` "Serializer")))
  (if _success
    (bind _success_2 (message `/Game/QuietRuntimeEditor/Serialization/BI_SerializerInterface.CacheScene` _value Actors TargetJson File DynamicMaterials))
    (return _success_2)))

(fn `SerializeObject`
  (params (object :type "Object Object Reference"))
  (returns (Success :type Boolean) (Json :type "JsonObjectWrapper Structure"))
  (bind (_success _value) (`/Game/QuietRuntimeEditor/Common/Blueprints/BP_Router.GetRegisterdObject` (`self.GetRouter` null) (struct :`TagName` "Serializer")))
  (if _success
    (bind _cache (message `/Game/QuietRuntimeEditor/Serialization/BI_SerializerInterface.CacheObject` _value object))
    (return true _cache)
    (else
      (return false (make `JsonObjectWrapper`)))))

(fn `SerializeRegisteredActor`
  (params (Actor :type "Actor Object Reference") (TargetJson :type "JsonObjectWrapper Structure (by ref)") (IncludeAttachment :type Boolean))
  (returns (Success :type Boolean))
  (bind (_success _value) (`/Game/QuietRuntimeEditor/Common/Blueprints/BP_Router.GetRegisterdObject` (`self.GetRouter` null) (struct :`TagName` "Serializer")))
  (if _success
    (message `/Game/QuietRuntimeEditor/Serialization/BI_SerializerInterface.CacheRegisteredActor` _value Actor TargetJson IncludeAttachment)
    (return true)
    (else
      (return false))))

(fn `SetPropertyByName`
  (params (Object :type "Object Object Reference") (Name :type String) (Value :type "JsonObjectWrapper Structure"))
  (returns (Success :type Boolean))
  (bind (_success _value) (`/Game/QuietRuntimeEditor/Common/Blueprints/BP_Router.GetRegisterdObject` (`self.GetRouter` null) (struct :`TagName` "Serializer")))
  (if _success
    (bind _success_2 (message `/Game/QuietRuntimeEditor/Serialization/BI_SerializerInterface.SetValueByName` _value Object Name Value))
    (return _success_2)
    (else
      (return false))))

(fn `SetUserInterfaceVisibility`
  (params (NewState :type Boolean))
  (returns (Success :type Boolean))
  (bind (_success _data) (`/Game/QuietRuntimeEditor/Common/Blueprints/BP_Router.Get Data with Tag` (`self.GetRouter` null) (struct :`TagName` "UserInterface") (struct :`TagName` "UserInterface.ToggleVisibility")))
  (bind _outvalue (`|GetJsonField` _data "Visible"))
  (if (!= _outvalue NewState)
    (bind _returnvalue (`/Game/QuietRuntimeEditor/Common/Blueprints/BP_Router.ThrowCommand` (`self.GetRouter` null) (struct :`TagName` "UserInterface") (struct :`TagName` "UserInterface.ToggleVisibility")))
    (return _returnvalue)))

(fn `SortStringArray`
  (params (Array :type "Array of String"))
  (returns (SortedArray :type "Array of String"))
  (locals (RawStrings :type "Array of String") (SortedStrings :type "Array of String") (First :type String))
  (`KismetArrayLibrary.Array_Shuffle` Array)
  (`self.QuickSortImpl` Array 0 (`KismetArrayLibrary.Array_LastIndex` Array))
  (return Array))

(fn `SplitByIndex`
  (params (String :type String))
  (returns (ReturnValue :type Boolean) (Left :type String) (Right :type String))
  (locals (Success :type Boolean) (Suffix :type String) (Numbers :type "Array of Integer"))
  (bind _returnvalue (`KismetStringLibrary.ToUpper` String))
  (bind _returnvalue_2 (`KismetStringLibrary.Len` _returnvalue))
  (for _index (range 1 (+ _returnvalue_2 1))
    (bind _returnvalue_3 (`KismetStringLibrary.Right` _returnvalue _index))
    (if (`KismetStringLibrary.IsNumeric` _returnvalue_3)
      (set `local.Suffix` _returnvalue_3)
      (set `local.Success` true)
      (else
        (bind _returnvalue_4 (`KismetStringLibrary.Left` _returnvalue (- _returnvalue_2 (- _index 1))))
        (bind _returnvalue_5 (`KismetStringLibrary.GetCharacterAsNumber` (`KismetStringLibrary.Right` _returnvalue_4 1)))
        (if (and (> _returnvalue_5 65) (< _returnvalue_5 91))
          (return (`local.Success`) _returnvalue_4 (`local.Suffix`))
          (else
            (set `local.Suffix` _returnvalue_3)
            (if (and (> _returnvalue_5 47) (< _returnvalue_5 58))
              (set `local.Success` true))))))))

(fn `SplitStringByIndex`
  (params (RawString :type String))
  (returns (String :type String) (Index :type Integer))
  (bind _returnvalue (`KismetStringLibrary.Len` RawString))
  (for _index (range 1 (+ _returnvalue 1))
    (bind _returnvalue_2 (- _returnvalue _index))
    (if (not (`KismetMathLibrary.InRange_IntInt` (`KismetStringLibrary.GetCharacterAsNumber` RawString _returnvalue_2) 48 57))
      (bind _returnvalue_3 (`KismetStringLibrary.GetSubstring` RawString 0 (+ _returnvalue_2 1)))
      (return (`KismetMathLibrary.SelectString` (`KismetStringLibrary.LeftChop` _returnvalue_3 1) _returnvalue_3 (`KismetStringLibrary.EndsWith` _returnvalue_3 " ")) (`KismetStringLibrary.Conv_StringToInt` (`KismetStringLibrary.GetSubstring` RawString _returnvalue_2 _index)))))
  (return "" (`KismetStringLibrary.Conv_StringToInt` RawString)))

(fn `SplitStringByIndexTrim`
  (params (RawString :type String))
  (returns (String :type String) (Index :type Integer))
  (bind _returnvalue (`KismetStringLibrary.Len` RawString))
  (for _index (range 1 (+ _returnvalue 1))
    (bind _returnvalue_2 (- _returnvalue _index))
    (if (not (`KismetMathLibrary.InRange_IntInt` (`KismetStringLibrary.GetCharacterAsNumber` RawString _returnvalue_2) 48 57))
      (bind _returnvalue_3 (`KismetStringLibrary.GetSubstring` RawString 0 (+ _returnvalue_2 1)))
      (return (`KismetMathLibrary.SelectString` (`KismetStringLibrary.LeftChop` _returnvalue_3 1) _returnvalue_3 (`KismetStringLibrary.EndsWith` _returnvalue_3 "_")) (`KismetStringLibrary.Conv_StringToInt` (`KismetStringLibrary.GetSubstring` RawString _returnvalue_2 _index)))))
  (return "" (`KismetStringLibrary.Conv_StringToInt` RawString)))

(fn `UnifyName`
  (params (SourceName :type "String (by ref)") (ExistingNames :type "Array of String"))
  (locals (Collection :type "Set of String") (Base :type String))
  (`BlueprintSetLibrary.Set_AddItems` (`local.Collection`) ExistingNames)
  (if (`BlueprintSetLibrary.Set_Contains` (`local.Collection`) SourceName)
    (if (not (`KismetStringLibrary.IsNumeric` SourceName))
      (if (`self.EndsWithNumber` SourceName) :!label _label
        (bind _string (`self.SplitStringByIndex` SourceName))
        (set `local.Base` _string)
        (else
          (set `local.Base` SourceName)))
      (for _index (range (+ (`BlueprintSetLibrary.Set_Length` (`local.Collection`)) 1))
        (bind _returnvalue (`KismetStringLibrary.Concat_StrStr` (`local.Base`) " " (`KismetStringLibrary.Conv_IntToString` _index)))
        (if (not (`BlueprintSetLibrary.Set_Contains` (`local.Collection`) _returnvalue))
          (`|VariableSetRef` SourceName _returnvalue)
          (return)))
      (elif (`KismetStringLibrary.Contains` SourceName " ")
        (goto _label)
        (else
          (bind _output_get (set `local.Base` (`KismetStringLibrary.Concat_StrStr` SourceName " 0")))
          (`self.UnifyName` _output_get ExistingNames)
          (`|VariableSetRef` SourceName _output_get))))))

(fn `UnifyNameTrim`
  (params (SourceName :type "String (by ref)") (ExistingNames :type "Array of String"))
  (locals (Collection :type "Set of String") (Base :type String))
  (`BlueprintSetLibrary.Set_AddItems` (`local.Collection`) ExistingNames)
  (if (`BlueprintSetLibrary.Set_Contains` (`local.Collection`) SourceName)
    (if (not (`KismetStringLibrary.IsNumeric` SourceName))
      (if (`self.EndsWithNumber` SourceName) :!label _label
        (bind _string (`self.SplitStringByIndexTrim` SourceName))
        (set `local.Base` _string)
        (else
          (set `local.Base` SourceName)))
      (for _index (range (+ (`BlueprintSetLibrary.Set_Length` (`local.Collection`)) 1))
        (bind _returnvalue (`KismetStringLibrary.Concat_StrStr` (`local.Base`) "_" (`KismetStringLibrary.Conv_IntToString` _index)))
        (if (not (`BlueprintSetLibrary.Set_Contains` (`local.Collection`) _returnvalue))
          (`|VariableSetRef` SourceName _returnvalue)
          (return)))
      (elif (`KismetStringLibrary.Contains` SourceName "_")
        (goto _label)
        (else
          (bind _output_get (set `local.Base` (`KismetStringLibrary.Concat_StrStr` SourceName "_0")))
          (`self.UnifyName` _output_get ExistingNames)
          (`|VariableSetRef` SourceName _output_get))))))