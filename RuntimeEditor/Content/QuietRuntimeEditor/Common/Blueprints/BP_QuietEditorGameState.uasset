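; Game state for the Quiet Runtime Editor that creates and holds the editor's router object.
; On BeginPlay it constructs a BP_Router, stores it and calls Init on it.
; GetRouterObject and TakeObjectWithTag return that router, the latter regardless of the request.
; The other tag-request functions are stubs: the two data functions report failure and TakeActorsWithTag returns nothing.
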(event `self.ReceiveBeginPlay`
  (bind _returnvalue (`|GenericCreateObject` "/Game/QuietRuntimeEditor/Common/Blueprints/BP_Router.BP_Router_C"))
  (bind _output_get (set `self.Router` _returnvalue))
  (`/Game/QuietRuntimeEditor/Common/Blueprints/BP_Router.Init` _output_get))

(fn `GetDataWithTag`
  (params (Request :type "GameplayTag Structure"))
  (returns (Success :type Boolean) (Data :type "JsonObjectWrapper Structure"))
  (return false))

(fn `GetRouterObject`
  (returns (Router :type "/Game/QuietRuntimeEditor/Common/Blueprints/BP_Router Object Reference"))
  (return (`self.Router`)))

(fn `ReturnDataByRequestWithTag`
  (params (Request :type "GameplayTag Structure") (InputData :type "JsonObjectWrapper Structure"))
  (returns (Success :type Boolean) (Data :type "JsonObjectWrapper Structure"))
  (return false))

(fn `TakeActorsWithTag`
  (params (Request :type "GameplayTag Structure"))
  (returns (Actors :type "Array of Actor Object Reference"))
  (return))

(fn `TakeObjectWithTag`
  (params (Request :type "GameplayTag Structure"))
  (returns (Object :type "Object Object Reference"))
  (return (`self.Router`)))

(fn `UserConstructionScript`)