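; BP_Router is a tag-keyed message router that decouples senders from objects implementing BI_QuietRoutingInterface.
; SubscribeWithTag stores objects in a map, and Throw, Request and Get functions forward commands, payloads and queries through that interface.
; A looping timer and actor destruction trigger ClearInvalidSubscribers, but its Contains check never matches stale entries.
; Only GetRegisterdObject validates a stored object and removes it when invalid.
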(event `Init`
  (`KismetSystemLibrary.K2_SetTimer` null "ClearInvalidSubscribers" 30.0 true))

(fn `ClearInvalidSubscribers`
  (bind _keys (`BlueprintMapLibrary.Map_Keys` (`self.Subscribers`)))
  (bind (_arrayindex _arrayelement) (`/Engine/EditorBlueprintResources/StandardMacros.ReverseForEachLoop` _keys)
    (:`LoopBody`
      (if (not (`BlueprintMapLibrary.Map_Contains` (`self.Subscribers`) _arrayelement))
        (`BlueprintMapLibrary.Map_Remove` (`self.Subscribers`) _arrayelement)))))

(fn `Get Data with Tag`
  (params (Target :type "GameplayTag Structure") (Request :type "GameplayTag Structure"))
  (returns (Success :type Boolean) (Data :type "JsonObjectWrapper Structure"))
  (bind _object (`self.FindSubscriberWithTag` Target))
  (bind (_success _data) (message `/Game/QuietRuntimeEditor/Common/Blueprints/BI_QuietRoutingInterface.GetDataWithTag` _object Request))
  (return true _data))

(fn `GetActorsWithTag`
  (params (Target :type "GameplayTag Structure") (DesiredObjects :type "GameplayTag Structure"))
  (returns (Actors :type "Array of Actor Object Reference"))
  (bind _object (`self.FindSubscriberWithTag` Target))
  (bind _actors (message `/Game/QuietRuntimeEditor/Common/Blueprints/BI_QuietRoutingInterface.TakeActorsWithTag` _object DesiredObjects))
  (return _actors))

(fn `GetRegisterdObject`
  (params (Key :type "GameplayTag Structure"))
  (returns (Success :type Boolean) (Value :type "Object Object Reference"))
  (bind _value (`BlueprintMapLibrary.Map_Find` (`self.Subscribers`) Key))
  (if (`BlueprintMapLibrary.Map_Contains` (`self.Subscribers`) Key)
    (`/Engine/EditorBlueprintResources/StandardMacros.IsValid` _value
      (:`Is Valid`
        (return true _value))
      (:`Is Not Valid`
        (`BlueprintMapLibrary.Map_Remove` (`self.Subscribers`) Key)
        (return false null)))
    (else
      (return false null))))

(fn `HandleOnSubscriberDestroyed`
  (params (DestroyedActor :type "Actor Object Reference"))
  (`self.ClearInvalidSubscribers`))

(fn `Request Data with Tag`
  (params (Target :type "GameplayTag Structure") (Request :type "GameplayTag Structure") (InputData :type "JsonObjectWrapper Structure"))
  (returns (Success :type Boolean) (ReturnData :type "JsonObjectWrapper Structure"))
  (bind _object (`self.FindSubscriberWithTag` Target))
  (bind (_success _data) (message `/Game/QuietRuntimeEditor/Common/Blueprints/BI_QuietRoutingInterface.ReturnDataByRequestWithTag` _object Request InputData))
  (return _success _data))

(fn `SubscribeWithTag`
  (params (Tag :type "GameplayTag Structure") (Object :type "Object Object Reference"))
  (returns (ReturnValue :type Boolean))
  (if (`KismetSystemLibrary.DoesImplementInterface` Object "/Game/QuietRuntimeEditor/Common/Blueprints/BI_QuietRoutingInterface.BI_QuietRoutingInterface_C")
    (`BlueprintMapLibrary.Map_Add` (`self.Subscribers`) Tag Object)
    (`|ExecutionSequence`
      (:`then_0`
        (bind _asactor (cast `Actor` Object))
        (add `Actor.OnDestroyed` _asactor (`|CreateDelegate` :!event `HandleOnSubscriberDestroyed`)))
      (:`then_1`
        (return true)))))

(fn `ThrowActor`
  (params (Target :type "GameplayTag Structure") (Action :type "GameplayTag Structure") (Actor :type "Actor Object Reference"))
  (returns (ReturnValue :type Boolean))
  (bind _object (`self.FindSubscriberWithTag` Target))
  (message `/Game/QuietRuntimeEditor/Common/Blueprints/BI_QuietRoutingInterface.ForwardActor` _object Action Actor)
  (return true))

(fn `ThrowCommand`
  (params (Target :type "GameplayTag Structure") (Command :type "GameplayTag Structure"))
  (returns (ReturnValue :type Boolean))
  (bind _object (`self.FindSubscriberWithTag` Target))
  (message `/Game/QuietRuntimeEditor/Common/Blueprints/BI_QuietRoutingInterface.ForwardCommand` _object Command)
  (return true))

(fn `ThrowJson`
  (params (Target :type "GameplayTag Structure") (Action :type "GameplayTag Structure") (Json :type "JsonObjectWrapper Structure"))
  (returns (ReturnValue :type Boolean))
  (bind _object (`self.FindSubscriberWithTag` Target))
  (message `/Game/QuietRuntimeEditor/Common/Blueprints/BI_QuietRoutingInterface.ForwardJson` _object Action Json)
  (return true))

(fn `ThrowMaterial`
  (params (Target :type "GameplayTag Structure") (Action :type "GameplayTag Structure") (Material :type "MaterialInterface Object Reference"))
  (returns (ReturnValue :type Boolean))
  (bind _object (`self.FindSubscriberWithTag` Target))
  (message `/Game/QuietRuntimeEditor/Common/Blueprints/BI_QuietRoutingInterface.ForwardMaterial` _object Action Material)
  (return true))

(fn `ThrowObject`
  (params (Target :type "GameplayTag Structure") (Action :type "GameplayTag Structure") (Object :type "Object Object Reference"))
  (returns (ReturnValue :type Boolean))
  (bind _object (`self.FindSubscriberWithTag` Target))
  (message `/Game/QuietRuntimeEditor/Common/Blueprints/BI_QuietRoutingInterface.ForwardObject` _object Action Object)
  (return true))