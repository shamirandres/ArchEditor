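; Illustrative scheme for QuietRuntimeEditor's manual, showing how a property edit travels from the details UI to selected actors at runtime.
; Details boxes the name and value in JSON, Manager forwards it for each selected actor, and Serializer picks a marshal from a class-keyed map.
; The marshal casts to the example actor and switches on property name to write float, int, string or bool fields.
; Selection and property-name helpers are empty stubs.
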(event `OnFloatPropertyValueChanged (Details)`
  (params (PropertyName :type String) (NewValue :type "Float (double-precision)"))
  ;[0 0 0] Details
  (bind _jsonobject (`self.NewJson`))
  (`|SetJsonField` _jsonobject PropertyName NewValue)
  (`self.RequestToChangePropery (Manager)` _jsonobject))

(event `RequestToChangePropery (Manager)`
  (params (BoxedProperty :type "JsonObjectWrapper Structure"))
  ;[0 0 0] Manager
  (for _array_element (`self.GetSelectedActors`)
    (`self.SendPropertyToMarshal (Serializer)` _array_element BoxedProperty)))

(event `SendPropertyToMarshal (Serializer)`
  (params (Object :type "Object Object Reference") (BoxedProperty :type "JsonObjectWrapper Structure"))
  ;[0 0 0] Serializer
  (`/Game/QuietRuntimeEditor/Serialization/Marshals/BP_MarshalBase.SetPropertyValue` (`BlueprintMapLibrary.Map_Find` (`self.MarshalsMap`) (`|ConvertAsset` (`GameplayStatics.GetObjectClass` Object))) Object (`self.GetPropertyName` BoxedProperty) BoxedProperty))

(event `SetProperty (Marshal)`
  (params (Object :type "Object Object Reference") (Property :type String) (JsonValue :type "JsonObjectWrapper Structure"))
  ;[0 0 0] Marshal
  (bind _asbp_serialization_example_actor (cast `/Game/QuietRuntimeEditor/Manual/Schemes/BP_SerializationExampleActor` Object))
  (switch `string` Property
    (:`SomeFloat`
      (bind _outvalue (`|GetJsonField` JsonValue Property))
      (set `/Game/QuietRuntimeEditor/Manual/Schemes/BP_SerializationExampleActor.SomeFloat` _outvalue _asbp_serialization_example_actor))
    (:`SomeInt`
      (bind _outvalue_2 (`|GetJsonField` JsonValue Property))
      (set `/Game/QuietRuntimeEditor/Manual/Schemes/BP_SerializationExampleActor.SomeInt` _outvalue_2 _asbp_serialization_example_actor))
    (:`SomeString`
      (bind _outvalue_3 (`|GetJsonField` JsonValue Property))
      (set `/Game/QuietRuntimeEditor/Manual/Schemes/BP_SerializationExampleActor.SomeString` _outvalue_3 _asbp_serialization_example_actor))
    (:`SomeBool`
      (bind _outvalue_4 (`|GetJsonField` JsonValue Property))
      (set `/Game/QuietRuntimeEditor/Manual/Schemes/BP_SerializationExampleActor.SomeBool` _outvalue_4 _asbp_serialization_example_actor))))

(fn `GetPropertyName`
  (params (Property :type "JsonObjectWrapper Structure (by ref)"))
  (returns (Name :type String))
  (return ""))

(fn `GetSelectedActors`
  (returns (Actors :type "Array of Actor Object Reference"))
  (return))

(fn `NewJson`
  (returns (JsonObject :type "JsonObjectWrapper Structure"))
  (return (make `JsonObjectWrapper`)))