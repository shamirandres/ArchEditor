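; Undo/redo history component for the Quiet runtime editor, storing actions as JSON objects in a capped, indexed stack.
; RegisterAction tags and records actions unless opted out via RegisterInHistory, optionally executing them through CallRedo.
; Undo and redo move the index and invoke CallUndo/CallRedo; registrations feed an unsaved-change counter.
; CutStack runs after appending and re-indexing, so undone entries stay in the stack.
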(event `RegisterAction`
  (params (Type :type "/Game/QuietRuntimeEditor/History/EQuietActionType Enum" :default "NewEnumerator11") (ActionData :type "JsonObjectWrapper Structure") (Execute :type Boolean))
  ;[0 0 0] Register Action
  (`|SetJsonField` ActionData "ActionType" Type)
  (bind _returnvalue (`JsonBlueprintFunctionLibrary.HasField` ActionData "RegisterInHistory"))
  (if _returnvalue
    (bind _outvalue (`|GetJsonField` ActionData "RegisterInHistory"))
    (if _outvalue
      (bind _returnvalue_2 (`KismetArrayLibrary.Array_Add` (`self.HistoryStack`) ActionData :!label _label))
      (set `self.CurrentStackIndex` _returnvalue_2)
      (`/Engine/EditorBlueprintResources/StandardMacros.IncrementInt` (`self.UnsavedCounter`)
        (:`  `
          (`|ExecutionSequence`
            (:`then_0`
              (`self.CutStack`)
              (if (== (`KismetArrayLibrary.Array_LastIndex` (`self.HistoryStack`)) (`self.HistoryStackLimit`))
                (`self.RemoveActionFromStack` (`|GetArrayItem` (`self.HistoryStack`)))
                (`/Engine/EditorBlueprintResources/StandardMacros.DecrementInt` (`self.CurrentStackIndex`))))
            (:`then_1`
              (if Execute :!label _label_2
                (`self.Redo` ActionData))))))
      (else
        (goto _label_2)))
    (else
      (goto _label))))

(event `UndoEvent`
  ;[0 0 0] UNDO
  (if (>= (`self.CurrentStackIndex`) 0)
    (`self.Undo` (`|GetArrayItem` (`self.HistoryStack`) (`self.CurrentStackIndex`)))
    (bind _result (`/Engine/EditorBlueprintResources/StandardMacros.DecrementInt` (`self.CurrentStackIndex`))
      (:`  `
        (set `self.CurrentStackIndex` (`KismetMathLibrary.Clamp` _result -1 (- (`self.HistoryStackLimit`) 1)))))))

(event `RedoEvent`
  (bind _returnvalue (+ (`self.CurrentStackIndex`) 1))
  ;[0 0 0] REDO
  (if (`KismetArrayLibrary.Array_IsValidIndex` (`self.HistoryStack`) _returnvalue)
    (`self.Redo` (`|GetArrayItem` (`self.HistoryStack`) _returnvalue))
    (`/Engine/EditorBlueprintResources/StandardMacros.IncrementInt` (`self.CurrentStackIndex`))))

(event `ClearHistory`
  ;[0 0 0] Clear History
  (set `self.CurrentStackIndex` -1)
  (`KismetArrayLibrary.Array_Clear` (`self.HistoryStack`))
  (`self.ResetUnsavedCounter`))

(event `ResetUnsavedCounter`
  ;[0 0 0] Reset Unsaved Steps
  (set `self.UnsavedCounter` 0))

(fn `AddToLastAction`
  (params (Json :type "JsonObjectWrapper Structure"))
  (bind _historystack (`self.HistoryStack`))
  (bind _returnvalue (`KismetArrayLibrary.Array_LastIndex` _historystack))
  (if (`KismetArrayLibrary.Array_IsValidIndex` _historystack _returnvalue)
    (`|SetJsonField` (`|GetArrayItem` _historystack _returnvalue) "Addition" Json)))

(fn `CutStack`
  (while (> (`KismetArrayLibrary.Array_LastIndex` (`self.HistoryStack`)) (`self.CurrentStackIndex`))
    (`self.RemoveActionFromStack` (`self.GetLastAction`))))

(fn `GetLastAction`
  (returns (Output :type "JsonObjectWrapper Structure"))
  (bind _historystack (`self.HistoryStack`))
  (return (`|GetArrayItem` _historystack (`KismetArrayLibrary.Array_LastIndex` _historystack))))

(fn `HasUnsavedSteps`
  (returns (ReturnValue :type Boolean))
  (return (> (`self.UnsavedCounter`) 0)))

(fn `RemoveActionFromStack`
  (params (Action :type "JsonObjectWrapper Structure (by ref)"))
  (`KismetArrayLibrary.Array_RemoveItem` (`self.HistoryStack`) Action))

(fn `UpdateLastAction`
  (params (Json :type "JsonObjectWrapper Structure"))
  (bind _historystack (`self.HistoryStack`))
  (if (`KismetArrayLibrary.Array_IsNotEmpty` (`self.HistoryStack`))
    (bind _pinned (`/Game/QuietRuntimeEditor/Common/Blueprints/BP_QuietJsonMacroLibrary.Pin` (`|GetArrayItem` _historystack (`KismetArrayLibrary.Array_LastIndex` _historystack))))
    (bind _outvalue (`|GetJsonField` Json "Cache"))
    (`|SetJsonField` _pinned "Cache" _outvalue)))