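; Blueprint function library for the runtime editor's outliner, working through the BP_QuietOutlinerComponent attached to actors.
; It gets or adds that component, giving new ones a fresh GUID and the actor's display name stripped of class suffixes.
; Helpers read names, GUIDs and selection state, set selection, and filter actors to those carrying the component.
; Batch GUID and parent lookups add empty entries for invalid items, keeping arrays index-aligned.
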(fn `AcquireOutlinerComponent`
  (params (Actor :type "Actor Object Reference"))
  (returns (TreeComponent :type "/Game/QuietRuntimeEditor/Outliner/Blueprints/BP_QuietOutlinerComponent Object Reference"))
  (bind _returnvalue (`Actor.GetComponentByClass` Actor "/Game/QuietRuntimeEditor/Outliner/Blueprints/BP_QuietOutlinerComponent.BP_QuietOutlinerComponent_C"))
  (`/Engine/EditorBlueprintResources/StandardMacros.IsValid` _returnvalue
    (:`Is Valid`
      (return _returnvalue))
    (:`Is Not Valid`
      (bind _returnvalue_2 (`|AddComponentByClass` Actor "/Game/QuietRuntimeEditor/Outliner/Blueprints/BP_QuietOutlinerComponent.BP_QuietOutlinerComponent_C" (`KismetGuidLibrary.NewGuid`) (`self.RemoveAssetSuffix` (`KismetSystemLibrary.GetDisplayName` Actor))))
      (return _returnvalue_2))))

(fn `CollectActorGuids`
  (params (Actors :type "Array of Actor Object Reference"))
  (returns (Guids :type "Array of Guid Structure"))
  (locals (CollectedNames :type "Array of Guid Structure"))
  (for _array_element Actors
    (`KismetArrayLibrary.Array_Add` (`local.CollectedNames`) (`/Game/QuietRuntimeEditor/Outliner/Blueprints/BP_QuietOutlinerComponent.GetGuid` (`Actor.GetComponentByClass` _array_element "/Game/QuietRuntimeEditor/Outliner/Blueprints/BP_QuietOutlinerComponent.BP_QuietOutlinerComponent_C"))))
  (return (`local.CollectedNames`)))

(fn `CollectActorNames`
  (params (Actors :type "Array of Actor Object Reference"))
  (returns (Names :type "Array of String"))
  (locals (CollectedNames :type "Array of String"))
  (for _array_element Actors
    (`KismetArrayLibrary.Array_Add` (`local.CollectedNames`) (`/Game/QuietRuntimeEditor/Outliner/Blueprints/BP_QuietOutlinerComponent.GetName` (`Actor.GetComponentByClass` _array_element "/Game/QuietRuntimeEditor/Outliner/Blueprints/BP_QuietOutlinerComponent.BP_QuietOutlinerComponent_C"))))
  (return (`local.CollectedNames`)))

(fn `FilterActorsArray`
  (params (Actors :type "Array of Actor Object Reference"))
  (returns (Filtered :type "Array of Actor Object Reference"))
  (locals (FilteredArray :type "Array of Actor Object Reference"))
  (for _array_element Actors
    (`/Engine/EditorBlueprintResources/StandardMacros.IsValid` (`Actor.GetComponentByClass` _array_element "/Game/QuietRuntimeEditor/Outliner/Blueprints/BP_QuietOutlinerComponent.BP_QuietOutlinerComponent_C")
      (:`Is Valid`
        (`KismetArrayLibrary.Array_Add` (`local.FilteredArray`) _array_element))))
  (return (`local.FilteredArray`)))

(fn `GetActorName`
  (params (Actor :type "Actor Object Reference"))
  (returns (Name :type String))
  (return (`/Game/QuietRuntimeEditor/Outliner/Blueprints/BP_QuietOutlinerComponent.GetName` (`Actor.GetComponentByClass` Actor "/Game/QuietRuntimeEditor/Outliner/Blueprints/BP_QuietOutlinerComponent.BP_QuietOutlinerComponent_C"))))

(fn `GetOutlinerComponent`
  (params (Object :type "Object Object Reference"))
  (returns (TreeComponent :type "/Game/QuietRuntimeEditor/Outliner/Blueprints/BP_QuietOutlinerComponent Object Reference"))
  (bind _asactor (cast `Actor` Object))
  (return (`Actor.GetComponentByClass` _asactor "/Game/QuietRuntimeEditor/Outliner/Blueprints/BP_QuietOutlinerComponent.BP_QuietOutlinerComponent_C")))

(fn `IsActorSelected`
  (params (Actor :type "Actor Object Reference"))
  (returns (State :type Boolean))
  (return (`/Game/QuietRuntimeEditor/Outliner/Blueprints/BP_QuietOutlinerComponent.GetSelectionState` (`Actor.GetComponentByClass` Actor "/Game/QuietRuntimeEditor/Outliner/Blueprints/BP_QuietOutlinerComponent.BP_QuietOutlinerComponent_C"))))

(fn `RemoveAssetSuffix`
  (params (SourceString :type String))
  (returns (ReturnValue :type String))
  (if (`KismetStringLibrary.EndsWith` SourceString "_C")
    (return (`KismetStringLibrary.LeftChop` SourceString 2))
    (elif (`KismetStringLibrary.Contains` SourceString "_C_")
      (return (`KismetStringLibrary.Replace` SourceString "_C_" "_" "CaseSensitive"))
      (else
        (return SourceString)))))

(fn `SetActorSelectionState`
  (params (Actor :type "Actor Object Reference") (NewState :type Boolean))
  (bind _returnvalue (`Actor.GetComponentByClass` Actor "/Game/QuietRuntimeEditor/Outliner/Blueprints/BP_QuietOutlinerComponent.BP_QuietOutlinerComponent_C"))
  (`/Engine/EditorBlueprintResources/StandardMacros.IsValid` Actor
    (:`Is Valid`
      (if (!= NewState (`/Game/QuietRuntimeEditor/Outliner/Blueprints/BP_QuietOutlinerComponent.GetSelectionState` _returnvalue))
        (if NewState
          (`/Game/QuietRuntimeEditor/Outliner/Blueprints/BP_QuietOutlinerComponent.Select` _returnvalue)
          (else
            (`/Game/QuietRuntimeEditor/Outliner/Blueprints/BP_QuietOutlinerComponent.Deselect` _returnvalue)))))
    (:`Is Not Valid`
      (`KismetSystemLibrary.PrintString` null "Attempt to select an invalid actor"))))

(fn `TakeActorGuid`
  (params (Actor :type "Actor Object Reference"))
  (returns (Guid :type "Guid Structure"))
  (bind _returnvalue (`Actor.GetComponentByClass` Actor "/Game/QuietRuntimeEditor/Outliner/Blueprints/BP_QuietOutlinerComponent.BP_QuietOutlinerComponent_C"))
  (`/Engine/EditorBlueprintResources/StandardMacros.IsValid` Actor
    (:`Is Valid`
      (`/Engine/EditorBlueprintResources/StandardMacros.IsValid` _returnvalue
        (:`Is Valid`
          (return (`/Game/QuietRuntimeEditor/Outliner/Blueprints/BP_QuietOutlinerComponent.GetGuid` _returnvalue)))
        (:`Is Not Valid`
          _)))
    (:`Is Not Valid`
      _))
  (return))

(fn `TakeActorGuids`
  (params (Actor :type "Array of Actor Object Reference"))
  (returns (Guids :type "Array of Guid Structure"))
  (locals (ActorGuids :type "Array of Guid Structure"))
  (bind _actorguids (`local.ActorGuids`))
  (for _array_element Actor
    (`/Engine/EditorBlueprintResources/StandardMacros.IsValid` _array_element
      (:`Is Valid`
        (bind _returnvalue (`Actor.GetComponentByClass` _array_element "/Game/QuietRuntimeEditor/Outliner/Blueprints/BP_QuietOutlinerComponent.BP_QuietOutlinerComponent_C"))
        (`/Engine/EditorBlueprintResources/StandardMacros.IsValid` _returnvalue
          (:`Is Valid`
            (`KismetArrayLibrary.Array_Add` _actorguids (`/Game/QuietRuntimeEditor/Outliner/Blueprints/BP_QuietOutlinerComponent.GetGuid` _returnvalue)))
          (:`Is Not Valid`
            (`KismetArrayLibrary.Array_Add` _actorguids :!label _label))))
      (:`Is Not Valid`
        (goto _label))))
  (return (`local.ActorGuids`)))

(fn `TakeActorParents`
  (params (Actors :type "Array of Actor Object Reference"))
  (returns (Parents :type "Array of Actor Object Reference") (Guids :type "Array of Guid Structure"))
  (locals (ParentActors :type "Array of Actor Object Reference") (ParentGuids :type "Array of Guid Structure"))
  (for _array_element Actors
    (bind _returnvalue (`Actor.GetAttachParentActor` _array_element))
    (`KismetArrayLibrary.Array_Add` (`local.ParentActors`) _returnvalue)
    (`/Engine/EditorBlueprintResources/StandardMacros.IsValid` _returnvalue
      (:`Is Valid`
        (`KismetArrayLibrary.Array_Add` (`local.ParentGuids`) (`self.TakeActorGuid` _returnvalue _returnvalue)))
      (:`Is Not Valid`
        (`KismetArrayLibrary.Array_Add` (`local.ParentGuids`)))))
  (return (`local.ParentActors`) (`local.ParentGuids`)))