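; Marshal for box collision components in the runtime editor, translating a BoxComponent's extent to and from JSON.
; Get and set calls try the parent marshal first, then handle BoxExtent, applying changes with an overlap update.
; Serialization adds BoxExtent to the parent's output.
; Property collection builds a Shape group with a bounded, class-defaulted vector parameter and copies in the parent's Collision group.
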(fn `CollectProperties`
  (params (Object :type "Object Object Reference") (TargetJson :type "JsonObjectWrapper Structure (by ref)"))
  (locals (Shape :type "Array of JsonObjectWrapper Structure"))
  (bind _asbox_collision (cast `BoxComponent` Object))
  (`|SetJsonField` (`local.TargetJson`) "GroupsState" (`|MakeArray` "Shape" "Collision"))
  (bind _jsonobject (`self.MakeVectorParam` "BoxExtent" "Box Extent" "" (`BoxComponent.BoxExtent` _asbox_collision) (defaults `Object` (`GameplayStatics.GetObjectClass` _asbox_collision)) 0.1 1.0 10000.0 1000.0))
  (`KismetArrayLibrary.Array_Add` (`local.Shape`) _jsonobject)
  (`|SetJsonField` (`local.TargetJson`) "Shape" (`local.Shape`))
  (bind _jsonobject_2 (`/Game/QuietRuntimeEditor/Common/Blueprints/BP_QuietJsonFunctionLibrary.NewJson`))
  (`parent.CollectProperties` Object _jsonobject_2)
  (bind _outvalue (`|GetJsonField` _jsonobject_2 "Collision"))
  (`|SetJsonField` (`local.TargetJson`) "Collision" _outvalue)
  (return))

(fn `GetPropertyValue`
  (params (Object :type "Object Object Reference") (Property :type String))
  (returns (Success :type Boolean) (Value :type "JsonObjectWrapper Structure"))
  (bind _property (`local.Property`))
  (bind (_success _value) (`parent.GetPropertyValue` Object Property))
  (if (not _success)
    (bind _asbox_collision (cast `BoxComponent` Object))
    (bind _jsonobject (`/Game/QuietRuntimeEditor/Common/Blueprints/BP_QuietJsonFunctionLibrary.NewJson`))
    (switch `string` _property
      (:`BoxExtent`
        (bind _returnvalue (`|SetJsonField` _jsonobject _property (`BoxComponent.BoxExtent` _asbox_collision)))
        (return _returnvalue _jsonobject)))
    (else
      (return true _value))))

(fn `SerializeObject`
  (params (Object :type "Object Object Reference") (TargetJson :type "JsonObjectWrapper Structure (by ref)"))
  (`parent.SerializeObject` Object TargetJson)
  (bind _asbox_collision (cast `BoxComponent` Object))
  (`|SetJsonField` TargetJson "BoxExtent" (`BoxComponent.BoxExtent` _asbox_collision))
  (return))

(fn `SetPropertyValue`
  (params (Object :type "Object Object Reference") (Property :type String) (JsonValue :type "JsonObjectWrapper Structure (by ref)"))
  (returns (Success :type Boolean))
  (bind _property (`local.Property`))
  (bind _success (`parent.SetPropertyValue` Object Property JsonValue))
  (if (not _success)
    (bind _asbox_collision (cast `BoxComponent` Object))
    (switch `string` _property
      (:`BoxExtent`
        (bind _newvalue (`/Game/QuietRuntimeEditor/Common/Blueprints/BP_QuietJsonMacroLibrary.ReadVectorWithCheck` (`local.JsonValue`) _property (`BoxComponent.BoxExtent` _asbox_collision))
          (:`then`
            (`BoxComponent.SetBoxExtent` _asbox_collision _newvalue true)
            (return true)))))
    (else
      (return true))))