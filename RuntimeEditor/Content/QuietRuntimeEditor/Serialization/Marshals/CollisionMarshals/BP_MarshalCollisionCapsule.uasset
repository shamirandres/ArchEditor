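; Marshal for CapsuleComponent in the runtime editor that converts capsule half height and radius to and from JSON.
; Property get and set try the parent marshal first, then handle the two capsule values, with setters updating overlaps.
; Serialization appends both values to the parent's output.
; Property collection builds a Shape group of ranged float parameters with class defaults and copies in the parent's Collision group.
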(fn `CollectProperties`
  (params (Object :type "Object Object Reference") (TargetJson :type "JsonObjectWrapper Structure (by ref)"))
  (locals (Shape :type "Array of JsonObjectWrapper Structure"))
  (bind _ascapsule_collision (cast `CapsuleComponent` Object))
  (`|SetJsonField` (`local.TargetJson`) "GroupsState" (`|MakeArray` "Shape" "Collision"))
  (bind (_capsulehalfheight _capsuleradius) (defaults `Object` (`GameplayStatics.GetObjectClass` _ascapsule_collision)))
  (bind _jsonobject (`self.MakeFloatParam` "CapsuleHalfHeight" "Capsule Half Height" "" (`CapsuleComponent.CapsuleHalfHeight` _ascapsule_collision) _capsulehalfheight 0.01 1.0 1000.0 100.0 1 3))
  (`KismetArrayLibrary.Array_Add` (`local.Shape`) _jsonobject)
  (bind _jsonobject_2 (`self.MakeFloatParam` "CapsuleRadius" "Capsule Radius" "" (`CapsuleComponent.CapsuleRadius` _ascapsule_collision) _capsuleradius 0.01 1.0 10000.0 400.0 1 3))
  (`KismetArrayLibrary.Array_Add` (`local.Shape`) _jsonobject_2)
  (`|SetJsonField` (`local.TargetJson`) "Shape" (`local.Shape`))
  (bind _jsonobject_3 (`/Game/QuietRuntimeEditor/Common/Blueprints/BP_QuietJsonFunctionLibrary.NewJson`))
  (`parent.CollectProperties` Object _jsonobject_3)
  (bind _outvalue (`|GetJsonField` _jsonobject_3 "Collision"))
  (`|SetJsonField` (`local.TargetJson`) "Collision" _outvalue)
  (return))

(fn `GetPropertyValue`
  (params (Object :type "Object Object Reference") (Property :type String))
  (returns (Success :type Boolean) (Value :type "JsonObjectWrapper Structure"))
  (bind _property (`local.Property`))
  (bind (_success _value) (`parent.GetPropertyValue` Object Property))
  (if (not _success)
    (bind _ascapsule_collision (cast `CapsuleComponent` Object))
    (bind _jsonobject (`/Game/QuietRuntimeEditor/Common/Blueprints/BP_QuietJsonFunctionLibrary.NewJson`))
    (switch `string` _property
      (:`CapsuleHalfHeight`
        (`|SetJsonField` _jsonobject _property (`CapsuleComponent.CapsuleHalfHeight` _ascapsule_collision)))
      (:`CapsuleRadius`
        (`|SetJsonField` _jsonobject _property (`CapsuleComponent.CapsuleRadius` _ascapsule_collision))))
    (return true _jsonobject)
    (else
      (return true _value))))

(fn `SerializeObject`
  (params (Object :type "Object Object Reference") (TargetJson :type "JsonObjectWrapper Structure (by ref)"))
  (`parent.SerializeObject` Object TargetJson)
  (bind _ascapsule_collision (cast `CapsuleComponent` Object))
  (`|SetJsonField` TargetJson "CapsuleHalfHeight" (`CapsuleComponent.CapsuleHalfHeight` _ascapsule_collision))
  (`|SetJsonField` TargetJson "CapsuleRadius" (`CapsuleComponent.CapsuleRadius` _ascapsule_collision))
  (return))

(fn `SetPropertyValue`
  (params (Object :type "Object Object Reference") (Property :type String) (JsonValue :type "JsonObjectWrapper Structure (by ref)"))
  (returns (Success :type Boolean))
  (bind _property (`local.Property`))
  (bind _jsonvalue (`local.JsonValue`))
  (bind _success (`parent.SetPropertyValue` Object Property JsonValue))
  (if (not _success)
    (bind _ascapsule_collision (cast `CapsuleComponent` Object))
    (switch `string` _property
      (:`CapsuleHalfHeight`
        (bind _newvalue (`/Game/QuietRuntimeEditor/Common/Blueprints/BP_QuietJsonMacroLibrary.ReadFloatWithCheck` _jsonvalue _property (`CapsuleComponent.CapsuleHalfHeight` _ascapsule_collision))
          (:`then`
            (`CapsuleComponent.SetCapsuleHalfHeight` _ascapsule_collision _newvalue true))))
      (:`CapsuleRadius`
        (bind _newvalue_2 (`/Game/QuietRuntimeEditor/Common/Blueprints/BP_QuietJsonMacroLibrary.ReadFloatWithCheck` _jsonvalue _property (`CapsuleComponent.CapsuleRadius` _ascapsule_collision))
          (:`then`
            (`CapsuleComponent.SetCapsuleRadius` _ascapsule_collision _newvalue_2 true)))))
    (return true)
    (else
      (return true))))