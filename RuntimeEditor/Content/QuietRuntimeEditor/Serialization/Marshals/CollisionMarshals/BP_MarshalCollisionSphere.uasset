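; Marshal Blueprint for sphere collision components in the runtime editor, serializing and exposing SphereRadius for editing.
; Property get and set try the parent marshal first, then handle the radius, applying changes via SetSphereRadius with overlap updates.
; Serialization appends the radius to the parent's output.
; Property collection builds a Shape group with a bounded radius slider and copies the parent's Collision group alongside it.
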(fn `CollectProperties`
  (params (Object :type "Object Object Reference") (TargetJson :type "JsonObjectWrapper Structure (by ref)"))
  (locals (Shape :type "Array of JsonObjectWrapper Structure"))
  (bind _assphere_collision (cast `SphereComponent` Object))
  (`|SetJsonField` (`local.TargetJson`) "GroupsState" (`|MakeArray` "Shape" "Collision"))
  (bind _jsonobject (`self.MakeFloatParam` "SphereRadius" "Sphere Radius" "" (`SphereComponent.SphereRadius` _assphere_collision) (defaults `Object` (`GameplayStatics.GetObjectClass` _assphere_collision)) 0.01 1.0 10000.0 400.0 1 3))
  (`KismetArrayLibrary.Array_Add` (`local.Shape`) _jsonobject)
  (`|SetJsonField` (`local.TargetJson`) "Shape" (`local.Shape`))
  (bind _jsonobject_2 (`/Game/QuietRuntimeEditor/Common/Blueprints/BP_QuietJsonFunctionLibrary.NewJson`))
  (`parent.CollectProperties` Object _jsonobject_2)
  (bind _outvalue (`|GetJsonField` _jsonobject_2 "Collision"))
  (`|SetJsonField` (`local.TargetJson`) "Collision" _outvalue)
  (return))

(fn `GetPropertyValue`
  (params (Object :type "Object Object Reference") (Property :type String))
  (returns (Success :type Boolean) (Value :type "JsonObjectWrapper Structure"))
  (bind _property (`local.Property`))
  (bind (_success _value) (`parent.GetPropertyValue` Object Property))
  (if (not _success)
    (bind _assphere_collision (cast `SphereComponent` Object))
    (bind _jsonobject (`/Game/QuietRuntimeEditor/Common/Blueprints/BP_QuietJsonFunctionLibrary.NewJson`))
    (switch `string` _property
      (:`SphereRadius`
        (bind _returnvalue (`|SetJsonField` _jsonobject _property (`SphereComponent.SphereRadius` _assphere_collision)))
        (return _returnvalue _jsonobject)))
    (else
      (return true _value))))

(fn `SerializeObject`
  (params (Object :type "Object Object Reference") (TargetJson :type "JsonObjectWrapper Structure (by ref)"))
  (`parent.SerializeObject` Object TargetJson)
  (bind _assphere_collision (cast `SphereComponent` Object))
  (`|SetJsonField` TargetJson "SphereRadius" (`SphereComponent.SphereRadius` _assphere_collision))
  (return))

(fn `SetPropertyValue`
  (params (Object :type "Object Object Reference") (Property :type String) (JsonValue :type "JsonObjectWrapper Structure (by ref)"))
  (returns (Success :type Boolean))
  (bind _property (`local.Property`))
  (bind _success (`parent.SetPropertyValue` Object Property JsonValue))
  (if (not _success)
    (bind _assphere_collision (cast `SphereComponent` Object))
    (switch `string` _property
      (:`SphereRadius`
        (bind _newvalue (`/Game/QuietRuntimeEditor/Common/Blueprints/BP_QuietJsonMacroLibrary.ReadFloatWithCheck` (`local.JsonValue`) _property (`SphereComponent.SphereRadius` _assphere_collision))
          (:`then`
            (`SphereComponent.SetSphereRadius` _assphere_collision _newvalue true)
            (return true)))))
    (else
      (return true))))