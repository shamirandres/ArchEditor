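; Marshal for actors in the Quiet runtime editor that converts them to and from JSON and exposes their properties for editing.
; Serialization writes class, transform, tags, hidden state, attach socket and the outliner component's GUID and name, which restore re-applies before calling the parent.
; Property setters change tags and visibility, and treat "Component.Slot" names as material assignments, with "None" applying a default material.
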(fn `CollectProperties`
  (params (Object :type "Object Object Reference") (TargetJson :type "JsonObjectWrapper Structure (by ref)"))
  (bind _asactor (cast `Actor` Object))
  (bind _jsonobject (`/Game/QuietRuntimeEditor/Serialization/Marshals/BP_MarshalMacroLibrary.MakeArrayJsonParam` "Name" "Tags" "Tags" "" (`Actor.Tags` _asactor) "None" (make `JsonObjectWrapper`)))
  (`|SetJsonField` TargetJson "Actor" (`|MakeArray` _jsonobject))
  (return))

(fn `GetActorGuid`
  (params (Actor :type "Actor Object Reference"))
  (returns (Success :type Boolean) (Guid :type "Guid Structure"))
  (bind _pinned (`/Game/QuietRuntimeEditor/Common/Blueprints/BP_QuietJsonMacroLibrary.Pin` (`Actor.GetComponentByClass` Actor "/Game/QuietRuntimeEditor/Outliner/Blueprints/BP_QuietOutlinerComponent.BP_QuietOutlinerComponent_C")))
  (`/Engine/EditorBlueprintResources/StandardMacros.IsValid` _pinned
    (:`Is Valid`
      (return true (`/Game/QuietRuntimeEditor/Outliner/Blueprints/BP_QuietOutlinerComponent.GetGuid` _pinned)))))

(fn `GetActorName`
  (params (Actor :type "Actor Object Reference"))
  (returns (Name :type String))
  (bind _pinned (`/Game/QuietRuntimeEditor/Common/Blueprints/BP_QuietJsonMacroLibrary.Pin` (`Actor.GetComponentByClass` Actor "/Game/QuietRuntimeEditor/Outliner/Blueprints/BP_QuietOutlinerComponent.BP_QuietOutlinerComponent_C")))
  (`/Engine/EditorBlueprintResources/StandardMacros.IsValid` _pinned
    (:`Is Valid`
      (return (`/Game/QuietRuntimeEditor/Outliner/Blueprints/BP_QuietOutlinerComponent.GetName` _pinned)))
    (:`Is Not Valid`
      (return (`KismetSystemLibrary.GetDisplayName` Actor)))))

(fn `GetPrimitiveByName`
  (params (Actor :type "Actor Object Reference") (Name :type String))
  (returns (Component :type "ActorComponent Object Reference"))
  (if (`KismetStringLibrary.EqualEqual_StrStr` Name "Root")
    (return (`Actor.RootComponent` Actor))
    (else
      (for _array_element (`Actor.K2_GetComponentsByClass` Actor "/Script/Engine.ActorComponent")
        (if (`KismetStringLibrary.EqualEqual_StrStr` (`KismetSystemLibrary.GetDisplayName` _array_element) Name)
          (return _array_element))))))

(fn `GetPropertyValue`
  (params (Object :type "Object Object Reference") (Property :type String))
  (returns (Success :type Boolean) (Value :type "JsonObjectWrapper Structure"))
  (bind _asactor (cast `Actor` Object))
  (bind _outjsonobject (`JsonBlueprintFunctionLibrary.FromString` "{ }"))
  (switch `string` Property
    (:`Tags`
      (`|SetJsonField` _outjsonobject Property (`Actor.Tags` _asactor))
      (return true _outjsonobject))
    (:`Hidden`
      (`|SetJsonField` _outjsonobject Property (`Actor.bHidden` _asactor))
      (return true _outjsonobject))
    (:`Socket`
      (`|SetJsonField` _outjsonobject Property (`Actor.GetAttachParentSocketName` _asactor))
      (return true _outjsonobject))
    (:`Guid`
      (bind (_success _guid) (`self.GetActorGuid` _asactor))
      (if _success
        (`|SetJsonField` _outjsonobject Property _guid)
        (return true _outjsonobject)))
    (:`Name`
      (bind _name (`self.GetActorName` _asactor))
      (`|SetJsonField` _outjsonobject Property _name)
      (return true _outjsonobject))))

(fn `RestoreObject`
  (params (Object :type "Object Object Reference") (JsonObject :type "JsonObjectWrapper Structure"))
  (`self.RestoreQuietComponent` Object JsonObject)
  (`parent.RestoreObject` Object JsonObject))

(fn `RestoreQuietComponent`
  (params (Object :type "Object Object Reference") (Json :type "JsonObjectWrapper Structure"))
  (bind _returnvalue (`JsonBlueprintFunctionLibrary.HasField` Json "QuietComponent"))
  (if _returnvalue
    (bind _asactor (cast `Actor` Object))
    (bind _outvalue (`|GetJsonField` Json "QuietComponent"))
    (bind _outvalue_2 (`|GetJsonField` _outvalue "Name"))
    (bind _outvalue_3 (`|GetJsonField` _outvalue "Guid"))
    (bind _returnvalue_2 (`Actor.GetComponentByClass` _asactor "/Game/QuietRuntimeEditor/Outliner/Blueprints/BP_QuietOutlinerComponent.BP_QuietOutlinerComponent_C"))
    (`/Engine/EditorBlueprintResources/StandardMacros.IsValid` _returnvalue_2
      (:`Is Valid`
        (bind _pinned (`/Game/QuietRuntimeEditor/Common/Blueprints/BP_QuietJsonMacroLibrary.Pin` _returnvalue_2))
        (`/Game/QuietRuntimeEditor/Outliner/Blueprints/BP_QuietOutlinerComponent.SetGuid` _pinned _outvalue_3)
        (`/Game/QuietRuntimeEditor/Outliner/Blueprints/BP_QuietOutlinerComponent.Rename` _pinned _outvalue_2 false))
      (:`Is Not Valid`
        (bind _returnvalue_3 (`|AddComponentByClass` _asactor "/Game/QuietRuntimeEditor/Outliner/Blueprints/BP_QuietOutlinerComponent.BP_QuietOutlinerComponent_C" _outvalue_3 _outvalue_2))
        (`/Game/QuietRuntimeEditor/Outliner/Blueprints/BP_QuietOutlinerComponent.Rename` _returnvalue_3 _outvalue_2 false)))))

(fn `SerializeObject`
  (params (Object :type "Object Object Reference") (TargetJson :type "JsonObjectWrapper Structure (by ref)"))
  (bind _asactor (cast `Actor` Object))
  (`self.SerializeOutlinerComponent` _asactor TargetJson)
  (`|ExecutionSequence`
    (:`then_0`
      (`|SetJsonField` TargetJson "Class" (`GameplayStatics.GetObjectClass` _asactor)))
    (:`then_1`
      (`|SetJsonField` TargetJson "Transform" (`Actor.GetTransform` _asactor)))
    (:`then_2`
      (`|SetJsonField` TargetJson "Tags" (`Actor.Tags` _asactor)))
    (:`then_3`
      (`|SetJsonField` TargetJson "Hidden" (`Actor.bHidden` _asactor)))
    (:`then_4`
      (`|SetJsonField` TargetJson "Socket" (`Actor.GetAttachParentSocketName` _asactor))
      (return))))

(fn `SerializeOutlinerComponent`
  (params (Actor :type "Actor Object Reference") (JsonObject :type "JsonObjectWrapper Structure (by ref)"))
  (bind _pinned (`/Game/QuietRuntimeEditor/Common/Blueprints/BP_QuietJsonMacroLibrary.Pin` (`Actor.GetComponentByClass` Actor "/Game/QuietRuntimeEditor/Outliner/Blueprints/BP_QuietOutlinerComponent.BP_QuietOutlinerComponent_C")))
  (`/Engine/EditorBlueprintResources/StandardMacros.IsValid` _pinned
    (:`Is Valid`
      (bind _jsonobject (`/Game/QuietRuntimeEditor/Common/Blueprints/BP_QuietJsonFunctionLibrary.NewJson`))
      (`|SetJsonField` _jsonobject "Guid" (`/Game/QuietRuntimeEditor/Outliner/Blueprints/BP_QuietOutlinerComponent.GetGuid` _pinned))
      (`|SetJsonField` _jsonobject "Name" (`/Game/QuietRuntimeEditor/Outliner/Blueprints/BP_QuietOutlinerComponent.GetName` _pinned))
      (`|SetJsonField` JsonObject "QuietComponent" _jsonobject))))

(fn `SetMaterial`
  (params (Actor :type "Actor Object Reference") (Property :type String) (Json :type "JsonObjectWrapper Structure"))
  (returns (Success :type Boolean))
  (bind (_lefts _rights) (`KismetStringLibrary.Split` Property "."))
  (bind _returnvalue (`KismetStringLibrary.Conv_StringToName` _rights))
  (if (`KismetStringLibrary.Contains` Property ".")
    (bind _returnvalue_2 (`JsonBlueprintFunctionLibrary.HasField` Json Property))
    (if _returnvalue_2
      (bind (_outvalue _returnvalue_3) (`|GetJsonField` Json Property))
      (if _returnvalue_3
        (bind _asmaterial_interface (cast `MaterialInterface` _outvalue)
          (:`then`
            (bind _component (`self.GetPrimitiveByName` Actor _lefts))
            (bind _asprimitive_component (cast `PrimitiveComponent` _component))
            (`PrimitiveComponent.SetMaterialByName` _asprimitive_component _returnvalue _asmaterial_interface)
            (return true))
          (:`CastFailed`
            (bind (_outvalue_2 _returnvalue_4) (`|GetJsonField` Json Property))
            (if _returnvalue_4
              (if (== _outvalue_2 "None")
                (bind _component_2 (`self.GetPrimitiveByName` Actor _lefts))
                (bind _asprimitive_component_2 (cast `PrimitiveComponent` _component_2))
                (`PrimitiveComponent.SetMaterialByName` _asprimitive_component_2 _returnvalue "/Engine/EngineMaterials/DefaultMaterial.DefaultMaterial")
                (return true)))))))))

(fn `SetPropertyValue`
  (params (Object :type "Object Object Reference") (Property :type String) (JsonValue :type "JsonObjectWrapper Structure (by ref)"))
  (returns (Success :type Boolean))
  (bind _asactor (cast `Actor` Object))
  (switch `string` Property
    (:`Default`
      (bind _success (`self.SetMaterial` _asactor Property JsonValue))
      (return _success))
    (:`Tags`
      (bind _array (`/Game/QuietRuntimeEditor/Serialization/Marshals/BP_MarshalMacroLibrary.EjectArray` JsonValue Property))
      (if (not (`KismetArrayLibrary.Array_Identical` _array (`Actor.Tags` _asactor)))
        (set `Actor.Tags` _array _asactor)
        (return true)))
    (:`Hidden`
      (bind _outvalue (`|GetJsonField` JsonValue Property))
      (if (!= _outvalue (`Actor.bHidden` _asactor))
        (`Actor.SetActorHiddenInGame` _asactor _outvalue)
        (return true)))))