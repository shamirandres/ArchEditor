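; Runtime editor marshal that serializes BP_ScatterMeshComponent scatter settings to JSON and exposes them for editing.
; CollectProperties builds typed UI parameter descriptors for the static mesh and placement settings like weight, height, orientation, scale and tilt.
; Property get/set and actions try the parent marshal first, then handle scatter-specific fields through checked JSON reads.
; The static mesh is editable but not written by this class's SerializeObject, and CallAction can clear instances.
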(fn `CallAction`
  (params (Object :type "Object Object Reference") (Action :type "JsonObjectWrapper Structure"))
  (returns (Success :type Boolean))
  (bind _success (`parent.CallAction` Object Action))
  (if (not _success)
    (bind _asbp_scatter_mesh_component (cast `/Game/QuietRuntimeEditor/Common/Features/QuietScatter/Blueprints/BP_ScatterMeshComponent` Object))
    (bind _outvalue (`|GetJsonField` (`local.Action`) "Action"))
    (switch `string` _outvalue
      (:`Clear`
        (`InstancedStaticMeshComponent.ClearInstances` _asbp_scatter_mesh_component)))
    (else
      (return true))))

(fn `CollectProperties`
  (params (Object :type "Object Object Reference") (TargetJson :type "JsonObjectWrapper Structure (by ref)"))
  (locals (Comp :type "Array of JsonObjectWrapper Structure"))
  (bind _asbp_scatter_mesh_component (cast `/Game/QuietRuntimeEditor/Common/Features/QuietScatter/Blueprints/BP_ScatterMeshComponent` Object))
  (bind _jsonobject (`self.MakeObjectParam` "StaticMesh" "Static Mesh" "" "/Script/Engine.StaticMesh" (`StaticMeshComponent.StaticMesh` _asbp_scatter_mesh_component)))
  (`KismetArrayLibrary.Array_Add` (`local.Comp`) _jsonobject)
  (bind (_weight _gravity _heightlimits _heightfallof _orientationlimit _scale_range _maxrandomtilt _maxrotationangle) (defaults `Object` (`GameplayStatics.GetObjectClass` _asbp_scatter_mesh_component)))
  (bind _jsonobject_2 (`self.MakeIntParam` "Weight" "Weight" "" (`/Game/QuietRuntimeEditor/Common/Features/QuietScatter/Blueprints/BP_ScatterMeshComponent.Weight` _asbp_scatter_mesh_component) _weight 0 0 100 20 true))
  (`KismetArrayLibrary.Array_Add` (`local.Comp`) _jsonobject_2)
  (bind _jsonobject_3 (`self.MakeFloatParam` "Gravity" "Gravity" "" (`/Game/QuietRuntimeEditor/Common/Features/QuietScatter/Blueprints/BP_ScatterMeshComponent.Gravity` _asbp_scatter_mesh_component) _gravity 0.0 0.0 1.0 1.0 1 3 true))
  (`KismetArrayLibrary.Array_Add` (`local.Comp`) _jsonobject_3)
  (bind _jsonobject_4 (`self.MakeVector2DParam` "HeightLimits" "Height Limits" "" (`/Game/QuietRuntimeEditor/Common/Features/QuietScatter/Blueprints/BP_ScatterMeshComponent.HeightLimits` _asbp_scatter_mesh_component) _heightlimits 0.0 0.0 0.0 0.0 1 3 true))
  (`KismetArrayLibrary.Array_Add` (`local.Comp`) _jsonobject_4)
  (bind _jsonobject_5 (`self.MakeFloatParam` "HeightFalloff" "Height Falloff" "" (`/Game/QuietRuntimeEditor/Common/Features/QuietScatter/Blueprints/BP_ScatterMeshComponent.HeightFallof` _asbp_scatter_mesh_component) _heightfallof 0.0 0.0 0.5 0.5 1 3 true))
  (`KismetArrayLibrary.Array_Add` (`local.Comp`) _jsonobject_5)
  (bind _jsonobject_6 (`self.MakeVector2DParam` "OrientationLimit" " Orientation Limit" "" (`/Game/QuietRuntimeEditor/Common/Features/QuietScatter/Blueprints/BP_ScatterMeshComponent.OrientationLimit` _asbp_scatter_mesh_component) _orientationlimit 0.0 0.0 0.0 0.0 1 3 true))
  (`KismetArrayLibrary.Array_Add` (`local.Comp`) _jsonobject_6)
  (bind _jsonobject_7 (`self.MakeVector2DParam` "ScaleRange" "Scale Range" "" (`/Game/QuietRuntimeEditor/Common/Features/QuietScatter/Blueprints/BP_ScatterMeshComponent.Scale Range` _asbp_scatter_mesh_component) _scale_range 0.0 0.0 0.0 0.0 1 3 true))
  (`KismetArrayLibrary.Array_Add` (`local.Comp`) _jsonobject_7)
  (bind _jsonobject_8 (`self.MakeFloatParam` "MaxRandomTilt" "Max Random Tilt" "" (`/Game/QuietRuntimeEditor/Common/Features/QuietScatter/Blueprints/BP_ScatterMeshComponent.MaxRandomTilt` _asbp_scatter_mesh_component) _maxrandomtilt 0.0 0.0 60.0 45.0 1 3 true))
  (`KismetArrayLibrary.Array_Add` (`local.Comp`) _jsonobject_8)
  (bind _jsonobject_9 (`self.MakeFloatParam` "MaxRotationAngle" "Max Rotation Angle" "" (`/Game/QuietRuntimeEditor/Common/Features/QuietScatter/Blueprints/BP_ScatterMeshComponent.MaxRotationAngle` _asbp_scatter_mesh_component) _maxrotationangle 0.0 0.0 180.0 180.0 1 3 true))
  (`KismetArrayLibrary.Array_Add` (`local.Comp`) _jsonobject_9)
  (`|SetJsonField` (`local.TargetJson`) "Component" (`local.Comp`))
  (return))

(fn `GetPropertyValue`
  (params (Object :type "Object Object Reference") (Property :type String))
  (returns (Success :type Boolean) (Value :type "JsonObjectWrapper Structure"))
  (bind _property (`local.Property`))
  (bind (_success _value) (`parent.GetPropertyValue` Object Property))
  (if (not _success)
    (bind _asbp_scatter_mesh_component (cast `/Game/QuietRuntimeEditor/Common/Features/QuietScatter/Blueprints/BP_ScatterMeshComponent` Object))
    (bind _jsonobject (`/Game/QuietRuntimeEditor/Common/Blueprints/BP_QuietJsonFunctionLibrary.NewJson`))
    (switch `string` (`local.Property`)
      (:`Weight`
        (`|SetJsonField` _jsonobject _property (`/Game/QuietRuntimeEditor/Common/Features/QuietScatter/Blueprints/BP_ScatterMeshComponent.Weight` _asbp_scatter_mesh_component)))
      (:`Gravity`
        (`|SetJsonField` _jsonobject _property (`/Game/QuietRuntimeEditor/Common/Features/QuietScatter/Blueprints/BP_ScatterMeshComponent.Gravity` _asbp_scatter_mesh_component)))
      (:`HeightLimits`
        (`|SetJsonField` _jsonobject _property (`/Game/QuietRuntimeEditor/Common/Features/QuietScatter/Blueprints/BP_ScatterMeshComponent.HeightLimits` _asbp_scatter_mesh_component)))
      (:`HeightFalloff`
        (`|SetJsonField` _jsonobject _property (`/Game/QuietRuntimeEditor/Common/Features/QuietScatter/Blueprints/BP_ScatterMeshComponent.HeightFallof` _asbp_scatter_mesh_component)))
      (:`OrientationLimit`
        (`|SetJsonField` _jsonobject _property (`/Game/QuietRuntimeEditor/Common/Features/QuietScatter/Blueprints/BP_ScatterMeshComponent.OrientationLimit` _asbp_scatter_mesh_component)))
      (:`ScaleRange`
        (`|SetJsonField` _jsonobject _property (`/Game/QuietRuntimeEditor/Common/Features/QuietScatter/Blueprints/BP_ScatterMeshComponent.Scale Range` _asbp_scatter_mesh_component)))
      (:`MaxRandomTilt`
        (`|SetJsonField` _jsonobject _property (`/Game/QuietRuntimeEditor/Common/Features/QuietScatter/Blueprints/BP_ScatterMeshComponent.MaxRandomTilt` _asbp_scatter_mesh_component)))
      (:`MaxRotationAngle`
        (`|SetJsonField` _jsonobject _property (`/Game/QuietRuntimeEditor/Common/Features/QuietScatter/Blueprints/BP_ScatterMeshComponent.MaxRotationAngle` _asbp_scatter_mesh_component))))
    (return true _jsonobject)
    (else
      (return true _value))))

(fn `SerializeObject`
  (params (Object :type "Object Object Reference") (TargetJson :type "JsonObjectWrapper Structure (by ref)"))
  (`parent.SerializeObject` Object TargetJson)
  (bind _asbp_scatter_mesh_component (cast `/Game/QuietRuntimeEditor/Common/Features/QuietScatter/Blueprints/BP_ScatterMeshComponent` Object))
  (`|SetJsonField` (`local.TargetJson`) "Weight" (`/Game/QuietRuntimeEditor/Common/Features/QuietScatter/Blueprints/BP_ScatterMeshComponent.Weight` _asbp_scatter_mesh_component))
  (`|SetJsonField` (`local.TargetJson`) "Gravity" (`/Game/QuietRuntimeEditor/Common/Features/QuietScatter/Blueprints/BP_ScatterMeshComponent.Gravity` _asbp_scatter_mesh_component))
  (`|SetJsonField` (`local.TargetJson`) "HeightLimits" (`/Game/QuietRuntimeEditor/Common/Features/QuietScatter/Blueprints/BP_ScatterMeshComponent.HeightLimits` _asbp_scatter_mesh_component))
  (`|SetJsonField` (`local.TargetJson`) "HeightFalloff" (`/Game/QuietRuntimeEditor/Common/Features/QuietScatter/Blueprints/BP_ScatterMeshComponent.HeightFallof` _asbp_scatter_mesh_component))
  (`|SetJsonField` (`local.TargetJson`) "OrientationLimit" (`/Game/QuietRuntimeEditor/Common/Features/QuietScatter/Blueprints/BP_ScatterMeshComponent.OrientationLimit` _asbp_scatter_mesh_component))
  (`|SetJsonField` (`local.TargetJson`) "ScaleRange" (`/Game/QuietRuntimeEditor/Common/Features/QuietScatter/Blueprints/BP_ScatterMeshComponent.Scale Range` _asbp_scatter_mesh_component))
  (`|SetJsonField` (`local.TargetJson`) "MaxRandomTilt" (`/Game/QuietRuntimeEditor/Common/Features/QuietScatter/Blueprints/BP_ScatterMeshComponent.MaxRandomTilt` _asbp_scatter_mesh_component))
  (`|SetJsonField` (`local.TargetJson`) "MaxRotationAngle" (`/Game/QuietRuntimeEditor/Common/Features/QuietScatter/Blueprints/BP_ScatterMeshComponent.MaxRotationAngle` _asbp_scatter_mesh_component))
  (return))

(fn `SetPropertyValue`
  (params (Object :type "Object Object Reference") (Property :type String) (JsonValue :type "JsonObjectWrapper Structure (by ref)"))
  (returns (Success :type Boolean))
  (bind _property (`local.Property`))
  (bind _success (`parent.SetPropertyValue` Object Property JsonValue))
  (if (not _success)
    (bind _asbp_scatter_mesh_component (cast `/Game/QuietRuntimeEditor/Common/Features/QuietScatter/Blueprints/BP_ScatterMeshComponent` Object))
    (switch `string` Property
      (:`Weight`
        (bind _newvalue (`/Game/QuietRuntimeEditor/Common/Blueprints/BP_QuietJsonMacroLibrary.ReadIntegerWithCheck` (`local.JsonValue`) _property (`/Game/QuietRuntimeEditor/Common/Features/QuietScatter/Blueprints/BP_ScatterMeshComponent.Weight` _asbp_scatter_mesh_component))
          (:`then`
            (set `/Game/QuietRuntimeEditor/Common/Features/QuietScatter/Blueprints/BP_ScatterMeshComponent.Weight` _newvalue _asbp_scatter_mesh_component))))
      (:`Gravity`
        (bind _newvalue_2 (`/Game/QuietRuntimeEditor/Common/Blueprints/BP_QuietJsonMacroLibrary.ReadFloatWithCheck` (`local.JsonValue`) _property (`/Game/QuietRuntimeEditor/Common/Features/QuietScatter/Blueprints/BP_ScatterMeshComponent.Gravity` _asbp_scatter_mesh_component))
          (:`then`
            (set `/Game/QuietRuntimeEditor/Common/Features/QuietScatter/Blueprints/BP_ScatterMeshComponent.Gravity` _newvalue_2 _asbp_scatter_mesh_component))))
      (:`HeightLimits`
        (bind _newvalue_3 (`/Game/QuietRuntimeEditor/Common/Blueprints/BP_QuietJsonMacroLibrary.ReadVector2DWithCheck` (`local.JsonValue`) _property (`/Game/QuietRuntimeEditor/Common/Features/QuietScatter/Blueprints/BP_ScatterMeshComponent.HeightLimits` _asbp_scatter_mesh_component))
          (:`then`
            (set `/Game/QuietRuntimeEditor/Common/Features/QuietScatter/Blueprints/BP_ScatterMeshComponent.HeightLimits` _newvalue_3 _asbp_scatter_mesh_component))))
      (:`HeightFalloff`
        (bind _newvalue_4 (`/Game/QuietRuntimeEditor/Common/Blueprints/BP_QuietJsonMacroLibrary.ReadFloatWithCheck` (`local.JsonValue`) _property (`/Game/QuietRuntimeEditor/Common/Features/QuietScatter/Blueprints/BP_ScatterMeshComponent.HeightFallof` _asbp_scatter_mesh_component))
          (:`then`
            (set `/Game/QuietRuntimeEditor/Common/Features/QuietScatter/Blueprints/BP_ScatterMeshComponent.HeightFallof` _newvalue_4 _asbp_scatter_mesh_component))))
      (:`OrientationLimit`
        (bind _newvalue_5 (`/Game/QuietRuntimeEditor/Common/Blueprints/BP_QuietJsonMacroLibrary.ReadVector2DWithCheck` (`local.JsonValue`) _property (`/Game/QuietRuntimeEditor/Common/Features/QuietScatter/Blueprints/BP_ScatterMeshComponent.OrientationLimit` _asbp_scatter_mesh_component))
          (:`then`
            (set `/Game/QuietRuntimeEditor/Common/Features/QuietScatter/Blueprints/BP_ScatterMeshComponent.OrientationLimit` _newvalue_5 _asbp_scatter_mesh_component))))
      (:`ScaleRange`
        (bind _newvalue_6 (`/Game/QuietRuntimeEditor/Common/Blueprints/BP_QuietJsonMacroLibrary.ReadVector2DWithCheck` (`local.JsonValue`) _property (`/Game/QuietRuntimeEditor/Common/Features/QuietScatter/Blueprints/BP_ScatterMeshComponent.Scale Range` _asbp_scatter_mesh_component))
          (:`then`
            (set `/Game/QuietRuntimeEditor/Common/Features/QuietScatter/Blueprints/BP_ScatterMeshComponent.Scale Range` _newvalue_6 _asbp_scatter_mesh_component))))
      (:`MaxRandomTilt`
        (bind _newvalue_7 (`/Game/QuietRuntimeEditor/Common/Blueprints/BP_QuietJsonMacroLibrary.ReadFloatWithCheck` (`local.JsonValue`) _property (`/Game/QuietRuntimeEditor/Common/Features/QuietScatter/Blueprints/BP_ScatterMeshComponent.MaxRandomTilt` _asbp_scatter_mesh_component))
          (:`then`
            (set `/Game/QuietRuntimeEditor/Common/Features/QuietScatter/Blueprints/BP_ScatterMeshComponent.MaxRandomTilt` _newvalue_7 _asbp_scatter_mesh_component))))
      (:`MaxRotationAngle`
        (bind _newvalue_8 (`/Game/QuietRuntimeEditor/Common/Blueprints/BP_QuietJsonMacroLibrary.ReadFloatWithCheck` (`local.JsonValue`) _property (`/Game/QuietRuntimeEditor/Common/Features/QuietScatter/Blueprints/BP_ScatterMeshComponent.MaxRotationAngle` _asbp_scatter_mesh_component))
          (:`then`
            (set `/Game/QuietRuntimeEditor/Common/Features/QuietScatter/Blueprints/BP_ScatterMeshComponent.MaxRotationAngle` _newvalue_8 _asbp_scatter_mesh_component))))
      (:`StaticMesh`
        (bind _newvalue_9 (`/Game/QuietRuntimeEditor/Common/Blueprints/BP_QuietJsonMacroLibrary.ReadMeshWithCheck` (`local.JsonValue`) _property (`StaticMeshComponent.StaticMesh` _asbp_scatter_mesh_component))
          (:`then`
            (bind _returnvalue (`StaticMeshComponent.SetStaticMesh` _asbp_scatter_mesh_component _newvalue_9))
            (return _returnvalue)))))
    (return true)
    (else
      (return true))))