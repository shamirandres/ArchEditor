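; Runtime-editor marshal for BP_QuietScatter, a brush and fill mesh-scattering actor, bridging it to JSON for saving and details editing.
; Serializes settings and meshes via the source's cached-object messages; its own restore step rebuilds only the meshes.
; Builds property groups that vary with projection and curvature, and maps actions to scatter and mesh operations.
; Edits route dotted "Name.Index" properties to one mesh, while common mesh settings propagate to all.
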(fn `CallAction`
  (params (Object :type "Object Object Reference") (Action :type "JsonObjectWrapper Structure"))
  (returns (Success :type Boolean))
  (bind _success (`parent.CallAction` Object Action))
  (if (not _success)
    (bind _asquiet_scatter (cast `/Game/QuietRuntimeEditor/Common/Features/QuietScatter/BP_QuietScatter` Object))
    (bind _outvalue (`|GetJsonField` (`local.Action`) "Action"))
    (switch `string` _outvalue
      (:`Default`
        ;[0 0 0] Remove Secondary Mesh
        (if (`KismetStringLibrary.StartsWith` _outvalue "Remove")
          (`/Game/QuietRuntimeEditor/Common/Features/QuietScatter/BP_QuietScatter.RemoveSecondaryMesh` _asquiet_scatter (`KismetStringLibrary.Conv_StringToInt` (`KismetStringLibrary.Replace` _outvalue "Remove")) true)
          (`/Game/QuietRuntimeEditor/Common/Features/QuietScatter/BP_QuietScatter.RefreshDetails` _asquiet_scatter)
          (return true)))
      (:`Clear`
        (`/Game/QuietRuntimeEditor/Common/Features/QuietScatter/BP_QuietScatter.Clear` _asquiet_scatter true)
        (return true))
      (:`Fill`
        (`/Game/QuietRuntimeEditor/Common/Features/QuietScatter/BP_QuietScatter.ExecuteScatter` _asquiet_scatter)
        (return true))
      (:`Add New Mesh`
        (`/Game/QuietRuntimeEditor/Common/Features/QuietScatter/BP_QuietScatter.Add Secondary Mesh` _asquiet_scatter true)
        (`/Game/QuietRuntimeEditor/Common/Features/QuietScatter/BP_QuietScatter.RefreshDetails` _asquiet_scatter)
        (return true)))
    (else
      (return true))))

(fn `CollectCommonProps`
  (params (Component :type "InstancedStaticMeshComponent Object Reference"))
  (returns (CommonParams :type "Array of JsonObjectWrapper Structure"))
  (locals (Collision :type "Array of JsonObjectWrapper Structure") (ECollisionEnabled :type "Array of String") (EObjectType :type "Array of String") (Lighting :type "Array of JsonObjectWrapper Structure") (DefaultChannels :type "LightingChannels Structure") (Render :type "Array of JsonObjectWrapper Structure") (MeshCommonParams :type "Array of JsonObjectWrapper Structure"))
  (bind _returnvalue (`PrimitiveComponent.GetCollisionProfileName` Component))
  (`|ExecutionSequence`
    (:`then_0`
      ;[0 0 0] Collision
      (bind _jsonobject (`self.MakeBoolParam` "GenerateOverlapEvents" "Generate Overlap Events" "" (`PrimitiveComponent.bGenerateOverlapEvents` Component)))
      (`KismetArrayLibrary.Array_Add` (`local.Collision`) _jsonobject)
      (bind _jsonobject_2 (`self.MakeComboStringParam` "CollisionProfileName" "Collision Profile Name" "" (`|MakeArray` "NoCollision" "BlockAll" "OverlapAll" "BlockAllDynamic" "OverlapAllDynamic" "IgnoreOnlyPawn" "OverlapOnlyPawn" "Pawn" "Spectator" "CharacterMesh" "PhysicsActor" "Destructible" "InvisibleWall" "InvisibleWallDynamic" "Trigger" "Ragdoll" "Vehicle" "UI" "Custom") (`KismetStringLibrary.Conv_NameToString` _returnvalue) "BlockAll"))
      (`|SetJsonField` _jsonobject_2 "Dependencies" (`|MakeArray`))
      (`KismetArrayLibrary.Array_Add` (`local.Collision`) _jsonobject_2)
      (if (== _returnvalue "Custom")
        (bind _jsonobject_3 (`self.MakeEnumParam` "CollisionEnabled" "Collision Enabled" "" (`local.ECollisionEnabled`) (`KismetMathLibrary.Conv_ByteToInt` (`PrimitiveComponent.GetCollisionEnabled` Component)) 3))
        (`KismetArrayLibrary.Array_Add` (`local.Collision`) _jsonobject_3)
        (bind _jsonobject_4 (`self.MakeEnumParam` "ObjectType" "Object Type" "" (`local.EObjectType`) (`KismetMathLibrary.Conv_ByteToInt` (`PrimitiveComponent.GetCollisionObjectType` Component))))
        (`KismetArrayLibrary.Array_Add` (`local.Collision`) _jsonobject_4))
      (bind _jsonobject_5 (`self.MakeParamSubgroup` "Collision" (`local.Collision`)))
      (`KismetArrayLibrary.Array_Add` (`local.MeshCommonParams`) _jsonobject_5))
    (:`then_1`
      ;[0 0 0] Rendering
      (bind _jsonobject_6 (`self.MakeBoolParam` "RenderInMainPass" "Render in Main Pass" "" (`PrimitiveComponent.bRenderInMainPass` Component) true))
      (`KismetArrayLibrary.Array_Add` (`local.Render`) _jsonobject_6)
      (bind _jsonobject_7 (`self.MakeBoolParam` "RenderInDepthPass" "Render in Depth Pass" "" (`PrimitiveComponent.bRenderInDepthPass` Component) true))
      (`KismetArrayLibrary.Array_Add` (`local.Render`) _jsonobject_7)
      (bind _jsonobject_8 (`self.MakeBoolParam` "ReceivesDecals" "Receives Decals" "" (`PrimitiveComponent.bReceivesDecals` Component) true))
      (`KismetArrayLibrary.Array_Add` (`local.Render`) _jsonobject_8)
      (bind _jsonobject_9 (`self.MakeBoolParam` "OwnerNoSee" "Owner No See" "" (`PrimitiveComponent.bOwnerNoSee` Component)))
      (`KismetArrayLibrary.Array_Add` (`local.Render`) _jsonobject_9)
      (bind _jsonobject_10 (`self.MakeBoolParam` "OnlyOwnerSee" "Only Owner See" "" (`PrimitiveComponent.bOnlyOwnerSee` Component)))
      (`KismetArrayLibrary.Array_Add` (`local.Render`) _jsonobject_10)
      (bind _jsonobject_11 (`self.MakeBoolParam` "VisibleInSceneCaptureOnly" "Visible in Scene Capture Only" "" (`PrimitiveComponent.bVisibleInSceneCaptureOnly` Component)))
      (`KismetArrayLibrary.Array_Add` (`local.Render`) _jsonobject_11)
      (bind _jsonobject_12 (`self.MakeBoolParam` "HiddenInSceneCapture" "Hidden in Scene Capture" "" (`PrimitiveComponent.bHiddenInSceneCapture` Component)))
      (`KismetArrayLibrary.Array_Add` (`local.Render`) _jsonobject_12)
      (bind _jsonobject_13 (`self.MakeParamSubgroup` "Rendering" (`local.Render`)))
      (`KismetArrayLibrary.Array_Add` (`local.MeshCommonParams`) _jsonobject_13))
    (:`then_2`
      ;[0 0 0] Lighting
      (bind _jsonobject_14 (`self.MakeBoolParam` "CastShadow" "Cast Shadow" "" (`PrimitiveComponent.CastShadow` Component) true))
      (`KismetArrayLibrary.Array_Add` (`local.Lighting`) _jsonobject_14)
      (bind _jsonobject_15 (`self.MakeBoolParam` "ContactShadow" "Contact Shadow" "" (`PrimitiveComponent.bCastContactShadow` Component) true))
      (`KismetArrayLibrary.Array_Add` (`local.Lighting`) _jsonobject_15)
      (bind _jsonobject_16 (`self.MakeBoolParam` "DynamicInsetShadow" "Dynamic Inset Shadow" "" (`PrimitiveComponent.bCastInsetShadow` Component)))
      (`KismetArrayLibrary.Array_Add` (`local.Lighting`) _jsonobject_16)
      (bind _jsonobject_17 (`self.MakeBoolParam` "HiddenShadow" "Hidden Shadow" "" (`PrimitiveComponent.bCastHiddenShadow` Component)))
      (`KismetArrayLibrary.Array_Add` (`local.Lighting`) _jsonobject_17)
      (bind _jsonobject_18 (`self.MakeLightingChannelsParam` "LightingChannels" "Lighting Channels" "" (`PrimitiveComponent.LightingChannels` Component) (`local.DefaultChannels`)))
      (`KismetArrayLibrary.Array_Add` (`local.Lighting`) _jsonobject_18)
      (bind _jsonobject_19 (`self.MakeParamSubgroup` "Lighting" (`local.Lighting`)))
      (`KismetArrayLibrary.Array_Add` (`local.MeshCommonParams`) _jsonobject_19)
      (return (`local.MeshCommonParams`)))))

(fn `CollectProperties`
  (params (Object :type "Object Object Reference") (TargetJson :type "JsonObjectWrapper Structure (by ref)"))
  (locals (ScatterActor :type "/Game/QuietRuntimeEditor/Common/Features/QuietScatter/BP_QuietScatter Object Reference") (Brush :type "Array of JsonObjectWrapper Structure") (Spawn :type "Array of JsonObjectWrapper Structure") (Scatter :type "Array of JsonObjectWrapper Structure"))
  (bind _scatteractor (`local.ScatterActor`))
  (bind _projection (`/Game/QuietRuntimeEditor/Common/Features/QuietScatter/BP_QuietScatter.GetProjectionMode` (`local.ScatterActor`)))
  (bind _asquiet_scatter (cast `/Game/QuietRuntimeEditor/Common/Features/QuietScatter/BP_QuietScatter` Object))
  (set `local.ScatterActor` _asquiet_scatter)
  (`|ExecutionSequence`
    (:`then_0`
      (bind _jsonobject (`self.MakeRadioParam` "BrushMode" "Brush Mode" "" (`/Game/QuietRuntimeEditor/Common/Features/QuietScatter/BP_QuietScatter.BrushOptions` _scatteractor) (`/Game/QuietRuntimeEditor/Common/Features/QuietScatter/BP_QuietScatter.GetBrushModeIndex` _scatteractor)))
      (`KismetArrayLibrary.Array_Add` (`local.Brush`) _jsonobject)
      (bind _jsonobject_2 (`self.MakeFloatParam` "BrushSize" "Brush Size" "" (`/Game/QuietRuntimeEditor/Common/Features/QuietScatter/BP_QuietScatter.BrushSize` (`local.ScatterActor`)) 30.0 1.0 10.0 1000.0 500.0 1 1 true))
      (`KismetArrayLibrary.Array_Add` (`local.Brush`) _jsonobject_2)
      (bind _jsonobject_3 (`self.MakeLinearColorParam` "BrushColor" "Brush Color" "" (`/Game/QuietRuntimeEditor/Common/Features/QuietScatter/BP_QuietScatter.BrushColor` (`local.ScatterActor`)) (struct :`G` 0.219526 :`B` 0.752942 :`A` 0.6)))
      (`KismetArrayLibrary.Array_Add` (`local.Brush`) _jsonobject_3))
    (:`then_1`
      (bind _param (`self.MakeActionsParam` (`|MakeArray` "Fill" "Clear")))
      (`KismetArrayLibrary.Array_Add` (`local.Spawn`) _param)
      (bind _jsonobject_4 (`self.MakeIntParam` "FillCount" "Fill Count" "" (`/Game/QuietRuntimeEditor/Common/Features/QuietScatter/BP_QuietScatter.FillCount` (`local.ScatterActor`)) 100 0 0 100000 10000 true))
      (`KismetArrayLibrary.Array_Add` (`local.Spawn`) _jsonobject_4)
      (bind _jsonobject_5 (`self.MakeFloatParam` "CellSize" "Cell Size" "" (`/Game/QuietRuntimeEditor/Common/Features/QuietScatter/BP_QuietScatter.CellSize` (`local.ScatterActor`)) 10.0 1.0 1.0 1000.0 500.0 1 3 true))
      (`KismetArrayLibrary.Array_Add` (`local.Spawn`) _jsonobject_5)
      (bind _jsonobject_6 (`self.MakeBoolParam` "IgnoreCollisions" "Ignore Collisions" "" (`/Game/QuietRuntimeEditor/Common/Features/QuietScatter/BP_QuietScatter.IgnoreCollisions` (`local.ScatterActor`))))
      (`KismetArrayLibrary.Array_Add` (`local.Spawn`) _jsonobject_6)
      (bind _jsonobject_7 (`self.MakeEnumParam` "Projection" "Projection" "" (`|MakeArray` "Plane" "Box" "Sphere" "Spline") (`KismetMathLibrary.Conv_ByteToInt` (cast `/Game/QuietRuntimeEditor/Common/Features/QuietScatter/Blueprints/EScatterProjection` _projection))))
      (`KismetArrayLibrary.Array_Add` (`local.Spawn`) _jsonobject_7)
      (switch `/Game/QuietRuntimeEditor/Common/Features/QuietScatter/Blueprints/EScatterProjection` _projection
        (:`NewEnumerator0`
          (bind _jsonobject_8 (`self.MakeVectorParam` "BoxExtent" "Box Extent" "" (`/Game/QuietRuntimeEditor/Common/Features/QuietScatter/BP_QuietScatter.BoxExtent` (`local.ScatterActor`)) (300.0 300.0 200.0) :!label _label))
          (`KismetArrayLibrary.Array_Add` (`local.Spawn`) _jsonobject_8))
        (:`NewEnumerator1`
          (goto _label))
        (:`NewEnumerator2`
          (bind _jsonobject_9 (`self.MakeFloatParam` "Radius" "Sphere Radius" "" (`/Game/QuietRuntimeEditor/Common/Features/QuietScatter/BP_QuietScatter.Radius` (`local.ScatterActor`)) 500.0 0.0 0.0 1000000.0 5000.0 1 3))
          (`KismetArrayLibrary.Array_Add` (`local.Spawn`) _jsonobject_9))
        (:`NewEnumerator4`
          (bind _jsonobject_10 (`self.MakeFloatParam` "SplineWidth" "Spline Width" "" (`/Game/QuietRuntimeEditor/Common/Features/QuietScatter/BP_QuietScatter.SplineWidth` (`local.ScatterActor`)) 50.0 0.0 0.0 1000000.0 1000.0 1 3 true))
          (`KismetArrayLibrary.Array_Add` (`local.Spawn`) _jsonobject_10)))
      (bind _jsonobject_11 (`self.MakeFloatParam` "ProjectionFalloff" "Projection Falloff" "" (`/Game/QuietRuntimeEditor/Common/Features/QuietScatter/BP_QuietScatter.ProjectionFalloff` (`local.ScatterActor`)) 0.0 0.0 0.0 1.0 0.5 1 3 true))
      (`KismetArrayLibrary.Array_Add` (`local.Spawn`) _jsonobject_11)
      (bind _jsonobject_12 (`self.MakeEnumParam` "SurfaceCurvature" "Surface Curvature" "" (`|MakeArray` "None" "Concave" "Convex") (`KismetMathLibrary.Conv_ByteToInt` (`/Game/QuietRuntimeEditor/Common/Features/QuietScatter/BP_QuietScatter.Curvature` (`local.ScatterActor`)))))
      (`|SetJsonField` _jsonobject_12 "Enabled" false)
      (`KismetArrayLibrary.Array_Add` (`local.Spawn`) _jsonobject_12)
      (switch `/Game/QuietRuntimeEditor/Common/Features/QuietScatter/Blueprints/ESurfaceCurvatureProcessing` (`/Game/QuietRuntimeEditor/Common/Features/QuietScatter/BP_QuietScatter.Curvature` (`local.ScatterActor`))
        (:`NewEnumerator1`
          _)
        (:`NewEnumerator2`
          _))
      (bind _jsonobject_13 (`self.MakeFloatParam` "CurvatureSpreading" "Curvature Spreading" "" (`/Game/QuietRuntimeEditor/Common/Features/QuietScatter/BP_QuietScatter.CurvatureSpreading` (`local.ScatterActor`)) 50.0 1.0 1.0 1000000.0 1000.0 1 3 true))
      (`KismetArrayLibrary.Array_Add` (`local.Spawn`) _jsonobject_13))
    (:`then_2`
      (`|SetJsonField` (`local.TargetJson`) "GroupsState" (`|MakeArray` "Brush" "Spawn" "Scatter" "Meshes"))
      (`|SetJsonField` (`local.TargetJson`) "Brush" (`local.Brush`))
      (`|SetJsonField` (`local.TargetJson`) "Scatter" (`local.Spawn`))
      (bind _group (`self.MakeMeshesGroup` (`local.ScatterActor`)))
      (`|SetJsonField` (`local.TargetJson`) "Meshes" _group)
      (bind _commonparams (`self.CollectCommonProps` (`/Game/QuietRuntimeEditor/Common/Features/QuietScatter/BP_QuietScatter.ComplexMesh` (`local.ScatterActor`))))
      (`|SetJsonField` (`local.TargetJson`) "Common Mesh Settings" _commonparams)
      (`parent.CollectProperties` (`local.ScatterActor`) (`local.TargetJson`))
      (return))))

(fn `GetPropertyValue`
  (params (Object :type "Object Object Reference") (Property :type String))
  (returns (Success :type Boolean) (Value :type "JsonObjectWrapper Structure"))
  (locals (TargetJson :type "JsonObjectWrapper Structure"))
  (bind _targetjson (`local.TargetJson`))
  (bind _property (`local.Property`))
  (bind (_success _value) (`parent.GetPropertyValue` Object Property))
  (if (not _success)
    (bind _asquiet_scatter (cast `/Game/QuietRuntimeEditor/Common/Features/QuietScatter/BP_QuietScatter` Object))
    (bind _jsonobject (`/Game/QuietRuntimeEditor/Common/Blueprints/BP_QuietJsonFunctionLibrary.NewJson`))
    (set `local.TargetJson` _jsonobject)
    (switch `string` _property
      (:`BrushMode`
        (`|SetJsonField` _targetjson _property (`/Game/QuietRuntimeEditor/Common/Features/QuietScatter/BP_QuietScatter.BrushMode` _asquiet_scatter)))
      (:`BrushSize`
        (`|SetJsonField` _targetjson _property (`/Game/QuietRuntimeEditor/Common/Features/QuietScatter/BP_QuietScatter.BrushSize` _asquiet_scatter)))
      (:`BrushColor`
        (`|SetJsonField` _targetjson _property (`/Game/QuietRuntimeEditor/Common/Features/QuietScatter/BP_QuietScatter.BrushColor` _asquiet_scatter)))
      (:`FillCount`
        (`|SetJsonField` _targetjson _property (`/Game/QuietRuntimeEditor/Common/Features/QuietScatter/BP_QuietScatter.FillCount` _asquiet_scatter)))
      (:`CellSize`
        (`|SetJsonField` _targetjson _property (`/Game/QuietRuntimeEditor/Common/Features/QuietScatter/BP_QuietScatter.CellSize` _asquiet_scatter)))
      (:`IgnoreCollisions`
        (`|SetJsonField` _targetjson _property (`/Game/QuietRuntimeEditor/Common/Features/QuietScatter/BP_QuietScatter.IgnoreCollisions` _asquiet_scatter)))
      (:`Projection`
        (`|SetJsonField` _targetjson _property (`/Game/QuietRuntimeEditor/Common/Features/QuietScatter/BP_QuietScatter.GetProjectionMode` _asquiet_scatter)))
      (:`BoxExtent`
        (`|SetJsonField` _targetjson _property (`/Game/QuietRuntimeEditor/Common/Features/QuietScatter/BP_QuietScatter.BoxExtent` _asquiet_scatter)))
      (:`Radius`
        (`|SetJsonField` _targetjson _property (`/Game/QuietRuntimeEditor/Common/Features/QuietScatter/BP_QuietScatter.Radius` _asquiet_scatter)))
      (:`SplineWidth`
        (`|SetJsonField` _targetjson _property (`/Game/QuietRuntimeEditor/Common/Features/QuietScatter/BP_QuietScatter.SplineWidth` _asquiet_scatter)))
      (:`ProjectionFalloff`
        (`|SetJsonField` _targetjson _property (`/Game/QuietRuntimeEditor/Common/Features/QuietScatter/BP_QuietScatter.ProjectionFalloff` _asquiet_scatter)))
      (:`SurfaceCurvature`
        (`|SetJsonField` _targetjson _property (`/Game/QuietRuntimeEditor/Common/Features/QuietScatter/BP_QuietScatter.Curvature` _asquiet_scatter)))
      (:`CurvatureSpreading`
        (`|SetJsonField` _targetjson _property (`/Game/QuietRuntimeEditor/Common/Features/QuietScatter/BP_QuietScatter.CurvatureSpreading` _asquiet_scatter))))
    (return true (`local.TargetJson`))
    (else
      (return true _value))))

(fn `MakeMeshElement`
  (params (Component :type "/Game/QuietRuntimeEditor/Common/Features/QuietScatter/Blueprints/BP_ScatterMeshComponent Object Reference") (Index :type Integer))
  (returns (Element :type "JsonObjectWrapper Structure"))
  (locals (Comp :type "Array of JsonObjectWrapper Structure") (Params :type "Array of JsonObjectWrapper Structure"))
  (bind _returnvalue (`KismetStringLibrary.Conv_IntToString` Index))
  (bind _jsonobject (`/Game/QuietRuntimeEditor/Common/Blueprints/BP_QuietJsonFunctionLibrary.NewJson`))
  (message `/Game/QuietRuntimeEditor/Serialization/BI_SerializerInterface.GrabDetails` (`self.GetSource`) Component _jsonobject)
  (bind _outvalue (`|GetJsonField` _jsonobject "Component"))
  (for _array_element _outvalue
    (`|SetJsonField` _array_element "Component" _returnvalue))
  (bind _jsonobject_2 (`self.MakeParamSubgroup` (`KismetStringLibrary.Concat_StrStr` "Mesh [ " _returnvalue " ]") _outvalue))
  (if (> Index 0)
    (`|SetJsonField` _jsonobject_2 "Class" "Mesh"))
  (return _jsonobject_2))

(fn `MakeMeshesGroup`
  (params (Scatter :type "/Game/QuietRuntimeEditor/Common/Features/QuietScatter/BP_QuietScatter Object Reference"))
  (returns (Group :type "Array of JsonObjectWrapper Structure"))
  (locals (Array :type "Array of JsonObjectWrapper Structure"))
  (bind _param (`self.MakeActionsParam` (`|MakeArray` "Add New Mesh" "Clear Secondary Meshes")))
  (`KismetArrayLibrary.Array_Add` (`local.Array`) _param)
  (bind _element (`self.MakeMeshElement` (`/Game/QuietRuntimeEditor/Common/Features/QuietScatter/BP_QuietScatter.ComplexMesh` Scatter)))
  (`KismetArrayLibrary.Array_Add` (`local.Array`) _element)
  (for (_array_element _array_index) (`/Game/QuietRuntimeEditor/Common/Features/QuietScatter/BP_QuietScatter.GetSecondaryMeshes` Scatter)
    (bind _element_2 (`self.MakeMeshElement` _array_element (+ _array_index 1)))
    (`KismetArrayLibrary.Array_Add` (`local.Array`) _element_2))
  (return (`local.Array`)))

(fn `RestoreObject`
  (params (Object :type "Object Object Reference") (JsonObject :type "JsonObjectWrapper Structure"))
  (`parent.RestoreObject` Object JsonObject)
  (bind _asquiet_scatter (cast `/Game/QuietRuntimeEditor/Common/Features/QuietScatter/BP_QuietScatter` Object))
  (bind _outvalue (`|GetJsonField` (`local.JsonObject`) "Root"))
  (message `/Game/QuietRuntimeEditor/Serialization/BI_SerializerInterface.RestoreObject` (`self.GetSource`) (`Actor.RootComponent` _asquiet_scatter) _outvalue)
  (bind _outvalue_2 (`|GetJsonField` (`local.JsonObject`) "Secondary"))
  (for _array_element _outvalue_2
    (bind _component (`/Game/QuietRuntimeEditor/Common/Features/QuietScatter/BP_QuietScatter.Add Secondary Mesh` _asquiet_scatter false))
    (message `/Game/QuietRuntimeEditor/Serialization/BI_SerializerInterface.RestoreObject` (`self.GetSource`) _component _array_element)))

(fn `SerializeObject`
  (params (Object :type "Object Object Reference") (TargetJson :type "JsonObjectWrapper Structure (by ref)"))
  (locals (Actor :type "/Game/QuietRuntimeEditor/Common/Features/QuietScatter/BP_QuietScatter Object Reference") (Secondary :type "Array of JsonObjectWrapper Structure"))
  (`parent.SerializeObject` Object TargetJson)
  (bind _asquiet_scatter (cast `/Game/QuietRuntimeEditor/Common/Features/QuietScatter/BP_QuietScatter` Object))
  (set `local.Actor` _asquiet_scatter)
  (`|ExecutionSequence`
    (:`then_0`
      (`|SetJsonField` (`local.TargetJson`) "BrushMode" (`/Game/QuietRuntimeEditor/Common/Features/QuietScatter/BP_QuietScatter.GetBrushModeIndex` (`local.Actor`)))
      (`|SetJsonField` (`local.TargetJson`) "BrushSize" (`/Game/QuietRuntimeEditor/Common/Features/QuietScatter/BP_QuietScatter.BrushSize` (`local.Actor`)))
      (`|SetJsonField` (`local.TargetJson`) "BrushColor" (`/Game/QuietRuntimeEditor/Common/Features/QuietScatter/BP_QuietScatter.BrushColor` (`local.Actor`)))
      (`|SetJsonField` (`local.TargetJson`) "FillCount" (`/Game/QuietRuntimeEditor/Common/Features/QuietScatter/BP_QuietScatter.FillCount` (`local.Actor`)))
      (`|SetJsonField` (`local.TargetJson`) "CellSize" (`/Game/QuietRuntimeEditor/Common/Features/QuietScatter/BP_QuietScatter.CellSize` (`local.Actor`)))
      (`|SetJsonField` (`local.TargetJson`) "IgnoreCollisions" (`/Game/QuietRuntimeEditor/Common/Features/QuietScatter/BP_QuietScatter.IgnoreCollisions` (`local.Actor`)))
      (`|SetJsonField` (`local.TargetJson`) "Projection" (`KismetMathLibrary.Conv_ByteToInt` (`/Game/QuietRuntimeEditor/Common/Features/QuietScatter/BP_QuietScatter.GetProjectionMode` (`local.Actor`))))
      (`|SetJsonField` (`local.TargetJson`) "BoxExtent" (`/Game/QuietRuntimeEditor/Common/Features/QuietScatter/BP_QuietScatter.BoxExtent` (`local.Actor`)))
      (`|SetJsonField` (`local.TargetJson`) "Radius" (`/Game/QuietRuntimeEditor/Common/Features/QuietScatter/BP_QuietScatter.Radius` (`local.Actor`)))
      (`|SetJsonField` (`local.TargetJson`) "SplineWidth" (`/Game/QuietRuntimeEditor/Common/Features/QuietScatter/BP_QuietScatter.SplineWidth` (`local.Actor`)))
      (`|SetJsonField` (`local.TargetJson`) "ProjectionFalloff" (`/Game/QuietRuntimeEditor/Common/Features/QuietScatter/BP_QuietScatter.ProjectionFalloff` (`local.Actor`)))
      (`|SetJsonField` (`local.TargetJson`) "SurfaceCurvature" (`KismetMathLibrary.Conv_ByteToInt` (`/Game/QuietRuntimeEditor/Common/Features/QuietScatter/BP_QuietScatter.Curvature` (`local.Actor`))))
      (`|SetJsonField` (`local.TargetJson`) "CurvatureSpreading" (`/Game/QuietRuntimeEditor/Common/Features/QuietScatter/BP_QuietScatter.CurvatureSpreading` (`local.Actor`))))
    (:`then_1`
      ;[0 0 0] Meshes
      (bind _cache (message `/Game/QuietRuntimeEditor/Serialization/BI_SerializerInterface.CacheObject` (`self.GetSource`) (`/Game/QuietRuntimeEditor/Common/Features/QuietScatter/BP_QuietScatter.ComplexMesh` (`local.Actor`))))
      (`|SetJsonField` (`local.TargetJson`) "Root" _cache)
      (for _array_element (`/Game/QuietRuntimeEditor/Common/Features/QuietScatter/BP_QuietScatter.GetSecondaryMeshes` (`local.Actor`))
        (bind _cache_2 (message `/Game/QuietRuntimeEditor/Serialization/BI_SerializerInterface.CacheObject` (`self.GetSource`) _array_element))
        (`KismetArrayLibrary.Array_Add` (`local.Secondary`) _cache_2))
      (`|SetJsonField` (`local.TargetJson`) "Secondary" (`local.Secondary`))
      (return))))

(fn `Set Common Mesh Param`
  (params (Scatter :type "/Game/QuietRuntimeEditor/Common/Features/QuietScatter/BP_QuietScatter Object Reference") (Property :type String) (JsonValue :type "JsonObjectWrapper Structure"))
  (returns (Success :type Boolean))
  (bind _success (message `/Game/QuietRuntimeEditor/Serialization/BI_SerializerInterface.SetValueByName` (`self.GetSource`) (`/Game/QuietRuntimeEditor/Common/Features/QuietScatter/BP_QuietScatter.ComplexMesh` Scatter) Property JsonValue))
  (if _success
    (for _array_element (`/Game/QuietRuntimeEditor/Common/Features/QuietScatter/BP_QuietScatter.GetSecondaryMeshes` Scatter)
      (message `/Game/QuietRuntimeEditor/Serialization/BI_SerializerInterface.SetValueByName` (`self.GetSource`) _array_element Property JsonValue))
    (return true)
    (else
      (return false))))

(fn `SetPropertyValue`
  (params (Object :type "Object Object Reference") (Property :type String) (JsonValue :type "JsonObjectWrapper Structure (by ref)"))
  (returns (Success :type Boolean))
  (locals (Scatter :type "/Game/QuietRuntimeEditor/Common/Features/QuietScatter/BP_QuietScatter Object Reference"))
  (bind _property (`local.Property`))
  (bind _jsonvalue (`local.JsonValue`))
  (bind _scatter (`local.Scatter`))
  (bind _scatter_2 (`local.Scatter`))
  (bind (_lefts _rights) (`KismetStringLibrary.Split` (`local.Property`) "."))
  (bind _success (`parent.SetPropertyValue` Object Property JsonValue))
  (if (not _success)
    (bind _asquiet_scatter (cast `/Game/QuietRuntimeEditor/Common/Features/QuietScatter/BP_QuietScatter` Object))
    (set `local.Scatter` _asquiet_scatter)
    (if (not (`KismetStringLibrary.Contains` (`local.Property`) "."))
      (switch `string` _property
        (:`Default`
          (bind _success_2 (`self.Set Common Mesh Param` (`local.Scatter`) (`local.Property`) (`local.JsonValue`)))
          (return _success_2))
        (:`BrushMode`
          (bind _newvalue (`/Game/QuietRuntimeEditor/Common/Blueprints/BP_QuietJsonMacroLibrary.ReadIntegerWithCheck` _jsonvalue _property (`/Game/QuietRuntimeEditor/Common/Features/QuietScatter/BP_QuietScatter.GetBrushModeIndex` _scatter_2))
            (:`then`
              (`/Game/QuietRuntimeEditor/Common/Features/QuietScatter/BP_QuietScatter.SetBrushMode` (`local.Scatter`) _newvalue))))
        (:`BrushSize`
          (bind _newvalue_2 (`/Game/QuietRuntimeEditor/Common/Blueprints/BP_QuietJsonMacroLibrary.ReadFloatWithCheck` _jsonvalue _property (`/Game/QuietRuntimeEditor/Common/Features/QuietScatter/BP_QuietScatter.BrushSize` _scatter_2))
            (:`then`
              (`/Game/QuietRuntimeEditor/Common/Features/QuietScatter/BP_QuietScatter.SetBrushSize` (`local.Scatter`) _newvalue_2))))
        (:`BrushColor`
          (bind _newvalue_3 (`/Game/QuietRuntimeEditor/Common/Blueprints/BP_QuietJsonMacroLibrary.ReadLinearColorWithCheck` _jsonvalue _property (`/Game/QuietRuntimeEditor/Common/Features/QuietScatter/BP_QuietScatter.BrushColor` _scatter_2))
            (:`then`
              (`/Game/QuietRuntimeEditor/Common/Features/QuietScatter/BP_QuietScatter.SetBrushColor` (`local.Scatter`) _newvalue_3))))
        (:`FillCount`
          (bind _newvalue_4 (`/Game/QuietRuntimeEditor/Common/Blueprints/BP_QuietJsonMacroLibrary.ReadIntegerWithCheck` _jsonvalue _property (`/Game/QuietRuntimeEditor/Common/Features/QuietScatter/BP_QuietScatter.FillCount` _scatter_2))
            (:`then`
              (set `/Game/QuietRuntimeEditor/Common/Features/QuietScatter/BP_QuietScatter.FillCount` _newvalue_4 (`local.Scatter`)))))
        (:`CellSize`
          (bind _newvalue_5 (`/Game/QuietRuntimeEditor/Common/Blueprints/BP_QuietJsonMacroLibrary.ReadFloatWithCheck` _jsonvalue _property (`/Game/QuietRuntimeEditor/Common/Features/QuietScatter/BP_QuietScatter.CellSize` _scatter_2))
            (:`then`
              (set `/Game/QuietRuntimeEditor/Common/Features/QuietScatter/BP_QuietScatter.CellSize` _newvalue_5 (`local.Scatter`)))))
        (:`IgnoreCollisions`
          (bind _newvalue_6 (`/Game/QuietRuntimeEditor/Common/Blueprints/BP_QuietJsonMacroLibrary.ReadBoolWithCheck` _jsonvalue _property (`/Game/QuietRuntimeEditor/Common/Features/QuietScatter/BP_QuietScatter.IgnoreCollisions` _scatter_2))
            (:`then`
              (set `/Game/QuietRuntimeEditor/Common/Features/QuietScatter/BP_QuietScatter.IgnoreCollisions` _newvalue_6 _scatter))))
        (:`Projection`
          (bind _newvalue_7 (`/Game/QuietRuntimeEditor/Common/Blueprints/BP_QuietJsonMacroLibrary.ReadEnumWithCheck` _jsonvalue _property (`/Game/QuietRuntimeEditor/Common/Features/QuietScatter/BP_QuietScatter.GetProjectionMode` _scatter_2))
            (:`then`
              (`/Game/QuietRuntimeEditor/Common/Features/QuietScatter/BP_QuietScatter.SetProjectionMode` _scatter (cast `/Game/QuietRuntimeEditor/Common/Features/QuietScatter/Blueprints/EScatterProjection` _newvalue_7)))))
        (:`BoxExtent`
          (bind _newvalue_8 (`/Game/QuietRuntimeEditor/Common/Blueprints/BP_QuietJsonMacroLibrary.ReadVectorWithCheck` _jsonvalue _property (`/Game/QuietRuntimeEditor/Common/Features/QuietScatter/BP_QuietScatter.BoxExtent` _scatter_2))
            (:`then`
              (set `/Game/QuietRuntimeEditor/Common/Features/QuietScatter/BP_QuietScatter.BoxExtent` _newvalue_8 (`local.Scatter`))
              (`/Game/QuietRuntimeEditor/Common/Features/QuietScatter/BP_QuietScatter.UpdateBounds` (`local.Scatter`))
              (return true))))
        (:`Radius`
          (bind _newvalue_9 (`/Game/QuietRuntimeEditor/Common/Blueprints/BP_QuietJsonMacroLibrary.ReadFloatWithCheck` _jsonvalue _property (`/Game/QuietRuntimeEditor/Common/Features/QuietScatter/BP_QuietScatter.Radius` _scatter_2))
            (:`then`
              (set `/Game/QuietRuntimeEditor/Common/Features/QuietScatter/BP_QuietScatter.Radius` _newvalue_9 (`local.Scatter`))
              (`/Game/QuietRuntimeEditor/Common/Features/QuietScatter/BP_QuietScatter.UpdateBounds` (`local.Scatter`))
              (return true))))
        (:`SplineWidth`
          (bind _newvalue_10 (`/Game/QuietRuntimeEditor/Common/Blueprints/BP_QuietJsonMacroLibrary.ReadFloatWithCheck` _jsonvalue _property (`/Game/QuietRuntimeEditor/Common/Features/QuietScatter/BP_QuietScatter.SplineWidth` _scatter_2))
            (:`then`
              (set `/Game/QuietRuntimeEditor/Common/Features/QuietScatter/BP_QuietScatter.SplineWidth` _newvalue_10 (`local.Scatter`))
              (return true))))
        (:`ProjectionFalloff`
          (bind _newvalue_11 (`/Game/QuietRuntimeEditor/Common/Blueprints/BP_QuietJsonMacroLibrary.ReadFloatWithCheck` _jsonvalue _property (`/Game/QuietRuntimeEditor/Common/Features/QuietScatter/BP_QuietScatter.ProjectionFalloff` _scatter_2))
            (:`then`
              (set `/Game/QuietRuntimeEditor/Common/Features/QuietScatter/BP_QuietScatter.ProjectionFalloff` _newvalue_11 (`local.Scatter`))
              (return true))))
        (:`SurfaceCurvature`
          (bind _newvalue_12 (`/Game/QuietRuntimeEditor/Common/Blueprints/BP_QuietJsonMacroLibrary.ReadEnumWithCheck` _jsonvalue _property (`/Game/QuietRuntimeEditor/Common/Features/QuietScatter/BP_QuietScatter.Curvature` _scatter_2))
            (:`then`
              (set `/Game/QuietRuntimeEditor/Common/Features/QuietScatter/BP_QuietScatter.Curvature` (cast `/Game/QuietRuntimeEditor/Common/Features/QuietScatter/Blueprints/ESurfaceCurvatureProcessing` _newvalue_12) (`local.Scatter`))
              (return true))))
        (:`CurvatureSpreading`
          (bind _newvalue_13 (`/Game/QuietRuntimeEditor/Common/Blueprints/BP_QuietJsonMacroLibrary.ReadFloatWithCheck` _jsonvalue _property (`/Game/QuietRuntimeEditor/Common/Features/QuietScatter/BP_QuietScatter.CurvatureSpreading` _scatter_2))
            (:`then`
              (set `/Game/QuietRuntimeEditor/Common/Features/QuietScatter/BP_QuietScatter.CurvatureSpreading` _newvalue_13 (`local.Scatter`))
              (return true)))))
      (return true)
      (else
        ;[0 0 0] Secondary Mesh Property
        (bind _pinned (`/Game/QuietRuntimeEditor/Common/Blueprints/BP_QuietJsonMacroLibrary.Pin` _lefts)) ; Property
        (bind _pinned_2 (`/Game/QuietRuntimeEditor/Common/Blueprints/BP_QuietJsonMacroLibrary.Pin` (`KismetStringLibrary.Conv_StringToInt` _rights))) ; Index
        (bind _component (`/Game/QuietRuntimeEditor/Common/Features/QuietScatter/BP_QuietScatter.GetMeshComponent` (`local.Scatter`) _pinned_2))
        (bind _success_3 (message `/Game/QuietRuntimeEditor/Serialization/BI_SerializerInterface.SetValueByName` (`self.GetSource`) _component _pinned (`local.JsonValue`)))
        (if _success_3
          (if (== _pinned "Weight")
            (`/Game/QuietRuntimeEditor/Common/Features/QuietScatter/BP_QuietScatter.WeightMeshes` (`local.Scatter`)))
          (return true))))
    (else
      (return true))))