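; Marshal Blueprint in the Quiet Runtime Editor that saves and restores Instanced Static Mesh Components as JSON.
; Saving runs the parent serialization, then writes every instance's local-space transform to an "Instances" array field.
; Restoring runs the parent restore, clears existing instances and re-adds each saved transform in local space.
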(fn `RestoreObject`
  (params (Object :type "Object Object Reference") (JsonObject :type "JsonObjectWrapper Structure"))
  (`parent.RestoreObject` Object JsonObject)
  (bind _asinstanced_static_mesh_component (cast `InstancedStaticMeshComponent` Object))
  (`InstancedStaticMeshComponent.ClearInstances` _asinstanced_static_mesh_component)
  (bind _outvalue (`|GetJsonField` JsonObject "Instances"))
  (for _array_element _outvalue
    (`InstancedStaticMeshComponent.AddInstance` _asinstanced_static_mesh_component _array_element false)))

(fn `SerializeObject`
  (params (Object :type "Object Object Reference") (TargetJson :type "JsonObjectWrapper Structure (by ref)"))
  (locals (Instances :type "Array of Transform Structure"))
  (`parent.SerializeObject` Object TargetJson)
  (bind _asinstanced_static_mesh_component (cast `InstancedStaticMeshComponent` Object))
  (for _index (range (`InstancedStaticMeshComponent.GetInstanceCount` _asinstanced_static_mesh_component))
    (`KismetArrayLibrary.Array_Add` (`local.Instances`) (`InstancedStaticMeshComponent.GetInstanceTransform` _asinstanced_static_mesh_component _index false)))
  (`|SetJsonField` (`local.TargetJson`) "Instances" (`local.Instances`))
  (return))