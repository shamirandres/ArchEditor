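; Marshal for StaticMeshComponent in the runtime editor, converting mesh, materials and reverse culling to and from JSON.
; Property get/set tries the parent marshal first; setting a mesh applies its default slot materials, while material arrays serialize and restore through the source's cache messages.
; CollectProperties builds grouped editor parameters with one entry per material slot, omitting mesh selection for Datasmith runtime actors.
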(fn `Collect Mesh Materials`
  (params (Component :type "StaticMeshComponent Object Reference"))
  (returns (Params :type "Array of JsonObjectWrapper Structure"))
  (locals (Parameters :type "Array of JsonObjectWrapper Structure"))
  (bind _staticmesh (`StaticMeshComponent.StaticMesh` Component))
  (for (_array_element _array_index) (`MeshComponent.GetMaterials` Component)
    (bind _returnvalue (`KismetStringLibrary.Conv_NameToString` (`|GetArrayItem` (`MeshComponent.GetMaterialSlotNames` Component) _array_index)))
    (bind _jsonobject (`self.MakeObjectParam` (`KismetStringLibrary.Concat_StrStr` (`KismetMathLibrary.SelectString` "Root" (`KismetSystemLibrary.GetDisplayName` Component) (== Component (`Actor.RootComponent` (`self.GetOwner` Component)))) "." _returnvalue) _returnvalue "" "/Script/Engine.MaterialInstanceConstant" _array_element (`KismetMathLibrary.SelectObject` "/Engine/EngineMaterials/WorldGridMaterial.WorldGridMaterial" (`StaticMesh.GetMaterial` _staticmesh _array_index) (`KismetSystemLibrary.IsValid` _staticmesh))))
    (`KismetArrayLibrary.Array_Add` (`local.Parameters`) _jsonobject))
  (return (`local.Parameters`)))

(fn `CollectProperties`
  (params (Object :type "Object Object Reference") (TargetJson :type "JsonObjectWrapper Structure (by ref)"))
  (locals (MeshGroup :type "Array of JsonObjectWrapper Structure"))
  (bind _asstatic_mesh_component (cast `StaticMeshComponent` Object))
  (`|SetJsonField` TargetJson "GroupsState" (`|MakeArray` "Static Mesh" "Materials" "Actor"))
  (if (not (`Actor.ActorHasTag` (`self.GetOwner` _asstatic_mesh_component) "Datasmith.Runtime.Tag"))
    (bind _jsonobject (`self.MakeObjectParam` "StaticMesh" "Static Mesh" "" "/Script/Engine.StaticMesh" (`StaticMeshComponent.StaticMesh` _asstatic_mesh_component)))
    (`|SetJsonField` _jsonobject "Dependencies" (`|MakeArray`))
    (`KismetArrayLibrary.Array_Add` (`local.MeshGroup`) _jsonobject))
  (bind _jsonobject_2 (`self.MakeBoolParam` "ReverseCulling" "Reverse Culling" "" (`StaticMeshComponent.bReverseCulling` _asstatic_mesh_component)))
  (`KismetArrayLibrary.Array_Add` (`local.MeshGroup`) _jsonobject_2)
  (`|SetJsonField` TargetJson "Static Mesh" (`local.MeshGroup`))
  (bind _params (`self.Collect Mesh Materials` _asstatic_mesh_component))
  (`|SetJsonField` TargetJson "Materials" _params)
  (`parent.CollectProperties` _asstatic_mesh_component TargetJson)
  (return))

(fn `GetPropertyValue`
  (params (Object :type "Object Object Reference") (Property :type String))
  (returns (Success :type Boolean) (Value :type "JsonObjectWrapper Structure"))
  (bind (_success _value) (`parent.GetPropertyValue` Object Property))
  (if (not _success)
    (bind _asstatic_mesh_component (cast `StaticMeshComponent` Object))
    (bind _outjsonobject (`JsonBlueprintFunctionLibrary.FromString` "{ }"))
    (switch `string` (`local.Property`)
      (:`StaticMesh`
        (`|SetJsonField` _outjsonobject (`local.Property`) (`StaticMeshComponent.StaticMesh` _asstatic_mesh_component))
        (return true _outjsonobject))
      (:`ReverseCulling`
        (bind _returnvalue (`|SetJsonField` _outjsonobject (`local.Property`) (`StaticMeshComponent.bReverseCulling` _asstatic_mesh_component)))
        (return _returnvalue _outjsonobject)))
    (else
      (return true _value))))

(fn `SerializeObject`
  (params (Object :type "Object Object Reference") (TargetJson :type "JsonObjectWrapper Structure (by ref)"))
  (`parent.SerializeObject` Object TargetJson)
  (bind _asstatic_mesh_component (cast `StaticMeshComponent` Object))
  (`|ExecutionSequence`
    (:`then_0`
      (`|SetJsonField` TargetJson "StaticMesh" (`StaticMeshComponent.StaticMesh` _asstatic_mesh_component))
      (bind _cache (message `/Game/QuietRuntimeEditor/Serialization/BI_SerializerInterface.CacheMatArray` (`self.GetSource`) (`MeshComponent.GetMaterials` _asstatic_mesh_component)))
      (`|SetJsonField` TargetJson "Materials" _cache))
    (:`then_1`
      (`|SetJsonField` TargetJson "ReverseCulling" (`StaticMeshComponent.bReverseCulling` _asstatic_mesh_component))
      (return))))

(fn `SetPropertyValue`
  (params (Object :type "Object Object Reference") (Property :type String) (JsonValue :type "JsonObjectWrapper Structure (by ref)"))
  (returns (Success :type Boolean))
  (bind _success (`parent.SetPropertyValue` Object Property JsonValue))
  (if (not _success)
    (bind _asstatic_mesh_component (cast `StaticMeshComponent` Object))
    (switch `string` (`local.Property`)
      (:`StaticMesh`
        ;[0 0 0] Restore Mesh
        (bind (_newvalue _invaliddata) (`/Game/QuietRuntimeEditor/Common/Blueprints/BP_QuietJsonMacroLibrary.ReadMeshWithCheck` JsonValue (`local.Property`) (`StaticMeshComponent.StaticMesh` _asstatic_mesh_component))
          (:`then`
            (bind _returnvalue (`StaticMeshComponent.SetStaticMesh` _asstatic_mesh_component _newvalue))
            (for _array_element (`StaticMesh.StaticMaterials` _newvalue)
              (bind (_materialinterface _materialslotname) (break `StaticMaterial` _array_element))
              (`PrimitiveComponent.SetMaterialByName` _asstatic_mesh_component _materialslotname _materialinterface))
            (return _returnvalue))
          (:`Null`
            _)
          (:`Failed`
            (`self.CheckInvalidData` _invaliddata)))
        (bind _returnvalue_2 (`StaticMeshComponent.SetStaticMesh` _asstatic_mesh_component null))
        (return _returnvalue_2))
      (:`ReverseCulling`
        (bind _newvalue_2 (`/Game/QuietRuntimeEditor/Common/Blueprints/BP_QuietJsonMacroLibrary.ReadBoolWithCheck` JsonValue (`local.Property`) (`StaticMeshComponent.bReverseCulling` _asstatic_mesh_component))
          (:`then`
            (`StaticMeshComponent.SetReverseCulling` _asstatic_mesh_component _newvalue_2)
            (return true))))
      (:`Materials`
        ;[0 0 0] Restore Materials
        (bind _outvalue (`|GetJsonField` JsonValue (`local.Property`)))
        (bind _materials (message `/Game/QuietRuntimeEditor/Serialization/BI_SerializerInterface.RestoreMatArray` (`self.GetSource`) _outvalue))
        (for (_array_element_2 _array_index) _materials
          (`/Engine/EditorBlueprintResources/StandardMacros.IsValid` _array_element_2
            (:`Is Valid`
              (`PrimitiveComponent.SetMaterial` _asstatic_mesh_component _array_index _array_element_2))))))
    (else
      (return true))))