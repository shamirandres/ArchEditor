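; Marshal that lets the runtime editor save, restore, inspect and edit BP_SunSky actors as JSON.
; It serializes orientation and sky settings, and hands the nested SUN object to the source for caching, restoring and unmatched property access.
; Setters write only changed values, then refresh the sky material, also updating orientation for angle changes.
; CollectProperties builds grouped editor parameters with class defaults, merging in the SUN's light detail groups.
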(fn `CollectProperties`
  (params (Object :type "Object Object Reference") (TargetJson :type "JsonObjectWrapper Structure (by ref)"))
  (locals (SkyParams :type "Array of JsonObjectWrapper Structure") (Override :type "Array of JsonObjectWrapper Structure") (Orientation :type "Array of JsonObjectWrapper Structure"))
  (bind _asbp_sun_sky (cast `/Game/QuietRuntimeEditor/Common/QuietActors/BP_SunSky` Object))
  (`|ExecutionSequence`
    (:`then_0`
      (bind (_skymaterial _refresh_material _colors_determined_by_sun_position _sunheight _sunbrightness _horizonfalloff _zenithcolor _horizoncolor _cloudcolor _overallcolor _cloudspeed _cloudopacity _starsbrightness _horizoncolorcurve _zenithcolorcurve _cloudcolorcurve _sunangle _azimuth) (defaults `Object` (`GameplayStatics.GetObjectClass` _asbp_sun_sky)))
      (bind _jsonobject (`self.MakeFloatParam` "SunAngle" "Sun Angle" "" (`/Game/QuietRuntimeEditor/Common/QuietActors/BP_SunSky.SunAngle` _asbp_sun_sky) _sunangle -360.0 -360.0 360.0 360.0 1 1))
      (`KismetArrayLibrary.Array_Add` (`local.Orientation`) _jsonobject)
      (bind _jsonobject_2 (`self.MakeFloatParam` "Azimuth" "Azimuth" "" (`/Game/QuietRuntimeEditor/Common/QuietActors/BP_SunSky.Azimuth` _asbp_sun_sky) _azimuth -360.0 -360.0 360.0 360.0 1 1))
      (`KismetArrayLibrary.Array_Add` (`local.Orientation`) _jsonobject_2))
    (:`then_1`
      (bind _jsonobject_3 (`self.MakeBoolParam` "ColorsDeterminedBySunPosition" "Colors Determined By Sun Position" "" (`/Game/QuietRuntimeEditor/Common/QuietActors/BP_SunSky.Colors determined by sun position` _asbp_sun_sky) _colors_determined_by_sun_position))
      (`KismetArrayLibrary.Array_Add` (`local.SkyParams`) _jsonobject_3)
      (bind _jsonobject_4 (`self.MakeFloatParam` "SunBrightness" "Sun Brightness" "" (`/Game/QuietRuntimeEditor/Common/QuietActors/BP_SunSky.SunBrightness` _asbp_sun_sky) _sunbrightness 0.0 0.0 1000.0 10000.0 1 2))
      (`KismetArrayLibrary.Array_Add` (`local.SkyParams`) _jsonobject_4)
      (bind _jsonobject_5 (`self.MakeFloatParam` "CloudSpeed" "Cloud Speed" "" (`/Game/QuietRuntimeEditor/Common/QuietActors/BP_SunSky.CloudSpeed` _asbp_sun_sky) _cloudspeed 0.0 0.0 0.0 0.0 1 3))
      (`KismetArrayLibrary.Array_Add` (`local.SkyParams`) _jsonobject_5)
      (bind _jsonobject_6 (`self.MakeFloatParam` "CloudOpacity" "Cloud Opacity" "" (`/Game/QuietRuntimeEditor/Common/QuietActors/BP_SunSky.CloudOpacity` _asbp_sun_sky) _cloudopacity 0.0 0.0 1.0 1.0 1 3))
      (`KismetArrayLibrary.Array_Add` (`local.SkyParams`) _jsonobject_6)
      (bind _jsonobject_7 (`self.MakeFloatParam` "StarsBrightness" "Stars Brightness" "" (`/Game/QuietRuntimeEditor/Common/QuietActors/BP_SunSky.StarsBrightness` _asbp_sun_sky) _starsbrightness 0.0 0.0 0.0 0.0 1 3))
      (`KismetArrayLibrary.Array_Add` (`local.SkyParams`) _jsonobject_7))
    (:`then_2`
      (bind _jsonobject_8 (`self.MakeFloatParam` "SunHeight" "Sun Height" "" (`/Game/QuietRuntimeEditor/Common/QuietActors/BP_SunSky.SunHeight` _asbp_sun_sky) _sunheight 0.0 0.0 1.0 1.0 1 3))
      (`KismetArrayLibrary.Array_Add` (`local.Override`) _jsonobject_8)
      (bind _jsonobject_9 (`self.MakeFloatParam` "HorizonFalloff" "Horizon Falloff" "" (`/Game/QuietRuntimeEditor/Common/QuietActors/BP_SunSky.HorizonFalloff` _asbp_sun_sky) _horizonfalloff 0.0 0.0 0.0 0.0 1 3))
      (`KismetArrayLibrary.Array_Add` (`local.Override`) _jsonobject_9)
      (bind _jsonobject_10 (`self.MakeLinearColorParam` "ZenithColor" "Zenith Color" "" (`/Game/QuietRuntimeEditor/Common/QuietActors/BP_SunSky.ZenithColor` _asbp_sun_sky) _zenithcolor))
      (`KismetArrayLibrary.Array_Add` (`local.Override`) _jsonobject_10)
      (bind _jsonobject_11 (`self.MakeLinearColorParam` "HorizonColor" "Horizon Color" "" (`/Game/QuietRuntimeEditor/Common/QuietActors/BP_SunSky.HorizonColor` _asbp_sun_sky) _horizoncolor))
      (`KismetArrayLibrary.Array_Add` (`local.Override`) _jsonobject_11)
      (bind _jsonobject_12 (`self.MakeLinearColorParam` "CloudColor" "Cloud Color" "" (`/Game/QuietRuntimeEditor/Common/QuietActors/BP_SunSky.CloudColor` _asbp_sun_sky) _cloudcolor))
      (`KismetArrayLibrary.Array_Add` (`local.Override`) _jsonobject_12)
      (bind _jsonobject_13 (`self.MakeLinearColorParam` "OverallColor" "Overall Color" "" (`/Game/QuietRuntimeEditor/Common/QuietActors/BP_SunSky.OverallColor` _asbp_sun_sky) _overallcolor))
      (`KismetArrayLibrary.Array_Add` (`local.Override`) _jsonobject_13))
    (:`then_3`
      (`|SetJsonField` TargetJson "GroupsState" (`|MakeArray` "Orientation" "Sun" "Sky Sphere"))
      (`|SetJsonField` TargetJson "Orientation" (`local.Orientation`))
      (bind _jsonobject_14 (`/Game/QuietRuntimeEditor/Common/Blueprints/BP_QuietJsonFunctionLibrary.NewJson`))
      (message `/Game/QuietRuntimeEditor/Serialization/BI_SerializerInterface.GrabDetails` (`self.GetSource`) (`/Game/QuietRuntimeEditor/Common/QuietActors/BP_SunSky.SUN` _asbp_sun_sky) _jsonobject_14)
      (bind _outvalue (`|GetJsonField` _jsonobject_14 "Light"))
      (`|SetJsonField` TargetJson "Sun" _outvalue)
      (bind _jsonobject_15 (`self.MakeParamSubgroup` "Override Settings" (`local.Override`)))
      (`KismetArrayLibrary.Array_Add` (`local.SkyParams`) _jsonobject_15)
      (`|SetJsonField` TargetJson "Sky Sphere" (`local.SkyParams`))
      (bind _outvalue_2 (`|GetJsonField` _jsonobject_14 "Ray Tracing"))
      (`|SetJsonField` TargetJson "Ray Tracing" _outvalue_2)
      (bind _outvalue_3 (`|GetJsonField` _jsonobject_14 "Light Shafts"))
      (`|SetJsonField` TargetJson "Light Shafts" _outvalue_3)
      (bind _outvalue_4 (`|GetJsonField` _jsonobject_14 "Cascaded Shadow Maps"))
      (`|SetJsonField` TargetJson "Cascaded Shadow Maps" _outvalue_4)
      (`parent.CollectProperties` Object TargetJson)
      (return))))

(fn `GetPropertyValue`
  (params (Object :type "Object Object Reference") (Property :type String))
  (returns (Success :type Boolean) (Value :type "JsonObjectWrapper Structure"))
  (bind (_success _value) (`parent.GetPropertyValue` Object Property))
  (if (not _success)
    (bind _outjsonobject (`JsonBlueprintFunctionLibrary.FromString` "{ }"))
    (bind _asbp_sun_sky (cast `/Game/QuietRuntimeEditor/Common/QuietActors/BP_SunSky` Object))
    (switch `string` Property
      (:`Default`
        (bind (_success_2 _boxedvalue) (message `/Game/QuietRuntimeEditor/Serialization/BI_SerializerInterface.GetValueByName` (`self.GetSource`) (`/Game/QuietRuntimeEditor/Common/QuietActors/BP_SunSky.SUN` _asbp_sun_sky) Property))
        (return _success_2 _boxedvalue))
      (:`SunAngle`
        (`|SetJsonField` _outjsonobject Property (`/Game/QuietRuntimeEditor/Common/QuietActors/BP_SunSky.SunAngle` _asbp_sun_sky))
        (return true _outjsonobject))
      (:`Azimuth`
        (`|SetJsonField` _outjsonobject Property (`/Game/QuietRuntimeEditor/Common/QuietActors/BP_SunSky.Azimuth` _asbp_sun_sky))
        (return true _outjsonobject))
      (:`ColorsDeterminedBySunPosition`
        (`|SetJsonField` _outjsonobject Property (`/Game/QuietRuntimeEditor/Common/QuietActors/BP_SunSky.Colors determined by sun position` _asbp_sun_sky))
        (return true _outjsonobject))
      (:`SunBrightness`
        (`|SetJsonField` _outjsonobject Property (`/Game/QuietRuntimeEditor/Common/QuietActors/BP_SunSky.SunBrightness` _asbp_sun_sky))
        (return true _outjsonobject))
      (:`CloudSpeed`
        (`|SetJsonField` _outjsonobject Property (`/Game/QuietRuntimeEditor/Common/QuietActors/BP_SunSky.CloudSpeed` _asbp_sun_sky))
        (return true _outjsonobject))
      (:`CloudOpacity`
        (`|SetJsonField` _outjsonobject Property (`/Game/QuietRuntimeEditor/Common/QuietActors/BP_SunSky.CloudOpacity` _asbp_sun_sky))
        (return true _outjsonobject))
      (:`StarsBrightness`
        (`|SetJsonField` _outjsonobject Property (`/Game/QuietRuntimeEditor/Common/QuietActors/BP_SunSky.StarsBrightness` _asbp_sun_sky))
        (return true _outjsonobject))
      (:`SunHeight`
        (`|SetJsonField` _outjsonobject Property (`/Game/QuietRuntimeEditor/Common/QuietActors/BP_SunSky.SunHeight` _asbp_sun_sky))
        (return true _outjsonobject))
      (:`HorizonFalloff`
        (`|SetJsonField` _outjsonobject Property (`/Game/QuietRuntimeEditor/Common/QuietActors/BP_SunSky.HorizonFalloff` _asbp_sun_sky))
        (return true _outjsonobject))
      (:`ZenithColor`
        (`|SetJsonField` _outjsonobject Property (`/Game/QuietRuntimeEditor/Common/QuietActors/BP_SunSky.ZenithColor` _asbp_sun_sky))
        (return true _outjsonobject))
      (:`HorizonColor`
        (`|SetJsonField` _outjsonobject Property (`/Game/QuietRuntimeEditor/Common/QuietActors/BP_SunSky.HorizonColor` _asbp_sun_sky))
        (return true _outjsonobject))
      (:`CloudColor`
        (`|SetJsonField` _outjsonobject Property (`/Game/QuietRuntimeEditor/Common/QuietActors/BP_SunSky.CloudColor` _asbp_sun_sky))
        (return true _outjsonobject))
      (:`OverallColor`
        (`|SetJsonField` _outjsonobject Property (`/Game/QuietRuntimeEditor/Common/QuietActors/BP_SunSky.OverallColor` _asbp_sun_sky))
        (return true _outjsonobject)))
    (else
      (return true _value))))

(fn `RestoreObject`
  (params (Object :type "Object Object Reference") (JsonObject :type "JsonObjectWrapper Structure"))
  (`parent.RestoreObject` Object JsonObject)
  (bind _returnvalue (`JsonBlueprintFunctionLibrary.HasField` JsonObject "Sun"))
  (if _returnvalue
    (bind _outvalue (`|GetJsonField` JsonObject "Sun"))
    (bind _asbp_sun_sky (cast `/Game/QuietRuntimeEditor/Common/QuietActors/BP_SunSky` Object))
    (message `/Game/QuietRuntimeEditor/Serialization/BI_SerializerInterface.RestoreObject` (`self.GetSource`) (`/Game/QuietRuntimeEditor/Common/QuietActors/BP_SunSky.SUN` _asbp_sun_sky) _outvalue)))

(fn `SerializeObject`
  (params (Object :type "Object Object Reference") (TargetJson :type "JsonObjectWrapper Structure (by ref)"))
  (`parent.SerializeObject` Object TargetJson)
  (bind _asbp_sun_sky (cast `/Game/QuietRuntimeEditor/Common/QuietActors/BP_SunSky` Object))
  (`|ExecutionSequence`
    (:`then_0`
      (bind _cache (message `/Game/QuietRuntimeEditor/Serialization/BI_SerializerInterface.CacheObject` (`self.GetSource`) (`/Game/QuietRuntimeEditor/Common/QuietActors/BP_SunSky.SUN` _asbp_sun_sky)))
      (`|SetJsonField` TargetJson "Sun" _cache))
    (:`then_1`
      (`|SetJsonField` TargetJson "ColorsDeterminedBySunPosition" (`/Game/QuietRuntimeEditor/Common/QuietActors/BP_SunSky.Colors determined by sun position` _asbp_sun_sky)))
    (:`then_2`
      (`|SetJsonField` TargetJson "SunBrightness" (`/Game/QuietRuntimeEditor/Common/QuietActors/BP_SunSky.SunBrightness` _asbp_sun_sky)))
    (:`then_3`
      (`|SetJsonField` TargetJson "CloudSpeed" (`/Game/QuietRuntimeEditor/Common/QuietActors/BP_SunSky.CloudSpeed` _asbp_sun_sky)))
    (:`then_4`
      (`|SetJsonField` TargetJson "CloudOpacity" (`/Game/QuietRuntimeEditor/Common/QuietActors/BP_SunSky.CloudOpacity` _asbp_sun_sky)))
    (:`then_5`
      (`|SetJsonField` TargetJson "StarsBrightness" (`/Game/QuietRuntimeEditor/Common/QuietActors/BP_SunSky.StarsBrightness` _asbp_sun_sky)))
    (:`then_6`
      (`|SetJsonField` TargetJson "SunHeight" (`/Game/QuietRuntimeEditor/Common/QuietActors/BP_SunSky.SunHeight` _asbp_sun_sky)))
    (:`then_7`
      (`|SetJsonField` TargetJson "HorizonFalloff" (`/Game/QuietRuntimeEditor/Common/QuietActors/BP_SunSky.HorizonFalloff` _asbp_sun_sky)))
    (:`then_8`
      (`|SetJsonField` TargetJson "ZenithColor" (`/Game/QuietRuntimeEditor/Common/QuietActors/BP_SunSky.ZenithColor` _asbp_sun_sky)))
    (:`then_9`
      (`|SetJsonField` TargetJson "HorizonColor" (`/Game/QuietRuntimeEditor/Common/QuietActors/BP_SunSky.HorizonColor` _asbp_sun_sky)))
    (:`then_10`
      (`|SetJsonField` TargetJson "CloudColor" (`/Game/QuietRuntimeEditor/Common/QuietActors/BP_SunSky.CloudColor` _asbp_sun_sky)))
    (:`then_11`
      (`|SetJsonField` TargetJson "OverallColor" (`/Game/QuietRuntimeEditor/Common/QuietActors/BP_SunSky.OverallColor` _asbp_sun_sky)))
    (:`then_12`
      (`|SetJsonField` TargetJson "SunAngle" (`/Game/QuietRuntimeEditor/Common/QuietActors/BP_SunSky.SunAngle` _asbp_sun_sky)))
    (:`then_13`
      (`|SetJsonField` TargetJson "Azimuth" (`/Game/QuietRuntimeEditor/Common/QuietActors/BP_SunSky.Azimuth` _asbp_sun_sky)))
    (:`then_14`
      (return))))

(fn `SetPropertyValue`
  (params (Object :type "Object Object Reference") (Property :type String) (JsonValue :type "JsonObjectWrapper Structure (by ref)"))
  (returns (Success :type Boolean))
  (`parent.SetPropertyValue` Object Property JsonValue)
  (bind _asbp_sun_sky (cast `/Game/QuietRuntimeEditor/Common/QuietActors/BP_SunSky` Object))
  (switch `string` Property
    (:`Default`
      (bind _success (message `/Game/QuietRuntimeEditor/Serialization/BI_SerializerInterface.SetValueByName` (`self.GetSource`) (`/Game/QuietRuntimeEditor/Common/QuietActors/BP_SunSky.SUN` _asbp_sun_sky) Property JsonValue))
      (return _success))
    (:`SunAngle`
      (bind _newvalue (`/Game/QuietRuntimeEditor/Common/Blueprints/BP_QuietJsonMacroLibrary.ReadFloatWithCheck` JsonValue Property (`/Game/QuietRuntimeEditor/Common/QuietActors/BP_SunSky.SunAngle` _asbp_sun_sky))
        (:`then`
          (set `/Game/QuietRuntimeEditor/Common/QuietActors/BP_SunSky.SunAngle` _newvalue _asbp_sun_sky)
          (`/Game/QuietRuntimeEditor/Common/QuietActors/BP_SunSky.UpdateOrientation` _asbp_sun_sky :!label _label)
          (`/Game/QuietRuntimeEditor/Common/QuietActors/BP_SunSky.RefreshMaterial` _asbp_sun_sky :!label _label_2)
          (return true))))
    (:`Azimuth`
      (bind _newvalue_2 (`/Game/QuietRuntimeEditor/Common/Blueprints/BP_QuietJsonMacroLibrary.ReadFloatWithCheck` JsonValue Property (`/Game/QuietRuntimeEditor/Common/QuietActors/BP_SunSky.Azimuth` _asbp_sun_sky))
        (:`then`
          (set `/Game/QuietRuntimeEditor/Common/QuietActors/BP_SunSky.Azimuth` _newvalue_2 _asbp_sun_sky)
          (goto _label))))
    (:`ColorsDeterminedBySunPosition`
      (bind _newvalue_3 (`/Game/QuietRuntimeEditor/Common/Blueprints/BP_QuietJsonMacroLibrary.ReadBoolWithCheck` JsonValue Property (`/Game/QuietRuntimeEditor/Common/QuietActors/BP_SunSky.Colors determined by sun position` _asbp_sun_sky))
        (:`then`
          (set `/Game/QuietRuntimeEditor/Common/QuietActors/BP_SunSky.Colors determined by sun position` _newvalue_3 _asbp_sun_sky)
          (goto _label_2))))
    (:`SunBrightness`
      (bind _newvalue_4 (`/Game/QuietRuntimeEditor/Common/Blueprints/BP_QuietJsonMacroLibrary.ReadFloatWithCheck` JsonValue Property (`/Game/QuietRuntimeEditor/Common/QuietActors/BP_SunSky.SunBrightness` _asbp_sun_sky))
        (:`then`
          (set `/Game/QuietRuntimeEditor/Common/QuietActors/BP_SunSky.SunBrightness` _newvalue_4 _asbp_sun_sky)
          (goto _label_2))))
    (:`CloudSpeed`
      (bind _newvalue_5 (`/Game/QuietRuntimeEditor/Common/Blueprints/BP_QuietJsonMacroLibrary.ReadFloatWithCheck` JsonValue Property (`/Game/QuietRuntimeEditor/Common/QuietActors/BP_SunSky.CloudSpeed` _asbp_sun_sky))
        (:`then`
          (set `/Game/QuietRuntimeEditor/Common/QuietActors/BP_SunSky.CloudSpeed` _newvalue_5 _asbp_sun_sky)
          (goto _label_2))))
    (:`CloudOpacity`
      (bind _newvalue_6 (`/Game/QuietRuntimeEditor/Common/Blueprints/BP_QuietJsonMacroLibrary.ReadFloatWithCheck` JsonValue Property (`/Game/QuietRuntimeEditor/Common/QuietActors/BP_SunSky.CloudOpacity` _asbp_sun_sky))
        (:`then`
          (set `/Game/QuietRuntimeEditor/Common/QuietActors/BP_SunSky.CloudOpacity` _newvalue_6 _asbp_sun_sky)
          (goto _label_2))))
    (:`StarsBrightness`
      (bind _newvalue_7 (`/Game/QuietRuntimeEditor/Common/Blueprints/BP_QuietJsonMacroLibrary.ReadFloatWithCheck` JsonValue Property (`/Game/QuietRuntimeEditor/Common/QuietActors/BP_SunSky.StarsBrightness` _asbp_sun_sky))
        (:`then`
          (set `/Game/QuietRuntimeEditor/Common/QuietActors/BP_SunSky.StarsBrightness` _newvalue_7 _asbp_sun_sky)
          (goto _label_2))))
    (:`SunHeight`
      (bind _newvalue_8 (`/Game/QuietRuntimeEditor/Common/Blueprints/BP_QuietJsonMacroLibrary.ReadFloatWithCheck` JsonValue Property (`/Game/QuietRuntimeEditor/Common/QuietActors/BP_SunSky.SunHeight` _asbp_sun_sky))
        (:`then`
          (set `/Game/QuietRuntimeEditor/Common/QuietActors/BP_SunSky.SunHeight` _newvalue_8 _asbp_sun_sky)
          (goto _label_2))))
    (:`HorizonFalloff`
      (bind _newvalue_9 (`/Game/QuietRuntimeEditor/Common/Blueprints/BP_QuietJsonMacroLibrary.ReadFloatWithCheck` JsonValue Property (`/Game/QuietRuntimeEditor/Common/QuietActors/BP_SunSky.HorizonFalloff` _asbp_sun_sky))
        (:`then`
          (set `/Game/QuietRuntimeEditor/Common/QuietActors/BP_SunSky.HorizonFalloff` _newvalue_9 _asbp_sun_sky)
          (goto _label_2))))
    (:`ZenithColor`
      (bind _outvalue (`|GetJsonField` JsonValue Property))
      (if (not (`KismetMathLibrary.LinearColor_IsNearEqual` _outvalue (`/Game/QuietRuntimeEditor/Common/QuietActors/BP_SunSky.ZenithColor` _asbp_sun_sky)))
        (set `/Game/QuietRuntimeEditor/Common/QuietActors/BP_SunSky.ZenithColor` _outvalue _asbp_sun_sky)
        (goto _label_2)))
    (:`HorizonColor`
      (bind _outvalue_2 (`|GetJsonField` JsonValue Property))
      (if (not (`KismetMathLibrary.LinearColor_IsNearEqual` _outvalue_2 (`/Game/QuietRuntimeEditor/Common/QuietActors/BP_SunSky.HorizonColor` _asbp_sun_sky)))
        (set `/Game/QuietRuntimeEditor/Common/QuietActors/BP_SunSky.HorizonColor` _outvalue_2 _asbp_sun_sky)
        (goto _label_2)))
    (:`CloudColor`
      (bind _outvalue_3 (`|GetJsonField` JsonValue Property))
      (if (not (`KismetMathLibrary.LinearColor_IsNearEqual` _outvalue_3 (`/Game/QuietRuntimeEditor/Common/QuietActors/BP_SunSky.CloudColor` _asbp_sun_sky)))
        (set `/Game/QuietRuntimeEditor/Common/QuietActors/BP_SunSky.CloudColor` _outvalue_3 _asbp_sun_sky)
        (goto _label_2)))
    (:`OverallColor`
      (bind _outvalue_4 (`|GetJsonField` JsonValue Property))
      (if (not (`KismetMathLibrary.LinearColor_IsNearEqual` _outvalue_4 (`/Game/QuietRuntimeEditor/Common/QuietActors/BP_SunSky.OverallColor` _asbp_sun_sky)))
        (set `/Game/QuietRuntimeEditor/Common/QuietActors/BP_SunSky.OverallColor` _outvalue_4 _asbp_sun_sky)
        (goto _label_2)))))