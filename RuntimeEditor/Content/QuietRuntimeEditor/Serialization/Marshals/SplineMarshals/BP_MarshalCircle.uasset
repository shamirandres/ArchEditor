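; Marshal that exposes BP_Circle spline objects to the runtime editor's property editing and JSON serialization.
; It adds Radius and point count as bounded, commit-only parameters in a Circle group and writes both during serialization.
; Property reads and writes go to the parent marshal first, with circle fields handled only when it does not.
; Setters use checked JSON reads against current values and refresh the circle after assigning.
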(fn `CollectProperties`
  (params (Object :type "Object Object Reference") (TargetJson :type "JsonObjectWrapper Structure (by ref)"))
  (locals (Circle :type "Array of JsonObjectWrapper Structure"))
  (bind _ascircleactor (cast `/Game/QuietRuntimeEditor/Common/Features/QuietSplineSystem/Blueprints/BP_Circle` Object))
  (bind (_radius _pointscount) (defaults `Object` (`GameplayStatics.GetObjectClass` _ascircleactor)))
  (bind _jsonobject (`self.MakeFloatParam` "Radius" "Radius" "" (`/Game/QuietRuntimeEditor/Common/Features/QuietSplineSystem/Blueprints/BP_Circle.Radius` _ascircleactor) _radius 0.01 0.1 10000.0 1000.0 1 2 true))
  (`KismetArrayLibrary.Array_Add` (`local.Circle`) _jsonobject)
  (bind _jsonobject_2 (`self.MakeIntParam` "PointsCount" "Points Count" "" (`/Game/QuietRuntimeEditor/Common/Features/QuietSplineSystem/Blueprints/BP_Circle.PointsCount` _ascircleactor) _pointscount 2 2 24 24 true))
  (`KismetArrayLibrary.Array_Add` (`local.Circle`) _jsonobject_2)
  (`|SetJsonField` (`local.TargetJson`) "GroupsState" (`|MakeArray` "Circle" "Spline"))
  (`|SetJsonField` (`local.TargetJson`) "Circle" (`local.Circle`))
  (`parent.CollectProperties` _ascircleactor (`local.TargetJson`))
  (return))

(fn `GetPropertyValue`
  (params (Object :type "Object Object Reference") (Property :type String))
  (returns (Success :type Boolean) (Value :type "JsonObjectWrapper Structure"))
  (bind _property (`local.Property`))
  (bind (_success _value) (`parent.GetPropertyValue` Object Property))
  (if (not _success)
    (bind _ascircleactor (cast `/Game/QuietRuntimeEditor/Common/Features/QuietSplineSystem/Blueprints/BP_Circle` Object))
    (bind _jsonobject (`/Game/QuietRuntimeEditor/Common/Blueprints/BP_QuietJsonFunctionLibrary.NewJson`))
    (switch `string` (`local.Property`)
      (:`Radius`
        (`|SetJsonField` _jsonobject _property (`/Game/QuietRuntimeEditor/Common/Features/QuietSplineSystem/Blueprints/BP_Circle.Radius` _ascircleactor)))
      (:`PointsCount`
        (`|SetJsonField` _jsonobject _property (`/Game/QuietRuntimeEditor/Common/Features/QuietSplineSystem/Blueprints/BP_Circle.PointsCount` _ascircleactor))))
    (return true _jsonobject)
    (else
      (return true _value))))

(fn `SerializeObject`
  (params (Object :type "Object Object Reference") (TargetJson :type "JsonObjectWrapper Structure (by ref)"))
  (`parent.SerializeObject` Object TargetJson)
  (bind _ascircleactor (cast `/Game/QuietRuntimeEditor/Common/Features/QuietSplineSystem/Blueprints/BP_Circle` Object))
  (`|SetJsonField` (`local.TargetJson`) "Radius" (`/Game/QuietRuntimeEditor/Common/Features/QuietSplineSystem/Blueprints/BP_Circle.Radius` _ascircleactor))
  (`|SetJsonField` (`local.TargetJson`) "PointsCount" (`/Game/QuietRuntimeEditor/Common/Features/QuietSplineSystem/Blueprints/BP_Circle.PointsCount` _ascircleactor))
  (return))

(fn `SetPropertyValue`
  (params (Object :type "Object Object Reference") (Property :type String) (JsonValue :type "JsonObjectWrapper Structure (by ref)"))
  (returns (Success :type Boolean))
  (bind _property (`local.Property`))
  (bind _jsonvalue (`local.JsonValue`))
  (bind _success (`parent.SetPropertyValue` Object Property JsonValue))
  (if (not _success)
    (bind _ascircleactor (cast `/Game/QuietRuntimeEditor/Common/Features/QuietSplineSystem/Blueprints/BP_Circle` Object))
    (switch `string` (`local.Property`)
      (:`Radius`
        (bind _newvalue (`/Game/QuietRuntimeEditor/Common/Blueprints/BP_QuietJsonMacroLibrary.ReadFloatWithCheck` _jsonvalue _property (`/Game/QuietRuntimeEditor/Common/Features/QuietSplineSystem/Blueprints/BP_Circle.Radius` _ascircleactor))
          (:`then`
            (set `/Game/QuietRuntimeEditor/Common/Features/QuietSplineSystem/Blueprints/BP_Circle.Radius` _newvalue _ascircleactor))))
      (:`PointsCount`
        (bind _newvalue_2 (`/Game/QuietRuntimeEditor/Common/Blueprints/BP_QuietJsonMacroLibrary.ReadIntegerWithCheck` _jsonvalue _property (`/Game/QuietRuntimeEditor/Common/Features/QuietSplineSystem/Blueprints/BP_Circle.PointsCount` _ascircleactor))
          (:`then`
            (set `/Game/QuietRuntimeEditor/Common/Features/QuietSplineSystem/Blueprints/BP_Circle.PointsCount` _newvalue_2 _ascircleactor)))))
    (`/Game/QuietRuntimeEditor/Common/Features/QuietSplineSystem/Blueprints/BP_QuietSplineActorBase.Refresh` _ascircleactor)
    (return true)
    (else
      (return _success))))