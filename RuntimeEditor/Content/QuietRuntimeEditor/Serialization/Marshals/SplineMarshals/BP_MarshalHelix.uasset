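; Marshal for BP_Helix in the runtime editor, translating the helix spline's shape properties to and from JSON.
; CollectProperties builds ranged, commit-only editor parameters in a Helix group, then lets the parent add its own properties.
; Get and Set defer to the parent first, handling helix fields only if it fails; a set value passes a read check before refreshing the helix.
; SerializeObject appends the helix fields after the parent's data.
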(fn `CollectProperties`
  (params (Object :type "Object Object Reference") (TargetJson :type "JsonObjectWrapper Structure (by ref)"))
  (locals (Helix :type "Array of JsonObjectWrapper Structure"))
  (bind _ashelixactor (cast `/Game/QuietRuntimeEditor/Common/Features/QuietSplineSystem/Blueprints/BP_Helix` Object))
  (bind (_startradius _endradius _height _turns _bias _pointscount) (defaults `Object` (`GameplayStatics.GetObjectClass` _ashelixactor)))
  (bind _jsonobject (`self.MakeFloatParam` "StartRadius" "Start Radius" "" (`/Game/QuietRuntimeEditor/Common/Features/QuietSplineSystem/Blueprints/BP_Helix.StartRadius` _ashelixactor) _startradius 0.01 0.1 10000.0 1000.0 1 2 true))
  (`KismetArrayLibrary.Array_Add` (`local.Helix`) _jsonobject)
  (bind _jsonobject_2 (`self.MakeFloatParam` "EndRadius" "End Radius" "" (`/Game/QuietRuntimeEditor/Common/Features/QuietSplineSystem/Blueprints/BP_Helix.EndRadius` _ashelixactor) _endradius 0.01 0.1 10000.0 1000.0 1 2 true))
  (`KismetArrayLibrary.Array_Add` (`local.Helix`) _jsonobject_2)
  (bind _jsonobject_3 (`self.MakeFloatParam` "Height" "Height" "" (`/Game/QuietRuntimeEditor/Common/Features/QuietSplineSystem/Blueprints/BP_Helix.Height` _ashelixactor) _height 0.01 0.1 10000.0 1000.0 1 2 true))
  (`KismetArrayLibrary.Array_Add` (`local.Helix`) _jsonobject_3)
  (bind _jsonobject_4 (`self.MakeIntParam` "Turns" "Turns" "" (`/Game/QuietRuntimeEditor/Common/Features/QuietSplineSystem/Blueprints/BP_Helix.Turns` _ashelixactor) _turns 2 2 24 24 true))
  (`KismetArrayLibrary.Array_Add` (`local.Helix`) _jsonobject_4)
  (bind _jsonobject_5 (`self.MakeFloatParam` "Bias" "Bias" "" (`/Game/QuietRuntimeEditor/Common/Features/QuietSplineSystem/Blueprints/BP_Helix.Bias` _ashelixactor) _bias -1.0 -1.0 1.0 1.0 1 3 true))
  (`KismetArrayLibrary.Array_Add` (`local.Helix`) _jsonobject_5)
  (bind _jsonobject_6 (`self.MakeIntParam` "PointsCount" "Points Count" "" (`/Game/QuietRuntimeEditor/Common/Features/QuietSplineSystem/Blueprints/BP_Helix.PointsCount` _ashelixactor) _pointscount 2 2 24 24 true))
  (`KismetArrayLibrary.Array_Add` (`local.Helix`) _jsonobject_6)
  (`|SetJsonField` (`local.TargetJson`) "GroupsState" (`|MakeArray` "Helix" "Spline"))
  (`|SetJsonField` (`local.TargetJson`) "Helix" (`local.Helix`))
  (`parent.CollectProperties` _ashelixactor (`local.TargetJson`))
  (return))

(fn `GetPropertyValue`
  (params (Object :type "Object Object Reference") (Property :type String))
  (returns (Success :type Boolean) (Value :type "JsonObjectWrapper Structure"))
  (bind _property (`local.Property`))
  (bind (_success _value) (`parent.GetPropertyValue` Object Property))
  (if (not _success)
    (bind _ashelixactor (cast `/Game/QuietRuntimeEditor/Common/Features/QuietSplineSystem/Blueprints/BP_Helix` Object))
    (bind _jsonobject (`/Game/QuietRuntimeEditor/Common/Blueprints/BP_QuietJsonFunctionLibrary.NewJson`))
    (switch `string` (`local.Property`)
      (:`StartRadius`
        (`|SetJsonField` _jsonobject _property (`/Game/QuietRuntimeEditor/Common/Features/QuietSplineSystem/Blueprints/BP_Helix.StartRadius` _ashelixactor)))
      (:`EndRadius`
        (`|SetJsonField` _jsonobject _property (`/Game/QuietRuntimeEditor/Common/Features/QuietSplineSystem/Blueprints/BP_Helix.EndRadius` _ashelixactor)))
      (:`Height`
        (`|SetJsonField` _jsonobject _property (`/Game/QuietRuntimeEditor/Common/Features/QuietSplineSystem/Blueprints/BP_Helix.Height` _ashelixactor)))
      (:`PointsCount`
        (`|SetJsonField` _jsonobject _property (`/Game/QuietRuntimeEditor/Common/Features/QuietSplineSystem/Blueprints/BP_Helix.PointsCount` _ashelixactor)))
      (:`Turns`
        (`|SetJsonField` _jsonobject _property (`/Game/QuietRuntimeEditor/Common/Features/QuietSplineSystem/Blueprints/BP_Helix.Turns` _ashelixactor)))
      (:`Bias`
        (`|SetJsonField` _jsonobject _property (`/Game/QuietRuntimeEditor/Common/Features/QuietSplineSystem/Blueprints/BP_Helix.Bias` _ashelixactor))))
    (return true _jsonobject)
    (else
      (return true _value))))

(fn `SerializeObject`
  (params (Object :type "Object Object Reference") (TargetJson :type "JsonObjectWrapper Structure (by ref)"))
  (`parent.SerializeObject` Object TargetJson)
  (bind _ashelixactor (cast `/Game/QuietRuntimeEditor/Common/Features/QuietSplineSystem/Blueprints/BP_Helix` Object))
  (`|SetJsonField` (`local.TargetJson`) "StartRadius" (`/Game/QuietRuntimeEditor/Common/Features/QuietSplineSystem/Blueprints/BP_Helix.StartRadius` _ashelixactor))
  (`|SetJsonField` (`local.TargetJson`) "EndRadius" (`/Game/QuietRuntimeEditor/Common/Features/QuietSplineSystem/Blueprints/BP_Helix.EndRadius` _ashelixactor))
  (`|SetJsonField` (`local.TargetJson`) "Height" (`/Game/QuietRuntimeEditor/Common/Features/QuietSplineSystem/Blueprints/BP_Helix.Height` _ashelixactor))
  (`|SetJsonField` (`local.TargetJson`) "PointsCount" (`/Game/QuietRuntimeEditor/Common/Features/QuietSplineSystem/Blueprints/BP_Helix.PointsCount` _ashelixactor))
  (`|SetJsonField` (`local.TargetJson`) "Turns" (`/Game/QuietRuntimeEditor/Common/Features/QuietSplineSystem/Blueprints/BP_Helix.Turns` _ashelixactor))
  (`|SetJsonField` (`local.TargetJson`) "Bias" (`/Game/QuietRuntimeEditor/Common/Features/QuietSplineSystem/Blueprints/BP_Helix.Bias` _ashelixactor))
  (return))

(fn `SetPropertyValue`
  (params (Object :type "Object Object Reference") (Property :type String) (JsonValue :type "JsonObjectWrapper Structure (by ref)"))
  (returns (Success :type Boolean))
  (bind _property (`local.Property`))
  (bind _jsonvalue (`local.JsonValue`))
  (bind _success (`parent.SetPropertyValue` Object Property JsonValue))
  (if (not _success)
    (bind _ashelixactor (cast `/Game/QuietRuntimeEditor/Common/Features/QuietSplineSystem/Blueprints/BP_Helix` Object))
    (switch `string` _property
      (:`StartRadius`
        (bind _newvalue (`/Game/QuietRuntimeEditor/Common/Blueprints/BP_QuietJsonMacroLibrary.ReadFloatWithCheck` _jsonvalue _property (`/Game/QuietRuntimeEditor/Common/Features/QuietSplineSystem/Blueprints/BP_Helix.StartRadius` _ashelixactor))
          (:`then`
            (set `/Game/QuietRuntimeEditor/Common/Features/QuietSplineSystem/Blueprints/BP_Helix.StartRadius` _newvalue _ashelixactor))))
      (:`EndRadius`
        (bind _newvalue_2 (`/Game/QuietRuntimeEditor/Common/Blueprints/BP_QuietJsonMacroLibrary.ReadFloatWithCheck` _jsonvalue _property (`/Game/QuietRuntimeEditor/Common/Features/QuietSplineSystem/Blueprints/BP_Helix.EndRadius` _ashelixactor))
          (:`then`
            (set `/Game/QuietRuntimeEditor/Common/Features/QuietSplineSystem/Blueprints/BP_Helix.EndRadius` _newvalue_2 _ashelixactor))))
      (:`Height`
        (bind _newvalue_3 (`/Game/QuietRuntimeEditor/Common/Blueprints/BP_QuietJsonMacroLibrary.ReadFloatWithCheck` _jsonvalue _property (`/Game/QuietRuntimeEditor/Common/Features/QuietSplineSystem/Blueprints/BP_Helix.Height` _ashelixactor))
          (:`then`
            (set `/Game/QuietRuntimeEditor/Common/Features/QuietSplineSystem/Blueprints/BP_Helix.Height` _newvalue_3 _ashelixactor))))
      (:`PointsCount`
        (bind _newvalue_4 (`/Game/QuietRuntimeEditor/Common/Blueprints/BP_QuietJsonMacroLibrary.ReadIntegerWithCheck` _jsonvalue _property (`/Game/QuietRuntimeEditor/Common/Features/QuietSplineSystem/Blueprints/BP_Helix.PointsCount` _ashelixactor))
          (:`then`
            (set `/Game/QuietRuntimeEditor/Common/Features/QuietSplineSystem/Blueprints/BP_Helix.PointsCount` _newvalue_4 _ashelixactor))))
      (:`Turns`
        (bind _newvalue_5 (`/Game/QuietRuntimeEditor/Common/Blueprints/BP_QuietJsonMacroLibrary.ReadIntegerWithCheck` _jsonvalue _property (`/Game/QuietRuntimeEditor/Common/Features/QuietSplineSystem/Blueprints/BP_Helix.Turns` _ashelixactor))
          (:`then`
            (set `/Game/QuietRuntimeEditor/Common/Features/QuietSplineSystem/Blueprints/BP_Helix.Turns` _newvalue_5 _ashelixactor))))
      (:`Bias`
        (bind _newvalue_6 (`/Game/QuietRuntimeEditor/Common/Blueprints/BP_QuietJsonMacroLibrary.ReadFloatWithCheck` _jsonvalue _property (`/Game/QuietRuntimeEditor/Common/Features/QuietSplineSystem/Blueprints/BP_Helix.Bias` _ashelixactor))
          (:`then`
            (set `/Game/QuietRuntimeEditor/Common/Features/QuietSplineSystem/Blueprints/BP_Helix.Bias` _newvalue_6 _ashelixactor)))))
    (`/Game/QuietRuntimeEditor/Common/Features/QuietSplineSystem/Blueprints/BP_QuietSplineActorBase.Refresh` _ashelixactor)
    (return true)
    (else
      (return _success))))