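; Serialization marshal for BP_Rectangle splines in the runtime editor, exposing Length, Width and Fillet as JSON.
; Property get and set try the parent marshal first, then handle the rectangle's own fields, with checked float reads that call Refresh after a write.
; CollectProperties builds commit-only float parameters in a Rectangle group ahead of the parent's properties.
; SerializeObject appends the three fields to the parent's serialized output.
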(fn `CollectProperties`
  (params (Object :type "Object Object Reference") (TargetJson :type "JsonObjectWrapper Structure (by ref)"))
  (locals (Ellipse :type "Array of JsonObjectWrapper Structure"))
  (bind _asrectangleactor (cast `/Game/QuietRuntimeEditor/Common/Features/QuietSplineSystem/Blueprints/BP_Rectangle` Object))
  (bind (_length _width _fillet) (defaults `Object` (`GameplayStatics.GetObjectClass` _asrectangleactor)))
  (bind _jsonobject (`self.MakeFloatParam` "Length" "Length" "" (`/Game/QuietRuntimeEditor/Common/Features/QuietSplineSystem/Blueprints/BP_Rectangle.Length` _asrectangleactor) _length 0.01 0.1 10000.0 1000.0 1 2 true))
  (`KismetArrayLibrary.Array_Add` (`local.Ellipse`) _jsonobject)
  (bind _jsonobject_2 (`self.MakeFloatParam` "Width" "Width" "" (`/Game/QuietRuntimeEditor/Common/Features/QuietSplineSystem/Blueprints/BP_Rectangle.Width` _asrectangleactor) _width 0.01 0.1 10000.0 1000.0 1 2 true))
  (`KismetArrayLibrary.Array_Add` (`local.Ellipse`) _jsonobject_2)
  (bind _jsonobject_3 (`self.MakeFloatParam` "Fillet" "Fillet" "" (`/Game/QuietRuntimeEditor/Common/Features/QuietSplineSystem/Blueprints/BP_Rectangle.Fillet` _asrectangleactor) _fillet 0.0 0.0 10000.0 100.0 1 2 true))
  (`KismetArrayLibrary.Array_Add` (`local.Ellipse`) _jsonobject_3)
  (`|SetJsonField` (`local.TargetJson`) "GroupsState" (`|MakeArray` "Rectangle" "Spline"))
  (`|SetJsonField` (`local.TargetJson`) "Rectangle" (`local.Ellipse`))
  (`parent.CollectProperties` _asrectangleactor (`local.TargetJson`))
  (return))

(fn `GetPropertyValue`
  (params (Object :type "Object Object Reference") (Property :type String))
  (returns (Success :type Boolean) (Value :type "JsonObjectWrapper Structure"))
  (bind _property (`local.Property`))
  (bind (_success _value) (`parent.GetPropertyValue` Object Property))
  (if (not _success)
    (bind _asrectangleactor (cast `/Game/QuietRuntimeEditor/Common/Features/QuietSplineSystem/Blueprints/BP_Rectangle` Object))
    (bind _jsonobject (`/Game/QuietRuntimeEditor/Common/Blueprints/BP_QuietJsonFunctionLibrary.NewJson`))
    (switch `string` (`local.Property`)
      (:`Length`
        (`|SetJsonField` _jsonobject _property (`/Game/QuietRuntimeEditor/Common/Features/QuietSplineSystem/Blueprints/BP_Rectangle.Length` _asrectangleactor))
        (return true _jsonobject))
      (:`Width`
        (`|SetJsonField` _jsonobject _property (`/Game/QuietRuntimeEditor/Common/Features/QuietSplineSystem/Blueprints/BP_Rectangle.Width` _asrectangleactor))
        (return true _jsonobject))
      (:`Fillet`
        (`|SetJsonField` _jsonobject _property (`/Game/QuietRuntimeEditor/Common/Features/QuietSplineSystem/Blueprints/BP_Rectangle.Fillet` _asrectangleactor))))
    (else
      (return true _value))))

(fn `SerializeObject`
  (params (Object :type "Object Object Reference") (TargetJson :type "JsonObjectWrapper Structure (by ref)"))
  (`parent.SerializeObject` Object TargetJson)
  (bind _asrectangleactor (cast `/Game/QuietRuntimeEditor/Common/Features/QuietSplineSystem/Blueprints/BP_Rectangle` Object))
  (`|SetJsonField` (`local.TargetJson`) "Length" (`/Game/QuietRuntimeEditor/Common/Features/QuietSplineSystem/Blueprints/BP_Rectangle.Length` _asrectangleactor))
  (`|SetJsonField` (`local.TargetJson`) "Width" (`/Game/QuietRuntimeEditor/Common/Features/QuietSplineSystem/Blueprints/BP_Rectangle.Width` _asrectangleactor))
  (`|SetJsonField` (`local.TargetJson`) "Fillet" (`/Game/QuietRuntimeEditor/Common/Features/QuietSplineSystem/Blueprints/BP_Rectangle.Fillet` _asrectangleactor))
  (return))

(fn `SetPropertyValue`
  (params (Object :type "Object Object Reference") (Property :type String) (JsonValue :type "JsonObjectWrapper Structure (by ref)"))
  (returns (Success :type Boolean))
  (bind _property (`local.Property`))
  (bind _jsonvalue (`local.JsonValue`))
  (bind _success (`parent.SetPropertyValue` Object Property JsonValue))
  (if (not _success)
    (bind _asrectangleactor (cast `/Game/QuietRuntimeEditor/Common/Features/QuietSplineSystem/Blueprints/BP_Rectangle` Object))
    (switch `string` _property
      (:`Length`
        (bind _newvalue (`/Game/QuietRuntimeEditor/Common/Blueprints/BP_QuietJsonMacroLibrary.ReadFloatWithCheck` _jsonvalue _property (`/Game/QuietRuntimeEditor/Common/Features/QuietSplineSystem/Blueprints/BP_Rectangle.Length` _asrectangleactor))
          (:`then`
            (set `/Game/QuietRuntimeEditor/Common/Features/QuietSplineSystem/Blueprints/BP_Rectangle.Length` _newvalue _asrectangleactor))))
      (:`Width`
        (bind _newvalue_2 (`/Game/QuietRuntimeEditor/Common/Blueprints/BP_QuietJsonMacroLibrary.ReadFloatWithCheck` _jsonvalue _property (`/Game/QuietRuntimeEditor/Common/Features/QuietSplineSystem/Blueprints/BP_Rectangle.Width` _asrectangleactor))
          (:`then`
            (set `/Game/QuietRuntimeEditor/Common/Features/QuietSplineSystem/Blueprints/BP_Rectangle.Width` _newvalue_2 _asrectangleactor))))
      (:`Fillet`
        (bind _newvalue_3 (`/Game/QuietRuntimeEditor/Common/Blueprints/BP_QuietJsonMacroLibrary.ReadFloatWithCheck` _jsonvalue _property (`/Game/QuietRuntimeEditor/Common/Features/QuietSplineSystem/Blueprints/BP_Rectangle.Fillet` _asrectangleactor))
          (:`then`
            (set `/Game/QuietRuntimeEditor/Common/Features/QuietSplineSystem/Blueprints/BP_Rectangle.Fillet` _newvalue_3 _asrectangleactor)))))
    (`/Game/QuietRuntimeEditor/Common/Features/QuietSplineSystem/Blueprints/BP_QuietSplineActorBase.Refresh` _asrectangleactor)
    (return true)
    (else
      (return _success))))