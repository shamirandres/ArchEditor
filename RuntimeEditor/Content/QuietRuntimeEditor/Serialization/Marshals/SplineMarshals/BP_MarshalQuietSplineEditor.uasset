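; Marshal that exposes BP_QuietSplineEditorComponent to the Quiet runtime editor as JSON-described properties and actions.
; CollectProperties builds point parameters that depend on the selection count, with dependencies linking tangents and point type, plus spline-wide editor settings.
; Get and Set handlers map property names to component accessors, using checked reads on writes and supporting spline import from JSON.
; CallAction routes named commands to selection, point editing, whole-spline operations and point-type changes.
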(fn `CallAction`
  (params (Object :type "Object Object Reference") (Action :type "JsonObjectWrapper Structure"))
  (returns (Success :type Boolean))
  (bind _asquietspline (cast `/Game/QuietRuntimeEditor/Common/Features/QuietSplineSystem/Blueprints/BP_QuietSplineEditorComponent` Object))
  (bind _outvalue (`|GetJsonField` Action "Action"))
  (switch `string` _outvalue
    (:`SelectFirst`
      (`/Game/QuietRuntimeEditor/Common/Features/QuietSplineSystem/Blueprints/BP_QuietSplineEditorComponent.SelectPoint` _asquietspline _outvalue :!label _label))
    (:`AddPrevious`
      (goto _label))
    (:`SelectPrevious`
      (goto _label))
    (:`SelectAll`
      (goto _label))
    (:`SelectNext`
      (goto _label))
    (:`AddNext`
      (goto _label))
    (:`SelectLast`
      (goto _label))
    (:`ClearSelection`
      (goto _label))
    (:`Refresh`
      (`/Game/QuietRuntimeEditor/Common/Features/QuietSplineSystem/Blueprints/BP_QuietSplineEditorComponent.UpdateSpline` _asquietspline true)
      (`/Game/QuietRuntimeEditor/Common/Features/QuietSplineSystem/Blueprints/BP_QuietSplineEditorComponent.OnSplineUpdated` _asquietspline))
    (:`Add Point`
      (`/Game/QuietRuntimeEditor/Common/Features/QuietSplineSystem/Blueprints/BP_QuietSplineEditorComponent.AddAnotherPoint` _asquietspline true))
    (:`Remove Selected Points`
      (`/Game/QuietRuntimeEditor/Common/Features/QuietSplineSystem/Blueprints/BP_QuietSplineEditorComponent.RemoveSelectedPoints` _asquietspline true))
    (:`Clear Spline`
      (`/Game/QuietRuntimeEditor/Common/Features/QuietSplineSystem/Blueprints/BP_QuietSplineEditorComponent.ClearSpline` _asquietspline true))
    (:`Reverse`
      (`/Game/QuietRuntimeEditor/Common/Features/QuietSplineSystem/Blueprints/BP_QuietSplineEditorComponent.Reverse` _asquietspline true))
    (:`Make First`
      (`/Game/QuietRuntimeEditor/Common/Features/QuietSplineSystem/Blueprints/BP_QuietSplineEditorComponent.MakeFirst` _asquietspline true))
    (:`Outline`
      (`/Game/QuietRuntimeEditor/Common/Features/QuietSplineSystem/Blueprints/BP_QuietSplineEditorComponent.Outline` _asquietspline true))
    (:`Smooth Spline`
      (`/Game/QuietRuntimeEditor/Common/Features/QuietSplineSystem/Blueprints/BP_QuietSplineEditorComponent.SmoothSpline` _asquietspline true))
    (:`Linear Spline`
      (`/Game/QuietRuntimeEditor/Common/Features/QuietSplineSystem/Blueprints/BP_QuietSplineEditorComponent.MakeLinear` _asquietspline true))
    (:`Bezier Corner`
      (bind _index (`/Game/QuietRuntimeEditor/Common/Features/QuietSplineSystem/Blueprints/BP_QuietSplineEditorComponent.GetMainSelectedPoint` _asquietspline))
      (`/Game/QuietRuntimeEditor/Common/Features/QuietSplineSystem/Blueprints/BP_QuietSplineEditorComponent.ExecutePointTypeChange` _asquietspline "Bezier Corner" _index))
    (:`Bezier`
      (`/Game/QuietRuntimeEditor/Common/Features/QuietSplineSystem/Blueprints/BP_QuietSplineEditorComponent.ExecutePointTypeChange` _asquietspline "Bezier" _index))
    (:`Corner`
      (`/Game/QuietRuntimeEditor/Common/Features/QuietSplineSystem/Blueprints/BP_QuietSplineEditorComponent.ExecutePointTypeChange` _asquietspline "Corner" _index))
    (:`Smooth`
      (`/Game/QuietRuntimeEditor/Common/Features/QuietSplineSystem/Blueprints/BP_QuietSplineEditorComponent.ExecutePointTypeChange` _asquietspline "Smooth" _index)))
  (return true))

(fn `CollectProperties`
  (params (Object :type "Object Object Reference") (TargetJson :type "JsonObjectWrapper Structure (by ref)"))
  (locals (Control :type "/Game/QuietRuntimeEditor/Common/Widgets/QuietControls/WBP_QuietControlBase Soft Class Reference" :default "/Game/QuietRuntimeEditor/Common/Features/QuietSplineSystem/Widgets/WBP_SplinePointsSelector.WBP_SplinePointsSelector_C") (Selected :type "Array of JsonObjectWrapper Structure") (`Edit Spline` :type "Array of JsonObjectWrapper Structure") (Spline :type "/Game/QuietRuntimeEditor/Common/Features/QuietSplineSystem/Blueprints/BP_QuietSplineEditorComponent Object Reference") (Editor :type "Array of JsonObjectWrapper Structure") (Actions :type "Array of String"))
  (bind _asquietspline (cast `/Game/QuietRuntimeEditor/Common/Features/QuietSplineSystem/Blueprints/BP_QuietSplineEditorComponent` Object))
  (set `local.Spline` _asquietspline)
  (bind _jsonobject (`/Game/QuietRuntimeEditor/Common/Blueprints/BP_QuietJsonFunctionLibrary.NewJson`))
  (`|SetJsonField` _jsonobject "Type" (`local.Control`))
  (`|SetJsonField` _jsonobject "Dependencies" (`|MakeArray`))
  (`|SetJsonField` _jsonobject "Name" "SelectSplinePoint")
  (`KismetArrayLibrary.Array_Add` (`local.Selected`) _jsonobject)
  (`|ExecutionSequence`
    (:`then_0`
      (bind _pinned (`/Game/QuietRuntimeEditor/Common/Blueprints/BP_QuietJsonMacroLibrary.Pin` (`KismetArrayLibrary.Array_Length` (`/Game/QuietRuntimeEditor/Common/Features/QuietSplineSystem/Blueprints/BP_QuietSplineEditorComponent.SelectedSplinePoints` (`local.Spline`)))))
      (if (> _pinned 0)
        (`|ExecutionSequence`
          (:`then_0`
            (if (== _pinned 1)
              (bind _jsonobject_2 (`self.MakeVectorParam` "PointLocation" "Location" "" (`/Game/QuietRuntimeEditor/Common/Features/QuietSplineSystem/Blueprints/BP_QuietSplineEditorComponent.GetLocationAtSelectedPoint` (`local.Spline`)) (0.0 0.0 0.0) 0.0 0.0 0.0 0.0 1 3 true))
              (`KismetArrayLibrary.Array_Add` (`local.Selected`) _jsonobject_2)
              (bind _jsonobject_3 (`self.MakeVectorParam` "PointRotation" "Rotation" "" (`KismetMathLibrary.MakeVector` (.roll (`/Game/QuietRuntimeEditor/Common/Features/QuietSplineSystem/Blueprints/BP_QuietSplineEditorComponent.GetRotationAtSelectedPoint` (`local.Spline`))) (.pitch (`/Game/QuietRuntimeEditor/Common/Features/QuietSplineSystem/Blueprints/BP_QuietSplineEditorComponent.GetRotationAtSelectedPoint` (`local.Spline`))) (.yaw (`/Game/QuietRuntimeEditor/Common/Features/QuietSplineSystem/Blueprints/BP_QuietSplineEditorComponent.GetRotationAtSelectedPoint` (`local.Spline`)))) (0.0 0.0 0.0) -360.0 -180.0 360.0 180.0 1 1 true))
              (`KismetArrayLibrary.Array_Add` (`local.Selected`) _jsonobject_3)
              (bind _jsonobject_4 (`self.MakeVectorParam` "PointScale" "Scale" "" (`/Game/QuietRuntimeEditor/Common/Features/QuietSplineSystem/Blueprints/BP_QuietSplineEditorComponent.GetScaleAtSelectedPoint` (`local.Spline`)) (1.0 1.0 1.0) 0.0 0.0 0.0 0.0 1 3 true))
              (`KismetArrayLibrary.Array_Add` (`local.Selected`) _jsonobject_4)
              (bind _jsonobject_5 (`self.MakeVectorParam` "ArriveTangent" "Arrive Tangent" "" (`/Game/QuietRuntimeEditor/Common/Features/QuietSplineSystem/Blueprints/BP_QuietSplineEditorComponent.GetArriveTangentAtSelectedPoint` (`local.Spline`)) (100.0 0.0 0.0) 0.0 0.0 0.0 0.0 1 3 true))
              (`|SetJsonField` _jsonobject_5 "Dependencies" (`|MakeArray` "Selected Point.LeaveTangent" "Selected Point.SplinePointType"))
              (`KismetArrayLibrary.Array_Add` (`local.Selected`) _jsonobject_5)
              (bind _jsonobject_6 (`self.MakeVectorParam` "LeaveTangent" "Leave Tangent" "" (`/Game/QuietRuntimeEditor/Common/Features/QuietSplineSystem/Blueprints/BP_QuietSplineEditorComponent.GetLeaveTangentAtSelectedPoint` (`local.Spline`)) (100.0 0.0 0.0) 0.0 0.0 0.0 0.0 1 3 true))
              (`|SetJsonField` _jsonobject_6 "Dependencies" (`|MakeArray` "Selected Point.ArriveTangent" "Selected Point.SplinePointType"))
              (`KismetArrayLibrary.Array_Add` (`local.Selected`) _jsonobject_6)
              (`KismetArrayLibrary.Array_Add` (`local.Actions`) "Make First")))
          (:`then_1`
            (bind _jsonobject_7 (`self.MakeEnumParam` "SplinePointType" "Type" "" (`|MakeArray` "Bezier Corner" "Bezier" "Corner" "Smooth") (`KismetMathLibrary.Conv_ByteToInt` (`/Game/QuietRuntimeEditor/Common/Features/QuietSplineSystem/Blueprints/BP_QuietSplineEditorComponent.GetSelectedPointType` (`local.Spline`))) 0 true))
            (`|SetJsonField` _jsonobject_7 "Dependencies" (`|MakeArray` "Selected Point.LeaveTangent"))
            (`KismetArrayLibrary.Array_Add` (`local.Selected`) _jsonobject_7)
            (`KismetArrayLibrary.Array_Add` (`local.Actions`) "Remove Selected Points")
            (bind _param (`self.MakeActionsParam` (`local.Actions`)))
            (`KismetArrayLibrary.Array_Add` (`local.Selected`) _param)))))
    (:`then_1`
      (`|SetJsonField` (`local.TargetJson`) "Points" (`local.Selected`))
      (bind _jsonobject_8 (`self.MakeFloatParam` "OutlineWidth" "Outline Width" "" (`/Game/QuietRuntimeEditor/Common/Features/QuietSplineSystem/Blueprints/BP_QuietSplineEditorComponent.OutlineWidth` (`local.Spline`)) 10.0 0.0 0.0 0.0 0.0 1 3))
      (`KismetArrayLibrary.Array_Add` (`local.Editor`) _jsonobject_8)
      (bind _jsonobject_9 (`self.MakeStringParam` "ImportJson" "Import Json" "" (`/Game/QuietRuntimeEditor/Common/Features/QuietSplineSystem/Blueprints/BP_QuietSplineEditorComponent.JsonString` (`local.Spline`))))
      (`KismetArrayLibrary.Array_Add` (`local.Editor`) _jsonobject_9)
      (bind _jsonobject_10 (`self.MakeIntParam` "InterpolationSteps" "Interpolation Steps" "" (`/Game/QuietRuntimeEditor/Common/Features/QuietSplineSystem/Blueprints/BP_QuietSplineEditorComponent.GetInterpolationSteps` (`local.Spline`)) 12 1 1 24 24))
      (`KismetArrayLibrary.Array_Add` (`local.Editor`) _jsonobject_10)
      (bind _jsonobject_11 (`self.MakeBoolParam` "ClosedLoop" "Closed Loop" "" (`/Game/QuietRuntimeEditor/Common/Features/QuietSplineSystem/Blueprints/BP_QuietSplineEditorComponent.IsClosedLoop` (`local.Spline`)) true))
      (`KismetArrayLibrary.Array_Add` (`local.Editor`) _jsonobject_11)
      (`|SetJsonField` (`local.TargetJson`) "Editor" (`local.Editor`))
      (return))))

(fn `GetPropertyValue`
  (params (Object :type "Object Object Reference") (Property :type String))
  (returns (Success :type Boolean) (Value :type "JsonObjectWrapper Structure"))
  (bind _property (`local.Property`))
  (bind _asquietspline (cast `/Game/QuietRuntimeEditor/Common/Features/QuietSplineSystem/Blueprints/BP_QuietSplineEditorComponent` Object))
  (bind _jsonobject (`/Game/QuietRuntimeEditor/Common/Blueprints/BP_QuietJsonFunctionLibrary.NewJson`))
  (switch `string` (`local.Property`)
    (:`PointLocation`
      (`|SetJsonField` _jsonobject _property (`/Game/QuietRuntimeEditor/Common/Features/QuietSplineSystem/Blueprints/BP_QuietSplineEditorComponent.GetLocationAtSelectedPoint` _asquietspline)))
    (:`PointRotation`
      (`|SetJsonField` _jsonobject _property (`/Game/QuietRuntimeEditor/Common/Features/QuietSplineSystem/Blueprints/BP_QuietSplineEditorComponent.GetRotationAtSelectedPoint` _asquietspline)))
    (:`PointScale`
      (`|SetJsonField` _jsonobject _property (`/Game/QuietRuntimeEditor/Common/Features/QuietSplineSystem/Blueprints/BP_QuietSplineEditorComponent.GetScaleAtSelectedPoint` _asquietspline)))
    (:`ArriveTangent`
      (`|SetJsonField` _jsonobject _property (`/Game/QuietRuntimeEditor/Common/Features/QuietSplineSystem/Blueprints/BP_QuietSplineEditorComponent.GetArriveTangentAtSelectedPoint` _asquietspline)))
    (:`LeaveTangent`
      (`|SetJsonField` _jsonobject _property (`/Game/QuietRuntimeEditor/Common/Features/QuietSplineSystem/Blueprints/BP_QuietSplineEditorComponent.GetLeaveTangentAtSelectedPoint` _asquietspline)))
    (:`SplinePointType`
      (`|SetJsonField` _jsonobject _property (`/Game/QuietRuntimeEditor/Common/Features/QuietSplineSystem/Blueprints/BP_QuietSplineEditorComponent.GetSelectedPointType` _asquietspline)))
    (:`InterpolationSteps`
      (`|SetJsonField` _jsonobject _property (`/Game/QuietRuntimeEditor/Common/Features/QuietSplineSystem/Blueprints/BP_QuietSplineEditorComponent.GetInterpolationSteps` _asquietspline)))
    (:`ClosedLoop`
      (`|SetJsonField` _jsonobject _property (`/Game/QuietRuntimeEditor/Common/Features/QuietSplineSystem/Blueprints/BP_QuietSplineEditorComponent.IsClosedLoop` _asquietspline)))
    (:`OutlineWidth`
      (`|SetJsonField` _jsonobject _property (`/Game/QuietRuntimeEditor/Common/Features/QuietSplineSystem/Blueprints/BP_QuietSplineEditorComponent.OutlineWidth` _asquietspline))))
  (return true _jsonobject))

(fn `SetPropertyValue`
  (params (Object :type "Object Object Reference") (Property :type String) (JsonValue :type "JsonObjectWrapper Structure (by ref)"))
  (returns (Success :type Boolean))
  (bind _jsonvalue (`local.JsonValue`))
  (bind _property (`local.Property`))
  (bind _asquietspline (cast `/Game/QuietRuntimeEditor/Common/Features/QuietSplineSystem/Blueprints/BP_QuietSplineEditorComponent` Object))
  (switch `string` (`local.Property`)
    (:`SelectSplinePoint`
      (bind _outvalue (`|GetJsonField` _jsonvalue _property))
      (`/Game/QuietRuntimeEditor/Common/Features/QuietSplineSystem/Blueprints/BP_QuietSplineEditorComponent.SelectPoint` _asquietspline _outvalue))
    (:`PointLocation`
      (bind _newvalue (`/Game/QuietRuntimeEditor/Common/Blueprints/BP_QuietJsonMacroLibrary.ReadVectorWithCheck` _jsonvalue _property (`/Game/QuietRuntimeEditor/Common/Features/QuietSplineSystem/Blueprints/BP_QuietSplineEditorComponent.GetLocationAtSelectedPoint` _asquietspline))
        (:`then`
          (`/Game/QuietRuntimeEditor/Common/Features/QuietSplineSystem/Blueprints/BP_QuietSplineEditorComponent.SetLocationAtSelectedPoint` _asquietspline _newvalue)
          (return true))))
    (:`PointRotation`
      (bind _newvalue_2 (`/Game/QuietRuntimeEditor/Common/Blueprints/BP_QuietJsonMacroLibrary.ReadRotatorWithCheck` _jsonvalue _property (`/Game/QuietRuntimeEditor/Common/Features/QuietSplineSystem/Blueprints/BP_QuietSplineEditorComponent.GetRotationAtSelectedPoint` _asquietspline))
        (:`then`
          (`/Game/QuietRuntimeEditor/Common/Features/QuietSplineSystem/Blueprints/BP_QuietSplineEditorComponent.SetRotationAtSelectedPoint` _asquietspline _newvalue_2)
          (return true))))
    (:`PointScale`
      (bind _newvalue_3 (`/Game/QuietRuntimeEditor/Common/Blueprints/BP_QuietJsonMacroLibrary.ReadVectorWithCheck` _jsonvalue _property (`/Game/QuietRuntimeEditor/Common/Features/QuietSplineSystem/Blueprints/BP_QuietSplineEditorComponent.GetScaleAtSelectedPoint` _asquietspline))
        (:`then`
          (`/Game/QuietRuntimeEditor/Common/Features/QuietSplineSystem/Blueprints/BP_QuietSplineEditorComponent.SetScaleAtSelectedPoint` _asquietspline _newvalue_3)
          (return true))))
    (:`ArriveTangent`
      (bind _newvalue_4 (`/Game/QuietRuntimeEditor/Common/Blueprints/BP_QuietJsonMacroLibrary.ReadVectorWithCheck` _jsonvalue _property (`/Game/QuietRuntimeEditor/Common/Features/QuietSplineSystem/Blueprints/BP_QuietSplineEditorComponent.GetArriveTangentAtSelectedPoint` _asquietspline))
        (:`then`
          (`/Game/QuietRuntimeEditor/Common/Features/QuietSplineSystem/Blueprints/BP_QuietSplineEditorComponent.SetArriveTangentAtSelectedPoint` _asquietspline _newvalue_4)
          (return true))))
    (:`LeaveTangent`
      (bind _newvalue_5 (`/Game/QuietRuntimeEditor/Common/Blueprints/BP_QuietJsonMacroLibrary.ReadVectorWithCheck` _jsonvalue _property (`/Game/QuietRuntimeEditor/Common/Features/QuietSplineSystem/Blueprints/BP_QuietSplineEditorComponent.GetLeaveTangentAtSelectedPoint` _asquietspline))
        (:`then`
          (`/Game/QuietRuntimeEditor/Common/Features/QuietSplineSystem/Blueprints/BP_QuietSplineEditorComponent.SetLeaveTangentAtSelectedPoint` _asquietspline _newvalue_5)
          (return true))))
    (:`SplinePointType`
      (bind _newvalue_6 (`/Game/QuietRuntimeEditor/Common/Blueprints/BP_QuietJsonMacroLibrary.ReadEnumWithCheck` _jsonvalue _property (`/Game/QuietRuntimeEditor/Common/Features/QuietSplineSystem/Blueprints/BP_QuietSplineEditorComponent.GetSelectedPointType` _asquietspline))
        (:`then`
          (`/Game/QuietRuntimeEditor/Common/Features/QuietSplineSystem/Blueprints/BP_QuietSplineEditorComponent.SetSelectedPointType` _asquietspline (cast `/Game/QuietRuntimeEditor/Common/Features/QuietSplineSystem/Blueprints/E_QuietSplinePointType` _newvalue_6))
          (`/Game/QuietRuntimeEditor/Common/Features/QuietSplineSystem/Blueprints/BP_QuietSplineEditorComponent.RequestToUpdateGizmo` _asquietspline)
          (return true))))
    (:`InterpolationSteps`
      (bind _newvalue_7 (`/Game/QuietRuntimeEditor/Common/Blueprints/BP_QuietJsonMacroLibrary.ReadIntegerWithCheck` _jsonvalue _property (`/Game/QuietRuntimeEditor/Common/Features/QuietSplineSystem/Blueprints/BP_QuietSplineEditorComponent.GetInterpolationSteps` _asquietspline))
        (:`then`
          (`/Game/QuietRuntimeEditor/Common/Features/QuietSplineSystem/Blueprints/BP_QuietSplineEditorComponent.SetInterpolationSteps` _asquietspline _newvalue_7)
          (return true))))
    (:`ClosedLoop`
      (bind _newvalue_8 (`/Game/QuietRuntimeEditor/Common/Blueprints/BP_QuietJsonMacroLibrary.ReadBoolWithCheck` _jsonvalue _property (`/Game/QuietRuntimeEditor/Common/Features/QuietSplineSystem/Blueprints/BP_QuietSplineEditorComponent.IsClosedLoop` _asquietspline))
        (:`then`
          (`/Game/QuietRuntimeEditor/Common/Features/QuietSplineSystem/Blueprints/BP_QuietSplineEditorComponent.SetClosedLoop` _asquietspline _newvalue_8)
          (return true))))
    (:`ImportJson`
      (bind _newvalue_9 (`/Game/QuietRuntimeEditor/Common/Blueprints/BP_QuietJsonMacroLibrary.ReadStringWithCheck` _jsonvalue _property (`/Game/QuietRuntimeEditor/Common/Features/QuietSplineSystem/Blueprints/BP_QuietSplineEditorComponent.JsonString` _asquietspline))
        (:`then`
          (`/Game/QuietRuntimeEditor/Common/Features/QuietSplineSystem/Blueprints/BP_QuietSplineEditorComponent.DeserializeSpline` _asquietspline _newvalue_9)
          (return true))))
    (:`OutlineWidth`
      (bind _newvalue_10 (`/Game/QuietRuntimeEditor/Common/Blueprints/BP_QuietJsonMacroLibrary.ReadFloatWithCheck` _jsonvalue _property (`/Game/QuietRuntimeEditor/Common/Features/QuietSplineSystem/Blueprints/BP_QuietSplineEditorComponent.OutlineWidth` _asquietspline))
        (:`then`
          (set `/Game/QuietRuntimeEditor/Common/Features/QuietSplineSystem/Blueprints/BP_QuietSplineEditorComponent.OutlineWidth` _newvalue_10 _asquietspline)
          (return true))))))