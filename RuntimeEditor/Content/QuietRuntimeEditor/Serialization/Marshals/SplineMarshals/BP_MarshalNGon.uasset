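; Marshal for BP_NGon spline shapes in the runtime editor, exposing Radius, Sides and Fillet as JSON for editing and serialization.
; Property get and set try the parent marshal first, then handle the NGon fields, calling Refresh on the shape after a checked write.
; CollectProperties builds slider parameters with class-default values under an NGon group ahead of the parent's properties, and SerializeObject appends the three fields to the parent's output.
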(fn `CollectProperties`
  (params (Object :type "Object Object Reference") (TargetJson :type "JsonObjectWrapper Structure (by ref)"))
  (locals (NGon :type "Array of JsonObjectWrapper Structure"))
  (bind _asngonactor (cast `/Game/QuietRuntimeEditor/Common/Features/QuietSplineSystem/Blueprints/BP_NGon` Object))
  (bind (_radius _sides _fillet) (defaults `Object` (`GameplayStatics.GetObjectClass` _asngonactor)))
  (bind _jsonobject (`self.MakeFloatParam` "Radius" "Radius" "" (`/Game/QuietRuntimeEditor/Common/Features/QuietSplineSystem/Blueprints/BP_NGon.Radius` _asngonactor) _radius 0.01 0.1 10000.0 1000.0 1 2 true))
  (`KismetArrayLibrary.Array_Add` (`local.NGon`) _jsonobject)
  (bind _jsonobject_2 (`self.MakeIntParam` "Sides" "Sides" "" (`/Game/QuietRuntimeEditor/Common/Features/QuietSplineSystem/Blueprints/BP_NGon.Sides` _asngonactor) _sides 3 3 24 24 true))
  (`KismetArrayLibrary.Array_Add` (`local.NGon`) _jsonobject_2)
  (bind _jsonobject_3 (`self.MakeFloatParam` "Fillet" "Fillet" "" (`/Game/QuietRuntimeEditor/Common/Features/QuietSplineSystem/Blueprints/BP_NGon.Fillet` _asngonactor) _fillet 0.0 0.0 100.0 1000.0 1 3 true))
  (`KismetArrayLibrary.Array_Add` (`local.NGon`) _jsonobject_3)
  (`|SetJsonField` (`local.TargetJson`) "GroupsState" (`|MakeArray` "NGon" "Spline"))
  (`|SetJsonField` (`local.TargetJson`) "NGon" (`local.NGon`))
  (`parent.CollectProperties` _asngonactor (`local.TargetJson`))
  (return))

(fn `GetPropertyValue`
  (params (Object :type "Object Object Reference") (Property :type String))
  (returns (Success :type Boolean) (Value :type "JsonObjectWrapper Structure"))
  (bind _property (`local.Property`))
  (bind (_success _value) (`parent.GetPropertyValue` Object Property))
  (if (not _success)
    (bind _asngonactor (cast `/Game/QuietRuntimeEditor/Common/Features/QuietSplineSystem/Blueprints/BP_NGon` Object))
    (bind _jsonobject (`/Game/QuietRuntimeEditor/Common/Blueprints/BP_QuietJsonFunctionLibrary.NewJson`))
    (switch `string` (`local.Property`)
      (:`Radius`
        (`|SetJsonField` _jsonobject _property (`/Game/QuietRuntimeEditor/Common/Features/QuietSplineSystem/Blueprints/BP_NGon.Radius` _asngonactor)))
      (:`Sides`
        (`|SetJsonField` _jsonobject _property (`/Game/QuietRuntimeEditor/Common/Features/QuietSplineSystem/Blueprints/BP_NGon.Sides` _asngonactor)))
      (:`Fillet`
        (`|SetJsonField` _jsonobject _property (`/Game/QuietRuntimeEditor/Common/Features/QuietSplineSystem/Blueprints/BP_NGon.Fillet` _asngonactor))))
    (return true _jsonobject)
    (else
      (return true _value))))

(fn `SerializeObject`
  (params (Object :type "Object Object Reference") (TargetJson :type "JsonObjectWrapper Structure (by ref)"))
  (`parent.SerializeObject` Object TargetJson)
  (bind _asngonactor (cast `/Game/QuietRuntimeEditor/Common/Features/QuietSplineSystem/Blueprints/BP_NGon` Object))
  (`|SetJsonField` (`local.TargetJson`) "Radius" (`/Game/QuietRuntimeEditor/Common/Features/QuietSplineSystem/Blueprints/BP_NGon.Radius` _asngonactor))
  (`|SetJsonField` (`local.TargetJson`) "Sides" (`/Game/QuietRuntimeEditor/Common/Features/QuietSplineSystem/Blueprints/BP_NGon.Sides` _asngonactor))
  (`|SetJsonField` (`local.TargetJson`) "Fillet" (`/Game/QuietRuntimeEditor/Common/Features/QuietSplineSystem/Blueprints/BP_NGon.Fillet` _asngonactor))
  (return))

(fn `SetPropertyValue`
  (params (Object :type "Object Object Reference") (Property :type String) (JsonValue :type "JsonObjectWrapper Structure (by ref)"))
  (returns (Success :type Boolean))
  (bind _property (`local.Property`))
  (bind _jsonvalue (`local.JsonValue`))
  (bind _success (`parent.SetPropertyValue` Object Property JsonValue))
  (if (not _success)
    (bind _asngonactor (cast `/Game/QuietRuntimeEditor/Common/Features/QuietSplineSystem/Blueprints/BP_NGon` Object))
    (switch `string` (`local.Property`)
      (:`Radius`
        (bind _newvalue (`/Game/QuietRuntimeEditor/Common/Blueprints/BP_QuietJsonMacroLibrary.ReadFloatWithCheck` _jsonvalue _property (`/Game/QuietRuntimeEditor/Common/Features/QuietSplineSystem/Blueprints/BP_NGon.Radius` _asngonactor))
          (:`then`
            (set `/Game/QuietRuntimeEditor/Common/Features/QuietSplineSystem/Blueprints/BP_NGon.Radius` _newvalue _asngonactor))))
      (:`Sides`
        (bind _newvalue_2 (`/Game/QuietRuntimeEditor/Common/Blueprints/BP_QuietJsonMacroLibrary.ReadIntegerWithCheck` _jsonvalue _property (`/Game/QuietRuntimeEditor/Common/Features/QuietSplineSystem/Blueprints/BP_NGon.Sides` _asngonactor))
          (:`then`
            (set `/Game/QuietRuntimeEditor/Common/Features/QuietSplineSystem/Blueprints/BP_NGon.Sides` _newvalue_2 _asngonactor))))
      (:`Fillet`
        (bind _newvalue_3 (`/Game/QuietRuntimeEditor/Common/Blueprints/BP_QuietJsonMacroLibrary.ReadFloatWithCheck` _jsonvalue _property (`/Game/QuietRuntimeEditor/Common/Features/QuietSplineSystem/Blueprints/BP_NGon.Fillet` _asngonactor))
          (:`then`
            (set `/Game/QuietRuntimeEditor/Common/Features/QuietSplineSystem/Blueprints/BP_NGon.Fillet` _newvalue_3 _asngonactor)))))
    (`/Game/QuietRuntimeEditor/Common/Features/QuietSplineSystem/Blueprints/BP_QuietSplineActorBase.Refresh` _asngonactor)
    (return true)
    (else
      (return _success))))