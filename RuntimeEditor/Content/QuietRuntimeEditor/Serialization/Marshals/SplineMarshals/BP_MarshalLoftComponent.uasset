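; Marshal for BP_QuietLoftComponent in the runtime editor, converting loft properties such as mesh, material, shift, offset and twist to and from JSON.
; SetPropertyValue reads checked values into the component, clearing the mesh when null or invalid and rebuilding the spline after mesh or twist edits.
; GetPropertyValue returns a single property as JSON.
; SerializeObject writes the whole set, including the material only when override is enabled.
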(fn `GetPropertyValue`
  (params (Object :type "Object Object Reference") (Property :type String))
  (returns (Success :type Boolean) (Value :type "JsonObjectWrapper Structure"))
  (bind _asquietloftcomponent (cast `/Game/QuietRuntimeEditor/Common/Features/QuietSplineSystem/Blueprints/BP_QuietLoftComponent` Object))
  (bind _jsonobject (`/Game/QuietRuntimeEditor/Common/Blueprints/BP_QuietJsonFunctionLibrary.NewJson`))
  (switch `string` Property
    (:`StaticMesh`
      (`|SetJsonField` _jsonobject Property (`/Game/QuietRuntimeEditor/Common/Features/QuietSplineSystem/Blueprints/BP_QuietLoftComponent.GetStaticMesh` _asquietloftcomponent)))
    (:`Shift`
      (`|SetJsonField` _jsonobject Property (`/Game/QuietRuntimeEditor/Common/Features/QuietSplineSystem/Blueprints/BP_QuietLoftComponent.Shift` _asquietloftcomponent)))
    (:`Offset`
      (`|SetJsonField` _jsonobject Property (`/Game/QuietRuntimeEditor/Common/Features/QuietSplineSystem/Blueprints/BP_QuietLoftComponent.Offset` _asquietloftcomponent)))
    (:`Twist`
      (`|SetJsonField` _jsonobject Property (`/Game/QuietRuntimeEditor/Common/Features/QuietSplineSystem/Blueprints/BP_QuietLoftComponent.Twist` _asquietloftcomponent)))
    (:`Material`
      (`|SetJsonField` _jsonobject Property (`/Game/QuietRuntimeEditor/Common/Features/QuietSplineSystem/Blueprints/BP_QuietLoftComponent.Material` _asquietloftcomponent)))
    (:`OverrideMaterial`
      (`|SetJsonField` _jsonobject Property (`/Game/QuietRuntimeEditor/Common/Features/QuietSplineSystem/Blueprints/BP_QuietLoftComponent.GetOverrideMaterial` _asquietloftcomponent))))
  (return true _jsonobject))

(fn `SerializeObject`
  (params (Object :type "Object Object Reference") (TargetJson :type "JsonObjectWrapper Structure (by ref)"))
  (bind _asquietloftcomponent (cast `/Game/QuietRuntimeEditor/Common/Features/QuietSplineSystem/Blueprints/BP_QuietLoftComponent` Object))
  (`|SetJsonField` TargetJson "StaticMesh" (`/Game/QuietRuntimeEditor/Common/Features/QuietSplineSystem/Blueprints/BP_QuietLoftComponent.GetStaticMesh` _asquietloftcomponent))
  (bind _overridematerial (`/Game/QuietRuntimeEditor/Common/Features/QuietSplineSystem/Blueprints/BP_QuietLoftComponent.GetOverrideMaterial` _asquietloftcomponent))
  (`|SetJsonField` TargetJson "OverrideMaterial" _overridematerial)
  (if _overridematerial
    (`|SetJsonField` TargetJson "Material" (`/Game/QuietRuntimeEditor/Common/Features/QuietSplineSystem/Blueprints/BP_QuietLoftComponent.Material` _asquietloftcomponent)))
  (`|SetJsonField` TargetJson "Shift" (`/Game/QuietRuntimeEditor/Common/Features/QuietSplineSystem/Blueprints/BP_QuietLoftComponent.Shift` _asquietloftcomponent))
  (`|SetJsonField` TargetJson "Offset" (`/Game/QuietRuntimeEditor/Common/Features/QuietSplineSystem/Blueprints/BP_QuietLoftComponent.Offset` _asquietloftcomponent))
  (`|SetJsonField` TargetJson "Twist" (`/Game/QuietRuntimeEditor/Common/Features/QuietSplineSystem/Blueprints/BP_QuietLoftComponent.Twist` _asquietloftcomponent))
  (return))

(fn `SetPropertyValue`
  (params (Object :type "Object Object Reference") (Property :type String) (JsonValue :type "JsonObjectWrapper Structure (by ref)"))
  (returns (Success :type Boolean))
  (bind _asquietloftcomponent (cast `/Game/QuietRuntimeEditor/Common/Features/QuietSplineSystem/Blueprints/BP_QuietLoftComponent` Object))
  (switch `string` Property
    (:`StaticMesh`
      (bind (_newvalue _invaliddata) (`/Game/QuietRuntimeEditor/Common/Blueprints/BP_QuietJsonMacroLibrary.ReadMeshWithCheck` JsonValue Property (`/Game/QuietRuntimeEditor/Common/Features/QuietSplineSystem/Blueprints/BP_QuietLoftComponent.GetStaticMesh` _asquietloftcomponent))
        (:`then`
          (`/Game/QuietRuntimeEditor/Common/Features/QuietSplineSystem/Blueprints/BP_QuietLoftComponent.SetStaticMesh` _asquietloftcomponent _newvalue))
        (:`Null`
          (`/Game/QuietRuntimeEditor/Common/Features/QuietSplineSystem/Blueprints/BP_QuietLoftComponent.SetStaticMesh` _asquietloftcomponent null :!label _label))
        (:`Failed`
          (`self.CheckInvalidData` _invaliddata)
          (goto _label)))
      (`/Game/QuietRuntimeEditor/Common/Features/QuietSplineSystem/Blueprints/BP_QuietLoftComponent.RebuildSpline` _asquietloftcomponent :!label _label_2))
    (:`Shift`
      (bind _newvalue_2 (`/Game/QuietRuntimeEditor/Common/Blueprints/BP_QuietJsonMacroLibrary.ReadFloatWithCheck` JsonValue Property (`/Game/QuietRuntimeEditor/Common/Features/QuietSplineSystem/Blueprints/BP_QuietLoftComponent.Shift` _asquietloftcomponent))
        (:`then`
          (`/Game/QuietRuntimeEditor/Common/Features/QuietSplineSystem/Blueprints/BP_QuietLoftComponent.SetShift` _asquietloftcomponent _newvalue_2))))
    (:`Offset`
      (bind _newvalue_3 (`/Game/QuietRuntimeEditor/Common/Blueprints/BP_QuietJsonMacroLibrary.ReadVectorWithCheck` JsonValue Property (`/Game/QuietRuntimeEditor/Common/Features/QuietSplineSystem/Blueprints/BP_QuietLoftComponent.Offset` _asquietloftcomponent))
        (:`then`
          (`/Game/QuietRuntimeEditor/Common/Features/QuietSplineSystem/Blueprints/BP_QuietLoftComponent.SetLoftOffset` _asquietloftcomponent _newvalue_3))))
    (:`Twist`
      (bind _newvalue_4 (`/Game/QuietRuntimeEditor/Common/Blueprints/BP_QuietJsonMacroLibrary.ReadFloatWithCheck` JsonValue Property (`/Game/QuietRuntimeEditor/Common/Features/QuietSplineSystem/Blueprints/BP_QuietLoftComponent.Twist` _asquietloftcomponent))
        (:`then`
          (set `/Game/QuietRuntimeEditor/Common/Features/QuietSplineSystem/Blueprints/BP_QuietLoftComponent.Twist` _newvalue_4 _asquietloftcomponent)
          (goto _label_2))))
    (:`Material`
      (bind _newvalue_5 (`/Game/QuietRuntimeEditor/Common/Blueprints/BP_QuietJsonMacroLibrary.ReadMaterialWithCheck` JsonValue Property (`/Game/QuietRuntimeEditor/Common/Features/QuietSplineSystem/Blueprints/BP_QuietLoftComponent.Material` _asquietloftcomponent))
        (:`then`
          (`/Game/QuietRuntimeEditor/Common/Features/QuietSplineSystem/Blueprints/BP_QuietLoftComponent.SetMaterial` _asquietloftcomponent _newvalue_5))))
    (:`OverrideMaterial`
      (bind _newvalue_6 (`/Game/QuietRuntimeEditor/Common/Blueprints/BP_QuietJsonMacroLibrary.ReadBoolWithCheck` JsonValue Property (`/Game/QuietRuntimeEditor/Common/Features/QuietSplineSystem/Blueprints/BP_QuietLoftComponent.GetOverrideMaterial` _asquietloftcomponent))
        (:`then`
          (`/Game/QuietRuntimeEditor/Common/Features/QuietSplineSystem/Blueprints/BP_QuietLoftComponent.SetOverrideMaterial` _asquietloftcomponent _newvalue_6)))))
  (return true))