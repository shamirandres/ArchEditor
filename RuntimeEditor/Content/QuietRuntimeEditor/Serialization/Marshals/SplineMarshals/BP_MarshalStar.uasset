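; Marshal for BP_Star spline shapes in the runtime editor, exposing radii, sides and fillets as JSON for editing and serialization.
; Property get and set defer to the parent marshal first, then handle star fields, with checked writes calling UpdateShape to rebuild the shape.
; CollectProperties builds commit-only, range-limited parameters under a "Star" group alongside "Spline".
; SerializeObject appends the star fields to the parent's output.
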(fn `CollectProperties`
  (params (Object :type "Object Object Reference") (TargetJson :type "JsonObjectWrapper Structure (by ref)"))
  (locals (Helix :type "Array of JsonObjectWrapper Structure"))
  (bind _asstaractor (cast `/Game/QuietRuntimeEditor/Common/Features/QuietSplineSystem/Blueprints/BP_Star` Object))
  (bind (_radius1 _radius2 _sides _fillet1 _fillet2) (defaults `Object` (`GameplayStatics.GetObjectClass` _asstaractor)))
  (bind _jsonobject (`self.MakeFloatParam` "Radius1" "Radius 1" "" (`/Game/QuietRuntimeEditor/Common/Features/QuietSplineSystem/Blueprints/BP_Star.Radius1` _asstaractor) _radius1 0.01 0.1 10000.0 1000.0 1 2 true))
  (`KismetArrayLibrary.Array_Add` (`local.Helix`) _jsonobject)
  (bind _jsonobject_2 (`self.MakeFloatParam` "Radius2" "Radius 2" "" (`/Game/QuietRuntimeEditor/Common/Features/QuietSplineSystem/Blueprints/BP_Star.Radius2` _asstaractor) _radius2 0.01 0.1 10000.0 1000.0 1 2 true))
  (`KismetArrayLibrary.Array_Add` (`local.Helix`) _jsonobject_2)
  (bind _jsonobject_3 (`self.MakeIntParam` "Sides" "Sides" "" (`/Game/QuietRuntimeEditor/Common/Features/QuietSplineSystem/Blueprints/BP_Star.Sides` _asstaractor) _sides 3 3 24 24 true))
  (`KismetArrayLibrary.Array_Add` (`local.Helix`) _jsonobject_3)
  (bind _jsonobject_4 (`self.MakeFloatParam` "Fillet1" "Fillet 1" "" (`/Game/QuietRuntimeEditor/Common/Features/QuietSplineSystem/Blueprints/BP_Star.Fillet1` _asstaractor) _fillet1 0.0 0.0 10000.0 100.0 1 2 true))
  (`KismetArrayLibrary.Array_Add` (`local.Helix`) _jsonobject_4)
  (bind _jsonobject_5 (`self.MakeFloatParam` "Fillet2" "Fillet 2" "" (`/Game/QuietRuntimeEditor/Common/Features/QuietSplineSystem/Blueprints/BP_Star.Fillet2` _asstaractor) _fillet2 0.0 0.0 10000.0 100.0 1 2 true))
  (`KismetArrayLibrary.Array_Add` (`local.Helix`) _jsonobject_5)
  (`|SetJsonField` (`local.TargetJson`) "GroupsState" (`|MakeArray` "Star" "Spline"))
  (`|SetJsonField` (`local.TargetJson`) "Star" (`local.Helix`))
  (`parent.CollectProperties` _asstaractor (`local.TargetJson`))
  (return))

(fn `GetPropertyValue`
  (params (Object :type "Object Object Reference") (Property :type String))
  (returns (Success :type Boolean) (Value :type "JsonObjectWrapper Structure"))
  (bind _property (`local.Property`))
  (bind (_success _value) (`parent.GetPropertyValue` Object Property))
  (if (not _success)
    (bind _asstaractor (cast `/Game/QuietRuntimeEditor/Common/Features/QuietSplineSystem/Blueprints/BP_Star` Object))
    (bind _jsonobject (`/Game/QuietRuntimeEditor/Common/Blueprints/BP_QuietJsonFunctionLibrary.NewJson`))
    (switch `string` (`local.Property`)
      (:`Radius1`
        (`|SetJsonField` _jsonobject _property (`/Game/QuietRuntimeEditor/Common/Features/QuietSplineSystem/Blueprints/BP_Star.Radius1` _asstaractor)))
      (:`Radius2`
        (`|SetJsonField` _jsonobject _property (`/Game/QuietRuntimeEditor/Common/Features/QuietSplineSystem/Blueprints/BP_Star.Radius2` _asstaractor)))
      (:`Sides`
        (`|SetJsonField` _jsonobject _property (`/Game/QuietRuntimeEditor/Common/Features/QuietSplineSystem/Blueprints/BP_Star.Sides` _asstaractor)))
      (:`Fillet1`
        (`|SetJsonField` _jsonobject _property (`/Game/QuietRuntimeEditor/Common/Features/QuietSplineSystem/Blueprints/BP_Star.Fillet1` _asstaractor)))
      (:`Fillet2`
        (`|SetJsonField` _jsonobject _property (`/Game/QuietRuntimeEditor/Common/Features/QuietSplineSystem/Blueprints/BP_Star.Fillet2` _asstaractor))))
    (return true _jsonobject)
    (else
      (return true _value))))

(fn `SerializeObject`
  (params (Object :type "Object Object Reference") (TargetJson :type "JsonObjectWrapper Structure (by ref)"))
  (`parent.SerializeObject` Object TargetJson)
  (bind _asstaractor (cast `/Game/QuietRuntimeEditor/Common/Features/QuietSplineSystem/Blueprints/BP_Star` Object))
  (`|SetJsonField` (`local.TargetJson`) "Radius1" (`/Game/QuietRuntimeEditor/Common/Features/QuietSplineSystem/Blueprints/BP_Star.Radius1` _asstaractor))
  (`|SetJsonField` (`local.TargetJson`) "Radius2" (`/Game/QuietRuntimeEditor/Common/Features/QuietSplineSystem/Blueprints/BP_Star.Radius2` _asstaractor))
  (`|SetJsonField` (`local.TargetJson`) "Sides" (`/Game/QuietRuntimeEditor/Common/Features/QuietSplineSystem/Blueprints/BP_Star.Sides` _asstaractor))
  (`|SetJsonField` (`local.TargetJson`) "Fillet1" (`/Game/QuietRuntimeEditor/Common/Features/QuietSplineSystem/Blueprints/BP_Star.Fillet1` _asstaractor))
  (`|SetJsonField` (`local.TargetJson`) "Fillet2" (`/Game/QuietRuntimeEditor/Common/Features/QuietSplineSystem/Blueprints/BP_Star.Fillet2` _asstaractor))
  (return))

(fn `SetPropertyValue`
  (params (Object :type "Object Object Reference") (Property :type String) (JsonValue :type "JsonObjectWrapper Structure (by ref)"))
  (returns (Success :type Boolean))
  (bind _property (`local.Property`))
  (bind _jsonvalue (`local.JsonValue`))
  (bind _success (`parent.SetPropertyValue` Object Property JsonValue))
  (if (not _success)
    (bind _asstaractor (cast `/Game/QuietRuntimeEditor/Common/Features/QuietSplineSystem/Blueprints/BP_Star` Object))
    (switch `string` _property
      (:`Radius1`
        (bind _newvalue (`/Game/QuietRuntimeEditor/Common/Blueprints/BP_QuietJsonMacroLibrary.ReadFloatWithCheck` _jsonvalue _property (`/Game/QuietRuntimeEditor/Common/Features/QuietSplineSystem/Blueprints/BP_Star.Radius1` _asstaractor))
          (:`then`
            (set `/Game/QuietRuntimeEditor/Common/Features/QuietSplineSystem/Blueprints/BP_Star.Radius1` _newvalue _asstaractor))))
      (:`Radius2`
        (bind _newvalue_2 (`/Game/QuietRuntimeEditor/Common/Blueprints/BP_QuietJsonMacroLibrary.ReadFloatWithCheck` _jsonvalue _property (`/Game/QuietRuntimeEditor/Common/Features/QuietSplineSystem/Blueprints/BP_Star.Radius2` _asstaractor))
          (:`then`
            (set `/Game/QuietRuntimeEditor/Common/Features/QuietSplineSystem/Blueprints/BP_Star.Radius2` _newvalue_2 _asstaractor))))
      (:`Sides`
        (bind _newvalue_3 (`/Game/QuietRuntimeEditor/Common/Blueprints/BP_QuietJsonMacroLibrary.ReadIntegerWithCheck` _jsonvalue _property (`/Game/QuietRuntimeEditor/Common/Features/QuietSplineSystem/Blueprints/BP_Star.Sides` _asstaractor))
          (:`then`
            (set `/Game/QuietRuntimeEditor/Common/Features/QuietSplineSystem/Blueprints/BP_Star.Sides` _newvalue_3 _asstaractor))))
      (:`Fillet1`
        (bind _newvalue_4 (`/Game/QuietRuntimeEditor/Common/Blueprints/BP_QuietJsonMacroLibrary.ReadFloatWithCheck` _jsonvalue _property (`/Game/QuietRuntimeEditor/Common/Features/QuietSplineSystem/Blueprints/BP_Star.Fillet1` _asstaractor))
          (:`then`
            (set `/Game/QuietRuntimeEditor/Common/Features/QuietSplineSystem/Blueprints/BP_Star.Fillet1` _newvalue_4 _asstaractor))))
      (:`Fillet2`
        (bind _newvalue_5 (`/Game/QuietRuntimeEditor/Common/Blueprints/BP_QuietJsonMacroLibrary.ReadFloatWithCheck` _jsonvalue _property (`/Game/QuietRuntimeEditor/Common/Features/QuietSplineSystem/Blueprints/BP_Star.Fillet2` _asstaractor))
          (:`then`
            (set `/Game/QuietRuntimeEditor/Common/Features/QuietSplineSystem/Blueprints/BP_Star.Fillet2` _newvalue_5 _asstaractor)))))
    (`/Game/QuietRuntimeEditor/Common/Features/QuietSplineSystem/Blueprints/BP_QuietSplineActorBase.UpdateShape` _asstaractor)
    (return true)
    (else
      (return _success))))