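; Marshal for BP_Ellipse in the runtime editor that exposes and serializes its Length and Width as JSON.
; Get and set defer to the parent marshal first and handle the ellipse fields only if it fails; a set value triggers Refresh on the ellipse.
; CollectProperties builds clamped float parameters in an Ellipse group alongside the parent's properties.
; SerializeObject appends both dimensions to the parent's output.
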(fn `CollectProperties`
  (params (Object :type "Object Object Reference") (TargetJson :type "JsonObjectWrapper Structure (by ref)"))
  (locals (Ellipse :type "Array of JsonObjectWrapper Structure"))
  (bind _asellipseactor (cast `/Game/QuietRuntimeEditor/Common/Features/QuietSplineSystem/Blueprints/BP_Ellipse` Object))
  (bind (_length _width) (defaults `Object` (`GameplayStatics.GetObjectClass` _asellipseactor)))
  (bind _jsonobject (`self.MakeFloatParam` "Length" "Length" "" (`/Game/QuietRuntimeEditor/Common/Features/QuietSplineSystem/Blueprints/BP_Ellipse.Length` _asellipseactor) _length 0.01 0.1 10000.0 1000.0 1 2 true))
  (`KismetArrayLibrary.Array_Add` (`local.Ellipse`) _jsonobject)
  (bind _jsonobject_2 (`self.MakeFloatParam` "Width" "Width" "" (`/Game/QuietRuntimeEditor/Common/Features/QuietSplineSystem/Blueprints/BP_Ellipse.Width` _asellipseactor) _width 0.01 0.1 10000.0 1000.0 1 2 true))
  (`KismetArrayLibrary.Array_Add` (`local.Ellipse`) _jsonobject_2)
  (`|SetJsonField` (`local.TargetJson`) "GroupsState" (`|MakeArray` "Ellipse" "Spline"))
  (`|SetJsonField` (`local.TargetJson`) "Ellipse" (`local.Ellipse`))
  (`parent.CollectProperties` _asellipseactor (`local.TargetJson`))
  (return))

(fn `GetPropertyValue`
  (params (Object :type "Object Object Reference") (Property :type String))
  (returns (Success :type Boolean) (Value :type "JsonObjectWrapper Structure"))
  (bind _property (`local.Property`))
  (bind (_success _value) (`parent.GetPropertyValue` Object Property))
  (if (not _success)
    (bind _asellipseactor (cast `/Game/QuietRuntimeEditor/Common/Features/QuietSplineSystem/Blueprints/BP_Ellipse` Object))
    (bind _jsonobject (`/Game/QuietRuntimeEditor/Common/Blueprints/BP_QuietJsonFunctionLibrary.NewJson`))
    (switch `string` (`local.Property`)
      (:`Length`
        (`|SetJsonField` _jsonobject _property (`/Game/QuietRuntimeEditor/Common/Features/QuietSplineSystem/Blueprints/BP_Ellipse.Length` _asellipseactor)))
      (:`Width`
        (`|SetJsonField` _jsonobject _property (`/Game/QuietRuntimeEditor/Common/Features/QuietSplineSystem/Blueprints/BP_Ellipse.Width` _asellipseactor))))
    (return true _jsonobject)
    (else
      (return true _value))))

(fn `SerializeObject`
  (params (Object :type "Object Object Reference") (TargetJson :type "JsonObjectWrapper Structure (by ref)"))
  (`parent.SerializeObject` Object TargetJson)
  (bind _asellipseactor (cast `/Game/QuietRuntimeEditor/Common/Features/QuietSplineSystem/Blueprints/BP_Ellipse` Object))
  (`|SetJsonField` (`local.TargetJson`) "Length" (`/Game/QuietRuntimeEditor/Common/Features/QuietSplineSystem/Blueprints/BP_Ellipse.Length` _asellipseactor))
  (`|SetJsonField` (`local.TargetJson`) "Width" (`/Game/QuietRuntimeEditor/Common/Features/QuietSplineSystem/Blueprints/BP_Ellipse.Width` _asellipseactor))
  (return))

(fn `SetPropertyValue`
  (params (Object :type "Object Object Reference") (Property :type String) (JsonValue :type "JsonObjectWrapper Structure (by ref)"))
  (returns (Success :type Boolean))
  (bind _property (`local.Property`))
  (bind _jsonvalue (`local.JsonValue`))
  (bind _success (`parent.SetPropertyValue` Object Property JsonValue))
  (if (not _success)
    (bind _asellipseactor (cast `/Game/QuietRuntimeEditor/Common/Features/QuietSplineSystem/Blueprints/BP_Ellipse` Object))
    (switch `string` _property
      (:`Length`
        (bind _newvalue (`/Game/QuietRuntimeEditor/Common/Blueprints/BP_QuietJsonMacroLibrary.ReadFloatWithCheck` _jsonvalue _property (`/Game/QuietRuntimeEditor/Common/Features/QuietSplineSystem/Blueprints/BP_Ellipse.Length` _asellipseactor))
          (:`then`
            (set `/Game/QuietRuntimeEditor/Common/Features/QuietSplineSystem/Blueprints/BP_Ellipse.Length` _newvalue _asellipseactor))))
      (:`Width`
        (bind _newvalue_2 (`/Game/QuietRuntimeEditor/Common/Blueprints/BP_QuietJsonMacroLibrary.ReadFloatWithCheck` _jsonvalue _property (`/Game/QuietRuntimeEditor/Common/Features/QuietSplineSystem/Blueprints/BP_Ellipse.Width` _asellipseactor))
          (:`then`
            (set `/Game/QuietRuntimeEditor/Common/Features/QuietSplineSystem/Blueprints/BP_Ellipse.Width` _newvalue_2 _asellipseactor)))))
    (`/Game/QuietRuntimeEditor/Common/Features/QuietSplineSystem/Blueprints/BP_QuietSplineActorBase.Refresh` _asellipseactor)
    (return true)
    (else
      (return _success))))