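; Marshal for BP_SpacingTool in the runtime editor, converting its mesh, count, randomness, and transform offset properties to and from JSON.
; Get and Set try the parent marshal first, then switch on property name.
; Checked reads gate writes, which call PopulateEvent, except the mesh, which uses SetStaticMesh.
; SerializeObject appends the fields to the parent's output but omits Uniform Scale, whose getter case also lacks the success return.
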(fn `GetPropertyValue`
  (params (Object :type "Object Object Reference") (Property :type String))
  (returns (Success :type Boolean) (Value :type "JsonObjectWrapper Structure"))
  (bind (_success _value) (`parent.GetPropertyValue` Object Property))
  (if (not _success)
    (bind _asspacingtool (cast `/Game/QuietRuntimeEditor/Common/Features/QuietSplineSystem/Blueprints/BP_SpacingTool` Object))
    (bind _jsonobject (`/Game/QuietRuntimeEditor/Common/Blueprints/BP_QuietJsonFunctionLibrary.NewJson`))
    (switch `string` Property
      (:`StaticMesh`
        (`|SetJsonField` _jsonobject Property (`StaticMeshComponent.StaticMesh` _asspacingtool))
        (return true _jsonobject))
      (:`Count`
        (`|SetJsonField` _jsonobject Property (`/Game/QuietRuntimeEditor/Common/Features/QuietSplineSystem/Blueprints/BP_SpacingTool.Count` _asspacingtool))
        (return true _jsonobject))
      (:`RandomHoleChance`
        (`|SetJsonField` _jsonobject Property (`/Game/QuietRuntimeEditor/Common/Features/QuietSplineSystem/Blueprints/BP_SpacingTool.RandomHoleChance` _asspacingtool))
        (return true _jsonobject))
      (:`StartOffset`
        (`|SetJsonField` _jsonobject Property (`/Game/QuietRuntimeEditor/Common/Features/QuietSplineSystem/Blueprints/BP_SpacingTool.StartOffset` _asspacingtool))
        (return true _jsonobject))
      (:`EndOffset`
        (`|SetJsonField` _jsonobject Property (`/Game/QuietRuntimeEditor/Common/Features/QuietSplineSystem/Blueprints/BP_SpacingTool.EndOffset` _asspacingtool))
        (return true _jsonobject))
      (:`RandomOffset`
        (`|SetJsonField` _jsonobject Property (`/Game/QuietRuntimeEditor/Common/Features/QuietSplineSystem/Blueprints/BP_SpacingTool.RandomOffset` _asspacingtool))
        (return true _jsonobject))
      (:`Bias`
        (`|SetJsonField` _jsonobject Property (`/Game/QuietRuntimeEditor/Common/Features/QuietSplineSystem/Blueprints/BP_SpacingTool.Bias` _asspacingtool))
        (return true _jsonobject))
      (:`Shift`
        (`|SetJsonField` _jsonobject Property (`/Game/QuietRuntimeEditor/Common/Features/QuietSplineSystem/Blueprints/BP_SpacingTool.Shift` _asspacingtool))
        (return true _jsonobject))
      (:`StartRotationOffset`
        (`|SetJsonField` _jsonobject Property (`/Game/QuietRuntimeEditor/Common/Features/QuietSplineSystem/Blueprints/BP_SpacingTool.StartRotationOffset` _asspacingtool))
        (return true _jsonobject))
      (:`EndRotationOffset`
        (`|SetJsonField` _jsonobject Property (`/Game/QuietRuntimeEditor/Common/Features/QuietSplineSystem/Blueprints/BP_SpacingTool.EndRotationOffset` _asspacingtool))
        (return true _jsonobject))
      (:`RandomRotationOffset`
        (`|SetJsonField` _jsonobject Property (`/Game/QuietRuntimeEditor/Common/Features/QuietSplineSystem/Blueprints/BP_SpacingTool.RandomRotation` _asspacingtool))
        (return true _jsonobject))
      (:`StartScaleOffset`
        (`|SetJsonField` _jsonobject Property (`/Game/QuietRuntimeEditor/Common/Features/QuietSplineSystem/Blueprints/BP_SpacingTool.StartScaleOffset` _asspacingtool))
        (return true _jsonobject))
      (:`EndScaleOffset`
        (`|SetJsonField` _jsonobject Property (`/Game/QuietRuntimeEditor/Common/Features/QuietSplineSystem/Blueprints/BP_SpacingTool.EndScaleOffset` _asspacingtool))
        (return true _jsonobject))
      (:`RandomScaleOffset`
        (`|SetJsonField` _jsonobject Property (`/Game/QuietRuntimeEditor/Common/Features/QuietSplineSystem/Blueprints/BP_SpacingTool.RandomScaleOffset` _asspacingtool))
        (return true _jsonobject))
      (:`UniformScale`
        (`|SetJsonField` _jsonobject Property (`/Game/QuietRuntimeEditor/Common/Features/QuietSplineSystem/Blueprints/BP_SpacingTool.UniformScale` _asspacingtool))))
    (else
      (return true _value))))

(fn `SerializeObject`
  (params (Object :type "Object Object Reference") (TargetJson :type "JsonObjectWrapper Structure (by ref)"))
  (`parent.SerializeObject` Object TargetJson)
  (bind _asspacingtool (cast `/Game/QuietRuntimeEditor/Common/Features/QuietSplineSystem/Blueprints/BP_SpacingTool` Object))
  (`|SetJsonField` TargetJson "StaticMesh" (`StaticMeshComponent.StaticMesh` _asspacingtool))
  (`|SetJsonField` TargetJson "Count" (`/Game/QuietRuntimeEditor/Common/Features/QuietSplineSystem/Blueprints/BP_SpacingTool.Count` _asspacingtool))
  (`|SetJsonField` TargetJson "RandomHoleChance" (`/Game/QuietRuntimeEditor/Common/Features/QuietSplineSystem/Blueprints/BP_SpacingTool.RandomHoleChance` _asspacingtool))
  (`|SetJsonField` TargetJson "StartOffset" (`/Game/QuietRuntimeEditor/Common/Features/QuietSplineSystem/Blueprints/BP_SpacingTool.StartOffset` _asspacingtool))
  (`|SetJsonField` TargetJson "EndOffset" (`/Game/QuietRuntimeEditor/Common/Features/QuietSplineSystem/Blueprints/BP_SpacingTool.EndOffset` _asspacingtool))
  (`|SetJsonField` TargetJson "RandomOffset" (`/Game/QuietRuntimeEditor/Common/Features/QuietSplineSystem/Blueprints/BP_SpacingTool.RandomOffset` _asspacingtool))
  (`|SetJsonField` TargetJson "Bias" (`/Game/QuietRuntimeEditor/Common/Features/QuietSplineSystem/Blueprints/BP_SpacingTool.Bias` _asspacingtool))
  (`|SetJsonField` TargetJson "Shift" (`/Game/QuietRuntimeEditor/Common/Features/QuietSplineSystem/Blueprints/BP_SpacingTool.Shift` _asspacingtool))
  (`|SetJsonField` TargetJson "StartRotationOffset" (`/Game/QuietRuntimeEditor/Common/Features/QuietSplineSystem/Blueprints/BP_SpacingTool.StartRotationOffset` _asspacingtool))
  (`|SetJsonField` TargetJson "EndRotationOffset" (`/Game/QuietRuntimeEditor/Common/Features/QuietSplineSystem/Blueprints/BP_SpacingTool.EndRotationOffset` _asspacingtool))
  (`|SetJsonField` TargetJson "RandomRotationOffset" (`/Game/QuietRuntimeEditor/Common/Features/QuietSplineSystem/Blueprints/BP_SpacingTool.RandomRotation` _asspacingtool))
  (`|SetJsonField` TargetJson "StartScaleOffset" (`/Game/QuietRuntimeEditor/Common/Features/QuietSplineSystem/Blueprints/BP_SpacingTool.StartScaleOffset` _asspacingtool))
  (`|SetJsonField` TargetJson "EndScaleOffset" (`/Game/QuietRuntimeEditor/Common/Features/QuietSplineSystem/Blueprints/BP_SpacingTool.EndScaleOffset` _asspacingtool))
  (`|SetJsonField` TargetJson "RandomScaleOffset" (`/Game/QuietRuntimeEditor/Common/Features/QuietSplineSystem/Blueprints/BP_SpacingTool.RandomScaleOffset` _asspacingtool))
  (return))

(fn `SetPropertyValue`
  (params (Object :type "Object Object Reference") (Property :type String) (JsonValue :type "JsonObjectWrapper Structure (by ref)"))
  (returns (Success :type Boolean))
  (bind _success (`parent.SetPropertyValue` Object Property JsonValue))
  (if (not _success)
    (bind _asspacingtool (cast `/Game/QuietRuntimeEditor/Common/Features/QuietSplineSystem/Blueprints/BP_SpacingTool` Object))
    (switch `string` Property
      (:`StaticMesh`
        (bind _newvalue (`/Game/QuietRuntimeEditor/Common/Blueprints/BP_QuietJsonMacroLibrary.ReadMeshWithCheck` JsonValue Property (`StaticMeshComponent.StaticMesh` _asspacingtool))
          (:`then`
            (`StaticMeshComponent.SetStaticMesh` _asspacingtool _newvalue))))
      (:`Count`
        (bind _newvalue_2 (`/Game/QuietRuntimeEditor/Common/Blueprints/BP_QuietJsonMacroLibrary.ReadIntegerWithCheck` JsonValue Property (`/Game/QuietRuntimeEditor/Common/Features/QuietSplineSystem/Blueprints/BP_SpacingTool.Count` _asspacingtool))
          (:`then`
            (set `/Game/QuietRuntimeEditor/Common/Features/QuietSplineSystem/Blueprints/BP_SpacingTool.Count` _newvalue_2 _asspacingtool)
            (`/Game/QuietRuntimeEditor/Common/Features/QuietSplineSystem/Blueprints/BP_SpacingTool.PopulateEvent` _asspacingtool :!label _label))))
      (:`RandomHoleChance`
        (bind _newvalue_3 (`/Game/QuietRuntimeEditor/Common/Blueprints/BP_QuietJsonMacroLibrary.ReadIntegerWithCheck` JsonValue Property (`/Game/QuietRuntimeEditor/Common/Features/QuietSplineSystem/Blueprints/BP_SpacingTool.RandomHoleChance` _asspacingtool))
          (:`then`
            (set `/Game/QuietRuntimeEditor/Common/Features/QuietSplineSystem/Blueprints/BP_SpacingTool.RandomHoleChance` _newvalue_3 _asspacingtool)
            (goto _label))))
      (:`StartOffset`
        (bind _newvalue_4 (`/Game/QuietRuntimeEditor/Common/Blueprints/BP_QuietJsonMacroLibrary.ReadVectorWithCheck` JsonValue Property (`/Game/QuietRuntimeEditor/Common/Features/QuietSplineSystem/Blueprints/BP_SpacingTool.StartOffset` _asspacingtool))
          (:`then`
            (set `/Game/QuietRuntimeEditor/Common/Features/QuietSplineSystem/Blueprints/BP_SpacingTool.StartOffset` _newvalue_4 _asspacingtool)
            (goto _label))))
      (:`EndOffset`
        (bind _newvalue_5 (`/Game/QuietRuntimeEditor/Common/Blueprints/BP_QuietJsonMacroLibrary.ReadVectorWithCheck` JsonValue Property (`/Game/QuietRuntimeEditor/Common/Features/QuietSplineSystem/Blueprints/BP_SpacingTool.EndOffset` _asspacingtool))
          (:`then`
            (set `/Game/QuietRuntimeEditor/Common/Features/QuietSplineSystem/Blueprints/BP_SpacingTool.EndOffset` _newvalue_5 _asspacingtool)
            (goto _label))))
      (:`RandomOffset`
        (bind _newvalue_6 (`/Game/QuietRuntimeEditor/Common/Blueprints/BP_QuietJsonMacroLibrary.ReadVectorWithCheck` JsonValue Property (`/Game/QuietRuntimeEditor/Common/Features/QuietSplineSystem/Blueprints/BP_SpacingTool.RandomOffset` _asspacingtool))
          (:`then`
            (set `/Game/QuietRuntimeEditor/Common/Features/QuietSplineSystem/Blueprints/BP_SpacingTool.RandomOffset` _newvalue_6 _asspacingtool)
            (goto _label))))
      (:`Bias`
        (bind _newvalue_7 (`/Game/QuietRuntimeEditor/Common/Blueprints/BP_QuietJsonMacroLibrary.ReadFloatWithCheck` JsonValue Property (`/Game/QuietRuntimeEditor/Common/Features/QuietSplineSystem/Blueprints/BP_SpacingTool.Bias` _asspacingtool))
          (:`then`
            (set `/Game/QuietRuntimeEditor/Common/Features/QuietSplineSystem/Blueprints/BP_SpacingTool.Bias` _newvalue_7 _asspacingtool)
            (goto _label))))
      (:`Shift`
        (bind _newvalue_8 (`/Game/QuietRuntimeEditor/Common/Blueprints/BP_QuietJsonMacroLibrary.ReadFloatWithCheck` JsonValue Property (`/Game/QuietRuntimeEditor/Common/Features/QuietSplineSystem/Blueprints/BP_SpacingTool.Shift` _asspacingtool))
          (:`then`
            (set `/Game/QuietRuntimeEditor/Common/Features/QuietSplineSystem/Blueprints/BP_SpacingTool.Shift` _newvalue_8 _asspacingtool)
            (goto _label))))
      (:`StartRotationOffset`
        (bind _newvalue_9 (`/Game/QuietRuntimeEditor/Common/Blueprints/BP_QuietJsonMacroLibrary.ReadRotatorWithCheck` JsonValue Property (`/Game/QuietRuntimeEditor/Common/Features/QuietSplineSystem/Blueprints/BP_SpacingTool.StartRotationOffset` _asspacingtool))
          (:`then`
            (set `/Game/QuietRuntimeEditor/Common/Features/QuietSplineSystem/Blueprints/BP_SpacingTool.StartRotationOffset` _newvalue_9 _asspacingtool)
            (goto _label))))
      (:`EndRotationOffset`
        (bind _newvalue_10 (`/Game/QuietRuntimeEditor/Common/Blueprints/BP_QuietJsonMacroLibrary.ReadRotatorWithCheck` JsonValue Property (`/Game/QuietRuntimeEditor/Common/Features/QuietSplineSystem/Blueprints/BP_SpacingTool.EndRotationOffset` _asspacingtool))
          (:`then`
            (set `/Game/QuietRuntimeEditor/Common/Features/QuietSplineSystem/Blueprints/BP_SpacingTool.EndRotationOffset` _newvalue_10 _asspacingtool)
            (goto _label))))
      (:`RandomRotationOffset`
        (bind _newvalue_11 (`/Game/QuietRuntimeEditor/Common/Blueprints/BP_QuietJsonMacroLibrary.ReadRotatorWithCheck` JsonValue Property (`/Game/QuietRuntimeEditor/Common/Features/QuietSplineSystem/Blueprints/BP_SpacingTool.RandomRotation` _asspacingtool))
          (:`then`
            (set `/Game/QuietRuntimeEditor/Common/Features/QuietSplineSystem/Blueprints/BP_SpacingTool.RandomRotation` _newvalue_11 _asspacingtool)
            (goto _label))))
      (:`StartScaleOffset`
        (bind _newvalue_12 (`/Game/QuietRuntimeEditor/Common/Blueprints/BP_QuietJsonMacroLibrary.ReadVectorWithCheck` JsonValue Property (`/Game/QuietRuntimeEditor/Common/Features/QuietSplineSystem/Blueprints/BP_SpacingTool.StartScaleOffset` _asspacingtool))
          (:`then`
            (set `/Game/QuietRuntimeEditor/Common/Features/QuietSplineSystem/Blueprints/BP_SpacingTool.StartScaleOffset` _newvalue_12 _asspacingtool)
            (goto _label))))
      (:`EndScaleOffset`
        (bind _newvalue_13 (`/Game/QuietRuntimeEditor/Common/Blueprints/BP_QuietJsonMacroLibrary.ReadVectorWithCheck` JsonValue Property (`/Game/QuietRuntimeEditor/Common/Features/QuietSplineSystem/Blueprints/BP_SpacingTool.EndScaleOffset` _asspacingtool))
          (:`then`
            (set `/Game/QuietRuntimeEditor/Common/Features/QuietSplineSystem/Blueprints/BP_SpacingTool.EndScaleOffset` _newvalue_13 _asspacingtool)
            (goto _label))))
      (:`RandomScaleOffset`
        (bind _newvalue_14 (`/Game/QuietRuntimeEditor/Common/Blueprints/BP_QuietJsonMacroLibrary.ReadVectorWithCheck` JsonValue Property (`/Game/QuietRuntimeEditor/Common/Features/QuietSplineSystem/Blueprints/BP_SpacingTool.RandomScaleOffset` _asspacingtool))
          (:`then`
            (set `/Game/QuietRuntimeEditor/Common/Features/QuietSplineSystem/Blueprints/BP_SpacingTool.RandomScaleOffset` _newvalue_14 _asspacingtool)
            (goto _label))))
      (:`UniformScale`
        (bind _newvalue_15 (`/Game/QuietRuntimeEditor/Common/Blueprints/BP_QuietJsonMacroLibrary.ReadBoolWithCheck` JsonValue Property (`/Game/QuietRuntimeEditor/Common/Features/QuietSplineSystem/Blueprints/BP_SpacingTool.UniformScale` _asspacingtool))
          (:`then`
            (set `/Game/QuietRuntimeEditor/Common/Features/QuietSplineSystem/Blueprints/BP_SpacingTool.UniformScale` _newvalue_15 _asspacingtool)
            (goto _label)))))
    (return true)
    (else
      (return true))))