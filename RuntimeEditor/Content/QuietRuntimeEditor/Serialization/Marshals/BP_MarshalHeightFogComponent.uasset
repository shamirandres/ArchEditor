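; Runtime editor marshal that exposes Exponential Height Fog components to JSON-based property editing and serialization.
; SetPropertyValue and GetPropertyValue defer to the parent first, then match fog properties by name; writes check against current values before calling component setters.
; SerializeObject appends all fog fields to the parent's output.
; CollectProperties builds typed parameters with defaults and slider limits in height fog, inscattering texture, directional and volumetric groups, then calls the parent.
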(fn `CollectProperties`
  (params (Object :type "Object Object Reference") (TargetJson :type "JsonObjectWrapper Structure (by ref)"))
  (locals (HeightFog :type "Array of JsonObjectWrapper Structure") (InscatteringTexture :type "Array of JsonObjectWrapper Structure") (Directional :type "Array of JsonObjectWrapper Structure") (Volumetric :type "Array of JsonObjectWrapper Structure"))
  (bind _asexponential_height_fog_component (cast `ExponentialHeightFogComponent` Object))
  (`|ExecutionSequence`
    (:`then_0`
      (bind _jsonobject (`self.MakeFloatParam` "FogDensity" "Fog Density" "" (`ExponentialHeightFogComponent.FogDensity` _asexponential_height_fog_component) 0.05 0.0 0.0 10.0 0.05 1 4))
      (`KismetArrayLibrary.Array_Add` (`local.HeightFog`) _jsonobject)
      (bind _jsonobject_2 (`self.MakeFloatParam` "FogHeightFalloff" "Fog Height Falloff" "" (`ExponentialHeightFogComponent.FogHeightFalloff` _asexponential_height_fog_component) 0.2 0.0 0.001 2.0 2.0 1 4))
      (`KismetArrayLibrary.Array_Add` (`local.HeightFog`) _jsonobject_2)
      (bind _jsonobject_3 (`self.MakeLinearColorParam` "FogInscatteringColor" "Fog Inscattering Color" "" (`ExponentialHeightFogComponent.FogInscatteringLuminance` _asexponential_height_fog_component)))
      (`KismetArrayLibrary.Array_Add` (`local.HeightFog`) _jsonobject_3)
      (bind _jsonobject_4 (`self.MakeFloatParam` "FogMaxOpacity" "Fog Max Opacity" "" (`ExponentialHeightFogComponent.FogMaxOpacity` _asexponential_height_fog_component) 1.0 0.0 0.0 1.0 1.0 1 3))
      (`KismetArrayLibrary.Array_Add` (`local.HeightFog`) _jsonobject_4)
      (bind _jsonobject_5 (`self.MakeFloatParam` "StartDistance" "Start Distance" "" (`ExponentialHeightFogComponent.StartDistance` _asexponential_height_fog_component) 0.0 0.0 0.0 100000.0 5000.0 1 1))
      (`KismetArrayLibrary.Array_Add` (`local.HeightFog`) _jsonobject_5)
      (bind _jsonobject_6 (`self.MakeFloatParam` "FogCutoffDistance" "Fog Cutoff Distance" "" (`ExponentialHeightFogComponent.FogCutoffDistance` _asexponential_height_fog_component) 0.0 0.0 0.0 0.0 0.0 1 1))
      (`KismetArrayLibrary.Array_Add` (`local.HeightFog`) _jsonobject_6))
    (:`then_1`
      (bind _jsonobject_7 (`self.MakeObjectParam` "InscatteringColorCubemap" "Cubemap" "" "/Script/Engine.TextureCube" (`ExponentialHeightFogComponent.InscatteringColorCubemap` _asexponential_height_fog_component)))
      (`KismetArrayLibrary.Array_Add` (`local.InscatteringTexture`) _jsonobject_7)
      (bind _jsonobject_8 (`self.MakeFloatParam` "InscatteringColorCubemapAngle" "Cubemap Angle" "" (`ExponentialHeightFogComponent.InscatteringColorCubemapAngle` _asexponential_height_fog_component) 0.0 -360.0 -180.0 360.0 180.0 1 2))
      (`KismetArrayLibrary.Array_Add` (`local.InscatteringTexture`) _jsonobject_8)
      (bind _jsonobject_9 (`self.MakeLinearColorParam` "InscatteringTextureTint" "Texture Tint" "" (`ExponentialHeightFogComponent.InscatteringTextureTint` _asexponential_height_fog_component) (struct :`R` 1.0 :`G` 1.0 :`B` 1.0 :`A` 1.0)))
      (`KismetArrayLibrary.Array_Add` (`local.InscatteringTexture`) _jsonobject_9)
      (bind _jsonobject_10 (`self.MakeFloatParam` "DirectionalInscatteringExponent" "Exponent" "" (`ExponentialHeightFogComponent.DirectionalInscatteringExponent` _asexponential_height_fog_component) 4.0 0.0 2.0 1000.0 64.0 1 3))
      (`KismetArrayLibrary.Array_Add` (`local.Directional`) _jsonobject_10)
      (bind _jsonobject_11 (`self.MakeFloatParam` "DirectionalInscatteringStartDistance" "Start Distance" "" (`ExponentialHeightFogComponent.DirectionalInscatteringStartDistance` _asexponential_height_fog_component) 10000.0))
      (`KismetArrayLibrary.Array_Add` (`local.Directional`) _jsonobject_11)
      (bind _jsonobject_12 (`self.MakeLinearColorParam` "DirectionalInscatteringColor" "Color" "" (`ExponentialHeightFogComponent.DirectionalInscatteringLuminance` _asexponential_height_fog_component)))
      (`KismetArrayLibrary.Array_Add` (`local.Directional`) _jsonobject_12))
    (:`then_2`
      (bind _jsonobject_13 (`self.MakeBoolParam` "VolumetricFog" "Volumetric Fog" "" (`ExponentialHeightFogComponent.bEnableVolumetricFog` _asexponential_height_fog_component)))
      (`KismetArrayLibrary.Array_Add` (`local.Volumetric`) _jsonobject_13)
      (bind _jsonobject_14 (`self.MakeFloatParam` "ScatteringDistribution" "Scattering Distribution" "" (`ExponentialHeightFogComponent.VolumetricFogScatteringDistribution` _asexponential_height_fog_component) 0.2 -1000.0 -0.9 1000.0 0.9 1 3))
      (`KismetArrayLibrary.Array_Add` (`local.Volumetric`) _jsonobject_14)
      (bind _jsonobject_15 (`self.MakeLinearColorParam` "Albedo" "Albedo" "" (`KismetMathLibrary.Conv_ColorToLinearColor` (`ExponentialHeightFogComponent.VolumetricFogAlbedo` _asexponential_height_fog_component)) (struct :`R` 1.0 :`G` 1.0 :`B` 1.0 :`A` 1.0)))
      (`KismetArrayLibrary.Array_Add` (`local.Volumetric`) _jsonobject_15)
      (bind _jsonobject_16 (`self.MakeLinearColorParam` "Emissive" "Emissive" "" (`ExponentialHeightFogComponent.VolumetricFogEmissive` _asexponential_height_fog_component)))
      (`KismetArrayLibrary.Array_Add` (`local.Volumetric`) _jsonobject_16)
      (bind _jsonobject_17 (`self.MakeFloatParam` "ExtinctionScale" "Extinction Scale" "" (`ExponentialHeightFogComponent.VolumetricFogExtinctionScale` _asexponential_height_fog_component) 1.0 0.0 0.1 1000.0 10.0 1 4))
      (`KismetArrayLibrary.Array_Add` (`local.Volumetric`) _jsonobject_17)
      (`|SetJsonField` (`local.TargetJson`) "GroupsState" (`|MakeArray` "Exponential Height Fog" "Inscattering Texture"))
      (`|SetJsonField` (`local.TargetJson`) "Exponential Height Fog" (`local.HeightFog`))
      (`|SetJsonField` (`local.TargetJson`) "Inscattering Texture" (`local.InscatteringTexture`))
      (`|SetJsonField` (`local.TargetJson`) "Directional Inscattering" (`local.Directional`))
      (`|SetJsonField` (`local.TargetJson`) "Volumetric Fog" (`local.Volumetric`))
      (`parent.CollectProperties` _asexponential_height_fog_component (`local.TargetJson`))
      (return))))

(fn `GetPropertyValue`
  (params (Object :type "Object Object Reference") (Property :type String))
  (returns (Success :type Boolean) (Value :type "JsonObjectWrapper Structure"))
  (bind _property (`local.Property`))
  (bind (_success _value) (`parent.GetPropertyValue` Object Property))
  (if (not _success)
    (bind _asexponential_height_fog_component (cast `ExponentialHeightFogComponent` Object))
    (bind _jsonobject (`/Game/QuietRuntimeEditor/Common/Blueprints/BP_QuietJsonFunctionLibrary.NewJson`))
    (switch `string` _property
      (:`FogDensity`
        (`|SetJsonField` _jsonobject _property (`ExponentialHeightFogComponent.FogDensity` _asexponential_height_fog_component)))
      (:`FogHeightFalloff`
        (`|SetJsonField` _jsonobject _property (`ExponentialHeightFogComponent.FogHeightFalloff` _asexponential_height_fog_component)))
      (:`FogInscatteringColor`
        (`|SetJsonField` _jsonobject _property (`ExponentialHeightFogComponent.FogInscatteringLuminance` _asexponential_height_fog_component)))
      (:`FogMaxOpacity`
        (`|SetJsonField` _jsonobject _property (`ExponentialHeightFogComponent.FogMaxOpacity` _asexponential_height_fog_component)))
      (:`StartDistance`
        (`|SetJsonField` _jsonobject _property (`ExponentialHeightFogComponent.StartDistance` _asexponential_height_fog_component)))
      (:`FogCutoffDistance`
        (`|SetJsonField` _jsonobject _property (`ExponentialHeightFogComponent.FogCutoffDistance` _asexponential_height_fog_component)))
      (:`InscatteringColorCubemap`
        (`|SetJsonField` _jsonobject _property (`ExponentialHeightFogComponent.InscatteringColorCubemap` _asexponential_height_fog_component)))
      (:`InscatteringColorCubemapAngle`
        (`|SetJsonField` _jsonobject _property (`ExponentialHeightFogComponent.InscatteringColorCubemapAngle` _asexponential_height_fog_component)))
      (:`InscatteringTextureTint`
        (`|SetJsonField` _jsonobject _property (`ExponentialHeightFogComponent.InscatteringTextureTint` _asexponential_height_fog_component)))
      (:`DirectionalInscatteringExponent`
        (`|SetJsonField` _jsonobject _property (`ExponentialHeightFogComponent.DirectionalInscatteringExponent` _asexponential_height_fog_component)))
      (:`DirectionalInscatteringStartDistance`
        (`|SetJsonField` _jsonobject _property (`ExponentialHeightFogComponent.DirectionalInscatteringStartDistance` _asexponential_height_fog_component)))
      (:`DirectionalInscatteringColor`
        (`|SetJsonField` _jsonobject _property (`ExponentialHeightFogComponent.DirectionalInscatteringLuminance` _asexponential_height_fog_component)))
      (:`VolumetricFog`
        (`|SetJsonField` _jsonobject _property (`ExponentialHeightFogComponent.bEnableVolumetricFog` _asexponential_height_fog_component)))
      (:`ScatteringDistribution`
        (`|SetJsonField` _jsonobject _property (`ExponentialHeightFogComponent.VolumetricFogScatteringDistribution` _asexponential_height_fog_component)))
      (:`Albedo`
        (`|SetJsonField` _jsonobject _property (`ExponentialHeightFogComponent.VolumetricFogAlbedo` _asexponential_height_fog_component)))
      (:`Emissive`
        (`|SetJsonField` _jsonobject _property (`ExponentialHeightFogComponent.VolumetricFogEmissive` _asexponential_height_fog_component)))
      (:`ExtinctionScale`
        (`|SetJsonField` _jsonobject _property (`ExponentialHeightFogComponent.VolumetricFogExtinctionScale` _asexponential_height_fog_component))))
    (return true _jsonobject)
    (else
      (return true _value))))

(fn `SerializeObject`
  (params (Object :type "Object Object Reference") (TargetJson :type "JsonObjectWrapper Structure (by ref)"))
  (`parent.SerializeObject` Object TargetJson)
  (bind _asexponential_height_fog_component (cast `ExponentialHeightFogComponent` Object))
  (`|SetJsonField` (`local.TargetJson`) "FogDensity" (`ExponentialHeightFogComponent.FogDensity` _asexponential_height_fog_component))
  (`|SetJsonField` (`local.TargetJson`) "FogHeightFalloff" (`ExponentialHeightFogComponent.FogHeightFalloff` _asexponential_height_fog_component))
  (`|SetJsonField` (`local.TargetJson`) "FogInscatteringColor" (`ExponentialHeightFogComponent.FogInscatteringLuminance` _asexponential_height_fog_component))
  (`|SetJsonField` (`local.TargetJson`) "FogMaxOpacity" (`ExponentialHeightFogComponent.FogMaxOpacity` _asexponential_height_fog_component))
  (`|SetJsonField` (`local.TargetJson`) "StartDistance" (`ExponentialHeightFogComponent.StartDistance` _asexponential_height_fog_component))
  (`|SetJsonField` (`local.TargetJson`) "FogCutoffDistance" (`ExponentialHeightFogComponent.FogCutoffDistance` _asexponential_height_fog_component))
  (`|SetJsonField` (`local.TargetJson`) "InscatteringColorCubemap" (`ExponentialHeightFogComponent.InscatteringColorCubemap` _asexponential_height_fog_component))
  (`|SetJsonField` (`local.TargetJson`) "InscatteringColorCubemapAngle" (`ExponentialHeightFogComponent.InscatteringColorCubemapAngle` _asexponential_height_fog_component))
  (`|SetJsonField` (`local.TargetJson`) "InscatteringTextureTint" (`ExponentialHeightFogComponent.InscatteringTextureTint` _asexponential_height_fog_component))
  (`|SetJsonField` (`local.TargetJson`) "DirectionalInscatteringExponent" (`ExponentialHeightFogComponent.DirectionalInscatteringExponent` _asexponential_height_fog_component))
  (`|SetJsonField` (`local.TargetJson`) "DirectionalInscatteringStartDistance" (`ExponentialHeightFogComponent.DirectionalInscatteringStartDistance` _asexponential_height_fog_component))
  (`|SetJsonField` (`local.TargetJson`) "DirectionalInscatteringColor" (`ExponentialHeightFogComponent.DirectionalInscatteringLuminance` _asexponential_height_fog_component))
  (`|SetJsonField` (`local.TargetJson`) "VolumetricFog" (`ExponentialHeightFogComponent.bEnableVolumetricFog` _asexponential_height_fog_component))
  (`|SetJsonField` (`local.TargetJson`) "ScatteringDistribution" (`ExponentialHeightFogComponent.VolumetricFogScatteringDistribution` _asexponential_height_fog_component))
  (`|SetJsonField` (`local.TargetJson`) "Albedo" (`ExponentialHeightFogComponent.VolumetricFogAlbedo` _asexponential_height_fog_component))
  (`|SetJsonField` (`local.TargetJson`) "Emissive" (`ExponentialHeightFogComponent.VolumetricFogEmissive` _asexponential_height_fog_component))
  (`|SetJsonField` (`local.TargetJson`) "ExtinctionScale" (`ExponentialHeightFogComponent.VolumetricFogExtinctionScale` _asexponential_height_fog_component))
  (return))

(fn `SetPropertyValue`
  (params (Object :type "Object Object Reference") (Property :type String) (JsonValue :type "JsonObjectWrapper Structure (by ref)"))
  (returns (Success :type Boolean))
  (bind _property (`local.Property`))
  (bind _jsonvalue (`local.JsonValue`))
  (bind _success (`parent.SetPropertyValue` Object Property JsonValue))
  (if (not _success)
    (bind _asexponential_height_fog_component (cast `ExponentialHeightFogComponent` Object))
    (switch `string` _property
      (:`FogDensity`
        (bind _newvalue (`/Game/QuietRuntimeEditor/Common/Blueprints/BP_QuietJsonMacroLibrary.ReadFloatWithCheck` _jsonvalue _property (`ExponentialHeightFogComponent.FogDensity` _asexponential_height_fog_component))
          (:`then`
            (`ExponentialHeightFogComponent.SetFogDensity` _asexponential_height_fog_component _newvalue)
            (return true))))
      (:`FogHeightFalloff`
        (bind _newvalue_2 (`/Game/QuietRuntimeEditor/Common/Blueprints/BP_QuietJsonMacroLibrary.ReadFloatWithCheck` _jsonvalue _property (`ExponentialHeightFogComponent.FogHeightFalloff` _asexponential_height_fog_component))
          (:`then`
            (`ExponentialHeightFogComponent.SetFogHeightFalloff` _asexponential_height_fog_component _newvalue_2)
            (return true))))
      (:`FogInscatteringColor`
        (bind _newvalue_3 (`/Game/QuietRuntimeEditor/Common/Blueprints/BP_QuietJsonMacroLibrary.ReadLinearColorWithCheck` _jsonvalue _property (`ExponentialHeightFogComponent.FogInscatteringLuminance` _asexponential_height_fog_component))
          (:`then`
            (`ExponentialHeightFogComponent.SetFogInscatteringColor` _asexponential_height_fog_component _newvalue_3)
            (return true))))
      (:`FogMaxOpacity`
        (bind _newvalue_4 (`/Game/QuietRuntimeEditor/Common/Blueprints/BP_QuietJsonMacroLibrary.ReadFloatWithCheck` _jsonvalue _property (`ExponentialHeightFogComponent.FogMaxOpacity` _asexponential_height_fog_component))
          (:`then`
            (`ExponentialHeightFogComponent.SetFogMaxOpacity` _asexponential_height_fog_component _newvalue_4)
            (return true))))
      (:`StartDistance`
        (bind _newvalue_5 (`/Game/QuietRuntimeEditor/Common/Blueprints/BP_QuietJsonMacroLibrary.ReadFloatWithCheck` _jsonvalue _property (`ExponentialHeightFogComponent.StartDistance` _asexponential_height_fog_component))
          (:`then`
            (`ExponentialHeightFogComponent.SetStartDistance` _asexponential_height_fog_component _newvalue_5)
            (return true))))
      (:`FogCutoffDistance`
        (bind _newvalue_6 (`/Game/QuietRuntimeEditor/Common/Blueprints/BP_QuietJsonMacroLibrary.ReadFloatWithCheck` _jsonvalue _property (`ExponentialHeightFogComponent.FogCutoffDistance` _asexponential_height_fog_component))
          (:`then`
            (`ExponentialHeightFogComponent.SetFogCutoffDistance` _asexponential_height_fog_component _newvalue_6)
            (return true))))
      (:`InscatteringColorCubemap`
        (bind _outvalue (`|GetJsonField` _jsonvalue _property))
        (if (!= _outvalue (`ExponentialHeightFogComponent.InscatteringColorCubemap` _asexponential_height_fog_component))
          (`ExponentialHeightFogComponent.SetInscatteringColorCubemap` _asexponential_height_fog_component _outvalue)
          (return true)))
      (:`InscatteringColorCubemapAngle`
        (bind _newvalue_7 (`/Game/QuietRuntimeEditor/Common/Blueprints/BP_QuietJsonMacroLibrary.ReadFloatWithCheck` _jsonvalue _property (`ExponentialHeightFogComponent.InscatteringColorCubemapAngle` _asexponential_height_fog_component))
          (:`then`
            (`ExponentialHeightFogComponent.SetInscatteringColorCubemapAngle` _asexponential_height_fog_component _newvalue_7)
            (return true))))
      (:`InscatteringTextureTint`
        (bind _newvalue_8 (`/Game/QuietRuntimeEditor/Common/Blueprints/BP_QuietJsonMacroLibrary.ReadLinearColorWithCheck` _jsonvalue _property (`ExponentialHeightFogComponent.InscatteringTextureTint` _asexponential_height_fog_component))
          (:`then`
            (`ExponentialHeightFogComponent.SetInscatteringTextureTint` _asexponential_height_fog_component _newvalue_8)
            (return true))))
      (:`DirectionalInscatteringExponent`
        (bind _newvalue_9 (`/Game/QuietRuntimeEditor/Common/Blueprints/BP_QuietJsonMacroLibrary.ReadFloatWithCheck` _jsonvalue _property (`ExponentialHeightFogComponent.DirectionalInscatteringExponent` _asexponential_height_fog_component))
          (:`then`
            (`ExponentialHeightFogComponent.SetDirectionalInscatteringExponent` _asexponential_height_fog_component _newvalue_9)
            (return true))))
      (:`DirectionalInscatteringStartDistance`
        (bind _newvalue_10 (`/Game/QuietRuntimeEditor/Common/Blueprints/BP_QuietJsonMacroLibrary.ReadFloatWithCheck` _jsonvalue _property (`ExponentialHeightFogComponent.DirectionalInscatteringStartDistance` _asexponential_height_fog_component))
          (:`then`
            (`ExponentialHeightFogComponent.SetDirectionalInscatteringStartDistance` _asexponential_height_fog_component _newvalue_10)
            (return true))))
      (:`DirectionalInscatteringColor`
        (bind _newvalue_11 (`/Game/QuietRuntimeEditor/Common/Blueprints/BP_QuietJsonMacroLibrary.ReadLinearColorWithCheck` _jsonvalue _property (`ExponentialHeightFogComponent.DirectionalInscatteringLuminance` _asexponential_height_fog_component))
          (:`then`
            (`ExponentialHeightFogComponent.SetDirectionalInscatteringColor` _asexponential_height_fog_component _newvalue_11)
            (return true))))
      (:`VolumetricFog`
        (bind _newvalue_12 (`/Game/QuietRuntimeEditor/Common/Blueprints/BP_QuietJsonMacroLibrary.ReadBoolWithCheck` _jsonvalue _property (`ExponentialHeightFogComponent.bEnableVolumetricFog` _asexponential_height_fog_component))
          (:`then`
            (`ExponentialHeightFogComponent.SetVolumetricFog` _asexponential_height_fog_component _newvalue_12)
            (return true))))
      (:`ScatteringDistribution`
        (bind _newvalue_13 (`/Game/QuietRuntimeEditor/Common/Blueprints/BP_QuietJsonMacroLibrary.ReadFloatWithCheck` _jsonvalue _property (`ExponentialHeightFogComponent.VolumetricFogScatteringDistribution` _asexponential_height_fog_component))
          (:`then`
            (`ExponentialHeightFogComponent.SetVolumetricFogScatteringDistribution` _asexponential_height_fog_component _newvalue_13)
            (return true))))
      (:`Albedo`
        (bind _newvalue_14 (`/Game/QuietRuntimeEditor/Common/Blueprints/BP_QuietJsonMacroLibrary.ReadLinearColorWithCheck` _jsonvalue _property (`KismetMathLibrary.Conv_ColorToLinearColor` (`ExponentialHeightFogComponent.VolumetricFogAlbedo` _asexponential_height_fog_component)))
          (:`then`
            (`ExponentialHeightFogComponent.SetVolumetricFogAlbedo` _asexponential_height_fog_component (`KismetMathLibrary.Conv_LinearColorToColor` _newvalue_14))
            (return true))))
      (:`Emissive`
        (bind _newvalue_15 (`/Game/QuietRuntimeEditor/Common/Blueprints/BP_QuietJsonMacroLibrary.ReadLinearColorWithCheck` _jsonvalue _property (`ExponentialHeightFogComponent.VolumetricFogEmissive` _asexponential_height_fog_component))
          (:`then`
            (`ExponentialHeightFogComponent.SetVolumetricFogEmissive` _asexponential_height_fog_component _newvalue_15)
            (return true))))
      (:`ExtinctionScale`
        (bind _newvalue_16 (`/Game/QuietRuntimeEditor/Common/Blueprints/BP_QuietJsonMacroLibrary.ReadFloatWithCheck` _jsonvalue _property (`ExponentialHeightFogComponent.VolumetricFogExtinctionScale` _asexponential_height_fog_component))
          (:`then`
            (`ExponentialHeightFogComponent.SetVolumetricFogExtinctionScale` _asexponential_height_fog_component _newvalue_16)
            (return true)))))
    (else
      (return true))))