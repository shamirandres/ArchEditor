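; Marshal that exposes LightComponentBase settings as JSON for the QuietRuntimeEditor's serialization and runtime property editing.
; SerializeObject writes the shared light properties to JSON, and GetPropertyValue returns a single one by name.
; CollectProperties builds typed parameter descriptors with defaults and limits, grouped into Light, Advanced and Ray Tracing.
; SetPropertyValue applies checked reads through component setters, but only for shadow, ray-tracing and sample-count properties.
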(fn `CollectProperties`
  (params (Object :type "Object Object Reference") (TargetJson :type "JsonObjectWrapper Structure (by ref)"))
  (locals (LightGroupArray :type "Array of JsonObjectWrapper Structure") (Advanced :type "Array of JsonObjectWrapper Structure") (RayTracing :type "Array of JsonObjectWrapper Structure"))
  (bind _aslight_component_base (cast `LightComponentBase` Object))
  (`|ExecutionSequence`
    (:`then_0`
      (`|ExecutionSequence`
        (:`then_0`
          (bind _jsonobject (`self.MakeFloatParam` "Intensity" "Intensity" "" (`LightComponentBase.Intensity` _aslight_component_base) 5.0 0.0 0.0 10000.0 150.0 1 3))
          (`KismetArrayLibrary.Array_Add` (`local.LightGroupArray`) _jsonobject))
        (:`then_1`
          (bind _jsonobject_2 (`self.MakeLinearColorParam` "LightColor" "Light Color" "" (`LightComponentBase.GetLightColor` _aslight_component_base) (struct :`R` 1.0 :`G` 1.0 :`B` 1.0 :`A` 1.0)))
          (`KismetArrayLibrary.Array_Add` (`local.LightGroupArray`) _jsonobject_2))
        (:`then_2`
          (bind _jsonobject_3 (`self.MakeBoolParam` "CastShadows" "Cast Shadows" "" (`LightComponentBase.CastShadows` _aslight_component_base) true))
          (`KismetArrayLibrary.Array_Add` (`local.LightGroupArray`) _jsonobject_3))))
    (:`then_1`
      (`|ExecutionSequence`
        (:`then_0`
          (bind _jsonobject_4 (`self.MakeFloatParam` "IndirectLightingIntensity" "Indirect Lighting Intensity" "" (`LightComponentBase.IndirectLightingIntensity` _aslight_component_base) 1.0 0.0 0.0 100.0 6.0 1 3))
          (`KismetArrayLibrary.Array_Add` (`local.Advanced`) _jsonobject_4))
        (:`then_1`
          (bind _jsonobject_5 (`self.MakeFloatParam` "VolumetricScatteringIntensity" "Volumetric Scattering Intensity" "" (`LightComponentBase.VolumetricScatteringIntensity` _aslight_component_base) 1.0 0.0 0.25 100.0 4.0 1 2))
          (`KismetArrayLibrary.Array_Add` (`local.Advanced`) _jsonobject_5))
        (:`then_2`
          (bind _jsonobject_6 (`self.MakeBoolParam` "AffectTranslucentLighting" "Affect Translucent Lighting" "" (`LightComponentBase.bAffectTranslucentLighting` _aslight_component_base) true))
          (`KismetArrayLibrary.Array_Add` (`local.Advanced`) _jsonobject_6))
        (:`then_3`
          (bind _jsonobject_7 (`self.MakeBoolParam` "Transmission" "Transmission" "" (`LightComponentBase.bTransmission` _aslight_component_base)))
          (`KismetArrayLibrary.Array_Add` (`local.Advanced`) _jsonobject_7))
        (:`then_4`
          (bind _jsonobject_8 (`self.MakeBoolParam` "CastVolumetricShadow" "Cast Volumetric Shadow" "" (`LightComponentBase.bCastVolumetricShadow` _aslight_component_base) true))
          (`KismetArrayLibrary.Array_Add` (`local.Advanced`) _jsonobject_8))
        (:`then_5`
          (bind _jsonobject_9 (`self.MakeBoolParam` "CastDeepShadow" "Cast Deep Shadow" "" (`LightComponentBase.bCastDeepShadow` _aslight_component_base)))
          (`KismetArrayLibrary.Array_Add` (`local.Advanced`) _jsonobject_9))))
    (:`then_2`
      (`|ExecutionSequence`
        (:`then_0`
          (bind _jsonobject_10 (`self.MakeEnumParam` "CastRayTracedShadows" "Cast Ray Traced Shadows" "" (`|MakeArray` "Disabled" "Use Project Setting" "Enabled") (`KismetMathLibrary.Conv_ByteToInt` (`LightComponentBase.CastRaytracedShadow` _aslight_component_base)) 1))
          (`KismetArrayLibrary.Array_Add` (`local.RayTracing`) _jsonobject_10))
        (:`then_1`
          (bind _jsonobject_11 (`self.MakeIntParam` "SamplesPerPixel" "Samples Per Pixel" "" (`LightComponentBase.SamplesPerPixel` _aslight_component_base) 1 0 0 512 64))
          (`KismetArrayLibrary.Array_Add` (`local.RayTracing`) _jsonobject_11))))
    (:`then_3`
      (`|SetJsonField` TargetJson "Light" (`local.LightGroupArray`))
      (`|SetJsonField` TargetJson "Advanced" (`local.Advanced`))
      (`|SetJsonField` TargetJson "Ray Tracing" (`local.RayTracing`))
      (return))))

(fn `GetPropertyValue`
  (params (Object :type "Object Object Reference") (Property :type String))
  (returns (Success :type Boolean) (Value :type "JsonObjectWrapper Structure"))
  (bind _aslight_component_base (cast `LightComponentBase` Object))
  (bind _outjsonobject (`JsonBlueprintFunctionLibrary.FromString` "{ }"))
  (switch `string` Property
    (:`CastShadows`
      (`|SetJsonField` _outjsonobject Property (`LightComponentBase.CastShadows` _aslight_component_base)))
    (:`IndirectLightingIntensity`
      (`|SetJsonField` _outjsonobject Property (`LightComponentBase.IndirectLightingIntensity` _aslight_component_base)))
    (:`VolumetricScatteringIntensity`
      (`|SetJsonField` _outjsonobject Property (`LightComponentBase.VolumetricScatteringIntensity` _aslight_component_base)))
    (:`Intensity`
      (`|SetJsonField` _outjsonobject Property (`LightComponentBase.Intensity` _aslight_component_base)))
    (:`LightColor`
      (`|SetJsonField` _outjsonobject Property (`LightComponentBase.GetLightColor` _aslight_component_base)))
    (:`AffectTranslucentLighting`
      (`|SetJsonField` _outjsonobject Property (`LightComponentBase.bAffectTranslucentLighting` _aslight_component_base)))
    (:`Transmission`
      (`|SetJsonField` _outjsonobject Property (`LightComponentBase.bTransmission` _aslight_component_base)))
    (:`CastVolumetricShadow`
      (`|SetJsonField` _outjsonobject Property (`LightComponentBase.bCastVolumetricShadow` _aslight_component_base)))
    (:`CastDeepShadow`
      (`|SetJsonField` _outjsonobject Property (`LightComponentBase.bCastDeepShadow` _aslight_component_base)))
    (:`CastRaytraceShadows`
      (`|SetJsonField` _outjsonobject Property (`LightComponentBase.CastRaytracedShadow` _aslight_component_base)))
    (:`SamplesPerPixel`
      (`|SetJsonField` _outjsonobject Property (`LightComponentBase.SamplesPerPixel` _aslight_component_base))))
  (return true _outjsonobject))

(fn `SerializeObject`
  (params (Object :type "Object Object Reference") (TargetJson :type "JsonObjectWrapper Structure (by ref)"))
  (bind _aslight_component_base (cast `LightComponentBase` Object))
  (`|ExecutionSequence`
    (:`then_0`
      (`|SetJsonField` TargetJson "CastShadows" (`LightComponentBase.CastShadows` _aslight_component_base)))
    (:`then_1`
      (`|SetJsonField` TargetJson "IndirectLightingIntensity" (`LightComponentBase.IndirectLightingIntensity` _aslight_component_base)))
    (:`then_2`
      (`|SetJsonField` TargetJson "VolumetricScatteringIntensity" (`LightComponentBase.VolumetricScatteringIntensity` _aslight_component_base)))
    (:`then_3`
      (`|SetJsonField` TargetJson "Intensity" (`LightComponentBase.Intensity` _aslight_component_base)))
    (:`then_4`
      (`|SetJsonField` TargetJson "LightColor" (`LightComponentBase.GetLightColor` _aslight_component_base)))
    (:`then_5`
      (`|SetJsonField` TargetJson "AffectTranslucentLighting" (`LightComponentBase.bAffectTranslucentLighting` _aslight_component_base)))
    (:`then_6`
      (`|SetJsonField` TargetJson "Transmission" (`LightComponentBase.bTransmission` _aslight_component_base)))
    (:`then_7`
      (`|SetJsonField` TargetJson "CastVolumetricShadow" (`LightComponentBase.bCastVolumetricShadow` _aslight_component_base)))
    (:`then_8`
      (`|SetJsonField` TargetJson "CastDeepShadow" (`LightComponentBase.bCastDeepShadow` _aslight_component_base)))
    (:`then_9`
      (`|SetJsonField` TargetJson "CastRaytraceShadows" (`LightComponentBase.CastRaytracedShadow` _aslight_component_base)))
    (:`then_10`
      (`|SetJsonField` TargetJson "SamplesPerPixel" (`LightComponentBase.SamplesPerPixel` _aslight_component_base))
      (return))))

(fn `SetPropertyValue`
  (params (Object :type "Object Object Reference") (Property :type String) (JsonValue :type "JsonObjectWrapper Structure (by ref)"))
  (returns (Success :type Boolean))
  (bind _aslight_component_base (cast `LightComponentBase` Object))
  (switch `string` (`local.Property`)
    (:`Default`
      (return false))
    (:`CastShadows`
      (bind _newvalue (`/Game/QuietRuntimeEditor/Common/Blueprints/BP_QuietJsonMacroLibrary.ReadBoolWithCheck` (`local.JsonValue`) (`local.Property`) (`LightComponentBase.CastShadows` _aslight_component_base))
        (:`then`
          (`LightComponentBase.SetCastShadows` _aslight_component_base _newvalue))))
    (:`CastVolumetricShadow`
      (bind _newvalue_2 (`/Game/QuietRuntimeEditor/Common/Blueprints/BP_QuietJsonMacroLibrary.ReadBoolWithCheck` (`local.JsonValue`) (`local.Property`) (`LightComponentBase.bCastVolumetricShadow` _aslight_component_base))
        (:`then`
          (`LightComponentBase.SetCastVolumetricShadow` _aslight_component_base _newvalue_2))))
    (:`CastDeepShadow`
      (bind _newvalue_3 (`/Game/QuietRuntimeEditor/Common/Blueprints/BP_QuietJsonMacroLibrary.ReadBoolWithCheck` (`local.JsonValue`) (`local.Property`) (`LightComponentBase.bCastDeepShadow` _aslight_component_base))
        (:`then`
          (`LightComponentBase.SetCastDeepShadow` _aslight_component_base _newvalue_3))))
    (:`CastRaytraceShadows`
      (bind _newvalue_4 (`/Game/QuietRuntimeEditor/Common/Blueprints/BP_QuietJsonMacroLibrary.ReadEnumWithCheck` (`local.JsonValue`) (`local.Property`) (`LightComponentBase.CastRaytracedShadow` _aslight_component_base))
        (:`then`
          (`LightComponentBase.SetCastRaytracedShadows` _aslight_component_base (cast `ECastRayTracedShadow` _newvalue_4)))))
    (:`SamplesPerPixel`
      (bind _newvalue_5 (`/Game/QuietRuntimeEditor/Common/Blueprints/BP_QuietJsonMacroLibrary.ReadIntegerWithCheck` (`local.JsonValue`) (`local.Property`) (`LightComponentBase.SamplesPerPixel` _aslight_component_base))
        (:`then`
          (`LightComponentBase.SetSamplesPerPixel` _aslight_component_base _newvalue_5)))))
  (return true))