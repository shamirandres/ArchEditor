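; Runtime editor marshal that serializes Spline Components to JSON and exposes their properties for reading and editing.
; SerializeObject writes duration, debug draw, closed loop, up vector and every point in local space, including tangents, rotation, scale and type.
; CollectProperties lists the scalar and vector settings as editable parameters, without points.
; GetPropertyValue tries the parent first, while SetPropertyValue applies checked values and rebuilds points by clearing and re-adding them.
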(fn `CollectProperties`
  (params (Object :type "Object Object Reference") (TargetJson :type "JsonObjectWrapper Structure (by ref)"))
  (locals (Spline :type "Array of JsonObjectWrapper Structure"))
  (bind _asspline_component (cast `SplineComponent` Object))
  (bind _jsonobject (`self.MakeFloatParam` "Duration" "Duration" "" (`SplineComponent.Duration` _asspline_component) 1.0 0.001 0.001 10000.0 100.0 1 3))
  (`KismetArrayLibrary.Array_Add` (`local.Spline`) _jsonobject)
  (bind _jsonobject_2 (`self.MakeBoolParam` "DrawDebug" "Draw Debug" "" (`SplineComponent.bDrawDebug` _asspline_component) true))
  (`KismetArrayLibrary.Array_Add` (`local.Spline`) _jsonobject_2)
  (bind _jsonobject_3 (`self.MakeBoolParam` "ClosedLoop" "Closed Loop" "" (`SplineComponent.IsClosedLoop` _asspline_component)))
  (`KismetArrayLibrary.Array_Add` (`local.Spline`) _jsonobject_3)
  (bind _jsonobject_4 (`self.MakeVectorParam` "DefaultUpVector" "Default Up Vector" "" (`SplineComponent.DefaultUpVector` _asspline_component) (0.0 0.0 1.0)))
  (`KismetArrayLibrary.Array_Add` (`local.Spline`) _jsonobject_4)
  (`|SetJsonField` (`local.TargetJson`) "Spline" (`local.Spline`))
  (return))

(fn `GetPropertyValue`
  (params (Object :type "Object Object Reference") (Property :type String))
  (returns (Success :type Boolean) (Value :type "JsonObjectWrapper Structure"))
  (bind _property (`local.Property`))
  (bind (_success _value) (`parent.GetPropertyValue` Object Property))
  (if (not _success)
    (bind _asspline_component (cast `SplineComponent` Object))
    (bind _jsonobject (`/Game/QuietRuntimeEditor/Common/Blueprints/BP_QuietJsonFunctionLibrary.NewJson`))
    (switch `string` (`local.Property`)
      (:`Duration`
        (`|SetJsonField` _jsonobject _property (`SplineComponent.Duration` _asspline_component)))
      (:`DrawDebug`
        (`|SetJsonField` _jsonobject _property (`SplineComponent.bDrawDebug` _asspline_component)))
      (:`ClosedLoop`
        (`|SetJsonField` _jsonobject _property (`SplineComponent.IsClosedLoop` _asspline_component)))
      (:`DefaultUpVector`
        (`|SetJsonField` _jsonobject _property (`SplineComponent.DefaultUpVector` _asspline_component))))
    (return true _jsonobject)
    (else
      (return true _value))))

(fn `SerializeObject`
  (params (Object :type "Object Object Reference") (TargetJson :type "JsonObjectWrapper Structure (by ref)"))
  (bind _asspline_component (cast `SplineComponent` Object))
  (`|SetJsonField` (`local.TargetJson`) "Duration" (`SplineComponent.Duration` _asspline_component))
  (`|SetJsonField` (`local.TargetJson`) "DrawDebug" (`SplineComponent.bDrawDebug` _asspline_component))
  (`|SetJsonField` (`local.TargetJson`) "ClosedLoop" (`SplineComponent.IsClosedLoop` _asspline_component))
  (`|SetJsonField` (`local.TargetJson`) "DefaultUpVector" (`SplineComponent.DefaultUpVector` _asspline_component))
  (bind _splinepoints (`self.SerializeSplinePoints` _asspline_component))
  (`|SetJsonField` (`local.TargetJson`) "SplinePoints" _splinepoints)
  (return))

(fn `SerializeSplinePoints`
  (params (Spline :type "SplineComponent Object Reference"))
  (returns (SplinePoints :type "Array of SplinePoint Structure"))
  (locals (Points :type "Array of SplinePoint Structure"))
  (for _index (range (`SplineComponent.GetNumberOfSplinePoints` Spline))
    (`KismetArrayLibrary.Array_Add` (`local.Points`) (make `SplinePoint` (`KismetMathLibrary.Conv_IntToDouble` _index) (`SplineComponent.GetLocationAtSplinePoint` Spline _index "Local") (`SplineComponent.GetArriveTangentAtSplinePoint` Spline _index "Local") (`SplineComponent.GetLeaveTangentAtSplinePoint` Spline _index "Local") (`SplineComponent.GetRotationAtSplinePoint` Spline _index "Local") (`SplineComponent.GetScaleAtSplinePoint` Spline _index) (`SplineComponent.GetSplinePointType` Spline _index))))
  (return (`local.Points`)))

(fn `SetPropertyValue`
  (params (Object :type "Object Object Reference") (Property :type String) (JsonValue :type "JsonObjectWrapper Structure (by ref)"))
  (returns (Success :type Boolean))
  (bind _jsonvalue (`local.JsonValue`))
  (bind _property (`local.Property`))
  (bind _asspline_component (cast `SplineComponent` Object))
  (switch `string` (`local.Property`)
    (:`Duration`
      (bind _newvalue (`/Game/QuietRuntimeEditor/Common/Blueprints/BP_QuietJsonMacroLibrary.ReadFloatWithCheck` _jsonvalue _property (`SplineComponent.Duration` _asspline_component))
        (:`then`
          (set `SplineComponent.Duration` _newvalue _asspline_component)
          (return true))))
    (:`DrawDebug`
      (bind _newvalue_2 (`/Game/QuietRuntimeEditor/Common/Blueprints/BP_QuietJsonMacroLibrary.ReadBoolWithCheck` _jsonvalue _property (`SplineComponent.bDrawDebug` _asspline_component))
        (:`then`
          (`SplineComponent.SetDrawDebug` _asspline_component _newvalue_2)
          (return true))))
    (:`ClosedLoop`
      (bind _newvalue_3 (`/Game/QuietRuntimeEditor/Common/Blueprints/BP_QuietJsonMacroLibrary.ReadBoolWithCheck` _jsonvalue _property (`SplineComponent.IsClosedLoop` _asspline_component))
        (:`then`
          (`SplineComponent.SetClosedLoop` _asspline_component _newvalue_3 true)
          (return true))))
    (:`DefaultUpVector`
      (bind _newvalue_4 (`/Game/QuietRuntimeEditor/Common/Blueprints/BP_QuietJsonMacroLibrary.ReadVectorWithCheck` _jsonvalue _property (`SplineComponent.DefaultUpVector` _asspline_component))
        (:`then`
          (`SplineComponent.SetDefaultUpVector` _asspline_component _newvalue_4 "Local")
          (return true))))
    (:`SplinePoints`
      (`SplineComponent.ClearSplinePoints` _asspline_component false)
      (bind _outvalue (`|GetJsonField` (`local.JsonValue`) "SplinePoints"))
      (`SplineComponent.AddPoints` _asspline_component _outvalue true))))