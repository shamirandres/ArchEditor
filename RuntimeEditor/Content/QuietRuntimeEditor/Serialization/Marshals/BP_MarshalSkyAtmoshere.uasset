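; Runtime editor marshal that exposes a SkyAtmosphereComponent's atmosphere, Rayleigh, Mie, absorption and art-direction settings as JSON.
; CollectProperties builds grouped float and color descriptors with defaults and ranges, while SerializeObject writes the raw values.
; Get/SetPropertyValue defer to the parent first, then match by property name, with setters using checked JSON reads.
; The Mie Absorption case in SetPropertyValue writes through SetOtherAbsorption.
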(fn `CollectProperties`
  (params (Object :type "Object Object Reference") (TargetJson :type "JsonObjectWrapper Structure (by ref)"))
  (locals (Atmosphere :type "Array of JsonObjectWrapper Structure") (Rayleigh :type "Array of JsonObjectWrapper Structure") (Mie :type "Array of JsonObjectWrapper Structure") (Absorption :type "Array of JsonObjectWrapper Structure") (ArtDirection :type "Array of JsonObjectWrapper Structure"))
  (`parent.CollectProperties` Object TargetJson)
  (bind _assky_atmosphere_component (cast `SkyAtmosphereComponent` Object))
  (bind _jsonobject (`self.MakeFloatParam` "AtmosphereHeight" "Atmosphere Height" "" (`SkyAtmosphereComponent.AtmosphereHeight` _assky_atmosphere_component) 60.0 0.1 1.0 100000.0 200.0 1 1))
  (`KismetArrayLibrary.Array_Add` (`local.Atmosphere`) _jsonobject)
  (bind _jsonobject_2 (`self.MakeFloatParam` "MultiScattering" "Multi Scattering" "" (`SkyAtmosphereComponent.MultiScatteringFactor` _assky_atmosphere_component) 1.0 0.0 0.0 2.0 1.0))
  (`KismetArrayLibrary.Array_Add` (`local.Atmosphere`) _jsonobject_2)
  (bind _jsonobject_3 (`self.MakeFloatParam` "RayleighScatteringScale" "Rayleigh Scattering Scale" "" (`SkyAtmosphereComponent.RayleighScatteringScale` _assky_atmosphere_component) 0.0331 0.0 0.0 2.0 2.0 1 4))
  (`KismetArrayLibrary.Array_Add` (`local.Rayleigh`) _jsonobject_3)
  (bind _jsonobject_4 (`self.MakeLinearColorParam` "RayleighScattering" "Rayleigh Scattering" "" (`SkyAtmosphereComponent.RayleighScattering` _assky_atmosphere_component) (struct :`R` 0.174647 :`G` 0.40724 :`B` 1.0 :`A` 1.0)))
  (`KismetArrayLibrary.Array_Add` (`local.Rayleigh`) _jsonobject_4)
  (bind _jsonobject_5 (`self.MakeFloatParam` "RayleighExponentialDistribution" "Rayleigh Exponential Distribution" "" (`SkyAtmosphereComponent.RayleighExponentialDistribution` _assky_atmosphere_component) 8.0 0.001 0.01 10000.0 20.0 1 4))
  (`KismetArrayLibrary.Array_Add` (`local.Rayleigh`) _jsonobject_5)
  (bind _jsonobject_6 (`self.MakeFloatParam` "MieScatteringScale" "Mie Scattering Scale" "" (`SkyAtmosphereComponent.MieScatteringScale` _assky_atmosphere_component) 0.003996 0.0 0.0 5.0 5.0))
  (`KismetArrayLibrary.Array_Add` (`local.Mie`) _jsonobject_6)
  (bind _jsonobject_7 (`self.MakeLinearColorParam` "MieScattering" "Mie Scattering" "" (`SkyAtmosphereComponent.MieScattering` _assky_atmosphere_component) (struct :`R` 1.0 :`G` 1.0 :`B` 1.0 :`A` 1.0)))
  (`KismetArrayLibrary.Array_Add` (`local.Mie`) _jsonobject_7)
  (bind _jsonobject_8 (`self.MakeFloatParam` "MieAbsorptionScale" "Mie Absorption Scale" "" (`SkyAtmosphereComponent.MieAbsorptionScale` _assky_atmosphere_component) 0.000444 0.0 0.0 5.0 5.0))
  (`KismetArrayLibrary.Array_Add` (`local.Mie`) _jsonobject_8)
  (bind _jsonobject_9 (`self.MakeLinearColorParam` "MieAbsorption" "Mie Absorption" "" (`SkyAtmosphereComponent.MieAbsorption` _assky_atmosphere_component) (struct :`R` 1.0 :`G` 1.0 :`B` 1.0 :`A` 1.0)))
  (`KismetArrayLibrary.Array_Add` (`local.Mie`) _jsonobject_9)
  (bind _jsonobject_10 (`self.MakeFloatParam` "MieAnisotropy" "Mie Anisotropy" "" (`SkyAtmosphereComponent.MieAnisotropy` _assky_atmosphere_component) 0.8 0.0 0.0 0.999 0.999))
  (`KismetArrayLibrary.Array_Add` (`local.Mie`) _jsonobject_10)
  (bind _jsonobject_11 (`self.MakeFloatParam` "MieExponentialDistribution" "Mie Exponential Distribution" "" (`SkyAtmosphereComponent.MieExponentialDistribution` _assky_atmosphere_component) 1.2 0.001 0.01 100000.0 10.0))
  (`KismetArrayLibrary.Array_Add` (`local.Mie`) _jsonobject_11)
  (bind _jsonobject_12 (`self.MakeFloatParam` "AbsorptionScale" "Absorption Scale" "" (`SkyAtmosphereComponent.OtherAbsorptionScale` _assky_atmosphere_component) 0.001881 0.0 0.0 1.0 0.2))
  (`KismetArrayLibrary.Array_Add` (`local.Absorption`) _jsonobject_12)
  (bind _jsonobject_13 (`self.MakeLinearColorParam` "Absorption" "Absorption" "" (`SkyAtmosphereComponent.OtherAbsorption` _assky_atmosphere_component) (struct :`R` 0.346704 :`G` 1.0 :`B` 0.045186 :`A` 1.0)))
  (`KismetArrayLibrary.Array_Add` (`local.Absorption`) _jsonobject_13)
  (bind _jsonobject_14 (`self.MakeLinearColorParam` "SkyLuminanceFactor" "Sky Luminance Factor" "" (`SkyAtmosphereComponent.SkyLuminanceFactor` _assky_atmosphere_component) (struct :`R` 1.0 :`G` 1.0 :`B` 1.0 :`A` 1.0)))
  (`KismetArrayLibrary.Array_Add` (`local.ArtDirection`) _jsonobject_14)
  (bind _jsonobject_15 (`self.MakeFloatParam` "AerialPerspectiveViewDistanceScale" "Aerial Perspective View Distance Scale" "" (`SkyAtmosphereComponent.AerialPespectiveViewDistanceScale` _assky_atmosphere_component) 1.0 0.0 0.0 1000.0 3.0))
  (`KismetArrayLibrary.Array_Add` (`local.Absorption`) _jsonobject_15)
  (bind _jsonobject_16 (`self.MakeFloatParam` "HeightFogContribution" "Height Fog Contribution" "" (`SkyAtmosphereComponent.HeightFogContribution` _assky_atmosphere_component) 1.0 0.0 0.0 1.0 1.0))
  (`KismetArrayLibrary.Array_Add` (`local.Absorption`) _jsonobject_16)
  (`|SetJsonField` (`local.TargetJson`) "GroupsState" (`|MakeArray` "Atmosphere"))
  (`|SetJsonField` (`local.TargetJson`) "Atmosphere" (`local.Atmosphere`))
  (`|SetJsonField` (`local.TargetJson`) "Atmosphere - Rayleigh" (`local.Rayleigh`))
  (`|SetJsonField` (`local.TargetJson`) "Atmosphere - Mie" (`local.Mie`))
  (`|SetJsonField` (`local.TargetJson`) "Atmosphere - Absorption" (`local.Absorption`))
  (`|SetJsonField` (`local.TargetJson`) "Art Direction" (`local.ArtDirection`))
  (return))

(fn `GetPropertyValue`
  (params (Object :type "Object Object Reference") (Property :type String))
  (returns (Success :type Boolean) (Value :type "JsonObjectWrapper Structure"))
  (bind _property (`local.Property`))
  (bind (_success _value) (`parent.GetPropertyValue` Object Property))
  (if (not _success)
    (bind _assky_atmosphere_component (cast `SkyAtmosphereComponent` Object))
    (bind _jsonobject (`/Game/QuietRuntimeEditor/Common/Blueprints/BP_QuietJsonFunctionLibrary.NewJson`))
    (switch `string` _property
      (:`AtmosphereHeight`
        (`|SetJsonField` _jsonobject _property (`SkyAtmosphereComponent.AtmosphereHeight` _assky_atmosphere_component)))
      (:`MultiScattering`
        (`|SetJsonField` _jsonobject _property (`SkyAtmosphereComponent.MultiScatteringFactor` _assky_atmosphere_component)))
      (:`RayleighScatteringScale`
        (`|SetJsonField` _jsonobject _property (`SkyAtmosphereComponent.RayleighScatteringScale` _assky_atmosphere_component)))
      (:`RayleighScattering`
        (`|SetJsonField` _jsonobject _property (`SkyAtmosphereComponent.RayleighScattering` _assky_atmosphere_component)))
      (:`RayleighExponentialDistribution`
        (`|SetJsonField` _jsonobject _property (`SkyAtmosphereComponent.RayleighExponentialDistribution` _assky_atmosphere_component)))
      (:`MieScatteringScale`
        (`|SetJsonField` _jsonobject _property (`SkyAtmosphereComponent.MieScatteringScale` _assky_atmosphere_component)))
      (:`MieScattering`
        (`|SetJsonField` _jsonobject _property (`SkyAtmosphereComponent.MieScattering` _assky_atmosphere_component)))
      (:`MieAbsorptionScale`
        (`|SetJsonField` _jsonobject _property (`SkyAtmosphereComponent.MieAbsorptionScale` _assky_atmosphere_component)))
      (:`MieAbsorption`
        (`|SetJsonField` _jsonobject _property (`SkyAtmosphereComponent.MieAbsorption` _assky_atmosphere_component)))
      (:`MieAnisotropy`
        (`|SetJsonField` _jsonobject _property (`SkyAtmosphereComponent.MieAnisotropy` _assky_atmosphere_component)))
      (:`MieExponentialDistribution`
        (`|SetJsonField` _jsonobject _property (`SkyAtmosphereComponent.MieExponentialDistribution` _assky_atmosphere_component)))
      (:`AbsorptionScale`
        (`|SetJsonField` _jsonobject _property (`SkyAtmosphereComponent.OtherAbsorptionScale` _assky_atmosphere_component)))
      (:`Absorption`
        (`|SetJsonField` _jsonobject _property (`SkyAtmosphereComponent.OtherAbsorption` _assky_atmosphere_component)))
      (:`SkyLuminanceFactor`
        (`|SetJsonField` _jsonobject _property (`SkyAtmosphereComponent.SkyLuminanceFactor` _assky_atmosphere_component)))
      (:`AerialPerspectiveViewDistanceScale`
        (`|SetJsonField` _jsonobject _property (`SkyAtmosphereComponent.AerialPespectiveViewDistanceScale` _assky_atmosphere_component)))
      (:`HeightFogContribution`
        (`|SetJsonField` _jsonobject _property (`SkyAtmosphereComponent.HeightFogContribution` _assky_atmosphere_component))))
    (return true _jsonobject)
    (else
      (return true _value))))

(fn `SerializeObject`
  (params (Object :type "Object Object Reference") (TargetJson :type "JsonObjectWrapper Structure (by ref)"))
  (locals (Atmosphere :type "Array of JsonObjectWrapper Structure") (Rayleigh :type "Array of JsonObjectWrapper Structure") (Mie :type "Array of JsonObjectWrapper Structure") (Absorption :type "Array of JsonObjectWrapper Structure") (ArtDirection :type "Array of JsonObjectWrapper Structure"))
  (`parent.SerializeObject` Object TargetJson)
  (bind _assky_atmosphere_component (cast `SkyAtmosphereComponent` Object))
  (`|SetJsonField` (`local.TargetJson`) "AtmosphereHeight" (`SkyAtmosphereComponent.AtmosphereHeight` _assky_atmosphere_component))
  (`|SetJsonField` (`local.TargetJson`) "MultiScattering" (`SkyAtmosphereComponent.MultiScatteringFactor` _assky_atmosphere_component))
  (`|SetJsonField` (`local.TargetJson`) "RayleighScatteringScale" (`SkyAtmosphereComponent.RayleighScatteringScale` _assky_atmosphere_component))
  (`|SetJsonField` (`local.TargetJson`) "RayleighScattering" (`SkyAtmosphereComponent.RayleighScattering` _assky_atmosphere_component))
  (`|SetJsonField` (`local.TargetJson`) "RayleighExponentialDistribution" (`SkyAtmosphereComponent.RayleighExponentialDistribution` _assky_atmosphere_component))
  (`|SetJsonField` (`local.TargetJson`) "MieScatteringScale" (`SkyAtmosphereComponent.MieScatteringScale` _assky_atmosphere_component))
  (`|SetJsonField` (`local.TargetJson`) "MieScattering" (`SkyAtmosphereComponent.MieScattering` _assky_atmosphere_component))
  (`|SetJsonField` (`local.TargetJson`) "MieAbsorptionScale" (`SkyAtmosphereComponent.MieAbsorptionScale` _assky_atmosphere_component))
  (`|SetJsonField` (`local.TargetJson`) "MieAbsorption" (`SkyAtmosphereComponent.MieAbsorption` _assky_atmosphere_component))
  (`|SetJsonField` (`local.TargetJson`) "MieAnisotropy" (`SkyAtmosphereComponent.MieAnisotropy` _assky_atmosphere_component))
  (`|SetJsonField` (`local.TargetJson`) "MieExponentialDistribution" (`SkyAtmosphereComponent.MieExponentialDistribution` _assky_atmosphere_component))
  (`|SetJsonField` (`local.TargetJson`) "AbsorptionScale" (`SkyAtmosphereComponent.OtherAbsorptionScale` _assky_atmosphere_component))
  (`|SetJsonField` (`local.TargetJson`) "Absorption" (`SkyAtmosphereComponent.OtherAbsorption` _assky_atmosphere_component))
  (`|SetJsonField` (`local.TargetJson`) "SkyLuminanceFactor" (`SkyAtmosphereComponent.SkyLuminanceFactor` _assky_atmosphere_component))
  (`|SetJsonField` (`local.TargetJson`) "AerialPerspectiveViewDistanceScale" (`SkyAtmosphereComponent.AerialPespectiveViewDistanceScale` _assky_atmosphere_component))
  (`|SetJsonField` (`local.TargetJson`) "HeightFogContribution" (`SkyAtmosphereComponent.HeightFogContribution` _assky_atmosphere_component))
  (return))

(fn `SetPropertyValue`
  (params (Object :type "Object Object Reference") (Property :type String) (JsonValue :type "JsonObjectWrapper Structure (by ref)"))
  (returns (Success :type Boolean))
  (bind _property (`local.Property`))
  (bind _jsonvalue (`local.JsonValue`))
  (bind _success (`parent.SetPropertyValue` Object Property JsonValue))
  (if (not _success)
    (bind _assky_atmosphere_component (cast `SkyAtmosphereComponent` Object))
    (switch `string` _property
      (:`AtmosphereHeight`
        (bind _newvalue (`/Game/QuietRuntimeEditor/Common/Blueprints/BP_QuietJsonMacroLibrary.ReadFloatWithCheck` _jsonvalue _property (`SkyAtmosphereComponent.AtmosphereHeight` _assky_atmosphere_component))
          (:`then`
            (`SkyAtmosphereComponent.SetAtmosphereHeight` _assky_atmosphere_component _newvalue))))
      (:`MultiScattering`
        (bind _newvalue_2 (`/Game/QuietRuntimeEditor/Common/Blueprints/BP_QuietJsonMacroLibrary.ReadFloatWithCheck` _jsonvalue _property (`SkyAtmosphereComponent.MultiScatteringFactor` _assky_atmosphere_component))
          (:`then`
            (`SkyAtmosphereComponent.SetMultiScatteringFactor` _assky_atmosphere_component _newvalue_2))))
      (:`RayleighScatteringScale`
        (bind _newvalue_3 (`/Game/QuietRuntimeEditor/Common/Blueprints/BP_QuietJsonMacroLibrary.ReadFloatWithCheck` _jsonvalue _property (`SkyAtmosphereComponent.RayleighScatteringScale` _assky_atmosphere_component))
          (:`then`
            (`SkyAtmosphereComponent.SetRayleighScatteringScale` _assky_atmosphere_component _newvalue_3))))
      (:`RayleighScattering`
        (bind _newvalue_4 (`/Game/QuietRuntimeEditor/Common/Blueprints/BP_QuietJsonMacroLibrary.ReadLinearColorWithCheck` _jsonvalue _property (`SkyAtmosphereComponent.RayleighScattering` _assky_atmosphere_component))
          (:`then`
            (`SkyAtmosphereComponent.SetRayleighScattering` _assky_atmosphere_component _newvalue_4))))
      (:`RayleighExponentialDistribution`
        (bind _newvalue_5 (`/Game/QuietRuntimeEditor/Common/Blueprints/BP_QuietJsonMacroLibrary.ReadFloatWithCheck` _jsonvalue _property (`SkyAtmosphereComponent.RayleighExponentialDistribution` _assky_atmosphere_component))
          (:`then`
            (`SkyAtmosphereComponent.SetRayleighExponentialDistribution` _assky_atmosphere_component _newvalue_5))))
      (:`MieScatteringScale`
        (bind _newvalue_6 (`/Game/QuietRuntimeEditor/Common/Blueprints/BP_QuietJsonMacroLibrary.ReadFloatWithCheck` _jsonvalue _property (`SkyAtmosphereComponent.MieScatteringScale` _assky_atmosphere_component))
          (:`then`
            (`SkyAtmosphereComponent.SetMieScatteringScale` _assky_atmosphere_component _newvalue_6))))
      (:`MieScattering`
        (bind _newvalue_7 (`/Game/QuietRuntimeEditor/Common/Blueprints/BP_QuietJsonMacroLibrary.ReadLinearColorWithCheck` _jsonvalue _property (`SkyAtmosphereComponent.MieScattering` _assky_atmosphere_component))
          (:`then`
            (`SkyAtmosphereComponent.SetMieScattering` _assky_atmosphere_component _newvalue_7))))
      (:`MieAbsorptionScale`
        (bind _newvalue_8 (`/Game/QuietRuntimeEditor/Common/Blueprints/BP_QuietJsonMacroLibrary.ReadFloatWithCheck` _jsonvalue _property (`SkyAtmosphereComponent.MieAbsorptionScale` _assky_atmosphere_component))
          (:`then`
            (`SkyAtmosphereComponent.SetMieAbsorptionScale` _assky_atmosphere_component _newvalue_8))))
      (:`MieAbsorption`
        (bind _newvalue_9 (`/Game/QuietRuntimeEditor/Common/Blueprints/BP_QuietJsonMacroLibrary.ReadLinearColorWithCheck` _jsonvalue _property (`SkyAtmosphereComponent.MieAbsorption` _assky_atmosphere_component))
          (:`then`
            (`SkyAtmosphereComponent.SetOtherAbsorption` _assky_atmosphere_component _newvalue_9))))
      (:`MieAnisotropy`
        (bind _newvalue_10 (`/Game/QuietRuntimeEditor/Common/Blueprints/BP_QuietJsonMacroLibrary.ReadFloatWithCheck` _jsonvalue _property (`SkyAtmosphereComponent.MieAnisotropy` _assky_atmosphere_component))
          (:`then`
            (`SkyAtmosphereComponent.SetMieAnisotropy` _assky_atmosphere_component _newvalue_10))))
      (:`MieExponentialDistribution`
        (bind _newvalue_11 (`/Game/QuietRuntimeEditor/Common/Blueprints/BP_QuietJsonMacroLibrary.ReadFloatWithCheck` _jsonvalue _property (`SkyAtmosphereComponent.MieExponentialDistribution` _assky_atmosphere_component))
          (:`then`
            (`SkyAtmosphereComponent.SetMieExponentialDistribution` _assky_atmosphere_component _newvalue_11))))
      (:`AbsorptionScale`
        (bind _newvalue_12 (`/Game/QuietRuntimeEditor/Common/Blueprints/BP_QuietJsonMacroLibrary.ReadFloatWithCheck` _jsonvalue _property (`SkyAtmosphereComponent.OtherAbsorptionScale` _assky_atmosphere_component))
          (:`then`
            (`SkyAtmosphereComponent.SetOtherAbsorptionScale` _assky_atmosphere_component _newvalue_12))))
      (:`Absorption`
        (bind _newvalue_13 (`/Game/QuietRuntimeEditor/Common/Blueprints/BP_QuietJsonMacroLibrary.ReadLinearColorWithCheck` _jsonvalue _property (`SkyAtmosphereComponent.OtherAbsorption` _assky_atmosphere_component))
          (:`then`
            (`SkyAtmosphereComponent.SetOtherAbsorption` _assky_atmosphere_component _newvalue_13))))
      (:`SkyLuminanceFactor`
        (bind _newvalue_14 (`/Game/QuietRuntimeEditor/Common/Blueprints/BP_QuietJsonMacroLibrary.ReadLinearColorWithCheck` _jsonvalue _property (`SkyAtmosphereComponent.SkyLuminanceFactor` _assky_atmosphere_component))
          (:`then`
            (`SkyAtmosphereComponent.SetSkyLuminanceFactor` _assky_atmosphere_component _newvalue_14))))
      (:`AerialPerspectiveViewDistanceScale`
        (bind _newvalue_15 (`/Game/QuietRuntimeEditor/Common/Blueprints/BP_QuietJsonMacroLibrary.ReadFloatWithCheck` _jsonvalue _property (`SkyAtmosphereComponent.AerialPespectiveViewDistanceScale` _assky_atmosphere_component))
          (:`then`
            (`SkyAtmosphereComponent.SetAerialPespectiveViewDistanceScale` _assky_atmosphere_component _newvalue_15))))
      (:`HeightFogContribution`
        (bind _newvalue_16 (`/Game/QuietRuntimeEditor/Common/Blueprints/BP_QuietJsonMacroLibrary.ReadFloatWithCheck` _jsonvalue _property (`SkyAtmosphereComponent.HeightFogContribution` _assky_atmosphere_component))
          (:`then`
            (`SkyAtmosphereComponent.SetHeightFogContribution` _assky_atmosphere_component _newvalue_16)))))
    (return true)
    (else
      (return true))))