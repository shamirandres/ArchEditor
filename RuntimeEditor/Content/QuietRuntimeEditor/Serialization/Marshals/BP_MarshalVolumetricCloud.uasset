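; Runtime editor marshal that exposes a VolumetricCloudComponent's layer, tracing, planet radius and ground albedo settings as JSON.
; Get and Set try the parent marshal first, then switch on property name, writing through checked reads and component setters, with sRGB conversion for albedo.
; SerializeObject appends these fields to the parent's output.
; CollectProperties builds ranged float and color parameter descriptors, grouped into Layer and Planet, for editing.
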(fn `CollectProperties`
  (params (Object :type "Object Object Reference") (TargetJson :type "JsonObjectWrapper Structure (by ref)"))
  (locals (Layer :type "Array of JsonObjectWrapper Structure") (Planet :type "Array of JsonObjectWrapper Structure"))
  (bind _asvolumetric_cloud_component (cast `VolumetricCloudComponent` Object))
  (bind _jsonobject (`self.MakeFloatParam` "LayerBottomAltitude" "Layer Bottom Altitude" "" (`VolumetricCloudComponent.LayerBottomAltitude` _asvolumetric_cloud_component) 5.0 -10000.0 0.0 10000.0 20.0 1 3))
  (`KismetArrayLibrary.Array_Add` (`local.Layer`) _jsonobject)
  (bind _jsonobject_2 (`self.MakeFloatParam` "LayerHeight" "Layer Height" "" (`VolumetricCloudComponent.LayerHeight` _asvolumetric_cloud_component) 10.0 0.1 0.1 10000.0 20.0 1 3))
  (`KismetArrayLibrary.Array_Add` (`local.Layer`) _jsonobject_2)
  (bind _jsonobject_3 (`self.MakeFloatParam` "TracingStartMaxDistance" "Tracing Start Max Distance" "" (`VolumetricCloudComponent.TracingStartMaxDistance` _asvolumetric_cloud_component) 350.0 1.0 100.0 1000000.0 500.0 1 1))
  (`KismetArrayLibrary.Array_Add` (`local.Layer`) _jsonobject_3)
  (bind _jsonobject_4 (`self.MakeFloatParam` "TracingMaxDistance" "Tracing Max Distance" "" (`VolumetricCloudComponent.TracingMaxDistance` _asvolumetric_cloud_component) 50.0 0.1 100.0 10000.0 7000.0 1 1))
  (`KismetArrayLibrary.Array_Add` (`local.Layer`) _jsonobject_4)
  (bind _jsonobject_5 (`self.MakeFloatParam` "PlanetRadius" "Planet Radius" "" (`VolumetricCloudComponent.PlanetRadius` _asvolumetric_cloud_component) 6360.0 0.1 100.0 10000.0 7000.0 1 1))
  (`KismetArrayLibrary.Array_Add` (`local.Planet`) _jsonobject_5)
  (bind _jsonobject_6 (`self.MakeLinearColorParam` "GroundAlbedo" "Ground Albedo" "" (`KismetMathLibrary.Conv_ColorToLinearColor` (`VolumetricCloudComponent.GroundAlbedo` _asvolumetric_cloud_component)) (struct :`R` 0.401978 :`G` 0.401978 :`B` 0.401978 :`A` 1.0)))
  (`KismetArrayLibrary.Array_Add` (`local.Planet`) _jsonobject_6)
  (`|SetJsonField` (`local.TargetJson`) "GroupsState" (`|MakeArray` "Layer" "Planet"))
  (`|SetJsonField` (`local.TargetJson`) "Layer" (`local.Layer`))
  (`|SetJsonField` (`local.TargetJson`) "Planet" (`local.Planet`))
  (return))

(fn `GetPropertyValue`
  (params (Object :type "Object Object Reference") (Property :type String))
  (returns (Success :type Boolean) (Value :type "JsonObjectWrapper Structure"))
  (bind _property (`local.Property`))
  (bind (_success _value) (`parent.GetPropertyValue` Object Property))
  (if (not _success)
    (bind _asvolumetric_cloud_component (cast `VolumetricCloudComponent` Object))
    (bind _jsonobject (`/Game/QuietRuntimeEditor/Common/Blueprints/BP_QuietJsonFunctionLibrary.NewJson`))
    (switch `string` _property
      (:`LayerBottomAltitude`
        (`|SetJsonField` _jsonobject _property (`VolumetricCloudComponent.LayerBottomAltitude` _asvolumetric_cloud_component)))
      (:`LayerHeight`
        (`|SetJsonField` _jsonobject _property (`VolumetricCloudComponent.LayerHeight` _asvolumetric_cloud_component)))
      (:`TracingStartMaxDistance`
        (`|SetJsonField` _jsonobject _property (`VolumetricCloudComponent.TracingStartMaxDistance` _asvolumetric_cloud_component)))
      (:`TracingMaxDistance`
        (`|SetJsonField` _jsonobject _property (`VolumetricCloudComponent.TracingMaxDistance` _asvolumetric_cloud_component)))
      (:`PlanetRadius`
        (`|SetJsonField` _jsonobject _property (`VolumetricCloudComponent.PlanetRadius` _asvolumetric_cloud_component)))
      (:`GroundAlbedo`
        (`|SetJsonField` _jsonobject _property (`VolumetricCloudComponent.GroundAlbedo` _asvolumetric_cloud_component))))
    (return true _jsonobject)
    (else
      (return true _value))))

(fn `SerializeObject`
  (params (Object :type "Object Object Reference") (TargetJson :type "JsonObjectWrapper Structure (by ref)"))
  (`parent.SerializeObject` Object TargetJson)
  (bind _asvolumetric_cloud_component (cast `VolumetricCloudComponent` Object))
  (`|SetJsonField` (`local.TargetJson`) "LayerBottomAltitude" (`VolumetricCloudComponent.LayerBottomAltitude` _asvolumetric_cloud_component))
  (`|SetJsonField` (`local.TargetJson`) "LayerHeight" (`VolumetricCloudComponent.LayerHeight` _asvolumetric_cloud_component))
  (`|SetJsonField` (`local.TargetJson`) "TracingStartMaxDistance" (`VolumetricCloudComponent.TracingStartMaxDistance` _asvolumetric_cloud_component))
  (`|SetJsonField` (`local.TargetJson`) "TracingMaxDistance" (`VolumetricCloudComponent.TracingMaxDistance` _asvolumetric_cloud_component))
  (`|SetJsonField` (`local.TargetJson`) "PlanetRadius" (`VolumetricCloudComponent.PlanetRadius` _asvolumetric_cloud_component))
  (`|SetJsonField` (`local.TargetJson`) "GroundAlbedo" (`VolumetricCloudComponent.GroundAlbedo` _asvolumetric_cloud_component))
  (return))

(fn `SetPropertyValue`
  (params (Object :type "Object Object Reference") (Property :type String) (JsonValue :type "JsonObjectWrapper Structure (by ref)"))
  (returns (Success :type Boolean))
  (bind _property (`local.Property`))
  (bind _jsonvalue (`local.JsonValue`))
  (bind _success (`parent.SetPropertyValue` Object Property JsonValue))
  (if (not _success)
    (bind _asvolumetric_cloud_component (cast `VolumetricCloudComponent` Object))
    (switch `string` _property
      (:`LayerBottomAltitude`
        (bind _newvalue (`/Game/QuietRuntimeEditor/Common/Blueprints/BP_QuietJsonMacroLibrary.ReadFloatWithCheck` _jsonvalue _property (`VolumetricCloudComponent.LayerBottomAltitude` _asvolumetric_cloud_component))
          (:`then`
            (`VolumetricCloudComponent.SetLayerBottomAltitude` _asvolumetric_cloud_component _newvalue))))
      (:`LayerHeight`
        (bind _newvalue_2 (`/Game/QuietRuntimeEditor/Common/Blueprints/BP_QuietJsonMacroLibrary.ReadFloatWithCheck` _jsonvalue _property (`VolumetricCloudComponent.LayerHeight` _asvolumetric_cloud_component))
          (:`then`
            (`VolumetricCloudComponent.SetLayerHeight` _asvolumetric_cloud_component _newvalue_2))))
      (:`TracingStartMaxDistance`
        (bind _newvalue_3 (`/Game/QuietRuntimeEditor/Common/Blueprints/BP_QuietJsonMacroLibrary.ReadFloatWithCheck` _jsonvalue _property (`VolumetricCloudComponent.TracingStartMaxDistance` _asvolumetric_cloud_component))
          (:`then`
            (`VolumetricCloudComponent.SetTracingStartMaxDistance` _asvolumetric_cloud_component _newvalue_3))))
      (:`TracingMaxDistance`
        (bind _newvalue_4 (`/Game/QuietRuntimeEditor/Common/Blueprints/BP_QuietJsonMacroLibrary.ReadFloatWithCheck` _jsonvalue _property (`VolumetricCloudComponent.TracingMaxDistance` _asvolumetric_cloud_component))
          (:`then`
            (`VolumetricCloudComponent.SetTracingMaxDistance` _asvolumetric_cloud_component _newvalue_4))))
      (:`PlanetRadius`
        (bind _newvalue_5 (`/Game/QuietRuntimeEditor/Common/Blueprints/BP_QuietJsonMacroLibrary.ReadFloatWithCheck` _jsonvalue _property (`VolumetricCloudComponent.PlanetRadius` _asvolumetric_cloud_component))
          (:`then`
            (`VolumetricCloudComponent.SetPlanetRadius` _asvolumetric_cloud_component _newvalue_5))))
      (:`GroundAlbedo`
        (bind _newvalue_6 (`/Game/QuietRuntimeEditor/Common/Blueprints/BP_QuietJsonMacroLibrary.ReadLinearColorWithCheck` _jsonvalue _property (`KismetMathLibrary.Conv_ColorToLinearColor` (`VolumetricCloudComponent.GroundAlbedo` _asvolumetric_cloud_component)))
          (:`then`
            (`VolumetricCloudComponent.SetGroundAlbedo` _asvolumetric_cloud_component (`KismetMathLibrary.Conv_LinearColorToColor` _newvalue_6))))))
    (return true)
    (else
      (return true))))