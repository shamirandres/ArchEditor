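; Marshal for CableComponent in the QuietRuntimeEditor serialization layer, converting cable properties to and from JSON for runtime editing.
; Set and Get defer to the parent first, then switch on property name; SerializeObject saves all cable fields, storing the attached actor as a GUID.
; CollectProperties builds a Cable parameter group with an Advanced subgroup, showing friction only while collision is enabled.
; Width and tiling edits double-toggle custom depth, apparently to force a render refresh.
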(fn `CollectProperties`
  (params (Object :type "Object Object Reference") (TargetJson :type "JsonObjectWrapper Structure (by ref)"))
  (locals (Cable :type "Array of JsonObjectWrapper Structure") (CableAdvanced :type "Array of JsonObjectWrapper Structure"))
  (bind _ascable_component (cast `CableComponent` Object))
  (`|ExecutionSequence`
    (:`then_0`
      (bind _jsonobject (`self.MakeObjectParam` "Material" "Material" "" "/Script/Engine.MaterialInstance" (`PrimitiveComponent.GetMaterial` _ascable_component 0)))
      (`KismetArrayLibrary.Array_Add` (`local.Cable`) _jsonobject)
      (bind _jsonobject_2 (`self.MakeBoolParam` "AttachStart" "Attach Start" "" (`CableComponent.bAttachStart` _ascable_component) true))
      (`KismetArrayLibrary.Array_Add` (`local.Cable`) _jsonobject_2)
      (bind _jsonobject_3 (`self.MakeBoolParam` "AttachEnd" "Attach End" "" (`CableComponent.bAttachEnd` _ascable_component) true))
      (`KismetArrayLibrary.Array_Add` (`local.Cable`) _jsonobject_3)
      (bind _jsonobject_4 (`self.MakeActorParam` "AttachEndTo" "Attach End To" "" (`CableComponent.GetAttachedActor` _ascable_component) null "/Script/Engine.Actor" (`|MakeSet`)))
      (`KismetArrayLibrary.Array_Add` (`local.Cable`) _jsonobject_4)
      (bind _jsonobject_5 (`self.MakeVectorParam` "EndLocation" "End Location" "" (`CableComponent.EndLocation` _ascable_component) (100.0 0.0 0.0)))
      (`KismetArrayLibrary.Array_Add` (`local.Cable`) _jsonobject_5)
      (bind _jsonobject_6 (`self.MakeFloatParam` "CableLength" "Cable Length" "" (`CableComponent.CableLength` _ascable_component) 100.0 1.0 10.0 10000.0 1000.0 1 3))
      (`KismetArrayLibrary.Array_Add` (`local.Cable`) _jsonobject_6)
      (bind _jsonobject_7 (`self.MakeIntParam` "SolverIterations" "Solver Iterations" "" (`CableComponent.SolverIterations` _ascable_component) 1 0 0 16 16 true))
      (`KismetArrayLibrary.Array_Add` (`local.Cable`) _jsonobject_7)
      (bind _jsonobject_8 (`self.MakeVectorParam` "CableForce" "Cable Force" "" (`CableComponent.CableForce` _ascable_component) (0.0 0.0 0.0) 0.0 0.0 0.0 0.0 1 3 true))
      (`KismetArrayLibrary.Array_Add` (`local.Cable`) _jsonobject_8)
      (bind _jsonobject_9 (`self.MakeFloatParam` "CableGravityScale" "Cable Gravity Scale" "" (`CableComponent.CableGravityScale` _ascable_component) 1.0 0.0 0.0 0.0 0.0 1 3))
      (`KismetArrayLibrary.Array_Add` (`local.Cable`) _jsonobject_9)
      (bind _jsonobject_10 (`self.MakeFloatParam` "CableWidth" "Cable Width" "" (`CableComponent.CableWidth` _ascable_component) 10.0 0.01 0.01 1000.0 50.0 1 3))
      (`KismetArrayLibrary.Array_Add` (`local.Cable`) _jsonobject_10)
      (bind _jsonobject_11 (`self.MakeFloatParam` "TileMaterial" "Tile Material" "" (`CableComponent.TileMaterial` _ascable_component) 1.0 0.001 0.1 1000.0 8.0 1 3))
      (`KismetArrayLibrary.Array_Add` (`local.Cable`) _jsonobject_11))
    (:`then_1`
      (bind _jsonobject_12 (`self.MakeBoolParam` "EnableStiffness" "Enable Stiffness" "" (`CableComponent.bEnableStiffness` _ascable_component)))
      (`KismetArrayLibrary.Array_Add` (`local.CableAdvanced`) _jsonobject_12)
      (bind _jsonobject_13 (`self.MakeBoolParam` "UseSubstepping" "Use Substepping" "" (`CableComponent.bUseSubstepping` _ascable_component) true))
      (`KismetArrayLibrary.Array_Add` (`local.CableAdvanced`) _jsonobject_13)
      (bind _jsonobject_14 (`self.MakeBoolParam` "SkipCableUpdateWhenNotVisible" "Skip Cable Update When No tVisible" "" (`CableComponent.bSkipCableUpdateWhenNotVisible` _ascable_component)))
      (`KismetArrayLibrary.Array_Add` (`local.CableAdvanced`) _jsonobject_14)
      (bind _benablecollision (`CableComponent.bEnableCollision` _ascable_component))
      (bind _jsonobject_15 (`self.MakeBoolParam` "EnableCollision" "Enable Collision" "" _benablecollision))
      (`|SetJsonField` _jsonobject_15 "Dependencies" (`|MakeArray`))
      (`KismetArrayLibrary.Array_Add` (`local.CableAdvanced`) _jsonobject_15)
      (if _benablecollision
        (bind _jsonobject_16 (`self.MakeFloatParam` "CollisionFriction" "Collision Friction" "" (`CableComponent.CollisionFriction` _ascable_component) 0.2 0.0 0.0 1.0 1.0 1 3 true))
        (`KismetArrayLibrary.Array_Add` (`local.CableAdvanced`) _jsonobject_16))
      (bind _jsonobject_17 (`self.MakeParamSubgroup` "Advanced" (`local.CableAdvanced`)))
      (`KismetArrayLibrary.Array_Add` (`local.Cable`) _jsonobject_17))
    (:`then_2`
      (`|SetJsonField` (`local.TargetJson`) "GroupsState" (`|MakeArray` "Cable"))
      (`|SetJsonField` (`local.TargetJson`) "Cable" (`local.Cable`))
      (`parent.CollectProperties` _ascable_component (`local.TargetJson`))
      (return))))

(fn `GetPropertyValue`
  (params (Object :type "Object Object Reference") (Property :type String))
  (returns (Success :type Boolean) (Value :type "JsonObjectWrapper Structure"))
  (bind _property (`local.Property`))
  (bind (_success _value) (`parent.GetPropertyValue` Object Property))
  (if (not _success)
    (bind _ascable_component (cast `CableComponent` Object))
    (bind _jsonobject (`/Game/QuietRuntimeEditor/Common/Blueprints/BP_QuietJsonFunctionLibrary.NewJson`))
    (switch `string` _property
      (:`Material`
        (`|SetJsonField` _jsonobject _property (`PrimitiveComponent.GetMaterial` _ascable_component 0)))
      (:`AttachStart`
        (`|SetJsonField` _jsonobject _property (`CableComponent.bAttachStart` _ascable_component)))
      (:`AttachEnd`
        (`|SetJsonField` _jsonobject _property (`CableComponent.bAttachEnd` _ascable_component)))
      (:`AttachEndTo`
        (`|SetJsonField` _jsonobject _property (`CableComponent.GetAttachedActor` _ascable_component)))
      (:`EndLocation`
        (`|SetJsonField` _jsonobject _property (`CableComponent.EndLocation` _ascable_component)))
      (:`CableLength`
        (`|SetJsonField` _jsonobject _property (`CableComponent.CableLength` _ascable_component)))
      (:`SolverIterations`
        (`|SetJsonField` _jsonobject _property (`CableComponent.SolverIterations` _ascable_component)))
      (:`EnableStiffness`
        (`|SetJsonField` _jsonobject _property (`CableComponent.bEnableStiffness` _ascable_component)))
      (:`UseSubstepping`
        (`|SetJsonField` _jsonobject _property (`CableComponent.bUseSubstepping` _ascable_component)))
      (:`SkipCableUpdateWhenNotVisible`
        (`|SetJsonField` _jsonobject _property (`CableComponent.bSkipCableUpdateWhenNotVisible` _ascable_component)))
      (:`EnableCollision`
        (`|SetJsonField` _jsonobject _property (`CableComponent.bEnableCollision` _ascable_component)))
      (:`CollisionFriction`
        (`|SetJsonField` _jsonobject _property (`CableComponent.CollisionFriction` _ascable_component)))
      (:`CableForce`
        (`|SetJsonField` _jsonobject _property (`CableComponent.CableForce` _ascable_component)))
      (:`CableGravityScale`
        (`|SetJsonField` _jsonobject _property (`CableComponent.CableGravityScale` _ascable_component)))
      (:`CableWidth`
        (`|SetJsonField` _jsonobject _property (`CableComponent.CableWidth` _ascable_component)))
      (:`TileMaterial`
        (`|SetJsonField` _jsonobject _property (`CableComponent.TileMaterial` _ascable_component))))
    (return true _jsonobject)
    (else
      (return true _value))))

(fn `SerializeObject`
  (params (Object :type "Object Object Reference") (TargetJson :type "JsonObjectWrapper Structure (by ref)"))
  (`parent.SerializeObject` Object TargetJson)
  (bind _ascable_component (cast `CableComponent` Object))
  (`|SetJsonField` (`local.TargetJson`) "Material" (`PrimitiveComponent.GetMaterial` _ascable_component 0))
  (`|SetJsonField` (`local.TargetJson`) "AttachStart" (`CableComponent.bAttachStart` _ascable_component))
  (`|SetJsonField` (`local.TargetJson`) "AttachEnd" (`CableComponent.bAttachEnd` _ascable_component))
  (`|SetJsonField` (`local.TargetJson`) "AttachEndTo" (`/Game/QuietRuntimeEditor/Outliner/Blueprints/BP_QuietOutlinerLibrary.TakeActorGuid` (`CableComponent.GetAttachedActor` _ascable_component)))
  (`|SetJsonField` (`local.TargetJson`) "EndLocation" (`CableComponent.EndLocation` _ascable_component))
  (`|SetJsonField` (`local.TargetJson`) "CableLength" (`CableComponent.CableLength` _ascable_component))
  (`|SetJsonField` (`local.TargetJson`) "SolverIterations" (`CableComponent.SolverIterations` _ascable_component))
  (`|SetJsonField` (`local.TargetJson`) "EnableStiffness" (`CableComponent.bEnableStiffness` _ascable_component))
  (`|SetJsonField` (`local.TargetJson`) "UseSubstepping" (`CableComponent.bUseSubstepping` _ascable_component))
  (`|SetJsonField` (`local.TargetJson`) "SkipCableUpdateWhenNotVisible" (`CableComponent.bSkipCableUpdateWhenNotVisible` _ascable_component))
  (`|SetJsonField` (`local.TargetJson`) "EnableCollision" (`CableComponent.bEnableCollision` _ascable_component))
  (`|SetJsonField` (`local.TargetJson`) "CollisionFriction" (`CableComponent.CollisionFriction` _ascable_component))
  (`|SetJsonField` (`local.TargetJson`) "CableForce" (`CableComponent.CableForce` _ascable_component))
  (`|SetJsonField` (`local.TargetJson`) "CableGravityScale" (`CableComponent.CableGravityScale` _ascable_component))
  (`|SetJsonField` (`local.TargetJson`) "CableWidth" (`CableComponent.CableWidth` _ascable_component))
  (`|SetJsonField` (`local.TargetJson`) "TileMaterial" (`CableComponent.TileMaterial` _ascable_component))
  (return))

(fn `SetPropertyValue`
  (params (Object :type "Object Object Reference") (Property :type String) (JsonValue :type "JsonObjectWrapper Structure (by ref)"))
  (returns (Success :type Boolean))
  (bind _property (`local.Property`))
  (bind _jsonvalue (`local.JsonValue`))
  (bind _success (`parent.SetPropertyValue` Object Property JsonValue))
  (if (not _success)
    (bind _ascable_component (cast `CableComponent` Object))
    (switch `string` _property
      (:`Material`
        (bind _newvalue (`/Game/QuietRuntimeEditor/Common/Blueprints/BP_QuietJsonMacroLibrary.ReadMaterialWithCheck` _jsonvalue _property (`PrimitiveComponent.GetMaterial` _ascable_component 0))
          (:`then`
            (`PrimitiveComponent.SetMaterial` _ascable_component 0 _newvalue)
            (return true))))
      (:`AttachStart`
        (bind _newvalue_2 (`/Game/QuietRuntimeEditor/Common/Blueprints/BP_QuietJsonMacroLibrary.ReadBoolWithCheck` _jsonvalue _property (`CableComponent.bAttachStart` _ascable_component))
          (:`then`
            (set `CableComponent.bAttachStart` _newvalue_2 _ascable_component)
            (return true))))
      (:`AttachEnd`
        (bind _newvalue_3 (`/Game/QuietRuntimeEditor/Common/Blueprints/BP_QuietJsonMacroLibrary.ReadBoolWithCheck` _jsonvalue _property (`CableComponent.bAttachEnd` _ascable_component))
          (:`then`
            (set `CableComponent.bAttachEnd` _newvalue_3 _ascable_component)
            (return true))))
      (:`AttachEndTo`
        (bind (_actor _success_2) (`self.ReadActorWithCheck` 1.0 _ascable_component _jsonvalue _property))
        (if _success_2
          (`CableComponent.SetAttachEndTo` _ascable_component _actor "None" "None")
          (return true)))
      (:`EndLocation`
        (bind _newvalue_4 (`/Game/QuietRuntimeEditor/Common/Blueprints/BP_QuietJsonMacroLibrary.ReadVectorWithCheck` _jsonvalue _property (`CableComponent.EndLocation` _ascable_component))
          (:`then`
            (set `CableComponent.EndLocation` _newvalue_4 _ascable_component)
            (return true))))
      (:`CableLength`
        (bind _newvalue_5 (`/Game/QuietRuntimeEditor/Common/Blueprints/BP_QuietJsonMacroLibrary.ReadFloatWithCheck` _jsonvalue _property (`CableComponent.CableLength` _ascable_component))
          (:`then`
            (set `CableComponent.CableLength` _newvalue_5 _ascable_component)
            (return true))))
      (:`SolverIterations`
        (bind _newvalue_6 (`/Game/QuietRuntimeEditor/Common/Blueprints/BP_QuietJsonMacroLibrary.ReadIntegerWithCheck` _jsonvalue _property (`CableComponent.SolverIterations` _ascable_component))
          (:`then`
            (set `CableComponent.SolverIterations` _newvalue_6 _ascable_component)
            (return true))))
      (:`EnableStiffness`
        (bind _newvalue_7 (`/Game/QuietRuntimeEditor/Common/Blueprints/BP_QuietJsonMacroLibrary.ReadBoolWithCheck` _jsonvalue _property (`CableComponent.bEnableStiffness` _ascable_component))
          (:`then`
            (set `CableComponent.bEnableStiffness` _newvalue_7 _ascable_component)
            (return true))))
      (:`UseSubstepping`
        (bind _newvalue_8 (`/Game/QuietRuntimeEditor/Common/Blueprints/BP_QuietJsonMacroLibrary.ReadBoolWithCheck` _jsonvalue _property (`CableComponent.bUseSubstepping` _ascable_component))
          (:`then`
            (set `CableComponent.bUseSubstepping` _newvalue_8 _ascable_component)
            (return true))))
      (:`SkipCableUpdateWhenNotVisible`
        (bind _newvalue_9 (`/Game/QuietRuntimeEditor/Common/Blueprints/BP_QuietJsonMacroLibrary.ReadBoolWithCheck` _jsonvalue _property (`CableComponent.bSkipCableUpdateWhenNotVisible` _ascable_component))
          (:`then`
            (set `CableComponent.bSkipCableUpdateWhenNotVisible` _newvalue_9 _ascable_component)
            (return true))))
      (:`EnableCollision`
        (bind _newvalue_10 (`/Game/QuietRuntimeEditor/Common/Blueprints/BP_QuietJsonMacroLibrary.ReadBoolWithCheck` _jsonvalue _property (`CableComponent.bEnableCollision` _ascable_component))
          (:`then`
            (set `CableComponent.bEnableCollision` _newvalue_10 _ascable_component)
            (return true))))
      (:`CollisionFriction`
        (bind _newvalue_11 (`/Game/QuietRuntimeEditor/Common/Blueprints/BP_QuietJsonMacroLibrary.ReadFloatWithCheck` _jsonvalue _property (`CableComponent.CollisionFriction` _ascable_component))
          (:`then`
            (set `CableComponent.CollisionFriction` _newvalue_11 _ascable_component)
            (return true))))
      (:`CableForce`
        (bind _newvalue_12 (`/Game/QuietRuntimeEditor/Common/Blueprints/BP_QuietJsonMacroLibrary.ReadVectorWithCheck` _jsonvalue _property (`CableComponent.CableForce` _ascable_component))
          (:`then`
            (set `CableComponent.CableForce` _newvalue_12 _ascable_component)
            (return true))))
      (:`CableGravityScale`
        (bind _newvalue_13 (`/Game/QuietRuntimeEditor/Common/Blueprints/BP_QuietJsonMacroLibrary.ReadFloatWithCheck` _jsonvalue _property (`CableComponent.CableGravityScale` _ascable_component))
          (:`then`
            (set `CableComponent.CableGravityScale` _newvalue_13 _ascable_component)
            (return true))))
      (:`CableWidth`
        (bind _newvalue_14 (`/Game/QuietRuntimeEditor/Common/Blueprints/BP_QuietJsonMacroLibrary.ReadFloatWithCheck` _jsonvalue _property (`CableComponent.CableWidth` _ascable_component))
          (:`then`
            (set `CableComponent.CableWidth` _newvalue_14 _ascable_component)
            (`self.UpdateComponent` _ascable_component :!label _label)
            (return true))))
      (:`TileMaterial`
        (bind _newvalue_15 (`/Game/QuietRuntimeEditor/Common/Blueprints/BP_QuietJsonMacroLibrary.ReadFloatWithCheck` _jsonvalue _property (`CableComponent.TileMaterial` _ascable_component))
          (:`then`
            (set `CableComponent.TileMaterial` _newvalue_15 _ascable_component)
            (goto _label)))))
    (else
      (return true))))

(fn `UpdateComponent`
  (params (Primitive :type "PrimitiveComponent Object Reference"))
  (bind _returnvalue (not (`PrimitiveComponent.bRenderCustomDepth` Primitive)))
  (`PrimitiveComponent.SetRenderCustomDepth` Primitive _returnvalue)
  (`PrimitiveComponent.SetRenderCustomDepth` Primitive _returnvalue))