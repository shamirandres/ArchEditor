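; Runtime editor marshal that exposes CameraComponent properties for editing and serializes them to JSON.
; It describes projection mode, field of view and blend weight as typed UI params, with get and set by property name.
; Post-process settings are read and written whole as "Settings".
; Editable post-process params and unrecognized property writes are delegated to a BP_MarshalPostprocess component, found or added on the owner on demand.
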(fn `AcquirePostprocessMarshal`
  (returns (Marshal :type "/Game/QuietRuntimeEditor/Serialization/Marshals/BP_MarshalPostprocess Object Reference"))
  (bind _pinned (`/Game/QuietRuntimeEditor/Common/Blueprints/BP_QuietJsonMacroLibrary.Pin` (`Actor.GetComponentByClass` (`self.GetOwner`) "/Game/QuietRuntimeEditor/Serialization/Marshals/BP_MarshalPostprocess.BP_MarshalPostprocess_C")))
  (`/Engine/EditorBlueprintResources/StandardMacros.IsValid` _pinned
    (:`Is Valid`
      (return _pinned))
    (:`Is Not Valid`
      (bind _returnvalue (`|AddComponentByClass` (`self.GetOwner`) "/Game/QuietRuntimeEditor/Serialization/Marshals/BP_MarshalPostprocess.BP_MarshalPostprocess_C"))
      (return _returnvalue))))

(fn `CollectProperties`
  (params (Object :type "Object Object Reference") (TargetJson :type "JsonObjectWrapper Structure (by ref)"))
  (locals (Options :type "Array of JsonObjectWrapper Structure"))
  (bind _ascamera_component (cast `CameraComponent` Object))
  (bind _jsonobject (`self.MakeEnumParam` "ProjectionMode" "Projection Mode" "" (`|MakeArray` "Perspective" "Orthographic") (`KismetMathLibrary.Conv_ByteToInt` (`CameraComponent.ProjectionMode` _ascamera_component))))
  (`KismetArrayLibrary.Array_Add` (`local.Options`) _jsonobject)
  (bind _jsonobject_2 (`self.MakeFloatParam` "FieldOfView" "Field Of View" "" (`CameraComponent.FieldOfView` _ascamera_component) 90.0 0.001 5.0 360.0 170.0 1 3))
  (`KismetArrayLibrary.Array_Add` (`local.Options`) _jsonobject_2)
  (bind _jsonobject_3 (`self.MakeFloatParam` "PostprocessBlendWeight" "Postprocess Blend Weight" "" (`CameraComponent.PostProcessBlendWeight` _ascamera_component) 1.0 0.0 0.0 1.0 1.0 1 3))
  (`KismetArrayLibrary.Array_Add` (`local.Options`) _jsonobject_3)
  (`|SetJsonField` (`local.TargetJson`) "Camera" (`local.Options`))
  (`/Game/QuietRuntimeEditor/Serialization/Marshals/BP_MarshalPostprocess.CollectPostprocessSettings` (`self.AcquirePostprocessMarshal`) (`CameraComponent.PostProcessSettings` _ascamera_component) (`local.TargetJson`))
  (return))

(fn `GetPropertyValue`
  (params (Object :type "Object Object Reference") (Property :type String))
  (returns (Success :type Boolean) (Value :type "JsonObjectWrapper Structure"))
  (bind _property (`local.Property`))
  (bind _ascamera_component (cast `CameraComponent` Object))
  (bind _jsonobject (`/Game/QuietRuntimeEditor/Common/Blueprints/BP_QuietJsonFunctionLibrary.NewJson`))
  (switch `string` _property
    (:`ProjectionMode`
      (`|SetJsonField` _jsonobject _property (`KismetMathLibrary.Conv_ByteToInt` (`CameraComponent.ProjectionMode` _ascamera_component))))
    (:`FieldOfView`
      (`|SetJsonField` _jsonobject _property (`CameraComponent.FieldOfView` _ascamera_component)))
    (:`PostprocessBlendWeight`
      (`|SetJsonField` _jsonobject _property (`CameraComponent.PostProcessBlendWeight` _ascamera_component)))
    (:`Settings`
      (`|SetJsonField` _jsonobject _property (`CameraComponent.PostProcessSettings` _ascamera_component))))
  (return true _jsonobject))

(fn `SerializeObject`
  (params (Object :type "Object Object Reference") (TargetJson :type "JsonObjectWrapper Structure (by ref)"))
  (bind _ascamera_component (cast `CameraComponent` Object))
  (`|SetJsonField` TargetJson "ProjectionMode" (`KismetMathLibrary.Conv_ByteToInt` (`CameraComponent.ProjectionMode` _ascamera_component)))
  (`|SetJsonField` TargetJson "FieldOfView" (`CameraComponent.FieldOfView` _ascamera_component))
  (`|SetJsonField` TargetJson "PostprocessBlendWeight" (`CameraComponent.PostProcessBlendWeight` _ascamera_component))
  (`|SetJsonField` TargetJson "Settings" (`CameraComponent.PostProcessSettings` _ascamera_component))
  (return))

(fn `SetPropertyValue`
  (params (Object :type "Object Object Reference") (Property :type String) (JsonValue :type "JsonObjectWrapper Structure (by ref)"))
  (returns (Success :type Boolean))
  (bind _property (`local.Property`))
  (bind _jsonvalue (`local.JsonValue`))
  (bind _ascamera_component (cast `CameraComponent` Object))
  (switch `string` _property
    (:`Default`
      (bind _newsettings (`/Game/QuietRuntimeEditor/Serialization/Marshals/BP_MarshalPostprocess.SetSettingsProperty` (`self.AcquirePostprocessMarshal`) (`CameraComponent.PostProcessSettings` _ascamera_component) (`local.JsonValue`) (`local.Property`)))
      (set `CameraComponent.PostProcessSettings` _newsettings _ascamera_component)
      (return true))
    (:`ProjectionMode`
      (bind _newvalue (`/Game/QuietRuntimeEditor/Common/Blueprints/BP_QuietJsonMacroLibrary.ReadEnumWithCheck` _jsonvalue _property (`CameraComponent.ProjectionMode` _ascamera_component))
        (:`then`
          (set `CameraComponent.ProjectionMode` (cast `ECameraProjectionMode` _newvalue) _ascamera_component)
          (return true))))
    (:`FieldOfView`
      (bind _newvalue_2 (`/Game/QuietRuntimeEditor/Common/Blueprints/BP_QuietJsonMacroLibrary.ReadFloatWithCheck` _jsonvalue _property (`CameraComponent.FieldOfView` _ascamera_component))
        (:`then`
          (`CameraComponent.SetFieldOfView` _ascamera_component _newvalue_2)
          (return true))))
    (:`PostprocessBlendWeight`
      (bind _newvalue_3 (`/Game/QuietRuntimeEditor/Common/Blueprints/BP_QuietJsonMacroLibrary.ReadFloatWithCheck` _jsonvalue _property (`CameraComponent.PostProcessBlendWeight` _ascamera_component))
        (:`then`
          (set `CameraComponent.PostProcessBlendWeight` _newvalue_3 _ascamera_component)
          (return true))))
    (:`Settings`
      (bind (_outvalue _returnvalue) (`|GetJsonField` _jsonvalue "Settings"))
      (if _returnvalue
        (set `CameraComponent.PostProcessSettings` _outvalue _ascamera_component)
        (return true)))))