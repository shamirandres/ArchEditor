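; Marshal that serializes and edits SpringArmComponent properties as JSON for the Quiet runtime editor.
; SerializeObject writes the arm, collision and camera lag settings, while GetPropertyValue and SetPropertyValue handle one named property, with writes passing through checked readers.
; CollectProperties builds typed editor params in Arm, Collision and Lag groups, adding probe channel and size only when collision testing is enabled.
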(fn `CollectProperties`
  (params (Object :type "Object Object Reference") (TargetJson :type "JsonObjectWrapper Structure (by ref)"))
  (locals (Arm :type "Array of JsonObjectWrapper Structure") (Collision :type "Array of JsonObjectWrapper Structure") (Lag :type "Array of JsonObjectWrapper Structure"))
  (bind _asspring_arm_component (cast `SpringArmComponent` Object))
  (bind _jsonobject (`self.MakeFloatParam` "TargetArmLength" "Target Arm Length" "" (`SpringArmComponent.TargetArmLength` _asspring_arm_component) 0.0 0.0 0.0 0.0 0.0 1 3))
  (`KismetArrayLibrary.Array_Add` (`local.Arm`) _jsonobject)
  (bind _jsonobject_2 (`self.MakeVectorParam` "SocketOffset" "Socket Offset" "" (`SpringArmComponent.SocketOffset` _asspring_arm_component)))
  (`KismetArrayLibrary.Array_Add` (`local.Arm`) _jsonobject_2)
  (bind _jsonobject_3 (`self.MakeVectorParam` "TargetOffset" "Target Offset" "" (`SpringArmComponent.TargetOffset` _asspring_arm_component)))
  (`KismetArrayLibrary.Array_Add` (`local.Arm`) _jsonobject_3)
  (bind _bdocollisiontest (`SpringArmComponent.bDoCollisionTest` _asspring_arm_component))
  (bind _jsonobject_4 (`self.MakeBoolParam` "DoCollisionTest" "DoCollisionTest" "" _bdocollisiontest))
  (`KismetArrayLibrary.Array_Add` (`local.Collision`) _jsonobject_4)
  (if _bdocollisiontest
    (bind _jsonobject_5 (`self.MakeEnumParam` "ProbeChannel" "Probe Channel" "" (`|MakeArray` "WorldStatic" "WorldDynamic" "Pawn" "Visibility" "Camera" "PhysicsBody" "Vehicle" "Destructible" "Gizmo" "Thumbnails") (`KismetMathLibrary.Conv_ByteToInt` (`SpringArmComponent.ProbeChannel` _asspring_arm_component)) 4))
    (`KismetArrayLibrary.Array_Add` (`local.Collision`) _jsonobject_5)
    (bind _jsonobject_6 (`self.MakeFloatParam` "ProbeSize" "Probe Size" "" (`SpringArmComponent.ProbeSize` _asspring_arm_component) 12.0 0.0 0.0 0.0 0.0 1 3))
    (`KismetArrayLibrary.Array_Add` (`local.Collision`) _jsonobject_6))
  (bind _jsonobject_7 (`self.MakeBoolParam` "EnableCameraLag" "Enable Camera Lag" "" (`SpringArmComponent.bEnableCameraLag` _asspring_arm_component)))
  (`KismetArrayLibrary.Array_Add` (`local.Lag`) _jsonobject_7)
  (bind _jsonobject_8 (`self.MakeBoolParam` "EnableCameraRotationLag" "Enable Camera Rotation Lag" "" (`SpringArmComponent.bEnableCameraRotationLag` _asspring_arm_component)))
  (`KismetArrayLibrary.Array_Add` (`local.Lag`) _jsonobject_8)
  (bind _jsonobject_9 (`self.MakeFloatParam` "CameraLagSpeed" "Camera Lag Speed" "" (`SpringArmComponent.CameraLagSpeed` _asspring_arm_component) 10.0 0.0 0.0 1000.0 30.0 1 3))
  (`KismetArrayLibrary.Array_Add` (`local.Lag`) _jsonobject_9)
  (bind _jsonobject_10 (`self.MakeFloatParam` "CameraRotationLagSpeed" "Camera Rotation Lag Speed" "" (`SpringArmComponent.CameraRotationLagSpeed` _asspring_arm_component) 10.0 0.0 0.0 1000.0 30.0 1 3))
  (`KismetArrayLibrary.Array_Add` (`local.Lag`) _jsonobject_10)
  (bind _jsonobject_11 (`self.MakeFloatParam` "CameraLagMaxDistance" "Camera Lag Max Distance" "" (`SpringArmComponent.CameraLagMaxDistance` _asspring_arm_component) 0.0 0.0 0.0 0.0 0.0 1 3))
  (`KismetArrayLibrary.Array_Add` (`local.Lag`) _jsonobject_11)
  (`|SetJsonField` (`local.TargetJson`) "GroupsState" (`|MakeArray` "Arm" "Collision" "Lag"))
  (`|SetJsonField` (`local.TargetJson`) "Arm" (`local.Arm`))
  (`|SetJsonField` (`local.TargetJson`) "Collision" (`local.Collision`))
  (`|SetJsonField` (`local.TargetJson`) "Lag" (`local.Lag`))
  (return))

(fn `GetPropertyValue`
  (params (Object :type "Object Object Reference") (Property :type String))
  (returns (Success :type Boolean) (Value :type "JsonObjectWrapper Structure"))
  (bind _property (`local.Property`))
  (bind _asspring_arm_component (cast `SpringArmComponent` Object))
  (bind _jsonobject (`/Game/QuietRuntimeEditor/Common/Blueprints/BP_QuietJsonFunctionLibrary.NewJson`))
  (switch `string` _property
    (:`TargetArmLength`
      (`|SetJsonField` _jsonobject _property (`SpringArmComponent.TargetArmLength` _asspring_arm_component)))
    (:`SocketOffset`
      (`|SetJsonField` _jsonobject _property (`SpringArmComponent.SocketOffset` _asspring_arm_component)))
    (:`TargetOffset`
      (`|SetJsonField` _jsonobject _property (`SpringArmComponent.TargetOffset` _asspring_arm_component)))
    (:`DoCollisionTest`
      (`|SetJsonField` _jsonobject _property (`SpringArmComponent.bDoCollisionTest` _asspring_arm_component)))
    (:`ProbeChannel`
      (`|SetJsonField` _jsonobject _property (`KismetMathLibrary.Conv_ByteToInt` (`SpringArmComponent.ProbeChannel` _asspring_arm_component))))
    (:`ProbeSize`
      (`|SetJsonField` _jsonobject _property (`SpringArmComponent.ProbeSize` _asspring_arm_component)))
    (:`EnableCameraLag`
      (`|SetJsonField` _jsonobject _property (`SpringArmComponent.bEnableCameraLag` _asspring_arm_component)))
    (:`EnableCameraRotationLag`
      (`|SetJsonField` _jsonobject _property (`SpringArmComponent.bEnableCameraRotationLag` _asspring_arm_component)))
    (:`CameraLagSpeed`
      (`|SetJsonField` _jsonobject _property (`SpringArmComponent.CameraLagSpeed` _asspring_arm_component)))
    (:`CameraRotationLagSpeed`
      (`|SetJsonField` _jsonobject _property (`SpringArmComponent.CameraRotationLagSpeed` _asspring_arm_component)))
    (:`CameraLagMaxDistance`
      (`|SetJsonField` _jsonobject _property (`SpringArmComponent.CameraLagMaxDistance` _asspring_arm_component))))
  (return true _jsonobject))

(fn `SerializeObject`
  (params (Object :type "Object Object Reference") (TargetJson :type "JsonObjectWrapper Structure (by ref)"))
  (bind _asspring_arm_component (cast `SpringArmComponent` Object))
  (`|SetJsonField` TargetJson "TargetArmLength" (`SpringArmComponent.TargetArmLength` _asspring_arm_component))
  (`|SetJsonField` TargetJson "SocketOffset" (`SpringArmComponent.SocketOffset` _asspring_arm_component))
  (`|SetJsonField` TargetJson "TargetOffset" (`SpringArmComponent.TargetOffset` _asspring_arm_component))
  (`|SetJsonField` TargetJson "DoCollisionTest" (`SpringArmComponent.bDoCollisionTest` _asspring_arm_component))
  (`|SetJsonField` TargetJson "ProbeChannel" (`KismetMathLibrary.Conv_ByteToInt` (`SpringArmComponent.ProbeChannel` _asspring_arm_component)))
  (`|SetJsonField` TargetJson "ProbeSize" (`SpringArmComponent.ProbeSize` _asspring_arm_component))
  (`|SetJsonField` TargetJson "EnableCameraLag" (`SpringArmComponent.bEnableCameraLag` _asspring_arm_component))
  (`|SetJsonField` TargetJson "EnableCameraRotationLag" (`SpringArmComponent.bEnableCameraRotationLag` _asspring_arm_component))
  (`|SetJsonField` TargetJson "CameraLagSpeed" (`SpringArmComponent.CameraLagSpeed` _asspring_arm_component))
  (`|SetJsonField` TargetJson "CameraRotationLagSpeed" (`SpringArmComponent.CameraRotationLagSpeed` _asspring_arm_component))
  (`|SetJsonField` TargetJson "CameraLagMaxDistance" (`SpringArmComponent.CameraLagMaxDistance` _asspring_arm_component))
  (return))

(fn `SetPropertyValue`
  (params (Object :type "Object Object Reference") (Property :type String) (JsonValue :type "JsonObjectWrapper Structure (by ref)"))
  (returns (Success :type Boolean))
  (bind _property (`local.Property`))
  (bind _jsonvalue (`local.JsonValue`))
  (bind _asspring_arm_component (cast `SpringArmComponent` Object))
  (switch `string` _property
    (:`TargetArmLength`
      (bind _newvalue (`/Game/QuietRuntimeEditor/Common/Blueprints/BP_QuietJsonMacroLibrary.ReadFloatWithCheck` _jsonvalue _property (`SpringArmComponent.TargetArmLength` _asspring_arm_component))
        (:`then`
          (set `SpringArmComponent.TargetArmLength` _newvalue _asspring_arm_component))))
    (:`SocketOffset`
      (bind _newvalue_2 (`/Game/QuietRuntimeEditor/Common/Blueprints/BP_QuietJsonMacroLibrary.ReadVectorWithCheck` _jsonvalue _property (`SpringArmComponent.SocketOffset` _asspring_arm_component))
        (:`then`
          (set `SpringArmComponent.SocketOffset` _newvalue_2 _asspring_arm_component))))
    (:`TargetOffset`
      (bind _newvalue_3 (`/Game/QuietRuntimeEditor/Common/Blueprints/BP_QuietJsonMacroLibrary.ReadVectorWithCheck` _jsonvalue _property (`SpringArmComponent.TargetOffset` _asspring_arm_component))
        (:`then`
          (set `SpringArmComponent.TargetOffset` _newvalue_3 _asspring_arm_component))))
    (:`DoCollisionTest`
      (bind _newvalue_4 (`/Game/QuietRuntimeEditor/Common/Blueprints/BP_QuietJsonMacroLibrary.ReadBoolWithCheck` _jsonvalue _property (`SpringArmComponent.bDoCollisionTest` _asspring_arm_component))
        (:`then`
          (set `SpringArmComponent.bDoCollisionTest` _newvalue_4 _asspring_arm_component))))
    (:`ProbeChannel`
      (bind _newvalue_5 (`/Game/QuietRuntimeEditor/Common/Blueprints/BP_QuietJsonMacroLibrary.ReadEnumWithCheck` _jsonvalue _property (`SpringArmComponent.ProbeChannel` _asspring_arm_component))
        (:`then`
          (set `SpringArmComponent.ProbeChannel` (cast `ECollisionChannel` _newvalue_5) _asspring_arm_component))))
    (:`ProbeSize`
      (bind _newvalue_6 (`/Game/QuietRuntimeEditor/Common/Blueprints/BP_QuietJsonMacroLibrary.ReadFloatWithCheck` _jsonvalue _property (`SpringArmComponent.ProbeSize` _asspring_arm_component))
        (:`then`
          (set `SpringArmComponent.ProbeSize` _newvalue_6 _asspring_arm_component))))
    (:`EnableCameraLag`
      (bind _newvalue_7 (`/Game/QuietRuntimeEditor/Common/Blueprints/BP_QuietJsonMacroLibrary.ReadBoolWithCheck` _jsonvalue _property (`SpringArmComponent.bEnableCameraLag` _asspring_arm_component))
        (:`then`
          (set `SpringArmComponent.bEnableCameraLag` _newvalue_7 _asspring_arm_component))))
    (:`EnableCameraRotationLag`
      (bind _newvalue_8 (`/Game/QuietRuntimeEditor/Common/Blueprints/BP_QuietJsonMacroLibrary.ReadBoolWithCheck` _jsonvalue _property (`SpringArmComponent.bEnableCameraRotationLag` _asspring_arm_component))
        (:`then`
          (set `SpringArmComponent.bEnableCameraRotationLag` _newvalue_8 _asspring_arm_component))))
    (:`CameraLagSpeed`
      (bind _newvalue_9 (`/Game/QuietRuntimeEditor/Common/Blueprints/BP_QuietJsonMacroLibrary.ReadFloatWithCheck` _jsonvalue _property (`SpringArmComponent.CameraLagSpeed` _asspring_arm_component))
        (:`then`
          (set `SpringArmComponent.CameraLagSpeed` _newvalue_9 _asspring_arm_component))))
    (:`CameraRotationLagSpeed`
      (bind _newvalue_10 (`/Game/QuietRuntimeEditor/Common/Blueprints/BP_QuietJsonMacroLibrary.ReadFloatWithCheck` _jsonvalue _property (`SpringArmComponent.CameraRotationLagSpeed` _asspring_arm_component))
        (:`then`
          (set `SpringArmComponent.CameraRotationLagSpeed` _newvalue_10 _asspring_arm_component))))
    (:`CameraLagMaxDistance`
      (bind _newvalue_11 (`/Game/QuietRuntimeEditor/Common/Blueprints/BP_QuietJsonMacroLibrary.ReadFloatWithCheck` _jsonvalue _property (`SpringArmComponent.CameraLagMaxDistance` _asspring_arm_component))
        (:`then`
          (set `SpringArmComponent.CameraLagMaxDistance` _newvalue_11 _asspring_arm_component)))))
  (return true))