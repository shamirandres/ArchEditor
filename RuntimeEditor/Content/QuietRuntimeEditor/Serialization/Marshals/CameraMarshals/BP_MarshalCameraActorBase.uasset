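; Marshal for BP_CameraActorBase in the runtime editor, exposing its properties and actions and saving its state as JSON.
; Property reads and writes try the parent, then the Camera and SpringArm components (in opposite order for writes), with LocalRotation mapped to the Socket's relative rotation.
; Serialize and restore delegate both components to the Source object.
; CollectProperties builds Camera and SpringArm groups, adding Activate, Deactivate, MoveAlongSpline and Stop actions, which CallAction dispatches.
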(fn `CallAction`
  (params (Object :type "Object Object Reference") (Action :type "JsonObjectWrapper Structure"))
  (returns (Success :type Boolean))
  (bind _success (`parent.CallAction` Object Action))
  (if (not _success)
    (bind _ascameraactorbase (cast `/Game/QuietRuntimeEditor/Common/QuietActors/BP_CameraActorBase` Object))
    (bind _outvalue (`|GetJsonField` Action "Action"))
    (switch `string` _outvalue
      (:`Activate`
        (`/Game/QuietRuntimeEditor/Common/QuietActors/BP_CameraActorBase.Activate` _ascameraactorbase))
      (:`Deactivate`
        (`/Game/QuietRuntimeEditor/Common/QuietActors/BP_CameraActorBase.Deactivate` _ascameraactorbase))
      (:`MoveAlongSpline`
        (`/Game/QuietRuntimeEditor/Common/QuietActors/BP_CameraActorBase.MoveAlongSpline` _ascameraactorbase))
      (:`Stop`
        (`/Game/QuietRuntimeEditor/Common/QuietActors/BP_CameraActorBase.Stop` _ascameraactorbase)))
    (else
      (return true))))

(fn `CollectProperties`
  (params (Object :type "Object Object Reference") (TargetJson :type "JsonObjectWrapper Structure (by ref)"))
  (locals (Camera :type "Array of JsonObjectWrapper Structure") (SpringArm :type "Array of JsonObjectWrapper Structure") (Postprocess :type "Array of JsonObjectWrapper Structure"))
  (bind _ascameraactorbase (cast `/Game/QuietRuntimeEditor/Common/QuietActors/BP_CameraActorBase` Object))
  (`|ExecutionSequence`
    (:`then_0`
      (bind _jsonobject (`/Game/QuietRuntimeEditor/Common/Blueprints/BP_QuietJsonFunctionLibrary.NewJson`))
      (message `/Game/QuietRuntimeEditor/Serialization/BI_SerializerInterface.GrabDetails` (`self.GetSource`) (`/Game/QuietRuntimeEditor/Common/QuietActors/BP_CameraActorBase.GetCamera` _ascameraactorbase) _jsonobject)
      (bind _outvalue (`|GetJsonField` _jsonobject "Camera"))
      (for _array_element _outvalue
        (`KismetArrayLibrary.Array_Add` (`local.Camera`) _array_element))
      (bind _param (`self.MakeActionsParam` (`|MakeArray` "Activate" "Deactivate" "MoveAlongSpline" "Stop")))
      (`KismetArrayLibrary.Array_Add` (`local.Camera`) _param))
    (:`then_1`
      (bind _jsonobject_2 (`/Game/QuietRuntimeEditor/Common/Blueprints/BP_QuietJsonFunctionLibrary.NewJson`))
      (message `/Game/QuietRuntimeEditor/Serialization/BI_SerializerInterface.GrabDetails` (`self.GetSource`) (`/Game/QuietRuntimeEditor/Common/QuietActors/BP_CameraActorBase.SpringArm` _ascameraactorbase) _jsonobject_2)
      (bind _fieldnames (`JsonBlueprintFunctionLibrary.GetFieldNames` _jsonobject_2))
      (for (_array_element_2 _array_index) _fieldnames
        (bind _outvalue_2 (`|GetJsonField` _jsonobject_2 _array_element_2))
        (bind _pinned (`/Game/QuietRuntimeEditor/Common/Blueprints/BP_QuietJsonMacroLibrary.PinArray` _outvalue_2))
        (switch `int` _array_index
          (:`Default`
            _)
          (:`1`
            (bind _jsonobject_3 (`self.MakeRotatorParam` "LocalRotation" "Rotation" "" (`SceneComponent.RelativeRotation` (`/Game/QuietRuntimeEditor/Common/QuietActors/BP_CameraActorBase.Socket` _ascameraactorbase))))
            (`KismetArrayLibrary.Array_Add` _pinned _jsonobject_3)))
        (bind _jsonobject_4 (`self.MakeParamSubgroup` _array_element_2 _pinned))
        (`KismetArrayLibrary.Array_Add` (`local.SpringArm`) _jsonobject_4)))
    (:`then_2`
      (`|SetJsonField` (`local.TargetJson`) "GroupsState" (`|MakeArray` "Camera" "SpringArm"))
      (`|SetJsonField` (`local.TargetJson`) "Camera" (`local.Camera`))
      (`|SetJsonField` (`local.TargetJson`) "SpringArm" (`local.SpringArm`))
      (bind _fieldnames_2 (`JsonBlueprintFunctionLibrary.GetFieldNames` _jsonobject))
      (for _index (range 1 (+ (`KismetArrayLibrary.Array_LastIndex` _fieldnames_2) 1))
        (bind _output (`|GetArrayItem` _fieldnames_2 _index))
        (bind _outvalue_3 (`|GetJsonField` _jsonobject _output))
        (`|SetJsonField` (`local.TargetJson`) _output _outvalue_3))
      (`parent.CollectProperties` _ascameraactorbase (`local.TargetJson`))
      (return))))

(fn `GetPropertyValue`
  (params (Object :type "Object Object Reference") (Property :type String))
  (returns (Success :type Boolean) (Value :type "JsonObjectWrapper Structure"))
  (bind _property (`local.Property`))
  (bind (_success _value) (`parent.GetPropertyValue` Object Property))
  (if (not _success)
    (bind _ascameraactorbase (cast `/Game/QuietRuntimeEditor/Common/QuietActors/BP_CameraActorBase` Object))
    (bind (_success_2 _boxedvalue) (message `/Game/QuietRuntimeEditor/Serialization/BI_SerializerInterface.GetValueByName` (`self.GetSource`) (`/Game/QuietRuntimeEditor/Common/QuietActors/BP_CameraActorBase.GetCamera` _ascameraactorbase) (`local.Property`)))
    (if (not _success_2)
      (bind _jsonobject (`/Game/QuietRuntimeEditor/Common/Blueprints/BP_QuietJsonFunctionLibrary.NewJson`))
      (switch `string` _property
        (:`Default`
          (bind (_success_3 _boxedvalue_2) (message `/Game/QuietRuntimeEditor/Serialization/BI_SerializerInterface.GetValueByName` (`self.GetSource`) (`/Game/QuietRuntimeEditor/Common/QuietActors/BP_CameraActorBase.SpringArm` _ascameraactorbase) (`local.Property`)))
          (return _success_3 _boxedvalue_2))
        (:`LocalRotation`
          (`|SetJsonField` _jsonobject _property (`SceneComponent.RelativeRotation` (`/Game/QuietRuntimeEditor/Common/QuietActors/BP_CameraActorBase.Socket` _ascameraactorbase)))
          (return true _jsonobject)))
      (else
        (return true _boxedvalue)))
    (else
      (return true _value))))

(fn `RestoreObject`
  (params (Object :type "Object Object Reference") (JsonObject :type "JsonObjectWrapper Structure"))
  (`parent.RestoreObject` Object JsonObject)
  (bind _ascameraactorbase (cast `/Game/QuietRuntimeEditor/Common/QuietActors/BP_CameraActorBase` Object))
  (bind _outvalue (`|GetJsonField` (`local.JsonObject`) "Camera"))
  (message `/Game/QuietRuntimeEditor/Serialization/BI_SerializerInterface.RestoreObject` (`self.GetSource`) (`/Game/QuietRuntimeEditor/Common/QuietActors/BP_CameraActorBase.GetCamera` _ascameraactorbase) _outvalue)
  (bind _outvalue_2 (`|GetJsonField` (`local.JsonObject`) "SpringArm"))
  (message `/Game/QuietRuntimeEditor/Serialization/BI_SerializerInterface.RestoreObject` (`self.GetSource`) (`/Game/QuietRuntimeEditor/Common/QuietActors/BP_CameraActorBase.SpringArm` _ascameraactorbase) _outvalue_2))

(fn `SerializeObject`
  (params (Object :type "Object Object Reference") (TargetJson :type "JsonObjectWrapper Structure (by ref)"))
  (`parent.SerializeObject` Object TargetJson)
  (bind _ascameraactorbase (cast `/Game/QuietRuntimeEditor/Common/QuietActors/BP_CameraActorBase` Object))
  (bind _cache (message `/Game/QuietRuntimeEditor/Serialization/BI_SerializerInterface.CacheObject` (`self.GetSource`) (`/Game/QuietRuntimeEditor/Common/QuietActors/BP_CameraActorBase.GetCamera` _ascameraactorbase)))
  (`|SetJsonField` (`local.TargetJson`) "Camera" _cache)
  (`|SetJsonField` (`local.TargetJson`) "LocalRotation" (`SceneComponent.RelativeRotation` (`/Game/QuietRuntimeEditor/Common/QuietActors/BP_CameraActorBase.Socket` _ascameraactorbase)))
  (bind _cache_2 (message `/Game/QuietRuntimeEditor/Serialization/BI_SerializerInterface.CacheObject` (`self.GetSource`) (`/Game/QuietRuntimeEditor/Common/QuietActors/BP_CameraActorBase.SpringArm` _ascameraactorbase)))
  (`|SetJsonField` (`local.TargetJson`) "SpringArm" _cache_2)
  (return))

(fn `SetPropertyValue`
  (params (Object :type "Object Object Reference") (Property :type String) (JsonValue :type "JsonObjectWrapper Structure (by ref)"))
  (returns (Success :type Boolean))
  (bind _property (`local.Property`))
  (bind _success (`parent.SetPropertyValue` Object Property JsonValue))
  (if (not _success)
    (bind _ascameraactorbase (cast `/Game/QuietRuntimeEditor/Common/QuietActors/BP_CameraActorBase` Object))
    (bind _success_2 (message `/Game/QuietRuntimeEditor/Serialization/BI_SerializerInterface.SetValueByName` (`self.GetSource`) (`/Game/QuietRuntimeEditor/Common/QuietActors/BP_CameraActorBase.SpringArm` _ascameraactorbase) (`local.Property`) (`local.JsonValue`)))
    (if (not _success_2)
      (switch `string` _property
        (:`Default`
          (bind _success_3 (message `/Game/QuietRuntimeEditor/Serialization/BI_SerializerInterface.SetValueByName` (`self.GetSource`) (`/Game/QuietRuntimeEditor/Common/QuietActors/BP_CameraActorBase.GetCamera` _ascameraactorbase) (`local.Property`) (`local.JsonValue`)))
          (return _success_3))
        (:`LocalRotation`
          (bind _socket (`/Game/QuietRuntimeEditor/Common/QuietActors/BP_CameraActorBase.Socket` _ascameraactorbase))
          (bind _newvalue (`/Game/QuietRuntimeEditor/Common/Blueprints/BP_QuietJsonMacroLibrary.ReadRotatorWithCheck` (`local.JsonValue`) _property (`SceneComponent.RelativeRotation` _socket))
            (:`then`
              (`SceneComponent.K2_SetRelativeRotation` _socket _newvalue false false)
              (return true)))))
      (else
        (return true)))
    (else
      (return true))))