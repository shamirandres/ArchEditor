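; Camera pawn for the Quiet runtime editor, providing fly, pan, Shift-orbit around the selection, focus, align and zoom-to-region navigation.
; Enhanced Input drives movement with a pinned, hidden cursor, while editor hotkeys are thrown as gameplay-tag commands through the Router.
; The pawn subscribes to the Router for camera and input-suspend commands, and serves transform and FOV as JSON.
; Camera moves feed a capped transform history for a separate camera undo.
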(event `/Game/QuietRuntimeEditor/Common/Blueprints/BI_QuietRoutingInterface.ForwardCommand`
  (params (Command :type "GameplayTag Structure"))
  (bind _returnvalue (pcsubsystem `EnhancedInputLocalPlayerSubsystem` (`GameplayStatics.GetPlayerController` 0)))
  ;[0 0 0] Camera
  (`|SwitchGameplayTag` Command
    (:`EditorPawn.Focus`
      (`self.FocusOnSelection`))
    (:`EditorPawn.AlignCamera`
      (`self.AlignCamera`))
    (:`EditorPawn.SuspendInput`
      (bind _returnvalue_2 (`KismetSystemLibrary.LoadAsset_Blocking` (`self.MappingContext`)))
      (bind _asinput_mapping_context (cast `InputMappingContext` _returnvalue_2))
      (`EnhancedInputSubsystemInterface.RemoveMappingContext` _returnvalue _asinput_mapping_context (struct)))
    (:`EditorPawn.ResumeInput`
      (bind _returnvalue_3 (`KismetSystemLibrary.LoadAsset_Blocking` (`self.MappingContext`)))
      (bind _asinput_mapping_context_2 (cast `InputMappingContext` _returnvalue_3))
      (`EnhancedInputSubsystemInterface.AddMappingContext` _returnvalue _asinput_mapping_context_2 0 (struct)))))

(event `/Game/QuietRuntimeEditor/Common/Blueprints/BI_QuietRoutingInterface.ForwardJson`
  (params (Action :type "GameplayTag Structure") (Json :type "JsonObjectWrapper Structure"))
  ;[0 0 0] Camera
  (`|SwitchGameplayTag` Action
    (:`EditorPawn.RestoreCamera`
      (bind _outvalue (`|GetJsonField` Json "Fov"))
      (bind _outvalue_2 (`|GetJsonField` Json "Transform"))
      (`self.SetupCamera` _outvalue_2 _outvalue))
    (:`EditorPawn.ZoomRegion`
      (bind _outvalue_3 (`|GetJsonField` Json "Size"))
      (bind _outvalue_4 (`|GetJsonField` Json "Position"))
      (`self.ZoomRegion` _outvalue_4 _outvalue_3))))

(event `EnhancedInput|/Game/QuietRuntimeEditor/EditorInput/Actions/IA_LeftMouseButton`
  (params (ActionValue :type Boolean) (ElapsedSeconds :type "Float (double-precision)") (TriggeredSeconds :type "Float (double-precision)") (InputAction :type "InputAction Object Reference" :default "/Game/QuietRuntimeEditor/EditorInput/Actions/IA_LeftMouseButton.IA_LeftMouseButton"))
  ;[0 0 0] Camera Inputs
  (:`Started`
    (`self.HideMouseCursor` :!label _label
      (:`then`
        (`self.SaveCameraTransform` false :!label _label_2))
      (:`End`
        (goto _label_2 :!via `Finish`))))
  (:`Completed`
    (goto _label :!via `Show`)))

(event `EnhancedInput|/Game/QuietRuntimeEditor/EditorInput/Actions/IA_Scour`
  (params (ActionValue :type "Vector2D Structure") (ElapsedSeconds :type "Float (double-precision)") (TriggeredSeconds :type "Float (double-precision)") (InputAction :type "InputAction Object Reference" :default "/Game/QuietRuntimeEditor/EditorInput/Actions/IA_Scour.IA_Scour"))
  (bind (_x _y) (`KismetMathLibrary.BreakVector2D` ActionValue))
  (bind (_returnvalue_roll _returnvalue_pitch _returnvalue_yaw) (`KismetMathLibrary.BreakRotator` (`self.GetControlRotation`)))
  ;[0 0 0] Camera Inputs
  ;;[0.001518 0.0356 0.03689] SCOUR
  (:`Triggered`
    (`self.FixMouse` :!label _label_3)
    (`self.AddControllerYawInput` _x)
    (`self.AddMovementInput` (`KismetMathLibrary.GetForwardVector` (`KismetMathLibrary.MakeRotator` _returnvalue_roll 0.0 _returnvalue_yaw)) _y))
  (:`Started`
    (goto _label_3 :!via `Started`)))

(event `self.ReceiveBeginPlay`
  ;[0.00736 0.01766 0.046] Begin Play - Setup
  (`self.EnableInput` (`GameplayStatics.GetPlayerController` 0))
  (`WidgetBlueprintLibrary.SetInputMode_GameAndUIEx` (`GameplayStatics.GetPlayerController` 0) null "DoNotLock" false)
  (`self.RegisterCameraAction` (`self.GetCurrentTransform`))
  (bind _object (`|LoadAsset` (`self.MappingContext`))
    (:`then`
      (`KismetSystemLibrary.Delay` 0.2)
      ;[0 0 0] Setup Router
      (`/Game/QuietRuntimeEditor/Common/Blueprints/BP_Router.SubscribeWithTag` (`/Game/QuietRuntimeEditor/Common/Blueprints/BP_QuietEditorUtilities.GetRouter`) (struct :`TagName` "EditorPawn") self))
    (:`Completed`
      (bind _asinput_mapping_context (cast `InputMappingContext` _object))
      (`EnhancedInputSubsystemInterface.AddMappingContext` (pcsubsystem `EnhancedInputLocalPlayerSubsystem` (`GameplayStatics.GetPlayerController` 0)) _asinput_mapping_context 0 (struct)))))

(event `EnhancedInput|/Game/QuietRuntimeEditor/EditorInput/Actions/IA_MiddleMouseButton`
  (params (ActionValue :type Boolean) (ElapsedSeconds :type "Float (double-precision)") (TriggeredSeconds :type "Float (double-precision)") (InputAction :type "InputAction Object Reference" :default "/Game/QuietRuntimeEditor/EditorInput/Actions/IA_MiddleMouseButton.IA_MiddleMouseButton"))
  ;[0 0 0] Camera Inputs
  (:`Started`
    (`self.HideMouseCursor` :!label _label_4
      (:`then`
        (`self.SaveCameraTransform` false :!label _label_5))
      (:`End`
        (goto _label_5 :!via `Finish`))))
  (:`Completed`
    (goto _label_4 :!via `Show`)))

(event `EnhancedInput|/Game/QuietRuntimeEditor/EditorInput/Actions/IA_PanTilt`
  (params (ActionValue :type "Vector2D Structure") (ElapsedSeconds :type "Float (double-precision)") (TriggeredSeconds :type "Float (double-precision)") (InputAction :type "InputAction Object Reference" :default "/Game/QuietRuntimeEditor/EditorInput/Actions/IA_PanTilt.IA_PanTilt"))
  (bind (_x _y) (`KismetMathLibrary.BreakVector2D` ActionValue))
  ;[0 0 0] Camera Inputs
  ;;[0.001518 0.0356 0.03689] PAN / TILT
  (:`Triggered`
    (`self.FixMouse` :!label _label_6)
    (`self.MoveRight` _x)
    (`self.MoveUp_World` _y))
  (:`Started`
    (goto _label_6 :!via `Started`)))

(event `EnhancedInput|/Game/QuietRuntimeEditor/EditorInput/Actions/IA_UndoCameraAction`
  (params (ActionValue :type Boolean) (ElapsedSeconds :type "Float (double-precision)") (TriggeredSeconds :type "Float (double-precision)") (InputAction :type "InputAction Object Reference" :default "/Game/QuietRuntimeEditor/EditorInput/Actions/IA_UndoCameraAction.IA_UndoCameraAction"))
  ;[0 0 0] History Input Actions
  (:`Triggered`
    (`self.UndoCameraAction`)))

(event `EnhancedInput|/Game/QuietRuntimeEditor/EditorInput/Actions/IA_Undo`
  (params (ActionValue :type Boolean) (ElapsedSeconds :type "Float (double-precision)") (TriggeredSeconds :type "Float (double-precision)") (InputAction :type "InputAction Object Reference" :default "/Game/QuietRuntimeEditor/EditorInput/Actions/IA_Undo.IA_Undo"))
  ;[0 0 0] History Input Actions
  (:`Triggered`
    (`/Game/QuietRuntimeEditor/Common/Blueprints/BP_Router.ThrowCommand` (`/Game/QuietRuntimeEditor/Common/Blueprints/BP_QuietEditorUtilities.GetRouter`) (struct :`TagName` "Manager") (struct :`TagName` "History.Undo"))))

(event `EnhancedInput|/Game/QuietRuntimeEditor/EditorInput/Actions/IA_Focus`
  (params (ActionValue :type Boolean) (ElapsedSeconds :type "Float (double-precision)") (TriggeredSeconds :type "Float (double-precision)") (InputAction :type "InputAction Object Reference" :default "/Game/QuietRuntimeEditor/EditorInput/Actions/IA_Focus.IA_Focus"))
  ;[0 0 0] Input Actions
  (:`Triggered`
    (`self.FocusOnSelection`)))

(event `EnhancedInput|/Game/QuietRuntimeEditor/EditorInput/Actions/IA_SaveCurrentScene`
  (params (ActionValue :type Boolean) (ElapsedSeconds :type "Float (double-precision)") (TriggeredSeconds :type "Float (double-precision)") (InputAction :type "InputAction Object Reference" :default "/Game/QuietRuntimeEditor/EditorInput/Actions/IA_SaveCurrentScene.IA_SaveCurrentScene"))
  ;[0 0 0] Input Actions
  ;;[0 0 0] Open/Save
  (:`Triggered`
    (`/Game/QuietRuntimeEditor/Common/Blueprints/BP_Router.ThrowCommand` (`/Game/QuietRuntimeEditor/Common/Blueprints/BP_QuietEditorUtilities.GetRouter`) (struct :`TagName` "Manager") (struct :`TagName` "Scenes.Save"))))

(event `EnhancedInput|/Game/QuietRuntimeEditor/EditorInput/Actions/IA_RightMouseButton`
  (params (ActionValue :type Boolean) (ElapsedSeconds :type "Float (double-precision)") (TriggeredSeconds :type "Float (double-precision)") (InputAction :type "InputAction Object Reference" :default "/Game/QuietRuntimeEditor/EditorInput/Actions/IA_RightMouseButton.IA_RightMouseButton"))
  ;[0 0 0] Camera Inputs
  (:`Started`
    (`self.HideMouseCursor` :!label _label_7
      (:`then`
        (`self.SaveCameraTransform` false :!label _label_8))
      (:`End`
        (goto _label_8 :!via `Finish`))))
  (:`Completed`
    (goto _label_7 :!via `Show`)))

(event `EnhancedInput|/Game/QuietRuntimeEditor/EditorInput/Actions/IA_Look`
  (params (ActionValue :type "Vector2D Structure") (ElapsedSeconds :type "Float (double-precision)") (TriggeredSeconds :type "Float (double-precision)") (InputAction :type "InputAction Object Reference" :default "/Game/QuietRuntimeEditor/EditorInput/Actions/IA_Look.IA_Look"))
  (bind (_x _y) (`KismetMathLibrary.BreakVector2D` ActionValue))
  ;[0 0 0] Camera Inputs
  ;;[0.001518 0.0356 0.03689] LOOK / ORBIT
  (:`Triggered`
    (`self.FixMouse` :!label _label_9)
    (bind _pivotlocation (`self.GetOrbitPivot`)
      (:`Orbit`
        (`self.OrbitRotation` false _pivotlocation _x)
        (`self.OrbitRotation` true _pivotlocation _y))
      (:`Default`
        (`self.AddControllerYawInput` _x)
        (`self.AddControllerPitchInput` _y))))
  (:`Started`
    (goto _label_9 :!via `Started`)))

(event `EnhancedInput|/Game/QuietRuntimeEditor/EditorInput/Actions/IA_Redo`
  (params (ActionValue :type Boolean) (ElapsedSeconds :type "Float (double-precision)") (TriggeredSeconds :type "Float (double-precision)") (InputAction :type "InputAction Object Reference" :default "/Game/QuietRuntimeEditor/EditorInput/Actions/IA_Redo.IA_Redo"))
  ;[0 0 0] History Input Actions
  (:`Triggered`
    (`/Game/QuietRuntimeEditor/Common/Blueprints/BP_Router.ThrowCommand` (`/Game/QuietRuntimeEditor/Common/Blueprints/BP_QuietEditorUtilities.GetRouter`) (struct :`TagName` "Manager") (struct :`TagName` "History.Redo"))))

(event `EnhancedInput|/Game/QuietRuntimeEditor/EditorInput/Actions/IA_Isolate`
  (params (ActionValue :type Boolean) (ElapsedSeconds :type "Float (double-precision)") (TriggeredSeconds :type "Float (double-precision)") (InputAction :type "InputAction Object Reference" :default "/Game/QuietRuntimeEditor/EditorInput/Actions/IA_Isolate.IA_Isolate"))
  ;[0 0 0] Input Actions
  (:`Triggered`
    (`/Game/QuietRuntimeEditor/Common/Blueprints/BP_Router.ThrowCommand` (`/Game/QuietRuntimeEditor/Common/Blueprints/BP_QuietEditorUtilities.GetRouter`) (struct :`TagName` "Manager") (struct :`TagName` "Outliner.IsolateSelection"))))

(event `EnhancedInput|/Game/QuietRuntimeEditor/EditorInput/Actions/IA_OpenScene`
  (params (ActionValue :type Boolean) (ElapsedSeconds :type "Float (double-precision)") (TriggeredSeconds :type "Float (double-precision)") (InputAction :type "InputAction Object Reference" :default "/Game/QuietRuntimeEditor/EditorInput/Actions/IA_OpenScene.IA_OpenScene"))
  ;[0 0 0] Input Actions
  ;;[0 0 0] Open/Save
  (:`Triggered`
    (`/Game/QuietRuntimeEditor/Common/Blueprints/BP_Router.ThrowCommand` (`/Game/QuietRuntimeEditor/Common/Blueprints/BP_QuietEditorUtilities.GetRouter`) (struct :`TagName` "Manager") (struct :`TagName` "Scenes.Open"))))

(event `EnhancedInput|/Game/QuietRuntimeEditor/EditorInput/Actions/IA_FastMoveForward`
  (params (ActionValue :type "Float (double-precision)") (ElapsedSeconds :type "Float (double-precision)") (TriggeredSeconds :type "Float (double-precision)") (InputAction :type "InputAction Object Reference" :default "/Game/QuietRuntimeEditor/EditorInput/Actions/IA_FastMoveForward.IA_FastMoveForward"))
  ;[0 0 0] Camera Inputs
  ;;[0 0.05729 0.056] WASD + Right Mouse Button
  (:`Triggered`
    (`self.MoveForward` ActionValue))
  (:`Started`
    (`self.SaveCameraTransform` true :!label _label_10))
  (:`Completed`
    (goto _label_10 :!via `Finish`)))

(event `EnhancedInput|/Game/QuietRuntimeEditor/EditorInput/Actions/IA_DeleteActors`
  (params (ActionValue :type Boolean) (ElapsedSeconds :type "Float (double-precision)") (TriggeredSeconds :type "Float (double-precision)") (InputAction :type "InputAction Object Reference" :default "/Game/QuietRuntimeEditor/EditorInput/Actions/IA_DeleteActors.IA_DeleteActors"))
  ;[0 0 0] Input Actions
  (:`Triggered`
    (`/Game/QuietRuntimeEditor/Common/Blueprints/BP_Router.ThrowCommand` (`/Game/QuietRuntimeEditor/Common/Blueprints/BP_QuietEditorUtilities.GetRouter`) (struct :`TagName` "Manager") (struct :`TagName` "Outliner.DeleteActors"))))

(event `EnhancedInput|/Game/QuietRuntimeEditor/EditorInput/Actions/IA_FastMoveBackward`
  (params (ActionValue :type "Float (double-precision)") (ElapsedSeconds :type "Float (double-precision)") (TriggeredSeconds :type "Float (double-precision)") (InputAction :type "InputAction Object Reference" :default "/Game/QuietRuntimeEditor/EditorInput/Actions/IA_FastMoveBackward.IA_FastMoveBackward"))
  ;[0 0 0] Camera Inputs
  ;;[0 0.05729 0.056] WASD + Right Mouse Button
  (:`Triggered`
    (`self.MoveForward` ActionValue))
  (:`Started`
    (`self.SaveCameraTransform` true :!label _label_11))
  (:`Completed`
    (goto _label_11 :!via `Finish`)))

(event `EnhancedInput|/Game/QuietRuntimeEditor/EditorInput/Actions/IA_MoveForward`
  (params (ActionValue :type "Float (double-precision)") (ElapsedSeconds :type "Float (double-precision)") (TriggeredSeconds :type "Float (double-precision)") (InputAction :type "InputAction Object Reference" :default "/Game/QuietRuntimeEditor/EditorInput/Actions/IA_MoveForward.IA_MoveForward"))
  ;[0 0 0] Camera Inputs
  ;;[0.001518 0.0356 0.03689] MOVE FORWARD
  (:`Triggered`
    (`self.MoveForward` ActionValue))
  (:`Started`
    (`self.SaveCameraTransform` true :!label _label_12))
  (:`Completed`
    (goto _label_12 :!via `Finish`)))

(event `EnhancedInput|/Game/QuietRuntimeEditor/EditorInput/Actions/IA_DeleteActorsWithAttachment`
  (params (ActionValue :type Boolean) (ElapsedSeconds :type "Float (double-precision)") (TriggeredSeconds :type "Float (double-precision)") (InputAction :type "InputAction Object Reference" :default "/Game/QuietRuntimeEditor/EditorInput/Actions/IA_DeleteActorsWithAttachment.IA_DeleteActorsWithAttachment"))
  ;[0 0 0] Input Actions
  (:`Triggered`
    (`/Game/QuietRuntimeEditor/Common/Blueprints/BP_Router.ThrowCommand` (`/Game/QuietRuntimeEditor/Common/Blueprints/BP_QuietEditorUtilities.GetRouter`) (struct :`TagName` "Manager") (struct :`TagName` "Outliner.DeleteBranches"))))

(event `EnhancedInput|/Game/QuietRuntimeEditor/EditorInput/Actions/IA_Play`
  (params (ActionValue :type Boolean) (ElapsedSeconds :type "Float (double-precision)") (TriggeredSeconds :type "Float (double-precision)") (InputAction :type "InputAction Object Reference" :default "/Game/QuietRuntimeEditor/EditorInput/Actions/IA_Play.IA_Play"))
  ;[0 0 0] Input Actions
  ;;[0.004887 0.04167 0.002457] PLAY / STOP
  (:`Triggered`
    (`/Game/QuietRuntimeEditor/Common/Blueprints/BP_Router.ThrowCommand` (`/Game/QuietRuntimeEditor/Common/Blueprints/BP_QuietEditorUtilities.GetRouter`) (struct :`TagName` "Manager") (struct :`TagName` "Modes.Play"))))

(event `ZoomRegion`
  (params (Position :type "Vector2D Structure") (Size :type "Vector2D Structure"))
  (bind _returnvalue (`WidgetLayoutLibrary.GetViewportSize`))
  (bind (_x _y) (`KismetMathLibrary.BreakVector2D` Size))
  (bind (_returnvalue_x _returnvalue_y) (`KismetMathLibrary.BreakVector2D` (/ Size _returnvalue)))
  (bind (_x_2 _y_2) (`KismetMathLibrary.BreakVector2D` _returnvalue))
  (bind _returnvalue_2 (/ (`PlayerCameraManager.GetFOVAngle` (`GameplayStatics.GetPlayerCameraManager` 0)) 2.0))
  (bind (_x_3 _y_3) (`KismetMathLibrary.BreakVector2D` (+ (* Position (`WidgetLayoutLibrary.GetViewportScale`)) (/ Size 2.0))))
  (bind (_worldlocation _worlddirection) (`PlayerController.DeprojectScreenPositionToWorld` (`GameplayStatics.GetPlayerController` 0) _x_3 _y_3))
  ;[0 0 0] ZOOM REGION
  (bind (_outhit _returnvalue_3) (`KismetSystemLibrary.LineTraceSingle` _worldlocation (+ _worldlocation (* _worlddirection 10000.0)) "TraceTypeQuery1" true))
  (if _returnvalue_3
    (`self.RegisterCameraAction` (`self.GetCurrentTransform`))
    (bind (_bblockinghit _binitialoverlap _time _distance _location) (`GameplayStatics.BreakHitResult` _outhit))
    (`self.K2_SetActorLocation` (+ _location (* (`KismetMathLibrary.NegateVector` _worlddirection) (* (* (* (`KismetMathLibrary.DegTan` _returnvalue_2) (`KismetMathLibrary.Vector_Distance` _worldlocation _location)) (`KismetMathLibrary.FMin` _returnvalue_x (* _returnvalue_y (/ (/ _x_2 _y_2) (/ _x _y))))) (`KismetMathLibrary.DegTan` (- 90.0 _returnvalue_2))))) false true)
    (`Controller.SetControlRotation` (`self.GetController`) (`KismetMathLibrary.Conv_VectorToRotator` _worlddirection))))

(event `EnhancedInput|/Game/QuietRuntimeEditor/EditorInput/Actions/IA_Stop`
  (params (ActionValue :type Boolean) (ElapsedSeconds :type "Float (double-precision)") (TriggeredSeconds :type "Float (double-precision)") (InputAction :type "InputAction Object Reference" :default "/Game/QuietRuntimeEditor/EditorInput/Actions/IA_Stop.IA_Stop"))
  ;[0 0 0] Input Actions
  ;;[0.004887 0.04167 0.002457] PLAY / STOP
  (:`Triggered`
    (`/Game/QuietRuntimeEditor/Common/Blueprints/BP_Router.ThrowCommand` (`/Game/QuietRuntimeEditor/Common/Blueprints/BP_QuietEditorUtilities.GetRouter`) (struct :`TagName` "Manager") (struct :`TagName` "Modes.Stop"))))

(event `EnhancedInput|/Game/QuietRuntimeEditor/EditorInput/Actions/IA_FastMoveLeft`
  (params (ActionValue :type "Float (double-precision)") (ElapsedSeconds :type "Float (double-precision)") (TriggeredSeconds :type "Float (double-precision)") (InputAction :type "InputAction Object Reference" :default "/Game/QuietRuntimeEditor/EditorInput/Actions/IA_FastMoveLeft.IA_FastMoveLeft"))
  ;[0 0 0] Camera Inputs
  ;;[0 0.05729 0.056] WASD + Right Mouse Button
  (:`Triggered`
    (`self.MoveRight` ActionValue))
  (:`Started`
    (`self.SaveCameraTransform` true :!label _label_13))
  (:`Completed`
    (goto _label_13 :!via `Finish`)))

(event `EnhancedInput|/Game/QuietRuntimeEditor/EditorInput/Actions/IA_Pan`
  (params (ActionValue :type "Float (double-precision)") (ElapsedSeconds :type "Float (double-precision)") (TriggeredSeconds :type "Float (double-precision)") (InputAction :type "InputAction Object Reference" :default "/Game/QuietRuntimeEditor/EditorInput/Actions/IA_Pan.IA_Pan"))
  ;[0 0 0] Camera Inputs
  ;;[0.001518 0.0356 0.03689] MOVE LEFT-RIGHT (PAN)
  (:`Triggered`
    (`self.FixMouse` :!label _label_14)
    (`self.MoveRight` ActionValue))
  (:`Started`
    (goto _label_14 :!via `Started`)))

(event `EnhancedInput|/Game/QuietRuntimeEditor/EditorInput/Actions/IA_SetGizmoIdleMode`
  (params (ActionValue :type Boolean) (ElapsedSeconds :type "Float (double-precision)") (TriggeredSeconds :type "Float (double-precision)") (InputAction :type "InputAction Object Reference" :default "/Game/QuietRuntimeEditor/EditorInput/Actions/IA_SetGizmoIdleMode.IA_SetGizmoIdleMode"))
  ;[0 0 0] Input Actions
  ;;[0 0 0] Gizmo
  (:`Triggered`
    (`/Game/QuietRuntimeEditor/Common/Blueprints/BP_Router.ThrowCommand` (`/Game/QuietRuntimeEditor/Common/Blueprints/BP_QuietEditorUtilities.GetRouter`) (struct :`TagName` "Manager") (struct :`TagName` "Gizmo.ToSelectMode"))))

(event `EnhancedInput|/Game/QuietRuntimeEditor/EditorInput/Actions/IA_FastMoveRight`
  (params (ActionValue :type "Float (double-precision)") (ElapsedSeconds :type "Float (double-precision)") (TriggeredSeconds :type "Float (double-precision)") (InputAction :type "InputAction Object Reference" :default "/Game/QuietRuntimeEditor/EditorInput/Actions/IA_FastMoveRight.IA_FastMoveRight"))
  ;[0 0 0] Camera Inputs
  ;;[0 0.05729 0.056] WASD + Right Mouse Button
  (:`Triggered`
    (`self.MoveRight` ActionValue))
  (:`Started`
    (`self.SaveCameraTransform` true :!label _label_15))
  (:`Completed`
    (goto _label_15 :!via `Finish`)))

(event `EnhancedInput|/Game/QuietRuntimeEditor/EditorInput/Actions/IA_Grid`
  (params (ActionValue :type Boolean) (ElapsedSeconds :type "Float (double-precision)") (TriggeredSeconds :type "Float (double-precision)") (InputAction :type "InputAction Object Reference" :default "/Game/QuietRuntimeEditor/EditorInput/Actions/IA_Grid.IA_Grid"))
  ;[0 0 0] Input Actions
  (:`Triggered`
    (`/Game/QuietRuntimeEditor/Common/Blueprints/BP_Router.ThrowCommand` (`/Game/QuietRuntimeEditor/Common/Blueprints/BP_QuietEditorUtilities.GetRouter`) (struct :`TagName` "Manager") (struct :`TagName` "Modes.Grid"))))

(event `EnhancedInput|/Game/QuietRuntimeEditor/EditorInput/Actions/IA_SetGizmoTranslateMode`
  (params (ActionValue :type Boolean) (ElapsedSeconds :type "Float (double-precision)") (TriggeredSeconds :type "Float (double-precision)") (InputAction :type "InputAction Object Reference" :default "/Game/QuietRuntimeEditor/EditorInput/Actions/IA_SetGizmoTranslateMode.IA_SetGizmoTranslateMode"))
  ;[0 0 0] Input Actions
  ;;[0 0 0] Gizmo
  (:`Triggered`
    (`/Game/QuietRuntimeEditor/Common/Blueprints/BP_Router.ThrowCommand` (`/Game/QuietRuntimeEditor/Common/Blueprints/BP_QuietEditorUtilities.GetRouter`) (struct :`TagName` "Manager") (struct :`TagName` "Gizmo.ToTranslateMode"))))

(event `EnhancedInput|/Game/QuietRuntimeEditor/EditorInput/Actions/IA_ToggleDebugMode`
  (params (ActionValue :type Boolean) (ElapsedSeconds :type "Float (double-precision)") (TriggeredSeconds :type "Float (double-precision)") (InputAction :type "InputAction Object Reference" :default "/Game/QuietRuntimeEditor/EditorInput/Actions/IA_ToggleDebugMode.IA_ToggleDebugMode"))
  ;[0 0 0] Input Actions
  (:`Triggered`
    (`/Game/QuietRuntimeEditor/Common/Blueprints/BP_Router.ThrowCommand` (`/Game/QuietRuntimeEditor/Common/Blueprints/BP_QuietEditorUtilities.GetRouter`) (struct :`TagName` "Manager") (struct :`TagName` "Modes.ToggleDebugMode"))))

(event `EnhancedInput|/Game/QuietRuntimeEditor/EditorInput/Actions/IA_SetGizmoRotateMode`
  (params (ActionValue :type Boolean) (ElapsedSeconds :type "Float (double-precision)") (TriggeredSeconds :type "Float (double-precision)") (InputAction :type "InputAction Object Reference" :default "/Game/QuietRuntimeEditor/EditorInput/Actions/IA_SetGizmoRotateMode.IA_SetGizmoRotateMode"))
  ;[0 0 0] Input Actions
  ;;[0 0 0] Gizmo
  (:`Triggered`
    (`/Game/QuietRuntimeEditor/Common/Blueprints/BP_Router.ThrowCommand` (`/Game/QuietRuntimeEditor/Common/Blueprints/BP_QuietEditorUtilities.GetRouter`) (struct :`TagName` "Manager") (struct :`TagName` "Gizmo.ToRotateMode"))))

(event `EnhancedInput|/Game/QuietRuntimeEditor/EditorInput/Actions/IA_ToggleUI`
  (params (ActionValue :type Boolean) (ElapsedSeconds :type "Float (double-precision)") (TriggeredSeconds :type "Float (double-precision)") (InputAction :type "InputAction Object Reference" :default "/Game/QuietRuntimeEditor/EditorInput/Actions/IA_ToggleUI.IA_ToggleUI"))
  ;[0 0 0] Input Actions
  (:`Triggered`
    (`/Game/QuietRuntimeEditor/Common/Blueprints/BP_Router.ThrowCommand` (`/Game/QuietRuntimeEditor/Common/Blueprints/BP_QuietEditorUtilities.GetRouter`) (struct :`TagName` "UserInterface") (struct :`TagName` "UserInterface.ToggleVisibility"))))

(event `EnhancedInput|/Game/QuietRuntimeEditor/EditorInput/Actions/IA_SetGizmoScaleMode`
  (params (ActionValue :type Boolean) (ElapsedSeconds :type "Float (double-precision)") (TriggeredSeconds :type "Float (double-precision)") (InputAction :type "InputAction Object Reference" :default "/Game/QuietRuntimeEditor/EditorInput/Actions/IA_SetGizmoScaleMode.IA_SetGizmoScaleMode"))
  ;[0 0 0] Input Actions
  ;;[0 0 0] Gizmo
  (:`Triggered`
    (`/Game/QuietRuntimeEditor/Common/Blueprints/BP_Router.ThrowCommand` (`/Game/QuietRuntimeEditor/Common/Blueprints/BP_QuietEditorUtilities.GetRouter`) (struct :`TagName` "Manager") (struct :`TagName` "Gizmo.ToScaleMode"))))

(event `EnhancedInput|/Game/QuietRuntimeEditor/EditorInput/Actions/IA_ToggleGizmoSnapMode`
  (params (ActionValue :type Boolean) (ElapsedSeconds :type "Float (double-precision)") (TriggeredSeconds :type "Float (double-precision)") (InputAction :type "InputAction Object Reference" :default "/Game/QuietRuntimeEditor/EditorInput/Actions/IA_ToggleGizmoSnapMode.IA_ToggleGizmoSnapMode"))
  ;[0 0 0] Input Actions
  ;;[0 0 0] Gizmo
  (:`Triggered`
    (`/Game/QuietRuntimeEditor/Common/Blueprints/BP_Router.ThrowCommand` (`/Game/QuietRuntimeEditor/Common/Blueprints/BP_QuietEditorUtilities.GetRouter`) (struct :`TagName` "Manager") (struct :`TagName` "Gizmo.ToggleSnap"))))

(event `EnhancedInput|/Game/QuietRuntimeEditor/EditorInput/Actions/IA_ToggleGizmoCoordsys`
  (params (ActionValue :type Boolean) (ElapsedSeconds :type "Float (double-precision)") (TriggeredSeconds :type "Float (double-precision)") (InputAction :type "InputAction Object Reference" :default "/Game/QuietRuntimeEditor/EditorInput/Actions/IA_ToggleGizmoCoordsys.IA_ToggleGizmoCoordsys"))
  ;[0 0 0] Input Actions
  ;;[0 0 0] Gizmo
  (:`Triggered`
    (`/Game/QuietRuntimeEditor/Common/Blueprints/BP_Router.ThrowCommand` (`/Game/QuietRuntimeEditor/Common/Blueprints/BP_QuietEditorUtilities.GetRouter`) (struct :`TagName` "Manager") (struct :`TagName` "Gizmo.ToggleRelative"))))

(fn `AlignCamera`
  (bind (_returnvalue_roll _returnvalue_pitch _returnvalue_yaw) (`KismetMathLibrary.BreakRotator` (`self.GetControlRotation`)))
  (`self.RegisterCameraAction` (`self.GetCurrentTransform`))
  (`Controller.SetControlRotation` (`self.GetController`) (`KismetMathLibrary.MakeRotator` _returnvalue_roll 0.0 _returnvalue_yaw)))

(fn `CompareTransform`
  (params (InTransform :type "Transform Structure (by ref)") (InTransform2 :type "Transform Structure (by ref)"))
  (returns (ReturnValue :type Boolean))
  (return (not (and (== (.location InTransform) (.location InTransform2) :`ErrorTolerance` 0.001) (== (.rotation InTransform) (.rotation InTransform2) :`ErrorTolerance` 0.001) (== (.scale InTransform) (.scale InTransform2) :`ErrorTolerance` 0.001)))))

(fn `FocusOnSelection`
  (bind _actors (`/Game/QuietRuntimeEditor/Common/Blueprints/BP_Router.GetActorsWithTag` (`/Game/QuietRuntimeEditor/Common/Blueprints/BP_QuietEditorUtilities.GetRouter`) (struct :`TagName` "Manager") (struct :`TagName` "Outliner.GetSelection")))
  (if (`KismetArrayLibrary.Array_IsNotEmpty` _actors)
    (bind (_center _boxextent) (`GameplayStatics.GetActorArrayBounds` _actors))
    (`|ExecutionSequence`
      (:`then_0`
        (`Controller.SetControlRotation` (`self.GetController`) (`KismetMathLibrary.FindLookAtRotation` (`self.K2_GetActorLocation`) _center)))
      (:`then_1`
        (`self.RegisterCameraAction` (`self.GetCurrentTransform`))
        (bind _returnvalue (`KismetMathLibrary.GetMaxElement` _boxextent))
        (bind _returnvalue_2 (`KismetMathLibrary.VSize` (`KismetMathLibrary.MakeVector` _returnvalue _returnvalue _returnvalue)))
        (`self.K2_SetActorLocation` (+ _center (* (`KismetMathLibrary.Conv_RotatorToVector` (`KismetMathLibrary.FindLookAtRotation` _center (`self.K2_GetActorLocation`))) (+ (/ _returnvalue_2 2.0) (* _returnvalue_2 (`KismetMathLibrary.DegTan` (- 90.0 (`KismetSystemLibrary.MakeLiteralDouble` (/ (`PlayerCameraManager.GetFOVAngle` (`GameplayStatics.GetPlayerCameraManager` 0)) 2.0)))))))) false true)))))

(fn `GetCurrentTransform`
  (returns (ReturnValue :type "Transform Structure"))
  (return (`KismetMathLibrary.MakeTransform` (`self.K2_GetActorLocation`) (`self.GetControlRotation`))))

(fn `GetDataWithTag`
  (params (Request :type "GameplayTag Structure"))
  (returns (Success :type Boolean) (Data :type "JsonObjectWrapper Structure"))
  (`|SwitchGameplayTag` Request
    (:`EditorPawn.GetSavedData`
      (bind _jsonobject (`/Game/QuietRuntimeEditor/Common/Blueprints/BP_QuietJsonFunctionLibrary.NewJson`))
      (`|SetJsonField` _jsonobject "Transform" (`self.GetCurrentTransform`))
      (`|SetJsonField` _jsonobject "Fov" (`PlayerCameraManager.GetFOVAngle` (`GameplayStatics.GetPlayerCameraManager` 0)))
      (return true _jsonobject))))

(fn `GetMovementScale`
  (returns (ReturnValue :type "Float (double-precision)"))
  (return (* (`self.MovementSpeed`) (`GameplayStatics.GetWorldDeltaSeconds`))))

(fn `Mouse X Scaled`
  (returns (Value :type "Float (double-precision)"))
  (return (* (`self.MovementSpeed`) (`self.GetInputAxisKeyValue`))))

(fn `Mouse Y Scaled`
  (returns (Value :type "Float (double-precision)"))
  (return (* (`self.MovementSpeed`) (`self.GetInputAxisKeyValue`))))

(fn `OrbitRotation`
  (params (Pitch :type Boolean) (Pivot :type "Vector Structure (by ref)") (Angle :type "Float (single-precision)"))
  (bind _returnvalue (`self.K2_GetActorLocation`))
  (bind _returnvalue_2 (+ Pivot (`KismetMathLibrary.RotateAngleAxis` (- _returnvalue Pivot) Angle (`KismetMathLibrary.SelectVector` (`KismetMathLibrary.GetRightVector` (`self.GetControlRotation`)) (0.0 0.0 1.0) Pitch))))
  (if Pitch
    (if (<= (`KismetMathLibrary.Abs` (.pitch (`KismetMathLibrary.FindLookAtRotation` _returnvalue_2 Pivot))) 80.0)
      (`self.K2_SetActorLocation` _returnvalue_2 :!label _label)
      (`Controller.SetControlRotation` (`self.GetController`) (`KismetMathLibrary.FindLookAtRotation` _returnvalue Pivot)))
    (else
      (goto _label))))

(fn `RegisterCameraAction`
  (params (Transform :type "Transform Structure"))
  (bind _cameraactionshistory (`self.CameraActionsHistory`))
  (bind _historylimit (`self.HistoryLimit`))
  (if (`KismetArrayLibrary.Array_IsValidIndex` _cameraactionshistory)
    (if (`self.CompareTransform` Transform (`|GetArrayItem` _cameraactionshistory (`KismetArrayLibrary.Array_LastIndex` _cameraactionshistory)))
      (bind _returnvalue (`KismetArrayLibrary.Array_Add` (`self.CameraActionsHistory`) Transform :!label _label))
      (if (== _returnvalue _historylimit)
        (`KismetArrayLibrary.Array_Remove` (`self.CameraActionsHistory`) _historylimit)))
    (else
      (goto _label))))

(fn `ReturnDataByRequestWithTag`
  (params (Request :type "GameplayTag Structure") (InputData :type "JsonObjectWrapper Structure"))
  (returns (Success :type Boolean) (Data :type "JsonObjectWrapper Structure"))
  (return false))

(fn `SetupCamera`
  (params (Transform :type "Transform Structure") (Fov :type "Float (double-precision)"))
  (`KismetArrayLibrary.Array_Clear` (`self.CameraActionsHistory`))
  (`self.K2_SetActorLocation` (.location Transform) false true)
  (`Controller.SetControlRotation` (`self.GetController`) (.rotation Transform))
  (set `PlayerCameraManager.DefaultFOV` Fov (`GameplayStatics.GetPlayerCameraManager` 0)))

(fn `TakeActorsWithTag`
  (params (Request :type "GameplayTag Structure"))
  (returns (Actors :type "Array of Actor Object Reference"))
  (return))

(fn `TakeObjectWithTag`
  (params (Request :type "GameplayTag Structure"))
  (returns (Object :type "Object Object Reference"))
  (return null))

(fn `UndoCameraAction`
  (bind (_returnvalue_location _returnvalue_rotation) (`KismetMathLibrary.BreakTransform` (`self.GetCurrentTransform`)))
  (bind _cameraactionshistory (`self.CameraActionsHistory`))
  (bind _cameraactionshistory_2 (`self.CameraActionsHistory`))
  (bind (_output_location _output_rotation) (`KismetMathLibrary.BreakTransform` (`|GetArrayItem` _cameraactionshistory_2 (`KismetArrayLibrary.Array_LastIndex` _cameraactionshistory_2))))
  (if (`KismetArrayLibrary.Array_IsValidIndex` _cameraactionshistory_2)
    (`|ExecutionSequence`
      (:`then_0`
        (if (!= _output_location _returnvalue_location :`ErrorTolerance` 0.001)
          (`self.K2_SetActorLocation` _output_location)))
      (:`then_1`
        (if (!= _output_rotation _returnvalue_rotation :`ErrorTolerance` 0.001)
          (`Controller.SetControlRotation` (`self.GetController`) _output_rotation)))
      (:`then_2`
        (`KismetArrayLibrary.Array_Remove` _cameraactionshistory (`KismetArrayLibrary.Array_LastIndex` _cameraactionshistory))))))

(fn `UserConstructionScript`)