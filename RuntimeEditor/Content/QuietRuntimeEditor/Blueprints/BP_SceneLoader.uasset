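; BP_SceneLoader loads a saved QuietRuntimeEditor scene and hands control to its character.
; Shortly after BeginPlay it has the Serializer restore the named scene's JSON file from the save directory, or shows an invalid-scene warning if the file is missing.
; A tick later, if a Character exists, it possesses it, captures the mouse for game input and disables debug mode on all BI_QuietActorsInterface actors.
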(event `self.ReceiveBeginPlay`
  (bind _returnvalue (`KismetStringLibrary.Concat_StrStr` (`/Game/QuietRuntimeEditor/Common/Blueprints/BP_PathAccessLibrary.GetSaveDirectory`) "/" (`self.Scene`) ".json"))
  (`KismetSystemLibrary.Delay` 0.2)
  (if (`BlueprintPathsLibrary.FileExists` _returnvalue)
    (message `/Game/QuietRuntimeEditor/Serialization/BI_SerializerInterface.RestoreScene` (`self.Serializer`) (make `FilePath` _returnvalue))
    (`KismetSystemLibrary.DelayUntilNextTick`)
    (bind _returnvalue_2 (`GameplayStatics.GetActorOfClass` "/Script/Engine.Character"))
    (`/Engine/EditorBlueprintResources/StandardMacros.IsValid` _returnvalue_2
      (:`Is Valid`
        (`Controller.Possess` (`GameplayStatics.GetPlayerController` 0) _returnvalue_2)
        (set `PlayerController.bShowMouseCursor` false (`GameplayStatics.GetPlayerController` 0))
        (`GameplayStatics.SetViewportMouseCaptureMode` "CapturePermanently")
        (`WidgetBlueprintLibrary.SetFocusToGameViewport`)
        (bind _outactors (`GameplayStatics.GetAllActorsWithInterface` "/Game/QuietRuntimeEditor/Common/QuietActors/Blueprints/BI_QuietActorsInterface.BI_QuietActorsInterface_C"))
        (for _array_element _outactors
          (message `/Game/QuietRuntimeEditor/Common/QuietActors/Blueprints/BI_QuietActorsInterface.EnableDebugMode` _array_element false))))
    (else
      (`/Game/QuietRuntimeEditor/Common/Blueprints/BP_QuietDialogLibrary.CallWarningDialogSimple` (`GameplayStatics.GetPlayerController` 0) "Loader.InvalidScene"))))

(fn `UserConstructionScript`)